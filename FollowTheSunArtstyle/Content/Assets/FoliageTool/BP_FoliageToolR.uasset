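; BP_FoliageToolR is a foliage placement tool that scatters flower instances over the surface beneath it when constructed.
; Its construction script picks seeded random offsets around Point relative to the actor, spanning both sides in X but only positive Y.
; Downward Visibility traces from those offsets supply locations for instanced static mesh instances, added without a hit check.
; Each instance gets an unseeded random yaw.
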(event EventBeginPlay)

(event Collision|EventActorBeginOverlap
  (params (OtherActor :type Actor%20Object%20Reference)))

(event EventTick
  (params (DeltaSeconds :type Float%20%28single-precision%29)))

(fn ConstructionScript
  (bind _returnvalue (* -1 0.0))
  (bind _point (Variables|Default|GetPoint))
  (bind _defaultsceneroot (Variables|Default|GetDefaultSceneRoot))
  (bind _max_x_distance (Variables|Default|GetMax%20X%20distance))
  (bind _seed (Variables|Default|GetSeed))
  (bind _max_y_distance (Variables|Default|GetMax%20Y%20distance))
  (bind _returnvalue_2 (Transformation|GetWorldLocation _defaultsceneroot))
  (bind _returnvalue_3 (Math|Random|RandomFloatinRangefromStream _returnvalue _max_y_distance _seed))
  (bind _returnvalue_4 (* -1 _max_x_distance))
  (bind _returnvalue_5 (Math|Random|RandomFloatinRangefromStream _returnvalue_4 _max_x_distance _seed))
  (bind _returnvalue_6 (+ _point _returnvalue_2 (Math|Vector|MakeVector _returnvalue_5 _returnvalue_3 0.0)))
  (for _index (range 1 (Variables|Default|GetNumber%20of%20Flowers))
    (bind _outhit (Collision|LineTraceByChannel _returnvalue_6 (+ _returnvalue_6 (Math|Vector|MakeVector 0.0 0.0 -1e+03)) "TraceTypeQuery1" false 0 "None"))
    (Components|InstancedStaticMesh|AddInstance (Variables|Default|GetInstancedStaticMesh) (Math|Transform|MakeTransform (- (.location _outhit) (Transformation|GetWorldLocation (Variables|Default|GetDefaultSceneRoot))) (Math|Rotator|MakeRotator 0.0 0.0 (Math|Random|RandomFloatinRange 0.0 3.6e+02)) "1,1,1"))))