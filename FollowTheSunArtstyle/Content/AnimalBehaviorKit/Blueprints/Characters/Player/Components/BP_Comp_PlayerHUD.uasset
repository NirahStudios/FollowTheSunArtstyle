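; Player HUD component from the Animal Behavior Kit that creates the player's HUD widget.
; Its create function stores prey and predator bait amounts, then finds the player controller through the owner's instigator.
; It creates and keeps a WBP_Player_HUD for that controller, adding it to the player screen only when ShowHUD is set.
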(fn FnCreateHUD
  (params (preyBait :type Integer) (predatorBait :type Integer))
  (LocalVariables|SetPreyBaitAmount preyBait)
  (LocalVariables|SetPredatorBaitAmount predatorBait)
  ;[1 1 1] Create Player HUD
  (bind _asplayer_controller (Utilities|Casting|CastToPlayerController (Pawn|GetController (Variables|/Script/Engine.Actor|GetInstigator (Components|GetOwner)))))
  (bind _returnvalue (UserInterface|CreateWidget "/Game/AnimalBehaviorKit/Blueprints/Widgets/WBP_Player_HUD.WBP_Player_HUD_C" _asplayer_controller))
  (Variables|Default|SetPlayerHUDRef _returnvalue)
  (if (Variables|Setup|GetShowHUD)
    (UserInterface|Viewport|AddtoPlayerScreen (Variables|Default|GetPlayerHUDRef))))