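; BP_AnimalBase is the base animal Blueprint, handling health, damage, tags and an overhead name/HP widget configured from AnimalDetails.
; Construction sets tags and initial HUD visibility; BeginPlay initializes HP and the widget, which Tick turns toward the player camera.
; AnyDamage filters causers by NoDamageTags, subtracts HP after a gated delay, and fires EventDead once for children to override.
; OnRep_CurrentHP updates either standard or companion HUD widgets.
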(event EventBeginPlay
  (|SAVEANIMALHP)
  (|SETHUDNAMEANDHPVISIBILITY))

(event EventTick
  (params (DeltaSeconds :type Float%20%28single-precision%29))
  (|ROTATEHUDTOWARDSPLAYER))

(fn ConstructionScript
  (bind _animal_details (Variables|Setup-General|GetAnimal_Details))
  (bind (_showhud_ _showhudonproximityonly) (Utilities|Struct|BreakBP_Struct_AnimalBase_AnimalDetail _animal_details))
  ;[1 1 1] Show the HUD permanently?
  (if (not _showhudonproximityonly)
    ;[1 1 1] Show HUD and set ShowingHUD to true
    (Rendering|SetVisibility (Variables|Default|GetWBP_HUD) _showhud_ false)
    (Variables|Default|SetShowingHUD true)
    (else
      (Rendering|SetVisibility (Variables|Default|GetWBP_HUD) false false)
      (Variables|Default|SetShowingHUD false)))
  (for _array_element (Variables|Setup-General|GetAdditionalTags)
    (Utilities|Array|Add (Variables|Setup-General|GetActorTags) _array_element))
  ;[1 1 1] Set default 'Animal' tag
  (Variables|Default|SetTags (Variables|Setup-General|GetActorTags)))

(fn FnGetAuthority
  (Networking|SwitchHasAuthority
    (:Authority
      (LocalVariables|Setauth true))
    (:Remote
      (LocalVariables|Setauth false)))
  (return (LocalVariables|Getauth)))

(fn OnRepCurrentHP
  (Utilities|FlowControl|Sequence
    (:then_0
      ;[0 1 1] [COMPANION CODE] Update HP Bar in the HUD
      (bind _aswbp_ats_ai_hud (Utilities|Casting|CastToWBP_ATS_AI_HUD (UserInterface|GetUserWidgetObject (Variables|Default|GetWBP_HUD))))
      (Default|FnSetHP _aswbp_ats_ai_hud (/ (Variables|Setup-AnimalDetails|GetCurrentHP) (Utilities|Struct|BreakBP_Struct_AnimalBase_AnimalDetail (Variables|Setup-General|GetAnimal_Details)))))
    (:then_1
      ;[1 1 1] Update HP Bar in the HUD
      (bind _aswbp_ai_hud (Utilities|Casting|CastToWBP_AI_HUD (UserInterface|GetUserWidgetObject (Variables|Default|GetWBP_HUD))))
      (Default|FnSetHP _aswbp_ai_hud (/ (Variables|Setup-AnimalDetails|GetCurrentHP) (Utilities|Struct|BreakBP_Struct_AnimalBase_AnimalDetail (Variables|Setup-General|GetAnimal_Details)))))))

(fn FnCanTakeDamage
  (params (Damage%20Causer :type Actor%20Object%20Reference))
  (LocalVariables|SetCauser Damage%20Causer)
  (bind _array_element (Utilities|Array|ForEachLoopwithBreak (Utilities|Struct|BreakBP_Struct_AnimalBase_AnimalDetail (Variables|Setup-General|GetAnimal_Details)) :!label _label)
    (:LoopBody
      ;[1 1 1] Is one of the No Damage Tags found on the Damage Causer?
      (if (Utilities|Array|ContainsItem (Variables|/Script/Engine.Actor|GetTags (LocalVariables|GetCauser)) _array_element)
        (LocalVariables|SetAllow false)
        (goto _label Break)
        (else
          (LocalVariables|SetAllow true))))
    (:Completed
      (return (LocalVariables|GetAllow)))))

(event Custom|EventDead
  ;[1 1 1] Base Event - Override in child blueprint
)

(event Game|Damage|EventAnyDamage
  (params (Damage :type Float%20%28single-precision%29) (DamageType :type Damage%20Type%20Object%20Reference) (InstigatedBy :type Controller%20Object%20Reference) (DamageCauser :type Actor%20Object%20Reference))
  (Variables|Default|SetDamageAmount Damage)
  (bind _output_get (Variables|Damage|SetDamageCauser DamageCauser))
  ;[1 1 1] Can we take damage?
  (bind _can_take_damage (CallFunction|FnCanTakeDamage _output_get))
  (if _can_take_damage
    (if (Variables|State|GetCanTakeDamage)
      (Variables|State|SetCanTakeDamage false)
      (Utilities|FlowControl|Delay (Variables|Damage|GetDamageFrequency))
      (Variables|State|SetCanTakeDamage true)
      ;[1 1 1] Reduce HP by Damage amount
      (Variables|Setup-AnimalDetails|SetCurrentHP (- (Variables|Setup-AnimalDetails|GetCurrentHP) (Variables|Default|GetDamageAmount)))
      ;[1 1 1] Is Animal dead?
      (if (<= (Variables|Setup-AnimalDetails|GetCurrentHP) 0.0)
        (Utilities|FlowControl|DoOnce false
          (:Completed
            (CallFunction|EventDead)))))))