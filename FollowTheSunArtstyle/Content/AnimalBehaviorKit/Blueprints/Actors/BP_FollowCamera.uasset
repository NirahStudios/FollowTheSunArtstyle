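; BP_FollowCamera is a toggleable orbit camera for the Animal Behavior Kit that follows TargetActor.
; When active, it takes over player 0's view, teleports to the target each tick, and applies camera FOV and global time dilation.
; Input rotates and zooms the CameraBoom, with clamped pitch that InvertYaw flips despite its name.
; It also gathers "Animal"-tagged actors into AnimalList, which this graph never reads.
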(event EventBeginPlay
  (if (Variables|Setup|GetActive)
    ;[1 1 1] Invert Yaw controls?
    (if (Variables|Setup|GetInvertYaw?)
      (Variables|Default|SetYawDirection -1.0)
      (else
        (Variables|Default|SetYawDirection 1.0)))
    (Game|Player|SetViewTargetwithBlend (Game|GetPlayerController 0) self 1.0 "VTBlend_Linear" 0.0 false)
    ;[1 1 1] Get all animals in the scene and add it to the AnimalList
    (bind _outactors (Actor|GetAllActorswithTag "Animal"))
    (for _array_element _outactors
      (Utilities|Array|Add (Variables|Setup|GetAnimalList) _array_element))
    (else
      ;[1 1 1] BP not active, do not consume input
      (Input|DisableInput self (Game|GetPlayerController 0)))))

(event EventTick
  (params (DeltaSeconds :type Float%20%28single-precision%29))
  (if (Variables|Setup|GetActive)
    ;[1 1 1] Set actor location to TargetActor
    (Transformation|SetActorLocation (Transformation|GetActorLocation (Variables|Setup|GetTargetActor)) false true)
    ;[1 1 1] Update Camera FOV
    (Camera|SetFieldOfView (Variables|Default|GetCamera) (Variables|Setup|GetCameraFOV))
    (Utilities|Time|SetGlobalTimeDilation (Variables|Setup|GetTimeDilation))))

(event Input|ActionEvents|InputActionZoomIn
  (params (Key :type Key%20Structure))
  ;[1 1 1] Zoom In and Out
  (:Pressed
    (Variables|/Script/Engine.SpringArmComponent|SetTargetArmLength (Variables|Default|GetCameraBoom) (- (Variables|/Script/Engine.SpringArmComponent|GetTargetArmLength (Variables|Default|GetCameraBoom)) (Variables|Setup|GetZoomAmount)))))

(event Input|ActionEvents|InputActionZoomOut
  (params (Key :type Key%20Structure))
  ;[1 1 1] Zoom In and Out
  (:Pressed
    (Variables|/Script/Engine.SpringArmComponent|SetTargetArmLength (Variables|Default|GetCameraBoom) (+ (Variables|/Script/Engine.SpringArmComponent|GetTargetArmLength (Variables|Default|GetCameraBoom)) (Variables|Setup|GetZoomAmount)))))

(event Input|AxisEvents|InputAxisLookUp
  (params (AxisValue :type Float%20%28single-precision%29))
  (bind _cameraboom (Variables|Default|GetCameraBoom))
  (bind _relativerotation (Variables|/Script/Engine.SceneComponent|GetRelativeRotation _cameraboom))
  ;[1 1 1] Rotate camera by moving the Mouse
  (Transformation|SetRelativeRotation (Variables|Default|GetCameraBoom) (Math|Rotator|MakeRotator (.roll _relativerotation) (Math|Float|Clamp(Float) (+ (.pitch _relativerotation) (* AxisValue 2.0 (Variables|Default|GetYawDirection))) -89.0 89.0) (.yaw _relativerotation)) false false))

(event Input|AxisEvents|InputAxisTurn
  (params (AxisValue :type Float%20%28single-precision%29))
  (bind _cameraboom (Variables|Default|GetCameraBoom))
  (bind _relativerotation (Variables|/Script/Engine.SceneComponent|GetRelativeRotation _cameraboom))
  ;[1 1 1] Rotate camera by moving the Mouse
  (Transformation|SetRelativeRotation (Variables|Default|GetCameraBoom) (Math|Rotator|MakeRotator (.roll _relativerotation) (.pitch _relativerotation) (+ (.yaw _relativerotation) (* AxisValue 2.0))) false false))

(fn ConstructionScript)