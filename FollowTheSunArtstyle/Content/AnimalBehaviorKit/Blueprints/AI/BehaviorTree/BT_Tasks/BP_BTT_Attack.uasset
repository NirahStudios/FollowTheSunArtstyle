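; Behavior tree task that makes a ground animal melee-attack its blackboard EngageActor.
; If a sphere trace finds the target in range, it plays the attack montage, then waits out its length and attack frequency.
; A dead target triggers hunger reset and disengage; dead or invalid targets return the animal to roaming.
; Tick optionally matches target speed in range, moves unless attacks are stationary, and turns toward the target, using line-traced impact points up close.
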(event EventReceiveExecuteAI
  (params (OwnerController :type AI%20Controller%20Object%20Reference) (ControlledPawn :type Pawn%20Object%20Reference))
  (Variables|Default|SetPawnRef ControlledPawn)
  (bind _asbp_ground_animal_base (Utilities|Casting|CastToBP_GroundAnimalBase (Variables|Default|GetPawnRef)))
  (Variables|Default|SetAnimalBase _asbp_ground_animal_base)
  ;[1 1 1] Check if we are in melee range
  (if (.In%20Range (CallFunction|FnGetEngageTargetSpeed))
    ;[1 1 1] Set Acceptance Radius
    (Variables|Default|SetAcceptanceRadius (Variables|/Game/AnimalBehaviorKit/Blueprints/Characters/Animals/GroundAnimals/BP_GroundAnimalBase.BP_GroundAnimalBase_C|GetMovementAcceptanceRadius (Variables|Default|GetAnimalBase)))
    ;[1 1 1] Set DisengageCD and StopMovement
    (Variables|Default|SetDisengageCD (.DisengageCD (Utilities|Struct|BreakBP_Struct_GroundAnimalBehavior_AnimalDetails_Attack (Variables|/Game/AnimalBehaviorKit/Blueprints/Characters/Animals/GroundAnimals/BP_GroundAnimalBase.BP_GroundAnimalBase_C|GetBehavior_Details_Attack (Variables|Default|GetAnimalBase)))))
    (Variables|Default|SetStopMovement (.Dontmovewhileattacking (Utilities|Struct|BreakBP_Struct_GroundAnimalBehavior_AnimalDetails_Attack (Variables|/Game/AnimalBehaviorKit/Blueprints/Characters/Animals/GroundAnimals/BP_GroundAnimalBase.BP_GroundAnimalBase_C|GetBehavior_Details_Attack (Variables|Default|GetAnimalBase)))))
    ;[1 1 1] Save the Max Walk Speed
    (Variables|Default|SetMaxWalkSpeed (Variables|/Script/Engine.CharacterMovementComponent|GetMaxWalkSpeed (Variables|/Script/Engine.Character|GetCharacterMovement (Variables|Default|GetAnimalBase))))
    ;[1 1 1] Check Engage Actor is Valid
    (Utilities|IsValid (AI|BehaviorTree|GetBlackboardValueasActor (Variables|Setup|GetEngageActor))
      (:Is%20Valid
        ;[1 1 1] Check that Engage Actor is NOT Dead
        (if (not (Actor|ActorHasTag (AI|BehaviorTree|GetBlackboardValueasActor (Variables|Setup|GetEngageActor)) "abkDead"))
          ;[1 1 1] Set State to Attacking
          (Variables|/Game/AnimalBehaviorKit/Blueprints/Characters/Animals/BP_AnimalBase.BP_AnimalBase_C|SetAttacking (Variables|Default|GetAnimalBase) true)
          ;[1 1 1] Play Attacking animation
          (Default|EventPlayAnimation (Variables|Default|GetAnimalBase) "NewEnumerator0")
          ;[1 1 1] Wait for the attack animation duration
          (bind _returnvalue (Animation|GetCurrentMontage (Variables|Default|GetAnimalBase) :!class /Script/Engine.Character))
          (Utilities|IsValid _returnvalue
            (:Is%20Valid
              (bind _returnvalue_2 (Animation|GetPlayLength _returnvalue))
              (Utilities|FlowControl|Delay (/ _returnvalue_2 (Utilities|Struct|BreakBP_Struct_GroundAnimal_CurrentMontage (Variables|/Game/AnimalBehaviorKit/Blueprints/Characters/Animals/GroundAnimals/BP_GroundAnimalBase.BP_GroundAnimalBase_C|GetCurrentAnimation (Variables|Default|GetAnimalBase))))))
            (:Is%20Not%20Valid
              _))
          ;[1 1 1] Stop attacking
          (Variables|/Game/AnimalBehaviorKit/Blueprints/Characters/Animals/BP_AnimalBase.BP_AnimalBase_C|SetAttacking (Variables|Default|GetAnimalBase) false)
          ;[1 1 1] Wait AttackFrequency before stopping the attack
          (Utilities|FlowControl|Delay (Utilities|Struct|BreakBP_Struct_GroundAnimalBehavior_AnimalDetails_Attack (Variables|/Game/AnimalBehaviorKit/Blueprints/Characters/Animals/GroundAnimals/BP_GroundAnimalBase.BP_GroundAnimalBase_C|GetBehavior_Details_Attack (Variables|Default|GetAnimalBase))))
          (AI|BehaviorTree|FinishExecute true)
          (else
            ;[1 1 1] Is Comp_NeedSystem present?
            (Utilities|IsValid (Actor|GetComponentbyClass (Variables|Default|GetAnimalBase) "/Game/AnimalBehaviorKit/Blueprints/AI/Components/GroundAnimals/BP_Comp_NeedSystem.BP_Comp_NeedSystem_C")
              (:Is%20Valid
                ;[1 1 1] Resets Hunger
                (Default|EventFinishedEating (Actor|GetComponentbyClass (Variables|Default|GetAnimalBase) "/Game/AnimalBehaviorKit/Blueprints/AI/Components/GroundAnimals/BP_Comp_NeedSystem.BP_Comp_NeedSystem_C")))
              (:Is%20Not%20Valid
                _))
            ;[1 1 1] Engage Actor is dead - Disengage
            (Default|FnDisengage (Variables|Default|GetAnimalBase))
            ;[1 1 1] Stop attacking
            (Variables|/Game/AnimalBehaviorKit/Blueprints/Characters/Animals/BP_AnimalBase.BP_AnimalBase_C|SetAttacking (Variables|Default|GetAnimalBase) false)
            ;[1 1 1] Set next Roam Behavior
            (bind _newroambehavior (Default|FnSetRoamBehavior (Variables|Default|GetAnimalBase)))
            (|SETNEXTBEHAVIORINTHEBLACKBOARD _newroambehavior
              (:OutputPin
                ;[1 1 1] Finished eating - set BiggestNeed to Roam again
                (Variables|/Game/AnimalBehaviorKit/Blueprints/Characters/Animals/GroundAnimals/BP_GroundAnimalBase.BP_GroundAnimalBase_C|SetBiggestNeed (Variables|Default|GetAnimalBase) "NewEnumerator3")
                (AI|BehaviorTree|FinishExecute true))))))
      (:Is%20Not%20Valid
        ;[1 1 1] Stop attacking
        (Variables|/Game/AnimalBehaviorKit/Blueprints/Characters/Animals/BP_AnimalBase.BP_AnimalBase_C|SetAttacking (Variables|Default|GetAnimalBase) false)
        ;[1 1 1] Set next Roam Behavior
        (bind _newroambehavior_2 (Default|FnSetRoamBehavior (Variables|Default|GetAnimalBase)))
        (|SETNEXTBEHAVIORINTHEBLACKBOARD_2 _newroambehavior_2
          (:OutputPin
            ;[1 1 1] Finished eating - set BiggestNeed to Roam again
            (Variables|/Game/AnimalBehaviorKit/Blueprints/Characters/Animals/GroundAnimals/BP_GroundAnimalBase.BP_GroundAnimalBase_C|SetBiggestNeed (Variables|Default|GetAnimalBase) "NewEnumerator3")
            (AI|BehaviorTree|FinishExecute true)))))
    (else
      (AI|BehaviorTree|FinishExecute true))))

(event EventReceiveTickAI
  (params (OwnerController :type AI%20Controller%20Object%20Reference) (ControlledPawn :type Pawn%20Object%20Reference) (DeltaSeconds :type Float%20%28single-precision%29))
  (bind (_in_range _newspeed) (CallFunction|FnGetEngageTargetSpeed))
  (bind _pawnref (Variables|Default|GetPawnRef))
  (bind _returnvalue (Transformation|GetActorRotation _pawnref))
  (bind (_roll _pitch) (Math|Rotator|BreakRotator _returnvalue))
  ;[1 1 1] Check Engage Actor is Valid
  (Utilities|IsValid (AI|BehaviorTree|GetBlackboardValueasActor (Variables|Setup|GetEngageActor))
    (:Is%20Valid
      (Utilities|FlowControl|Sequence
        (:then_0
          ;[1 1 1] Check if we want to use Accurate Target Detection
          (if (Utilities|Struct|BreakBP_Struct_GroundAnimalBehavior_AnimalDetails_Attack (Variables|/Game/AnimalBehaviorKit/Blueprints/Characters/Animals/GroundAnimals/BP_GroundAnimalBase.BP_GroundAnimalBase_C|GetBehavior_Details_Attack (Variables|Default|GetAnimalBase)))
            ;[1 1 1] Check if we are in melee range
            (if _in_range
              ;[1 1 1] Melee Range - match target speed
              (Variables|/Script/Engine.CharacterMovementComponent|SetMaxWalkSpeed (Variables|/Script/Engine.Character|GetCharacterMovement (Variables|Default|GetAnimalBase)) (Math|Float|Clamp(Float) _newspeed 0.0 (Variables|Default|GetMaxWalkSpeed)))
              (Variables|Default|SetInMeleeRange true)
              (else
                ;[1 1 1] Not in melee range
                (Variables|/Script/Engine.CharacterMovementComponent|SetMaxWalkSpeed (Variables|/Script/Engine.Character|GetCharacterMovement (Variables|Default|GetAnimalBase)) (Variables|Default|GetMaxWalkSpeed))
                (Variables|Default|SetInMeleeRange false)
                ;[1 1 1] Check that we are not currently attacking
                (if (not (Variables|/Game/AnimalBehaviorKit/Blueprints/Characters/Animals/BP_AnimalBase.BP_AnimalBase_C|GetAttacking (Variables|Default|GetAnimalBase)))
                  (AI|BehaviorTree|FinishExecute true))))))
        (:then_1
          ;[1 1 1] If StopMovement is False, move animal towards target
          (if (not (Variables|Default|GetStopMovement))
            ;[1 1 1] Set actor location to EngageActor
            (AI|AIMoveTo (Variables|Default|GetPawnRef) (select (Variables|Default|GetInMeleeRange) (Variables|Default|GetTargetLocation) (Transformation|GetActorLocation (AI|BehaviorTree|GetBlackboardValueasActor (Variables|Setup|GetEngageActor)))) 0 (Variables|Default|GetAcceptanceRadius) true
              (:then
                ;[1 1 1] Set Moving to True
                (Class|BTFunctionLibrary|SetBlackboardValueasBool (Variables|Default|GetMoving) false))
              (:OnSuccess
                ;[1 1 1] Set Moving to False
                (Class|BTFunctionLibrary|SetBlackboardValueasBool (Variables|Default|GetMoving) false))
              (:OnFail
                ;[1 1 1] Set Moving to False
                (Class|BTFunctionLibrary|SetBlackboardValueasBool (Variables|Default|GetMoving) false)))))
        (:then_2
          ;[1 1 1] Rotate towards target
          (Transformation|SetActorRotation (Variables|Default|GetPawnRef) (Math|Interpolation|RInterpTo _returnvalue (Math|Rotator|MakeRotator _roll _pitch (.yaw (Math|Rotator|FindLookatRotation (Transformation|GetActorLocation (Variables|Default|GetPawnRef)) (select (Variables|Default|GetInMeleeRange) (Variables|Default|GetTargetLocation) (Transformation|GetActorLocation (AI|BehaviorTree|GetBlackboardValueasActor (Variables|Setup|GetEngageActor))))))) (Utilities|Time|GetWorldDeltaSeconds) 1.0)))))))

(fn FnGetEngageTargetSpeed
  (bind _animalbase (Variables|Default|GetAnimalBase))
  (bind _animalbase_2 (Variables|Default|GetAnimalBase))
  (bind _returnvalue (Transformation|GetActorLocation _animalbase))
  (bind _collision_attack (Variables|/Game/AnimalBehaviorKit/Blueprints/Characters/Animals/GroundAnimals/BP_GroundAnimalBase.BP_GroundAnimalBase_C|GetCollision_Attack _animalbase_2))
  (bind _returnvalue_2 (Transformation|GetWorldLocation _collision_attack))
  (Utilities|IsValid (AI|BehaviorTree|GetBlackboardValueasActor (Variables|Setup|GetEngageActor))
    (:Is%20Valid
      (Utilities|FlowControl|Sequence
        (:then_0
          (if (Variables|Default|GetDebugMeleeRange)
            (LocalVariables|SetDebugType "ForOneFrame")
            (else
              (LocalVariables|SetDebugType "None")))
          ;[1 1 1] Check if we are in attack range with target
          (bind (_outhits _returnvalue_3) (Collision|MultiSphereTraceForObjects _returnvalue_2 (+ _returnvalue_2 "0, 0,0.010000") (* (Variables|/Script/Engine.SphereComponent|GetSphereRadius _collision_attack) (Variables|Default|GetCollisionRadiusMultiplier)) (Variables|/Game/AnimalBehaviorKit/Blueprints/Characters/Animals/GroundAnimals/BP_GroundAnimalBase.BP_GroundAnimalBase_C|GetDamageObjectTypes (Variables|Default|GetAnimalBase)) true (Utilities|Array|MakeArray (Variables|Default|GetAnimalBase)) (LocalVariables|GetDebugType)))
          (if _returnvalue_3
            (bind _array_element (Utilities|Array|ForEachLoopwithBreak _outhits :!label _label)
              (:LoopBody
                (if (== (AI|BehaviorTree|GetBlackboardValueasActor (Variables|Setup|GetEngageActor)) (Components|GetOwner (.HitComponent (Collision|BreakHitResult _array_element))))
                  (LocalVariables|SetInRange true)
                  (goto _label Break)))
              (:Completed
                ;[1 1 1] Check if we are in attack range with target
                (bind (_outhits_2 _returnvalue_4) (Class|KismetSystemLibrary|LineTraceMultiforObjects _returnvalue (+ _returnvalue (* (Math|Vector|GetForwardVector (Math|Rotator|FindLookatRotation _returnvalue (Transformation|GetActorLocation (AI|BehaviorTree|GetBlackboardValueasActor (Variables|Setup|GetEngageActor))))) (LocalVariables|GetTraceLength))) (Variables|/Game/AnimalBehaviorKit/Blueprints/Characters/Animals/GroundAnimals/BP_GroundAnimalBase.BP_GroundAnimalBase_C|GetDamageObjectTypes (Variables|Default|GetAnimalBase)) true (Utilities|Array|MakeArray (Variables|Default|GetAnimalBase)) (LocalVariables|GetDebugType) true))
                (if _returnvalue_4
                  (bind _array_element_2 (Utilities|Array|ForEachLoopwithBreak _outhits_2 :!label _label_2)
                    (:LoopBody
                      (if (== (AI|BehaviorTree|GetBlackboardValueasActor (Variables|Setup|GetEngageActor)) (Components|GetOwner (.HitComponent (Collision|BreakHitResult _array_element_2))))
                        (Variables|Default|SetTargetLocation (.ImpactPoint (Collision|BreakHitResult _array_element_2)))
                        (Variables|Default|SetTargetRotation (Math|Rotator|MakeRotfromXZ (.Normal (Collision|BreakHitResult _array_element_2)) (Transformation|GetActorUpVector (Variables|Default|GetAnimalBase))))
                        (goto _label_2 Break)))))))))
        (:then_1
          (if (LocalVariables|GetInRange)
            ;[1 1 1] Get EngageActor's speed and set it for this animal
            (LocalVariables|SetSpeed (Math|Vector|VectorLength (Transformation|GetVelocity (AI|BehaviorTree|GetBlackboardValueasActor (Variables|Setup|GetEngageActor)))))))
        (:then_2
          (return (LocalVariables|GetInRange) (LocalVariables|GetSpeed)))))))