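; Behavior tree task that sends a thirsty ground animal to the water in the NearestWater blackboard key to drink.
; It moves to the closest point on the water's spline, retrying at a random spline point if that fails.
; A self-calling event loops the drink montage until DrinkingTime ends.
; It then resets thirst and writes the next roam behavior to the blackboard, favoring home base when enabled.
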(event Custom|EventPlayDrinkAnimation
  (if (Variables|Default|GetCanDrink)
    ;[1 1 1] Check that the Biggest Need is Drinking
    (if (Utilities|Enum|Equal(Enum) (Variables|/Game/AnimalBehaviorKit/Blueprints/Characters/Animals/GroundAnimals/BP_GroundAnimalBase.BP_GroundAnimalBase_C|GetBiggestNeed (Variables|Default|GetAnimalBase)) "NewEnumerator1")
      ;[1 1 1] Play Drink animation
      (Default|EventPlayAnimation (Variables|Default|GetAnimalBase) "NewEnumerator4")
      ;[1 1 1] Wait for the drink animation duration
      (bind _returnvalue (Animation|GetCurrentMontage (Variables|Default|GetAnimalBase) :!class /Script/Engine.Character))
      (Utilities|IsValid _returnvalue
        (:Is%20Valid
          (bind _returnvalue_2 (Animation|GetPlayLength _returnvalue))
          (Utilities|FlowControl|Delay _returnvalue_2))
        (:Is%20Not%20Valid
          _))
      (CallFunction|EventPlayDrinkAnimation))
    (else
      ;[1 1 1] Stop current animation montage
      (bind _returnvalue_3 (Animation|GetCurrentMontage (Variables|Default|GetAnimalBase) :!class /Script/Engine.Character))
      (Animation|StopAnimMontage (Variables|Default|GetAnimalBase) _returnvalue_3))))

(event EventReceiveExecuteAI
  (params (OwnerController :type AI%20Controller%20Object%20Reference) (ControlledPawn :type Pawn%20Object%20Reference))
  (Variables|Default|SetPawnRef ControlledPawn)
  (bind _asbp_ground_animal_base (Utilities|Casting|CastToBP_GroundAnimalBase (Variables|Default|GetPawnRef)))
  (Variables|Default|SetAnimalBase _asbp_ground_animal_base)
  ;[1 1 1] Check if we have Comp_NeedSystem
  (Utilities|IsValid (Actor|GetComponentbyClass (Variables|Default|GetAnimalBase) "/Game/AnimalBehaviorKit/Blueprints/AI/Components/GroundAnimals/BP_Comp_NeedSystem.BP_Comp_NeedSystem_C")
    (:Is%20Valid
      ;[1 1 1] Save NeedSystem
      (Variables|Default|SetNeedSystem (Actor|GetComponentbyClass (Variables|Default|GetAnimalBase) "/Game/AnimalBehaviorKit/Blueprints/AI/Components/GroundAnimals/BP_Comp_NeedSystem.BP_Comp_NeedSystem_C"))
      ;[1 1 1] Use HomeBase?
      (Variables|Default|SetUseHomeBase? (Variables|/Game/AnimalBehaviorKit/Blueprints/Characters/Animals/GroundAnimals/BP_GroundAnimalBase.BP_GroundAnimalBase_C|GetUseHomeBase? (Variables|Default|GetAnimalBase)))
      ;[1 1 1] Set Acceptance Radius
      (Variables|Default|SetAcceptanceRadius (Variables|/Game/AnimalBehaviorKit/Blueprints/Characters/Animals/GroundAnimals/BP_GroundAnimalBase.BP_GroundAnimalBase_C|GetMovementAcceptanceRadius (Variables|Default|GetAnimalBase)))
      ;[1 1 1] Set DrinkingTime
      (Variables|Default|SetDrinkingTime (.DrinkingTime (Utilities|Struct|BreakBP_Struct_Need_Drink (Variables|/Game/AnimalBehaviorKit/Blueprints/AI/Components/GroundAnimals/BP_Comp_NeedSystem.BP_Comp_NeedSystem_C|GetThristDetails (Variables|Default|GetNeedSystem)))))
      ;[1 1 1] Check NearestWater is valid
      (Utilities|IsValid (Class|BTFunctionLibrary|GetBlackboardValueasObject (Variables|Setup|GetNearestWater))
        (:Is%20Valid
          ;[1 1 1] Get nearest water source and Move AI to that location
          (bind _asbp_ai_water (Utilities|Casting|CastToBP_AI_Water (Class|BTFunctionLibrary|GetBlackboardValueasObject (Variables|Setup|GetNearestWater))))
          (AI|AIMoveTo (Variables|Default|GetPawnRef) (Spline|FindLocationClosesttoWorldLocation (Variables|/Game/AnimalBehaviorKit/Blueprints/AI/Actors/Ground_AI/NeedSystem/BP_AI_Water.BP_AI_Water_C|GetSpline _asbp_ai_water) (Transformation|GetActorLocation (Variables|Default|GetPawnRef)) "World") 0 (Variables|Default|GetAcceptanceRadius) true
            (:then
              ;[1 1 1] Set Moving to True
              (Class|BTFunctionLibrary|SetBlackboardValueasBool (Variables|Default|GetMoving) true))
            (:OnSuccess
              ;[1 1 1] Set Moving to False
              (Class|BTFunctionLibrary|SetBlackboardValueasBool (Variables|Default|GetMoving) false)
              ;[1 1 1] Play Drink animation
              (CallFunction|EventPlayDrinkAnimation :!label _label)
              ;[1 1 1] Wait WaitAtDestination seconds
              (Utilities|FlowControl|Delay (Variables|Default|GetDrinkingTime))
              ;[1 1 1] Check if we are playing the animation montage and stop it
              (Variables|Default|SetCanDrink false)
              (bind _returnvalue (Animation|GetCurrentMontage (Variables|Default|GetAnimalBase) :!class /Script/Engine.Character))
              (Animation|StopAnimMontage (Variables|Default|GetAnimalBase) _returnvalue)
              ;[1 1 1] This delay accounts for the drinking montage's blend out time. You may need to adjust this depending on your animation
              (Utilities|FlowControl|Delay 1.5)
              (if (Variables|Default|GetUseHomeBase?)
                (Variables|/Game/AnimalBehaviorKit/Blueprints/Characters/Animals/GroundAnimals/BP_GroundAnimalBase.BP_GroundAnimalBase_C|SetRoamBehavior (Variables|Default|GetAnimalBase) "NewEnumerator6"))
              ;[1 1 1] Set next Roam Behavior
              (bind _newroambehavior (Default|FnSetRoamBehavior (Variables|Default|GetAnimalBase)))
              (|SETNEXTBEHAVIORINTHEBLACKBOARD _newroambehavior
                (:OutputPin
                  ;[1 1 1] Finished drinking - set BiggestNeed to Roam again
                  (Variables|/Game/AnimalBehaviorKit/Blueprints/Characters/Animals/GroundAnimals/BP_GroundAnimalBase.BP_GroundAnimalBase_C|SetBiggestNeed (Variables|Default|GetAnimalBase) "NewEnumerator3")
                  ;[1 1 1] Reset Thirst
                  (Default|EventFinishedDrinking (Variables|Default|GetNeedSystem))
                  (Variables|Default|SetCanDrink true)
                  (AI|BehaviorTree|FinishExecute true))))
            (:OnFail
              ;[1 1 1] Set Moving to False
              (Class|BTFunctionLibrary|SetBlackboardValueasBool (Variables|Default|GetMoving) false)
              (|RANDOMLOCATIONINWATERSPLINE
                (:OnSuccess
                  (goto _label))
                (:OnFail
                  (AI|BehaviorTree|FinishExecute false))))))
        (:Is%20Not%20Valid
          (AI|BehaviorTree|FinishExecute false))))
    (:Is%20Not%20Valid
      (AI|BehaviorTree|FinishExecute false))))