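; Behavior tree task that walks a ground animal to a custom target location stored in the blackboard.
; In Walk movement mode, it picks a random navigable point within the animal's acceptance radius of that location and runs AI MoveTo.
; It tracks the Moving key, clearing CustomTargetActive only on success.
; If the cast or Walk check fails, the task never calls FinishExecute.
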(event EventReceiveExecuteAI
  (params (OwnerController :type AI%20Controller%20Object%20Reference) (ControlledPawn :type Pawn%20Object%20Reference))
  (Variables|Default|SetPawnRef ControlledPawn)
  (bind _asbp_ground_animal_base (Utilities|Casting|CastToBP_GroundAnimalBase (Variables|Default|GetPawnRef)))
  (Variables|Default|SetAnimalBase _asbp_ground_animal_base)
  ;[1 1 1] Check that the current movement mode is Walk
  (if (Utilities|Enum|Equal(Enum) (Variables|/Game/AnimalBehaviorKit/Blueprints/Characters/Animals/GroundAnimals/BP_GroundAnimalBase.BP_GroundAnimalBase_C|GetCurrentMovementMode (Variables|Default|GetAnimalBase)) "NewEnumerator0")
    ;[1 1 1] Set Custom Target
    (Variables|Default|SetCustomLoc (Class|BTFunctionLibrary|GetBlackboardValueasVector (Variables|Default|GetCustomLocation)))
    ;[1 1 1] Set Acceptance Radius
    (Variables|Default|SetAcceptanceRadius (Variables|/Game/AnimalBehaviorKit/Blueprints/Characters/Animals/GroundAnimals/BP_GroundAnimalBase.BP_GroundAnimalBase_C|GetMovementAcceptanceRadius (Variables|Default|GetAnimalBase)))
    ;[1 1 1] Get target location
    (Variables|Default|SetTargetLocation (.RandomLocation (Class|NavigationSystem|GetRandomPointinNavigableRadius (Variables|Default|GetCustomLoc) (Variables|Default|GetAcceptanceRadius))))
    ;[1 1 1] Move towards CustomTarget
    (AI|AIMoveTo (Variables|Default|GetPawnRef) (Variables|Default|GetTargetLocation) 0 (Variables|Default|GetAcceptanceRadius) true
      (:then
        ;[1 1 1] Set Moving to True
        (Class|BTFunctionLibrary|SetBlackboardValueasBool (Variables|Default|GetMoving) true))
      (:OnSuccess
        ;[1 1 1] Set Moving to False
        (Class|BTFunctionLibrary|SetBlackboardValueasBool (Variables|Default|GetMoving) false)
        (Class|BTFunctionLibrary|SetBlackboardValueasBool (Variables|Default|GetCustomTargetActive) false)
        (AI|BehaviorTree|FinishExecute true))
      (:OnFail
        ;[1 1 1] Set Moving to False
        (Class|BTFunctionLibrary|SetBlackboardValueasBool (Variables|Default|GetMoving) false)
        (AI|BehaviorTree|FinishExecute false)))))