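; Behavior tree task that walks a ground animal along waypoints of its assigned path or the blackboard's nearest path.
; EventFollowPath re-calls itself per waypoint, randomizing speed and acceleration, then playing an animation and waiting on arrival.
; At path ends it loops or reverses in one roam mode, or hands off to GoToHomeBase and finishes when home base is used.
; A failed move only resets movement, without finishing the task.
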(event Custom|EventFollowPath
  (|SETRANDOMWALKSPEEDANDACCELERATION)
  (switch Utilities|FlowControl|Switch|SwitchonBP_Enum_PathSelection (Variables|Default|GetPathSelection)
    (:NewEnumerator0
      ;[1 1 1] Move AI to specified Path
      (AI|AIMoveTo (Variables|Default|GetPawnRef) (Transformation|GetActorLocation (Utilities|Array|Get(acopy) (Variables|/Game/AnimalBehaviorKit/Blueprints/AI/Actors/Ground_AI/Navigation/BP_AIPath.BP_AIPath_C|GetListOfWayPoints (Variables|Default|GetPathRef)) (Variables|Default|GetCurrentWayPoint))) 0 (Variables|Default|GetMoveRadius) true
        (:then
          ;[1 1 1] Set Moving to True
          (Class|BTFunctionLibrary|SetBlackboardValueasBool (Variables|Default|GetMoving) true))
        (:OnSuccess
          ;[1 1 1] Set Moving to False
          (Class|BTFunctionLibrary|SetBlackboardValueasBool (Variables|Default|GetMoving) false)
          ;[1 1 1] Play Idle animation
          (Default|EventPlayAnimation (Variables|Default|GetAnimalBase) "NewEnumerator6" :!label _label)
          ;[1 1 1] Wait for the idle animation duration
          (bind _returnvalue (Animation|GetCurrentMontage (Variables|Default|GetAnimalBase) :!class /Script/Engine.Character))
          (Utilities|IsValid _returnvalue
            (:Is%20Valid
              (bind _returnvalue_2 (Animation|GetPlayLength _returnvalue))
              (Utilities|FlowControl|Delay _returnvalue_2))
            (:Is%20Not%20Valid
              _))
          ;[1 1 1] Wait WaitAtDestination seconds
          (Utilities|FlowControl|Delay (Variables|Default|GetWaitAtWayPoint))
          ;[1 1 1] Are we going forward in the path?
          (if (Variables|Default|GetGoingForward?)
            ;[1 1 1] Is CurrentWayPoint Less Than the Last WayPoint in the Path?
            (if (< (Variables|Default|GetCurrentWayPoint) (- (Utilities|Array|Length (Variables|/Game/AnimalBehaviorKit/Blueprints/AI/Actors/Ground_AI/Navigation/BP_AIPath.BP_AIPath_C|GetListOfWayPoints (Variables|Default|GetPathRef))) 1))
              ;[1 1 1] Increase the CurrentWayPoint by 1
              (Math|Integer|IncrementInt (Variables|Default|GetCurrentWayPoint)
                (:%20%20
                  (|RESETWALKSPEEDANDACCELERATION_2 :!label _label_2)
                  ;[1 1 1] Call event again to go to the next WayPoint
                  (CallFunction|EventFollowPath)))
              (else
                ;[1 1 1] Do we NOT use the Home Base?
                (if (not (Variables|Default|GetUseHomeBase?))
                  ;[1 1 1] Is Roam Mode Specific?
                  (if (Utilities|Enum|Equal(Enum) (Variables|/Game/AnimalBehaviorKit/Blueprints/Characters/Animals/GroundAnimals/BP_GroundAnimalBase.BP_GroundAnimalBase_C|GetRoamMode (Variables|Default|GetAnimalBase)) "NewEnumerator0")
                    (if (Variables|Default|GetIsPathLooped?)
                      ;[1 1 1] Go to the first WayPoint
                      (Variables|Default|SetCurrentWayPoint 0)
                      (goto _label_2)
                      (else
                        ;[1 1 1] Go back 1 WayPoint
                        (Math|Integer|DecrementInt (Variables|Default|GetCurrentWayPoint)
                          (:%20%20
                            ;[1 1 1] Set to False so we now go back through the path
                            (Variables|Default|SetGoingForward? false)
                            (goto _label_2))))))
                  (else
                    (if (Variables|Default|GetUseHomeBase?)
                      ;[1 1 1] Set BB RoamBehavior to selected behavior
                      (Class|BTFunctionLibrary|SetBlackboardValueasEnum (Variables|Default|GetRoamBehavior) (Utilities|Enum|LiteralenumBP_Enum_AIRoamBehavior "NewEnumerator6"))
                      (Variables|/Game/AnimalBehaviorKit/Blueprints/Characters/Animals/GroundAnimals/BP_GroundAnimalBase.BP_GroundAnimalBase_C|SetRoamBehavior (Variables|Default|GetAnimalBase) "NewEnumerator6")
                      (else
                        ;[1 1 1] Set next Roam Behavior
                        (bind _newroambehavior (Default|FnSetRoamBehavior (Variables|Default|GetAnimalBase)))
                        (|SETNEXTBEHAVIORINTHEBLACKBOARD_2 _newroambehavior
                          (:OutputPin
                            ;[1 1 1] Finished drinking - set BiggestNeed to Roam again
                            (Variables|/Game/AnimalBehaviorKit/Blueprints/Characters/Animals/GroundAnimals/BP_GroundAnimalBase.BP_GroundAnimalBase_C|SetBiggestNeed (Variables|Default|GetAnimalBase) "NewEnumerator3")))))
                    (|RESETWALKSPEEDANDACCELERATION_3)
                    (AI|BehaviorTree|FinishExecute true)))))
            (else
              ;[1 1 1] Is CurrentWayPoint Bigger Than the First WayPoint in the Path?
              (if (> (Variables|Default|GetCurrentWayPoint) 0)
                ;[1 1 1] Decrease the CurrentWayPoint by 1
                (Math|Integer|DecrementInt (Variables|Default|GetCurrentWayPoint)
                  (:%20%20
                    (|RESETWALKSPEEDANDACCELERATION_4 :!label _label_3)
                    ;[1 1 1] Call event again to go to the next WayPoint
                    (CallFunction|EventFollowPath)))
                (else
                  ;[1 1 1] Do we NOT use the Home Base?
                  (if (not (Variables|Default|GetUseHomeBase?))
                    ;[1 1 1] Is Roam Mode Specific?
                    (if (Utilities|Enum|Equal(Enum) (Variables|/Game/AnimalBehaviorKit/Blueprints/Characters/Animals/GroundAnimals/BP_GroundAnimalBase.BP_GroundAnimalBase_C|GetRoamMode (Variables|Default|GetAnimalBase)) "NewEnumerator0")
                      (if (Variables|Default|GetIsPathLooped?)
                        ;[1 1 1] Go to the last WayPoint
                        (Variables|Default|SetCurrentWayPoint (- (Utilities|Array|Length (Variables|/Game/AnimalBehaviorKit/Blueprints/AI/Actors/Ground_AI/Navigation/BP_AIPath.BP_AIPath_C|GetListOfWayPoints (Variables|Default|GetPathRef))) 1))
                        (goto _label_3)
                        (else
                          ;[1 1 1] Go back 1 WayPoint
                          (Math|Integer|IncrementInt (Variables|Default|GetCurrentWayPoint)
                            (:%20%20
                              ;[1 1 1] Set to True so we now go forward through the path
                              (Variables|Default|SetGoingForward? true)
                              (goto _label_3))))))
                    (else
                      (if (Variables|Default|GetUseHomeBase?)
                        ;[1 1 1] Set BB RoamBehavior to selected behavior
                        (Class|BTFunctionLibrary|SetBlackboardValueasEnum (Variables|Default|GetRoamBehavior) (Utilities|Enum|LiteralenumBP_Enum_AIRoamBehavior "NewEnumerator6"))
                        (Variables|/Game/AnimalBehaviorKit/Blueprints/Characters/Animals/GroundAnimals/BP_GroundAnimalBase.BP_GroundAnimalBase_C|SetRoamBehavior (Variables|Default|GetAnimalBase) "NewEnumerator6")
                        (else
                          ;[1 1 1] Set next Roam Behavior
                          (bind _newroambehavior_2 (Default|FnSetRoamBehavior (Variables|Default|GetAnimalBase)))
                          (|SETNEXTBEHAVIORINTHEBLACKBOARD _newroambehavior_2
                            (:OutputPin
                              ;[1 1 1] Finished drinking - set BiggestNeed to Roam again
                              (Variables|/Game/AnimalBehaviorKit/Blueprints/Characters/Animals/GroundAnimals/BP_GroundAnimalBase.BP_GroundAnimalBase_C|SetBiggestNeed (Variables|Default|GetAnimalBase) "NewEnumerator3")))))
                      (|RESETWALKSPEEDANDACCELERATION_5)
                      (AI|BehaviorTree|FinishExecute true))))))))
        (:OnFail
          ;[1 1 1] Set Moving to False
          (Class|BTFunctionLibrary|SetBlackboardValueasBool (Variables|Default|GetMoving) false)
          (|RESETWALKSPEEDANDACCELERATION :!label _label_4))))
    (:NewEnumerator1
      ;[1 1 1] Move AI to nearest path
      (bind _asbp_aipath (Utilities|Casting|CastToBP_AIPath (Class|BTFunctionLibrary|GetBlackboardValueasObject (Variables|Default|GetNearestPath))))
      (Variables|Default|SetPathRef _asbp_aipath)
      (AI|AIMoveTo (Variables|Default|GetPawnRef) (Transformation|GetActorLocation (Utilities|Array|Get(acopy) (Variables|/Game/AnimalBehaviorKit/Blueprints/AI/Actors/Ground_AI/Navigation/BP_AIPath.BP_AIPath_C|GetListOfWayPoints _asbp_aipath) (Variables|Default|GetCurrentWayPoint))) 0 (Variables|Default|GetMoveRadius) true
        (:then
          ;[1 1 1] Set Moving to True
          (Class|BTFunctionLibrary|SetBlackboardValueasBool (Variables|Default|GetMoving) true))
        (:OnSuccess
          ;[1 1 1] Set Moving to False
          (Class|BTFunctionLibrary|SetBlackboardValueasBool (Variables|Default|GetMoving) false)
          (goto _label))
        (:OnFail
          ;[1 1 1] Set Moving to False
          (Class|BTFunctionLibrary|SetBlackboardValueasBool (Variables|Default|GetMoving) false)
          (goto _label_4))))))

(event EventReceiveExecuteAI
  (params (OwnerController :type AI%20Controller%20Object%20Reference) (ControlledPawn :type Pawn%20Object%20Reference))
  (bind _output_get (Variables|Default|SetPawnRef ControlledPawn))
  (Utilities|IsValid _output_get
    (:Is%20Valid
      (bind _asbp_ground_animal_base (Utilities|Casting|CastToBP_GroundAnimalBase (Variables|Default|GetPawnRef)))
      (Variables|Default|SetAnimalBase _asbp_ground_animal_base)
      ;[1 1 1] Use HomeBase?
      (Variables|Default|SetUseHomeBase? (Variables|/Game/AnimalBehaviorKit/Blueprints/Characters/Animals/GroundAnimals/BP_GroundAnimalBase.BP_GroundAnimalBase_C|GetUseHomeBase? (Variables|Default|GetAnimalBase)))
      ;[1 1 1] Set WaitAtDestination
      (Variables|Default|SetWaitAtWayPoint (Math|Random|RandomFloatinRange (.x (Utilities|Struct|BreakBP_Struct_GroundAnimalBehavior_FollowPath (Variables|/Game/AnimalBehaviorKit/Blueprints/Characters/Animals/GroundAnimals/BP_GroundAnimalBase.BP_GroundAnimalBase_C|GetBehavior_FollowPath (Variables|Default|GetAnimalBase)))) (.y (Utilities|Struct|BreakBP_Struct_GroundAnimalBehavior_FollowPath (Variables|/Game/AnimalBehaviorKit/Blueprints/Characters/Animals/GroundAnimals/BP_GroundAnimalBase.BP_GroundAnimalBase_C|GetBehavior_FollowPath (Variables|Default|GetAnimalBase))))))
      ;[1 1 1] Save the Path reference
      (Utilities|IsValid (Utilities|Struct|BreakBP_Struct_GroundAnimalBehavior_FollowPath (Variables|/Game/AnimalBehaviorKit/Blueprints/Characters/Animals/GroundAnimals/BP_GroundAnimalBase.BP_GroundAnimalBase_C|GetBehavior_FollowPath (Variables|Default|GetAnimalBase)))
        (:Is%20Valid
          (Variables|Default|SetPathRef (Utilities|Struct|BreakBP_Struct_GroundAnimalBehavior_FollowPath (Variables|/Game/AnimalBehaviorKit/Blueprints/Characters/Animals/GroundAnimals/BP_GroundAnimalBase.BP_GroundAnimalBase_C|GetBehavior_FollowPath (Variables|Default|GetAnimalBase))))
          ;[1 1 1] Set IsPathLooped?
          (Variables|Default|SetIsPathLooped? (Variables|/Game/AnimalBehaviorKit/Blueprints/AI/Actors/Ground_AI/Navigation/BP_AIPath.BP_AIPath_C|GetPathIsLooped? (Variables|Default|GetPathRef)))
          ;[1 1 1] Set GoingForward?
          (Variables|Default|SetGoingForward? (Variables|/Game/AnimalBehaviorKit/Blueprints/AI/Actors/Ground_AI/Navigation/BP_AIPath.BP_AIPath_C|GetGoingForward? (Variables|Default|GetPathRef)))
          ;[1 1 1] Set CurrentWayPoint
          (Variables|Default|SetCurrentWayPoint (Utilities|Struct|BreakBP_Struct_GroundAnimalBehavior_FollowPath (Variables|/Game/AnimalBehaviorKit/Blueprints/Characters/Animals/GroundAnimals/BP_GroundAnimalBase.BP_GroundAnimalBase_C|GetBehavior_FollowPath (Variables|Default|GetAnimalBase))))
          ;[1 1 1] Set PathSelection
          (Variables|Default|SetPathSelection (Utilities|Struct|BreakBP_Struct_GroundAnimalBehavior_FollowPath (Variables|/Game/AnimalBehaviorKit/Blueprints/Characters/Animals/GroundAnimals/BP_GroundAnimalBase.BP_GroundAnimalBase_C|GetBehavior_FollowPath (Variables|Default|GetAnimalBase))))
          ;[1 1 1] Get Movement Acceptance Radius
          (Variables|Default|SetMoveRadius (Variables|/Game/AnimalBehaviorKit/Blueprints/Characters/Animals/GroundAnimals/BP_GroundAnimalBase.BP_GroundAnimalBase_C|GetMovementAcceptanceRadius (Variables|Default|GetAnimalBase)))
          (CallFunction|EventFollowPath))
        (:Is%20Not%20Valid
          ;[1 1 1] Error Message
          (Development|PrintString (Utilities|String|Append (Utilities|GetDisplayName (Variables|Default|GetAnimalBase)) ": No Path found!") true true "(R=1.000000,G=0.000000,B=0.000000,A=1.000000)" 5.0))))))