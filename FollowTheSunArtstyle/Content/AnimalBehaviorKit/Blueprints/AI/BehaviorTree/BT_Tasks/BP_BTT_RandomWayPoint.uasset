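; Behavior tree task that sends a ground animal to the waypoint stored in the blackboard, if it lies within search radius.
; It randomly scales walk speed and acceleration, moves while updating the Moving key, then idles and waits on arrival.
; It then writes the next RoamBehavior, either home base or the animal's own selection, and restores movement values.
; A missing waypoint only prints an error, without finishing the task.
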(event EventReceiveExecuteAI
  (params (OwnerController :type AI%20Controller%20Object%20Reference) (ControlledPawn :type Pawn%20Object%20Reference))
  (bind _waypoint (Variables|Default|GetWayPoint))
  (bind _returnvalue (Class|BTFunctionLibrary|GetBlackboardValueasObject _waypoint))
  (bind _output_get (Variables|Default|SetPawnRef ControlledPawn))
  (Utilities|IsValid _output_get
    (:Is%20Valid
      (bind _asbp_ground_animal_base (Utilities|Casting|CastToBP_GroundAnimalBase (Variables|Default|GetPawnRef)))
      (Variables|Default|SetAnimalBase _asbp_ground_animal_base)
      ;[1 1 1] Use HomeBase?
      (Variables|Default|SetUseHomeBase? (Variables|/Game/AnimalBehaviorKit/Blueprints/Characters/Animals/GroundAnimals/BP_GroundAnimalBase.BP_GroundAnimalBase_C|GetUseHomeBase? (Variables|Default|GetAnimalBase)))
      ;[1 1 1] Set WaitAtDestination
      (Variables|Default|SetWaitAtDestination (Math|Random|RandomFloatinRange (.x (.Waitatlocationrange (Utilities|Struct|BreakBP_Struct_GroundAnimalBehavior_Location (Variables|/Game/AnimalBehaviorKit/Blueprints/Characters/Animals/GroundAnimals/BP_GroundAnimalBase.BP_GroundAnimalBase_C|GetBehavior_Location (Variables|Default|GetAnimalBase))))) (.y (.Waitatlocationrange (Utilities|Struct|BreakBP_Struct_GroundAnimalBehavior_Location (Variables|/Game/AnimalBehaviorKit/Blueprints/Characters/Animals/GroundAnimals/BP_GroundAnimalBase.BP_GroundAnimalBase_C|GetBehavior_Location (Variables|Default|GetAnimalBase)))))))
      ;[1 1 1] Set Search Radius
      (Variables|Default|SetSearchRadius (.SearchRadius (Utilities|Struct|BreakBP_Struct_GroundAnimalBehavior_Location (Variables|/Game/AnimalBehaviorKit/Blueprints/Characters/Animals/GroundAnimals/BP_GroundAnimalBase.BP_GroundAnimalBase_C|GetBehavior_Location (Variables|Default|GetAnimalBase)))))
      ;[1 1 1] Get Movement Acceptance Radius
      (Variables|Default|SetMoveRadius (Variables|/Game/AnimalBehaviorKit/Blueprints/Characters/Animals/GroundAnimals/BP_GroundAnimalBase.BP_GroundAnimalBase_C|GetMovementAcceptanceRadius (Variables|Default|GetAnimalBase)))
      ;[1 1 1] Choose random WayPoint from returned list and get location
      (Utilities|IsValid _returnvalue
        (:Is%20Valid
          (bind _asbp_ai_way_point (Utilities|Casting|CastToBP_AI_WayPoint _returnvalue))
          (Variables|Default|SetDestination (Transformation|GetActorLocation _asbp_ai_way_point))
          ;[1 1 1] Check that the Destination is within the Search Radius
          (if (<= (Math|Vector|VectorLength (- (Variables|Default|GetDestination) (Transformation|GetActorLocation (Variables|Default|GetPawnRef)))) (Variables|Default|GetSearchRadius))
            (|SETRANDOMWALKSPEEDANDACCELERATION)
            ;[1 1 1] Move to Destination
            (AI|AIMoveTo (Variables|Default|GetPawnRef) (Variables|Default|GetDestination) 0 (Variables|Default|GetMoveRadius) true
              (:then
                ;[1 1 1] Set Moving to True
                (Class|BTFunctionLibrary|SetBlackboardValueasBool (Variables|Default|GetMoving) true))
              (:OnSuccess
                ;[1 1 1] Set Moving to False
                (Class|BTFunctionLibrary|SetBlackboardValueasBool (Variables|Default|GetMoving) false)
                ;[1 1 1] Play Idle animation
                (Default|EventPlayAnimation (Variables|Default|GetAnimalBase) "NewEnumerator6")
                ;[1 1 1] Wait for the idle animation duration
                (bind _returnvalue_2 (Animation|GetCurrentMontage (Variables|Default|GetAnimalBase) :!class /Script/Engine.Character))
                (Utilities|IsValid _returnvalue_2
                  (:Is%20Valid
                    (bind _returnvalue_3 (Animation|GetPlayLength _returnvalue_2))
                    (Utilities|FlowControl|Delay _returnvalue_3))
                  (:Is%20Not%20Valid
                    _))
                ;[1 1 1] Wait WaitAtDestination seconds
                (Utilities|FlowControl|Delay (Variables|Default|GetWaitAtDestination))
                (if (Variables|Default|GetUseHomeBase?)
                  ;[1 1 1] Set BB RoamBehavior to selected behavior
                  (Class|BTFunctionLibrary|SetBlackboardValueasEnum (Variables|Default|GetRoamBehavior) (Utilities|Enum|LiteralenumBP_Enum_AIRoamBehavior "NewEnumerator6"))
                  (Variables|/Game/AnimalBehaviorKit/Blueprints/Characters/Animals/GroundAnimals/BP_GroundAnimalBase.BP_GroundAnimalBase_C|SetRoamBehavior (Variables|Default|GetAnimalBase) "NewEnumerator6")
                  (else
                    ;[1 1 1] Set next Roam Behavior
                    (bind _newroambehavior (Default|FnSetRoamBehavior (Variables|Default|GetAnimalBase)))
                    (|SETNEXTBEHAVIORINTHEBLACKBOARD _newroambehavior
                      (:OutputPin
                        ;[1 1 1] Finished drinking - set BiggestNeed to Roam again
                        (Variables|/Game/AnimalBehaviorKit/Blueprints/Characters/Animals/GroundAnimals/BP_GroundAnimalBase.BP_GroundAnimalBase_C|SetBiggestNeed (Variables|Default|GetAnimalBase) "NewEnumerator3")))))
                (|RESETWALKSPEEDANDACCELERATION_2)
                (AI|BehaviorTree|FinishExecute true))
              (:OnFail
                ;[1 1 1] Set Moving to False
                (Class|BTFunctionLibrary|SetBlackboardValueasBool (Variables|Default|GetMoving) false)
                (AI|BehaviorTree|FinishExecute false :!label _label)))
            (else
              (|RESETWALKSPEEDANDACCELERATION)
              (goto _label))))
        (:Is%20Not%20Valid
          ;[1 1 1] Error Message
          (Development|PrintString (Utilities|String|Append (Utilities|GetDisplayName (Variables|Default|GetAnimalBase)) ": No WayPoints found!") true true "(R=1.000000,G=0.000000,B=0.000000,A=1.000000)" 5.0))))))