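; Behavior tree task that performs predictive movement for ground animals by periodically teleporting the pawn instead of walking it.
; It reads settings from the animal, then a timed event picks a destination by roam behavior: random navmesh point, random point within bounds, or waypoint.
; Navmesh and bounds points are rejected when a vertical trace hits a no-spawn-tagged actor.
; The waypoint branch runs an EQS query and teleports to the blackboard's waypoint.
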(event Custom|EventMoveAI
  (Utilities|Time|SetTimerbyEvent (delegate Custom|EventMoveAI) (Variables|Default|GetUpdateRate) true)
  ;[1 1 1] Switch on AI's Roam Behavior
  (switch Utilities|FlowControl|Switch|SwitchonBP_Enum_AIRoamBehavior (Variables|/Game/AnimalBehaviorKit/Blueprints/Characters/Animals/GroundAnimals/BP_GroundAnimalBase.BP_GroundAnimalBase_C|GetRoamBehavior (Variables|Default|GetAnimalBase))
    (:NewEnumerator0
      (|RANDOMLOCATIONINNAVMESH))
    (:NewEnumerator3
      (|RANDOMLOCATIONINSIDEBOUNDS))
    (:NewEnumerator5
      (|GOTORANDOMWAYPOINT))))

(event EventReceiveExecuteAI
  (params (OwnerController :type AI%20Controller%20Object%20Reference) (ControlledPawn :type Pawn%20Object%20Reference))
  (Variables|Default|SetPawnRef ControlledPawn)
  (bind _asbp_ground_animal_base (Utilities|Casting|CastToBP_GroundAnimalBase (Variables|Default|GetPawnRef)))
  (bind _output_get (Variables|Default|SetAnimalBase _asbp_ground_animal_base))
  ;[1 1 1] Get Movement Update Rate
  (Variables|Default|SetUpdateRate (.PredictiveMovementupdaterate (Utilities|Struct|BreakBP_Struct_AnimalBase_SimDetails (Variables|/Game/AnimalBehaviorKit/Blueprints/Characters/Animals/BP_AnimalBase.BP_AnimalBase_C|GetSimulation_Details _output_get))))
  ;[1 1 1] Set No Spawn tag
  (Variables|Default|SetTag (.NoSpawntag (Utilities|Struct|BreakBP_Struct_AnimalBase_SimDetails (Variables|/Game/AnimalBehaviorKit/Blueprints/Characters/Animals/BP_AnimalBase.BP_AnimalBase_C|GetSimulation_Details _output_get))))
  ;[1 1 1] Set the Bounds reference
  (Variables|Default|SetBoundsRef (.BoundsReference (Utilities|Struct|BreakBP_Struct_GroundAnimalBehavior_Location (Variables|/Game/AnimalBehaviorKit/Blueprints/Characters/Animals/GroundAnimals/BP_GroundAnimalBase.BP_GroundAnimalBase_C|GetBehavior_Location (Variables|Default|GetAnimalBase)))))
  ;[1 1 1] Set Search Radius
  (Variables|Default|SetRadius (.SearchRadius (Utilities|Struct|BreakBP_Struct_GroundAnimalBehavior_Location (Variables|/Game/AnimalBehaviorKit/Blueprints/Characters/Animals/GroundAnimals/BP_GroundAnimalBase.BP_GroundAnimalBase_C|GetBehavior_Location (Variables|Default|GetAnimalBase)))))
  (CallFunction|EventMoveAI))

(fn FnCheckSpawnLocation
  (params (Location :type Vector))
  (LocalVariables|SetSpawnLocation Location)
  (bind _outhit (Collision|LineTraceByChannel (+ (LocalVariables|GetSpawnLocation) "0, 0,40000.000000") (- (LocalVariables|GetSpawnLocation) "0, 0,40000.000000") "TraceTypeQuery1" false 0 "None"))
  (if (Actor|ActorHasTag (.HitActor (Collision|BreakHitResult _outhit)) (Variables|Default|GetTag))
    (LocalVariables|SetSpawn false)
    (else
      (LocalVariables|SetSpawn true)))
  (return (LocalVariables|GetSpawn)))