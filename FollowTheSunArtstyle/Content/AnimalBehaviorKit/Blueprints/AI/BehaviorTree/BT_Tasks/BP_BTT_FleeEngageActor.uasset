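; Behavior tree task that makes a ground animal flee from an engaged actor by moving to the FleeLocation blackboard vector.
; It scales walk speed and acceleration by random engage multipliers, then runs AI MoveTo with the animal's acceptance radius while maintaining the Moving blackboard flag.
; When the move ends it restores engage speed and acceleration from BehaviorDetails, disengaging and succeeding on arrival, or failing otherwise.
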(event EventReceiveExecuteAI
  (params (OwnerController :type AI%20Controller%20Object%20Reference) (ControlledPawn :type Pawn%20Object%20Reference))
  (Variables|Default|SetPawnRef ControlledPawn)
  (bind _asbp_ground_animal_base (Utilities|Casting|CastToBP_GroundAnimalBase (Variables|Default|GetPawnRef)))
  (Variables|Default|SetAnimalBase _asbp_ground_animal_base)
  ;[1 1 1] Set Acceptance Radius
  (Variables|Default|SetAcceptanceRadius (Variables|/Game/AnimalBehaviorKit/Blueprints/Characters/Animals/GroundAnimals/BP_GroundAnimalBase.BP_GroundAnimalBase_C|GetMovementAcceptanceRadius (Variables|Default|GetAnimalBase)))
  (|SETRANDOMWALKSPEEDANDACCELERATION)
  ;[1 1 1] Move to Flee Location
  (AI|AIMoveTo (Variables|Default|GetPawnRef) (Class|BTFunctionLibrary|GetBlackboardValueasVector (Variables|Setup|GetFleeLocation)) 0 (Variables|Default|GetAcceptanceRadius) true
    (:then
      ;[1 1 1] Set Moving to True
      (Class|BTFunctionLibrary|SetBlackboardValueasBool (Variables|Default|GetMoving) true))
    (:OnSuccess
      ;[1 1 1] Set Moving to False
      (Class|BTFunctionLibrary|SetBlackboardValueasBool (Variables|Default|GetMoving) false)
      ;[1 1 1] Disengage
      (Default|FnDisengage (Variables|Default|GetAnimalBase))
      (|RESETWALKSPEEDANDACCELERATION)
      (AI|BehaviorTree|FinishExecute true))
    (:OnFail
      ;[1 1 1] Set Moving to False
      (Class|BTFunctionLibrary|SetBlackboardValueasBool (Variables|Default|GetMoving) false)
      (|RESETWALKSPEEDANDACCELERATION_2)
      (AI|BehaviorTree|FinishExecute false))))