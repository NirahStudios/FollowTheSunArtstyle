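; Behavior Tree task that sends a ground animal toward its parent, using the parent reference from its GrowOld component.
; It runs AIMoveTo with the animal's own movement acceptance radius.
; The Moving blackboard key is set while the move runs and cleared when it ends, and the task finishes with the move's result.
; Without a GrowOld component or a successful cast, the task never calls FinishExecute.
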(event EventReceiveExecuteAI
  (params (OwnerController :type AI%20Controller%20Object%20Reference) (ControlledPawn :type Pawn%20Object%20Reference))
  (Variables|Default|SetPawnRef ControlledPawn)
  (bind _asbp_ground_animal_base (Utilities|Casting|CastToBP_GroundAnimalBase (Variables|Default|GetPawnRef)))
  (Variables|Default|SetAnimalBase _asbp_ground_animal_base)
  ;[1 1 1] Set Acceptance Radius
  (Variables|Default|SetAcceptanceRadius (Variables|/Game/AnimalBehaviorKit/Blueprints/Characters/Animals/GroundAnimals/BP_GroundAnimalBase.BP_GroundAnimalBase_C|GetMovementAcceptanceRadius (Variables|Default|GetAnimalBase)))
  ;[1 1 1] Does the animal have the GrowOld component?
  (Utilities|IsValid (Actor|GetComponentbyClass (Variables|Default|GetAnimalBase) "/Game/AnimalBehaviorKit/Blueprints/AI/Components/GroundAnimals/BP_Comp_GrowOld.BP_Comp_GrowOld_C")
    (:Is%20Valid
      ;[1 1 1] Get parent reference
      (Variables|Default|SetNearbyParent (Variables|/Game/AnimalBehaviorKit/Blueprints/AI/Components/GroundAnimals/BP_Comp_GrowOld.BP_Comp_GrowOld_C|GetParentRef (Actor|GetComponentbyClass (Variables|Default|GetAnimalBase) "/Game/AnimalBehaviorKit/Blueprints/AI/Components/GroundAnimals/BP_Comp_GrowOld.BP_Comp_GrowOld_C")))
      ;[1 1 1] Move towards nearby Partner
      (AI|AIMoveTo (Variables|Default|GetPawnRef) "0, 0, 0" (Variables|Default|GetNearbyParent) (Variables|Default|GetAcceptanceRadius) true
        (:then
          ;[1 1 1] Set Moving to True
          (Class|BTFunctionLibrary|SetBlackboardValueasBool (Variables|Default|GetMoving) true))
        (:OnSuccess
          ;[1 1 1] Set Moving to False
          (Class|BTFunctionLibrary|SetBlackboardValueasBool (Variables|Default|GetMoving) false)
          (AI|BehaviorTree|FinishExecute true))
        (:OnFail
          ;[1 1 1] Set Moving to False
          (Class|BTFunctionLibrary|SetBlackboardValueasBool (Variables|Default|GetMoving) false)
          (AI|BehaviorTree|FinishExecute false))))))