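; Behavior Tree task that makes a ground animal defend its location by chasing and attacking the blackboard EngageActor.
; Each tick it moves toward the target at randomized speed, attacks within melee range for the montage length plus a cooldown, optionally rooting itself.
; A dead target resets hunger and sets a roam behavior.
; Exceeding max defense distance or losing the target sends it back, pausing engagement for an inspection delay.
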(event Custom|EventReturnToDefendLocation
  ;[1 1 1] Set CanEngage to False
  (Variables|Default|SetCanEngage false)
  (Variables|/Game/AnimalBehaviorKit/Blueprints/Characters/Animals/GroundAnimals/BP_GroundAnimalBase.BP_GroundAnimalBase_C|SetCanEngage (Variables|Default|GetAnimalBase) false)
  ;[1 1 1] Set DefenseState to 'Going to Defense Location'
  (Class|BTFunctionLibrary|SetBlackboardValueasEnum (Variables|Setup|GetDefenseState) (Utilities|Enum|LiteralenumBP_Enum_DefenseState "NewEnumerator0"))
  (Variables|/Game/AnimalBehaviorKit/Blueprints/Characters/Animals/GroundAnimals/BP_GroundAnimalBase.BP_GroundAnimalBase_C|SetDefenseState (Variables|Default|GetAnimalBase) "NewEnumerator0")
  ;[1 1 1] Stop attacking
  (Variables|/Game/AnimalBehaviorKit/Blueprints/Characters/Animals/BP_AnimalBase.BP_AnimalBase_C|SetAttacking (Variables|Default|GetAnimalBase) false)
  (Variables|Default|SetcanAttack true)
  (Utilities|FlowControl|Delay (Variables|Default|GetInspectionTime))
  (Variables|/Game/AnimalBehaviorKit/Blueprints/Characters/Animals/GroundAnimals/BP_GroundAnimalBase.BP_GroundAnimalBase_C|SetCanEngage (Variables|Default|GetAnimalBase) true)
  (|RESETWALKSPEEDANDACCELERATION)
  (AI|BehaviorTree|FinishExecute true))

(event EventReceiveExecuteAI
  (params (OwnerController :type AI%20Controller%20Object%20Reference) (ControlledPawn :type Pawn%20Object%20Reference))
  (Variables|Default|SetPawnRef ControlledPawn)
  (bind _asbp_ground_animal_base (Utilities|Casting|CastToBP_GroundAnimalBase (Variables|Default|GetPawnRef)))
  (Variables|Default|SetAnimalBase _asbp_ground_animal_base)
  ;[1 1 1] Set CanEngage
  (Variables|Default|SetCanEngage (Variables|/Game/AnimalBehaviorKit/Blueprints/Characters/Animals/GroundAnimals/BP_GroundAnimalBase.BP_GroundAnimalBase_C|GetCanEngage (Variables|Default|GetAnimalBase)))
  ;[1 1 1] Get Melee range
  (Variables|Default|SetMeleeRange (Components|Sphere|GetScaledSphereRadius (Variables|/Game/AnimalBehaviorKit/Blueprints/Characters/Animals/GroundAnimals/BP_GroundAnimalBase.BP_GroundAnimalBase_C|GetCollision_AI (Variables|Default|GetAnimalBase))))
  ;[1 1 1] Set Defense Behavior parameters
  (Variables|Setup|SetDefendBehavior (Variables|/Game/AnimalBehaviorKit/Blueprints/Characters/Animals/GroundAnimals/BP_GroundAnimalBase.BP_GroundAnimalBase_C|GetBehavior_Defend (Variables|Default|GetAnimalBase)))
  ;[1 1 1] Set Acceptance Radius
  (Variables|Default|SetAcceptanceRadius (Variables|/Game/AnimalBehaviorKit/Blueprints/Characters/Animals/GroundAnimals/BP_GroundAnimalBase.BP_GroundAnimalBase_C|GetMovementAcceptanceRadius (Variables|Default|GetAnimalBase)))
  ;[1 1 1] Set InspectionTime
  (Variables|Default|SetInspectionTime (Utilities|Struct|BreakBP_Struct_GroundAnimaBehavior_Defend (Variables|/Game/AnimalBehaviorKit/Blueprints/Characters/Animals/GroundAnimals/BP_GroundAnimalBase.BP_GroundAnimalBase_C|GetBehavior_Defend (Variables|Default|GetAnimalBase))))
  ;[1 1 1] Stop attacking
  (Variables|/Game/AnimalBehaviorKit/Blueprints/Characters/Animals/BP_AnimalBase.BP_AnimalBase_C|SetAttacking (Variables|Default|GetAnimalBase) false)
  (Variables|Default|SetcanAttack true)
  ;[1 1 1] Set StopMovement
  (Variables|Default|SetStopMovement (.Dontmovewhileattacking (Utilities|Struct|BreakBP_Struct_GroundAnimalBehavior_AnimalDetails_Attack (Variables|/Game/AnimalBehaviorKit/Blueprints/Characters/Animals/GroundAnimals/BP_GroundAnimalBase.BP_GroundAnimalBase_C|GetBehavior_Details_Attack (Variables|Default|GetAnimalBase))))))

(event EventReceiveTickAI
  (params (OwnerController :type AI%20Controller%20Object%20Reference) (ControlledPawn :type Pawn%20Object%20Reference) (DeltaSeconds :type Float%20%28single-precision%29))
  (bind _pawnref (Variables|Default|GetPawnRef))
  (bind _animalbase (Variables|Default|GetAnimalBase))
  (bind _animalbase_2 (Variables|Default|GetAnimalBase))
  (bind _returnvalue (Transformation|GetActorRotation _pawnref))
  (bind _returnvalue_2 (Actor|GetComponentbyClass _animalbase "/Game/AnimalBehaviorKit/Blueprints/AI/Components/GroundAnimals/BP_Comp_NeedSystem.BP_Comp_NeedSystem_C"))
  (bind (_roll _pitch) (Math|Rotator|BreakRotator _returnvalue))
  (if (Variables|Default|GetCanEngage)
    ;[1 1 1] Check Engage Actor is Valid
    (Utilities|IsValid (AI|BehaviorTree|GetBlackboardValueasActor (Variables|Setup|GetEngageActor))
      (:Is%20Valid
        (Utilities|FlowControl|Sequence
          (:then_0
            ;[1 1 1] Check that Engage Actor is NOT Dead
            (if (not (Actor|ActorHasTag (AI|BehaviorTree|GetBlackboardValueasActor (Variables|Setup|GetEngageActor)) "abkDead"))
              ;[1 1 1] Is animal in melee range to EngageActor?
              (if (<= (Math|Vector|VectorLength (- (Transformation|GetActorLocation (AI|BehaviorTree|GetBlackboardValueasActor (Variables|Setup|GetEngageActor))) (Transformation|GetActorLocation (Variables|Default|GetAnimalBase)))) (* (Variables|Default|GetMeleeRange) 2.0))
                (if (and (not (Variables|/Game/AnimalBehaviorKit/Blueprints/Characters/Animals/BP_AnimalBase.BP_AnimalBase_C|GetAttacking (Variables|Default|GetAnimalBase))) (Variables|Default|GetcanAttack))
                  (Variables|Default|SetcanAttack false)
                  ;[1 1 1] Set State to Attacking
                  (Variables|/Game/AnimalBehaviorKit/Blueprints/Characters/Animals/BP_AnimalBase.BP_AnimalBase_C|SetAttacking (Variables|Default|GetAnimalBase) true)
                  ;[1 1 1] Play Attacking animation
                  (Default|EventPlayAnimation (Variables|Default|GetAnimalBase) "NewEnumerator0")
                  (AI|Navigation|StopMovement
                    (:then
                      _)
                    (:OutputPin
                      _))
                  ;[1 1 1] Wait for the attack animation duration
                  (bind _returnvalue_3 (Animation|GetCurrentMontage (Variables|Default|GetAnimalBase) :!class /Script/Engine.Character))
                  (bind _returnvalue_4 (Animation|GetPlayLength _returnvalue_3))
                  (Utilities|FlowControl|Delay (/ _returnvalue_4 (Utilities|Struct|BreakBP_Struct_GroundAnimal_CurrentMontage (Variables|/Game/AnimalBehaviorKit/Blueprints/Characters/Animals/GroundAnimals/BP_GroundAnimalBase.BP_GroundAnimalBase_C|GetCurrentAnimation (Variables|Default|GetAnimalBase)))))
                  (|RESETMOVEMENTSPEED)
                  ;[1 1 1] Stop attacking
                  (Variables|/Game/AnimalBehaviorKit/Blueprints/Characters/Animals/BP_AnimalBase.BP_AnimalBase_C|SetAttacking (Variables|Default|GetAnimalBase) false)
                  ;[1 1 1] Wait AttackFrequency before stopping the attack
                  (Utilities|FlowControl|Delay (Utilities|Struct|BreakBP_Struct_GroundAnimalBehavior_AnimalDetails_Attack (Variables|/Game/AnimalBehaviorKit/Blueprints/Characters/Animals/GroundAnimals/BP_GroundAnimalBase.BP_GroundAnimalBase_C|GetBehavior_Details_Attack (Variables|Default|GetAnimalBase))))
                  (Variables|Default|SetcanAttack true)))
              (else
                ;[1 1 1] Is Comp_NeedSystem present?
                (Utilities|IsValid _returnvalue_2
                  (:Is%20Valid
                    ;[1 1 1] Resets Hunger
                    (Default|EventFinishedEating _returnvalue_2))
                  (:Is%20Not%20Valid
                    _))
                ;[1 1 1] Engage Actor is dead - Disengage
                (Default|FnDisengage (Variables|Default|GetAnimalBase))
                ;[1 1 1] Stop attacking
                (Variables|/Game/AnimalBehaviorKit/Blueprints/Characters/Animals/BP_AnimalBase.BP_AnimalBase_C|SetAttacking (Variables|Default|GetAnimalBase) false)
                ;[1 1 1] Set next Roam Behavior
                (bind _newroambehavior (Default|FnSetRoamBehavior (Variables|Default|GetAnimalBase)))
                (|SETNEXTBEHAVIORINTHEBLACKBOARD _newroambehavior
                  (:OutputPin
                    ;[1 1 1] Finished eating - set BiggestNeed to Roam again
                    (Variables|/Game/AnimalBehaviorKit/Blueprints/Characters/Animals/GroundAnimals/BP_GroundAnimalBase.BP_GroundAnimalBase_C|SetBiggestNeed (Variables|Default|GetAnimalBase) "NewEnumerator3")
                    (AI|BehaviorTree|FinishExecute true))))))
          (:then_1
            (|SETRANDOMWALKSPEEDANDACCELERATION)
            ;[1 1 1] Set actor location to EngageActor
            (AI|AIMoveTo (Variables|Default|GetPawnRef) "0, 0, 0" (AI|BehaviorTree|GetBlackboardValueasActor (Variables|Setup|GetEngageActor)) (* (Variables|Default|GetAcceptanceRadius) 0.25) true
              (:then
                ;[1 1 1] Check if animal is farther than MaxDistanceFromLocation
                (if (> (Math|Vector|VectorLength (- (Variables|/Game/AnimalBehaviorKit/Blueprints/Characters/Animals/GroundAnimals/BP_GroundAnimalBase.BP_GroundAnimalBase_C|GetDefenseLocation _animalbase_2) (Transformation|GetActorLocation _animalbase_2))) (Utilities|Struct|BreakBP_Struct_GroundAnimaBehavior_Defend (Variables|Setup|GetDefendBehavior)))
                  (CallFunction|EventReturntoDefendLocation)
                  (else
                    ;[1 1 1] Rotate towards target
                    (Transformation|SetActorRotation (Variables|Default|GetPawnRef) (Math|Interpolation|RInterpTo _returnvalue (Math|Rotator|MakeRotator _roll _pitch (.yaw (Math|Rotator|FindLookatRotation (Transformation|GetActorLocation (Variables|Default|GetPawnRef)) (Transformation|GetActorLocation (AI|BehaviorTree|GetBlackboardValueasActor (Variables|Setup|GetEngageActor)))))) (Utilities|Time|GetWorldDeltaSeconds) 2.0)))))
              (:OnSuccess
                (|RESETWALKSPEEDANDACCELERATION_3))
              (:OnFail
                (|RESETWALKSPEEDANDACCELERATION_2))))))
      (:Is%20Not%20Valid
        (CallFunction|EventReturntoDefendLocation)))))