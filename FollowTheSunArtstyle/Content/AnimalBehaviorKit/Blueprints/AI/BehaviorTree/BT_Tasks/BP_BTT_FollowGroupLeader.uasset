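; Behavior tree task that keeps a grouped ground animal following its group leader.
; It disengages the animal, then moves it to a random point around the leader, bounded by the group component's max leader distance.
; If the leader is invalid or that move fails, it heads for a random group member, and if that also fails it flags the animal as separated from the group.
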(event Custom|EventFollowLeader
  (bind _maxleaderdistance (Variables|Default|GetMaxLeaderDistance))
  (Default|FnDisengage (Variables|Default|GetAnimalBase))
  ;[1 1 1] Is the group leader valid?
  (Utilities|IsValid (Variables|/Game/AnimalBehaviorKit/Blueprints/AI/Actors/Ground_AI/Group/BP_GroupManager.BP_GroupManager_C|GetGroupLeader (Variables|/Game/AnimalBehaviorKit/Blueprints/AI/Components/GroundAnimals/BP_Comp_Group.BP_Comp_Group_C|GetGroupManager (Variables|Default|GetCompGroup)))
    (:Is%20Valid
      ;[1 1 1] Get Herd Leader's location and move towards it
      (AI|AIMoveTo (Variables|Default|GetPawnRef) (Math|Random|RandomPointinBoundingBox (Transformation|GetActorLocation (Variables|/Game/AnimalBehaviorKit/Blueprints/AI/Actors/Ground_AI/Group/BP_GroupManager.BP_GroupManager_C|GetGroupLeader (Variables|/Game/AnimalBehaviorKit/Blueprints/AI/Components/GroundAnimals/BP_Comp_Group.BP_Comp_Group_C|GetGroupManager (Variables|Default|GetCompGroup)))) (Math|Vector|MakeVector _maxleaderdistance _maxleaderdistance 1e+01)) 0 6e+02 true
        (:OnSuccess
          ;[1 1 1] Set Moving to False
          (Class|BTFunctionLibrary|SetBlackboardValueasBool (Variables|Default|GetMoving) false :!label _label)
          (AI|BehaviorTree|FinishExecute true))
        (:OnFail
          ;[1 1 1] Could not reach leader, get another random member and try to go to it
          (bind _randommember (Default|FnGetRandomMember (Variables|/Game/AnimalBehaviorKit/Blueprints/AI/Components/GroundAnimals/BP_Comp_Group.BP_Comp_Group_C|GetGroupManager (Variables|Default|GetCompGroup)) :!label _label_2))
          (AI|AIMoveTo (Variables|Default|GetPawnRef) "0, 0, 0" _randommember 6e+02 true
            (:then
              ;[1 1 1] Set Moving to True
              (Class|BTFunctionLibrary|SetBlackboardValueasBool (Variables|Default|GetMoving) true))
            (:OnSuccess
              (goto _label))
            (:OnFail
              ;[1 1 1] Separate from group
              (Variables|/Game/AnimalBehaviorKit/Blueprints/AI/Components/GroundAnimals/BP_Comp_Group.BP_Comp_Group_C|SetPartOfAGroup? (Variables|Default|GetCompGroup) false)
              (goto _label))))))
    (:Is%20Not%20Valid
      (goto _label_2))))

(event EventReceiveExecuteAI
  (params (OwnerController :type AI%20Controller%20Object%20Reference) (ControlledPawn :type Pawn%20Object%20Reference))
  (Variables|Default|SetPawnRef ControlledPawn)
  (bind _asbp_ground_animal_base (Utilities|Casting|CastToBP_GroundAnimalBase (Variables|Default|GetPawnRef)))
  (Variables|Default|SetAnimalBase _asbp_ground_animal_base)
  ;[1 1 1] Do we have component Comp_Group present?
  (Utilities|IsValid (Actor|GetComponentbyClass (Variables|Default|GetAnimalBase) "/Game/AnimalBehaviorKit/Blueprints/AI/Components/GroundAnimals/BP_Comp_Group.BP_Comp_Group_C")
    (:Is%20Valid
      (Variables|Default|SetCompGroup (Actor|GetComponentbyClass (Variables|Default|GetAnimalBase) "/Game/AnimalBehaviorKit/Blueprints/AI/Components/GroundAnimals/BP_Comp_Group.BP_Comp_Group_C"))
      ;[1 1 1] Set Max Leader Distance
      (Variables|Default|SetMaxLeaderDistance (Variables|/Game/AnimalBehaviorKit/Blueprints/AI/Components/GroundAnimals/BP_Comp_Group.BP_Comp_Group_C|GetMaxLeaderDistance (Variables|Default|GetCompGroup)))
      (CallFunction|EventFollowLeader))))