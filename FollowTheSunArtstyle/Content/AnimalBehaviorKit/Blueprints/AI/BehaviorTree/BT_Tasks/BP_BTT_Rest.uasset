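; Behavior tree task that sends a ground animal with a day-cycle component to rest at its home base.
; It moves the animal to a random point within the home base bounds, retrying whenever the move fails.
; On arrival it sets the resting flags, plays the rest animation, calls the day-cycle rest event and optionally hides the animal and ignores pawn collision.
; Execution finishes only after a successful move.
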(event Custom|EventGoToRestLocation
  (bind _homebase (Variables|Default|GetHomeBase))
  (bind _bounds (Variables|/Game/AnimalBehaviorKit/Blueprints/AI/Actors/Ground_AI/Navigation/BP_AI_POI_Base.BP_AI_POI_Base_C|GetBounds _homebase))
  (bind _returnvalue (Transformation|GetWorldLocation _bounds))
  (bind _returnvalue_2 (Components|Box|GetScaledBoxExtent _bounds))
  (bind _returnvalue_3 (Math|Random|RandomPointinBoundingBox _returnvalue _returnvalue_2))
  ;[1 1 1] Make sure we are not already resting
  (if (not (Class|BTFunctionLibrary|GetBlackboardValueasBool (Variables|Setup|GetResting?)))
    ;[1 1 1] Get random location inside the POI and move there
    (AI|AIMoveTo (Variables|Default|GetPawnRef) (Math|Vector|MakeVector (.x _returnvalue_3) (.y _returnvalue_3) (.z (Transformation|GetActorLocation (Variables|Default|GetPawnRef)))) 0 (Variables|Default|GetAcceptanceRadius) true
      (:OnSuccess
        ;[1 1 1] Set BB value Resting? as True
        (Class|BTFunctionLibrary|SetBlackboardValueasBool (Variables|Setup|GetResting?) true)
        ;[1 1 1] Play rest animation
        (Default|EventPlayAnimation (Variables|Default|GetAnimalBase) "NewEnumerator5")
        ;[1 1 1] Set Resting to True
        (Variables|/Game/AnimalBehaviorKit/Blueprints/Characters/Animals/BP_AnimalBase.BP_AnimalBase_C|SetResting (Variables|Default|GetAnimalBase) true)
        ;[1 1 1] Call custom event DayCycle_RestStart
        (Default|DayCycleRestStart (Variables|Default|GetAnimalBase))
        (if (Variables|Default|GetHideMesh)
          (Development|SetHiddeninGame (Variables|/Script/Engine.Character|GetCapsuleComponent (Variables|Default|GetAnimalBase)) true true)
          (Collision|SetCollisionResponsetoChannel (Variables|/Script/Engine.Character|GetCapsuleComponent (Variables|Default|GetAnimalBase)) "ECC_Pawn" "ECR_Ignore"))
        (AI|BehaviorTree|FinishExecute true))
      (:OnFail
        (CallFunction|EventGotoRestLocation)))))

(event EventReceiveExecuteAI
  (params (OwnerController :type AI%20Controller%20Object%20Reference) (ControlledPawn :type Pawn%20Object%20Reference))
  (Variables|Default|SetPawnRef ControlledPawn)
  (bind _asbp_ground_animal_base (Utilities|Casting|CastToBP_GroundAnimalBase (Variables|Default|GetPawnRef)))
  (Variables|Default|SetAnimalBase _asbp_ground_animal_base)
  ;[1 1 1] Check if animal has Day Night Cycle component
  (Utilities|IsValid (Actor|GetComponentbyClass (Variables|Default|GetAnimalBase) "/Game/AnimalBehaviorKit/Blueprints/AI/Components/AllAnimals/BP_Comp_DayCycle.BP_Comp_DayCycle_C")
    (:Is%20Valid
      (Variables|Default|SetHideMesh (Variables|/Game/AnimalBehaviorKit/Blueprints/AI/Components/AllAnimals/BP_Comp_DayCycle.BP_Comp_DayCycle_C|GetHideMeshWhileResting? (Actor|GetComponentbyClass (Variables|Default|GetAnimalBase) "/Game/AnimalBehaviorKit/Blueprints/AI/Components/AllAnimals/BP_Comp_DayCycle.BP_Comp_DayCycle_C")))
      ;[1 1 1] Get Home Base
      (Utilities|IsValid (Variables|/Game/AnimalBehaviorKit/Blueprints/Characters/Animals/GroundAnimals/BP_GroundAnimalBase.BP_GroundAnimalBase_C|GetHomeBase (Variables|Default|GetAnimalBase))
        (:Is%20Valid
          (Variables|Default|SetHomeBase (Variables|/Game/AnimalBehaviorKit/Blueprints/Characters/Animals/GroundAnimals/BP_GroundAnimalBase.BP_GroundAnimalBase_C|GetHomeBase (Variables|Default|GetAnimalBase)))
          ;[1 1 1] Set Acceptance Radius
          (Variables|Default|SetAcceptanceRadius (Variables|/Game/AnimalBehaviorKit/Blueprints/Characters/Animals/GroundAnimals/BP_GroundAnimalBase.BP_GroundAnimalBase_C|GetMovementAcceptanceRadius (Variables|Default|GetAnimalBase)))
          (CallFunction|EventGotoRestLocation))
        (:Is%20Not%20Valid
          ;[1 1 1] Error: No Homebase reference found
          (Development|PrintString (Utilities|String|Append (Utilities|GetDisplayName (Variables|Default|GetAnimalBase)) ": No Homebase reference found!")))))))