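; Behavior tree task that sends a hungry ground animal after the nearest prey as food.
; It asks the animal's Need System component for the nearest prey, then makes it the engaged actor, switches engage behavior to attack and sets the engage parameters.
; With no prey found, the animal either dies if its hunger settings allow it or resets its biggest need to roaming.
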(event EventReceiveExecuteAI
  (params (OwnerController :type AI%20Controller%20Object%20Reference) (ControlledPawn :type Pawn%20Object%20Reference))
  (Variables|Default|SetPawnRef ControlledPawn)
  (bind _asbp_ground_animal_base (Utilities|Casting|CastToBP_GroundAnimalBase (Variables|Default|GetPawnRef)))
  (Variables|Default|SetAnimalBase _asbp_ground_animal_base)
  ;[1 1 1] Does the animal have the component Need System?
  (Utilities|IsValid (Actor|GetComponentbyClass (Variables|Default|GetAnimalBase) "/Game/AnimalBehaviorKit/Blueprints/AI/Components/GroundAnimals/BP_Comp_NeedSystem.BP_Comp_NeedSystem_C")
    (:Is%20Valid
      (Variables|Default|SetNeedSystem (Actor|GetComponentbyClass (Variables|Default|GetAnimalBase) "/Game/AnimalBehaviorKit/Blueprints/AI/Components/GroundAnimals/BP_Comp_NeedSystem.BP_Comp_NeedSystem_C"))
      ;[1 1 1] Get nearest Prey
      (bind _nearestprey (Default|FnGetNearestPrey (Variables|Default|GetNeedSystem)))
      (Variables|Default|SetNearestPrey _nearestprey)
      ;[1 1 1] Check that NearestPrey is Valid
      (Utilities|IsValid (Variables|Default|GetNearestPrey)
        (:Is%20Valid
          ;[1 1 1] Set Engage Behavior to Attack
          (Variables|/Game/AnimalBehaviorKit/Blueprints/Characters/Animals/GroundAnimals/BP_GroundAnimalBase.BP_GroundAnimalBase_C|SetEngageBehavior (Variables|Default|GetAnimalBase) "NewEnumerator3")
          ;[1 1 1] Set Prey as EngagedActor
          (Variables|/Game/AnimalBehaviorKit/Blueprints/Characters/Animals/GroundAnimals/BP_GroundAnimalBase.BP_GroundAnimalBase_C|SetEngagedActor (Variables|Default|GetAnimalBase) (Variables|Default|GetNearestPrey))
          ;[1 1 1] Set Engage Parameters
          (Default|FnSetEngageParams (Variables|Default|GetAnimalBase))
          (AI|BehaviorTree|FinishExecute true))
        (:Is%20Not%20Valid
          ;[1 1 1] Check if animal dies from hunger
          (if (Utilities|Struct|BreakBP_Struct_Need_Eat (Variables|/Game/AnimalBehaviorKit/Blueprints/AI/Components/GroundAnimals/BP_Comp_NeedSystem.BP_Comp_NeedSystem_C|GetHungerDetails (Variables|Default|GetNeedSystem)))
            ;[1 1 1] Kill animal
            (Default|EventDead (Variables|Default|GetAnimalBase))
            (else
              ;[1 1 1] Set BiggestNeed to Roam again
              (Variables|/Game/AnimalBehaviorKit/Blueprints/Characters/Animals/GroundAnimals/BP_GroundAnimalBase.BP_GroundAnimalBase_C|SetBiggestNeed (Variables|Default|GetAnimalBase) "NewEnumerator3")
              (AI|BehaviorTree|FinishExecute true))))))))