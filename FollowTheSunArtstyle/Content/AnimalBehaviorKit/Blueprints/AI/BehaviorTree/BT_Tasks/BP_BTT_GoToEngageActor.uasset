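; Behavior Tree task that moves a ground animal to its blackboard EngageActor with AI MoveTo, updating the Moving key.
; It randomizes max walk speed and acceleration for the chase, then restores engage values before finishing.
; With accurate target detection enabled, a fast looping timer sphere-traces from the attack collision to finish successfully once the target is in melee range.
; The range check also returns target speed, which goes unused.
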(event Custom|EventTickReplacement
  (bind _returnvalue (Utilities|Time|SetTimerbyEvent (delegate Custom|EventTickReplacement) 0.01 true))
  (Variables|Default|SetTickHandler _returnvalue)
  ;[1 1 1] Check if we are in melee range
  (if (.Range (CallFunction|FnGetTargetSpeed))
    (|RESETWALKSPEEDANDACCELERATION_3)
    (AI|BehaviorTree|FinishExecute true)))

(event EventReceiveExecuteAI
  (params (OwnerController :type AI%20Controller%20Object%20Reference) (ControlledPawn :type Pawn%20Object%20Reference))
  (Variables|Default|SetPawnRef ControlledPawn)
  (bind _asbp_ground_animal_base (Utilities|Casting|CastToBP_GroundAnimalBase (Variables|Default|GetPawnRef)))
  (bind _output_get (Variables|Default|SetAnimalBase _asbp_ground_animal_base))
  ;[1 1 1] Set Acceptance Radius
  (Variables|Default|SetAcceptanceRadius (Variables|/Game/AnimalBehaviorKit/Blueprints/Characters/Animals/GroundAnimals/BP_GroundAnimalBase.BP_GroundAnimalBase_C|GetMovementAcceptanceRadius _output_get))
  ;[1 1 1] Check Engage Actor is Valid
  (Utilities|IsValid (AI|BehaviorTree|GetBlackboardValueasActor (Variables|Setup|GetEngageActor))
    (:Is%20Valid
      (|SETRANDOMWALKSPEEDANDACCELERATION)
      ;[1 1 1] Check if we want to use Accurate Target Detection
      (if (Utilities|Struct|BreakBP_Struct_GroundAnimalBehavior_AnimalDetails_Attack (Variables|/Game/AnimalBehaviorKit/Blueprints/Characters/Animals/GroundAnimals/BP_GroundAnimalBase.BP_GroundAnimalBase_C|GetBehavior_Details_Attack (Variables|Default|GetAnimalBase)))
        (CallFunction|EventTickReplacement))
      ;[1 1 1] Move towards Engage Actor
      (AI|AIMoveTo (Variables|Default|GetPawnRef) "0, 0, 0" (AI|BehaviorTree|GetBlackboardValueasActor (Variables|Setup|GetEngageActor)) 5.0 true
        (:then
          ;;[1 1 1] Set Moving to True
          (Class|BTFunctionLibrary|SetBlackboardValueasBool (Variables|Default|GetMoving) true))
        (:OnSuccess
          ;;[1 1 1] Set Moving to False
          (Class|BTFunctionLibrary|SetBlackboardValueasBool (Variables|Default|GetMoving) false)
          (|RESETWALKSPEEDANDACCELERATION)
          (AI|BehaviorTree|FinishExecute true))
        (:OnFail
          ;;[1 1 1] Set Moving to False
          (Class|BTFunctionLibrary|SetBlackboardValueasBool (Variables|Default|GetMoving) false)
          (|RESETWALKSPEEDANDACCELERATION_2)
          (AI|BehaviorTree|FinishExecute false))))))

(fn FnGetTargetSpeed
  (bind _engageactor (Variables|Setup|GetEngageActor))
  (bind _animalbase (Variables|Default|GetAnimalBase))
  (bind _returnvalue (AI|BehaviorTree|GetBlackboardValueasActor _engageactor))
  (bind _collision_attack (Variables|/Game/AnimalBehaviorKit/Blueprints/Characters/Animals/GroundAnimals/BP_GroundAnimalBase.BP_GroundAnimalBase_C|GetCollision_Attack _animalbase))
  (bind _returnvalue_2 (Transformation|GetWorldLocation _collision_attack))
  (Utilities|FlowControl|Sequence
    (:then_0
      (if (Variables|Default|GetDebugMeleeRange)
        (LocalVariables|SetDebugType "ForDuration")
        (else
          (LocalVariables|SetDebugType "None")))
      ;[1 1 1] Check if we are in attack range with target
      (bind (_outhits _returnvalue_3) (Collision|MultiSphereTraceForObjects _returnvalue_2 (+ _returnvalue_2 "0, 0,0.010000") (* (Variables|/Script/Engine.SphereComponent|GetSphereRadius _collision_attack) (Variables|Default|GetCollisionRadiusMultiplier)) (Variables|/Game/AnimalBehaviorKit/Blueprints/Characters/Animals/GroundAnimals/BP_GroundAnimalBase.BP_GroundAnimalBase_C|GetDamageObjectTypes (Variables|Default|GetAnimalBase)) false (Utilities|Array|MakeArray (Variables|Default|GetAnimalBase)) (LocalVariables|GetDebugType) true "(R=1.000000,G=0.000000,B=0.000000,A=1.000000)" "(R=0.000000,G=1.000000,B=0.000000,A=1.000000)" 1.0))
      (if _returnvalue_3
        (bind _array_element (Utilities|Array|ForEachLoopwithBreak _outhits :!label _label)
          (:LoopBody
            (if (== (AI|BehaviorTree|GetBlackboardValueasActor (Variables|Setup|GetEngageActor)) (Components|GetOwner (.HitComponent (Collision|BreakHitResult _array_element))))
              (LocalVariables|SetInRange true)
              (goto _label Break))))))
    (:then_1
      (if (LocalVariables|GetInRange)
        ;[1 1 1] Get EngageActor's speed and set it for this animal
        (Utilities|IsValid _returnvalue
          (:Is%20Valid
            (LocalVariables|SetSpeed (Math|Vector|VectorLength (Transformation|GetVelocity _returnvalue)))))))
    (:then_2
      (return (LocalVariables|GetInRange) (LocalVariables|GetSpeed)))))