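; Behavior tree task that sends a ground animal to the nearest point of interest from the Blackboard, cast by Prey or Predator feeding type.
; On arrival it loops through random moves within the POI bounds, randomizing speed and acceleration, playing an idle montage and waiting after each.
; It then sets the roam behavior to home base or a newly selected one and finishes successfully, while a failed move fails the task.
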(event Custom|EventMoveToPOI
  (|SETRANDOMWALKSPEEDANDACCELERATION)
  ;[1 1 1] Get nearest POI and move there
  (switch Utilities|FlowControl|Switch|SwitchonBP_Enum_FeedingBehavior (Utilities|Enum|ByteToEnumBP_Enum_FeedingBehavior (Class|BTFunctionLibrary|GetBlackboardValueasEnum (Variables|Setup|GetFeedingBehavior)))
    (:NewEnumerator0
      (bind _asbp_ai_poi_base (Utilities|Casting|CastToBP_AI_POI_Base (Class|BTFunctionLibrary|GetBlackboardValueasObject (Variables|Setup|GetNearestPOI))))
      (AI|AIMoveTo (Variables|Default|GetPawnRef) (Transformation|GetActorLocation _asbp_ai_poi_base) 0 (Variables|Default|GetMoveRadius) true
        (:then
          ;[1 1 1] Set Moving to True
          (Class|BTFunctionLibrary|SetBlackboardValueasBool (Variables|Default|GetMoving) true :!label _label))
        (:OnSuccess
          ;[1 1 1] Set Moving to False
          (Class|BTFunctionLibrary|SetBlackboardValueasBool (Variables|Default|GetMoving) false :!label _label_2)
          (CallFunction|EventMoveInsidePOI))
        (:OnFail
          ;[1 1 1] Set Moving to False
          (Class|BTFunctionLibrary|SetBlackboardValueasBool (Variables|Default|GetMoving) false :!label _label_3)
          (|RESETWALKSPEEDANDACCELERATION)
          (AI|BehaviorTree|FinishExecute false))))
    (:NewEnumerator1
      (bind _asbp_ai_poi_predator (Utilities|Casting|CastToBP_AI_POI_Predator (Class|BTFunctionLibrary|GetBlackboardValueasObject (Variables|Setup|GetNearestPOI))))
      (AI|AIMoveTo (Variables|Default|GetPawnRef) (Transformation|GetActorLocation _asbp_ai_poi_predator) 0 (Variables|Default|GetMoveRadius) true
        (:then
          (goto _label))
        (:OnSuccess
          (goto _label_2))
        (:OnFail
          (goto _label_3))))))

(event Custom|EventMoveInsidePOI
  ;[1 1 1] Is the MoveCounter Less Than the TotalMoves?
  (if (< (Variables|Default|GetMoveCounter) (Variables|Default|GetTotalMoves))
    ;[1 1 1] Increase the counter by 1
    (Math|Integer|IncrementInt (Variables|Default|GetMoveCounter)
      (:%20%20
        (|SETRANDOMWALKSPEEDANDACCELERATION_2)
        ;[1 1 1] Get random location inside the POI and move there
        (bind _asbp_ai_poi_base (Utilities|Casting|CastToBP_AI_POI_Base (Class|BTFunctionLibrary|GetBlackboardValueasObject (Variables|Setup|GetNearestPOI))))
        (AI|AIMoveTo (Variables|Default|GetPawnRef) (Math|Vector|MakeVector (.x (Math|Random|RandomPointinBoundingBox (Transformation|GetWorldLocation (Variables|/Game/AnimalBehaviorKit/Blueprints/AI/Actors/Ground_AI/Navigation/BP_AI_POI_Base.BP_AI_POI_Base_C|GetBounds _asbp_ai_poi_base)) (Components|Box|GetScaledBoxExtent (Variables|/Game/AnimalBehaviorKit/Blueprints/AI/Actors/Ground_AI/Navigation/BP_AI_POI_Base.BP_AI_POI_Base_C|GetBounds _asbp_ai_poi_base)))) (.y (Math|Random|RandomPointinBoundingBox (Transformation|GetWorldLocation (Variables|/Game/AnimalBehaviorKit/Blueprints/AI/Actors/Ground_AI/Navigation/BP_AI_POI_Base.BP_AI_POI_Base_C|GetBounds _asbp_ai_poi_base)) (Components|Box|GetScaledBoxExtent (Variables|/Game/AnimalBehaviorKit/Blueprints/AI/Actors/Ground_AI/Navigation/BP_AI_POI_Base.BP_AI_POI_Base_C|GetBounds _asbp_ai_poi_base)))) (.z (Transformation|GetActorLocation (Variables|Default|GetPawnRef)))) 0 (Variables|Default|GetMoveRadius) true
          (:then
            ;[1 1 1] Set Moving to True
            (Class|BTFunctionLibrary|SetBlackboardValueasBool (Variables|Default|GetMoving) true))
          (:OnSuccess
            ;[1 1 1] Set Moving to False
            (Class|BTFunctionLibrary|SetBlackboardValueasBool (Variables|Default|GetMoving) false)
            ;[1 1 1] Play Idle animation
            (Default|EventPlayAnimation (Variables|Default|GetAnimalBase) "NewEnumerator6")
            ;[1 1 1] Wait for the idle animation duration
            (bind _returnvalue (Animation|GetCurrentMontage (Variables|Default|GetAnimalBase) :!class /Script/Engine.Character))
            (Utilities|IsValid _returnvalue
              (:Is%20Valid
                (bind _returnvalue_2 (Animation|GetPlayLength _returnvalue))
                (Utilities|FlowControl|Delay _returnvalue_2))
              (:Is%20Not%20Valid
                _))
            (Utilities|FlowControl|Delay (Variables|Default|GetWaitTime))
            (|RESETWALKSPEEDANDACCELERATION_3)
            (CallFunction|EventMoveInsidePOI))
          (:OnFail
            ;[1 1 1] Set Moving to False
            (Class|BTFunctionLibrary|SetBlackboardValueasBool (Variables|Default|GetMoving) false)
            (|RESETWALKSPEEDANDACCELERATION_4)
            (AI|BehaviorTree|FinishExecute false)))))
    (else
      ;[1 1 1] Reset Move Counter
      (Variables|Default|SetMoveCounter 0)
      (if (Variables|Default|GetUseHomeBase?)
        ;[1 1 1] Set BB RoamBehavior to selected behavior
        (Class|BTFunctionLibrary|SetBlackboardValueasEnum (Variables|Default|GetRoamBehavior) (Utilities|Enum|LiteralenumBP_Enum_AIRoamBehavior "NewEnumerator6"))
        (Variables|/Game/AnimalBehaviorKit/Blueprints/Characters/Animals/GroundAnimals/BP_GroundAnimalBase.BP_GroundAnimalBase_C|SetRoamBehavior (Variables|Default|GetAnimalBase) "NewEnumerator6")
        (else
          ;[1 1 1] Set next Roam Behavior
          (bind _newroambehavior (Default|FnSetRoamBehavior (Variables|Default|GetAnimalBase)))
          (|SETNEXTBEHAVIORINTHEBLACKBOARD _newroambehavior
            (:OutputPin
              ;[1 1 1] Set BiggestNeed to Roam again
              (Variables|/Game/AnimalBehaviorKit/Blueprints/Characters/Animals/GroundAnimals/BP_GroundAnimalBase.BP_GroundAnimalBase_C|SetBiggestNeed (Variables|Default|GetAnimalBase) "NewEnumerator3")))))
      (|RESETWALKSPEEDANDACCELERATION_2)
      (AI|BehaviorTree|FinishExecute true))))

(event EventReceiveExecuteAI
  (params (OwnerController :type AI%20Controller%20Object%20Reference) (ControlledPawn :type Pawn%20Object%20Reference))
  (bind _output_get (Variables|Default|SetPawnRef ControlledPawn))
  (Utilities|IsValid _output_get
    (:Is%20Valid
      (bind _asbp_ground_animal_base (Utilities|Casting|CastToBP_GroundAnimalBase (Variables|Default|GetPawnRef)))
      (Variables|Default|SetAnimalBase _asbp_ground_animal_base)
      ;[1 1 1] Use HomeBase?
      (Variables|Default|SetUseHomeBase? (Variables|/Game/AnimalBehaviorKit/Blueprints/Characters/Animals/GroundAnimals/BP_GroundAnimalBase.BP_GroundAnimalBase_C|GetUseHomeBase? (Variables|Default|GetAnimalBase)))
      ;[1 1 1] Get Total Time spent inside the POI
      (Variables|Default|SetWaitTime (Math|Random|RandomFloatinRange (.x (Utilities|Struct|BreakBP_Struct_GroundAnimalBehavior_POI (Variables|/Game/AnimalBehaviorKit/Blueprints/Characters/Animals/GroundAnimals/BP_GroundAnimalBase.BP_GroundAnimalBase_C|GetBehavior_POI (Variables|Default|GetAnimalBase)))) (.y (Utilities|Struct|BreakBP_Struct_GroundAnimalBehavior_POI (Variables|/Game/AnimalBehaviorKit/Blueprints/Characters/Animals/GroundAnimals/BP_GroundAnimalBase.BP_GroundAnimalBase_C|GetBehavior_POI (Variables|Default|GetAnimalBase))))))
      ;[1 1 1] Get number of moves inside the POI
      (Variables|Default|SetTotalMoves (Utilities|Struct|BreakBP_Struct_GroundAnimalBehavior_POI (Variables|/Game/AnimalBehaviorKit/Blueprints/Characters/Animals/GroundAnimals/BP_GroundAnimalBase.BP_GroundAnimalBase_C|GetBehavior_POI (Variables|Default|GetAnimalBase))))
      ;[1 1 1] Get Movement Acceptance Radius
      (Variables|Default|SetMoveRadius (Variables|/Game/AnimalBehaviorKit/Blueprints/Characters/Animals/GroundAnimals/BP_GroundAnimalBase.BP_GroundAnimalBase_C|GetMovementAcceptanceRadius (Variables|Default|GetAnimalBase)))
      (CallFunction|EventMovetoPOI))))