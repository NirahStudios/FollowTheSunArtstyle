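; Behavior tree task that walks a ground animal to the NearestFood blackboard actor and has it eat.
; It reads eating time from the animal's need system component, moves via AI MoveTo, then replays the eat montage through a self-calling event until that time elapses.
; Afterwards it picks the next roam behavior, optionally favoring home base, writes it to the blackboard and resets hunger.
; It fails if the move fails or the component is missing.
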(event Custom|EventPlayEatAnimation
  (if (Variables|Default|GetCanEat)
    ;[1 1 1] Check that the Biggest Need is Eating
    (if (Utilities|Enum|Equal(Enum) (Variables|/Game/AnimalBehaviorKit/Blueprints/Characters/Animals/GroundAnimals/BP_GroundAnimalBase.BP_GroundAnimalBase_C|GetBiggestNeed (Variables|Default|GetAnimalBase)) "NewEnumerator0")
      ;[1 1 1] Play Eating animation
      (Default|EventPlayAnimation (Variables|Default|GetAnimalBase) "NewEnumerator3")
      ;[1 1 1] Wait for the eating animation duration
      (bind _returnvalue (Animation|GetCurrentMontage (Variables|Default|GetAnimalBase) :!class /Script/Engine.Character))
      (Utilities|IsValid _returnvalue
        (:Is%20Valid
          (bind _returnvalue_2 (Animation|GetPlayLength _returnvalue))
          (Utilities|FlowControl|Delay _returnvalue_2))
        (:Is%20Not%20Valid
          _))
      (CallFunction|EventPlayEatAnimation))
    (else
      ;[1 1 1] Stop current animation montage
      (bind _returnvalue_3 (Animation|GetCurrentMontage (Variables|Default|GetAnimalBase) :!class /Script/Engine.Character))
      (Animation|StopAnimMontage (Variables|Default|GetAnimalBase) _returnvalue_3))))

(event EventReceiveExecuteAI
  (params (OwnerController :type AI%20Controller%20Object%20Reference) (ControlledPawn :type Pawn%20Object%20Reference))
  (Variables|Default|SetPawnRef ControlledPawn)
  (bind _asbp_ground_animal_base (Utilities|Casting|CastToBP_GroundAnimalBase (Variables|Default|GetPawnRef)))
  (Variables|Default|SetAnimalBase _asbp_ground_animal_base)
  ;[1 1 1] Check if we have Comp_NeedSystem
  (Utilities|IsValid (Actor|GetComponentbyClass (Variables|Default|GetAnimalBase) "/Game/AnimalBehaviorKit/Blueprints/AI/Components/GroundAnimals/BP_Comp_NeedSystem.BP_Comp_NeedSystem_C")
    (:Is%20Valid
      ;[1 1 1] Save NeedSystem
      (Variables|Default|SetNeedSystem (Actor|GetComponentbyClass (Variables|Default|GetAnimalBase) "/Game/AnimalBehaviorKit/Blueprints/AI/Components/GroundAnimals/BP_Comp_NeedSystem.BP_Comp_NeedSystem_C"))
      ;[1 1 1] Use HomeBase?
      (Variables|Default|SetUseHomeBase? (Variables|/Game/AnimalBehaviorKit/Blueprints/Characters/Animals/GroundAnimals/BP_GroundAnimalBase.BP_GroundAnimalBase_C|GetUseHomeBase? (Variables|Default|GetAnimalBase)))
      ;[1 1 1] Set EatingTime
      (Variables|Default|SetEatingTime (.EatingTime (Utilities|Struct|BreakBP_Struct_Need_Eat (Variables|/Game/AnimalBehaviorKit/Blueprints/AI/Components/GroundAnimals/BP_Comp_NeedSystem.BP_Comp_NeedSystem_C|GetHungerDetails (Variables|Default|GetNeedSystem)))))
      ;[1 1 1] Get Movement Acceptance Radius
      (Variables|Default|SetMoveRadius (Variables|/Game/AnimalBehaviorKit/Blueprints/Characters/Animals/GroundAnimals/BP_GroundAnimalBase.BP_GroundAnimalBase_C|GetMovementAcceptanceRadius (Variables|Default|GetAnimalBase)))
      ;[1 1 1] Get nearest food source and Move AI to that location
      (bind _asbp_ai_food (Utilities|Casting|CastToBP_AI_Food (Class|BTFunctionLibrary|GetBlackboardValueasObject (Variables|Setup|GetNearestFood))))
      (AI|AIMoveTo (Variables|Default|GetPawnRef) (Transformation|GetActorLocation _asbp_ai_food) 0 (Variables|Default|GetMoveRadius) true
        (:then
          ;[1 1 1] Set Moving to True
          (Class|BTFunctionLibrary|SetBlackboardValueasBool (Variables|Default|GetMoving) true))
        (:OnSuccess
          ;[1 1 1] Set Moving to False
          (Class|BTFunctionLibrary|SetBlackboardValueasBool (Variables|Default|GetMoving) false)
          ;[1 1 1] Play Eating Animation
          (CallFunction|EventPlayEatAnimation)
          ;[1 1 1] Wait WaitAtDestination seconds
          (Utilities|FlowControl|Delay (Variables|Default|GetEatingTime))
          ;[1 1 1] Stop Eating animation
          (Variables|Default|SetCanEat false)
          (bind _returnvalue (Animation|GetCurrentMontage (Variables|Default|GetAnimalBase) :!class /Script/Engine.Character))
          (Animation|StopAnimMontage (Variables|Default|GetAnimalBase) _returnvalue)
          ;[1 1 1] This delay accounts for the eating montage's blend out time. You may need to adjust this depending on your animation
          (Utilities|FlowControl|Delay 1.5)
          (if (Variables|Default|GetUseHomeBase?)
            (Variables|/Game/AnimalBehaviorKit/Blueprints/Characters/Animals/GroundAnimals/BP_GroundAnimalBase.BP_GroundAnimalBase_C|SetRoamBehavior (Variables|Default|GetAnimalBase) "NewEnumerator6"))
          ;[1 1 1] Set next Roam Behavior
          (bind _newroambehavior (Default|FnSetRoamBehavior (Variables|Default|GetAnimalBase)))
          (|SETNEXTBEHAVIORINTHEBLACKBOARD _newroambehavior
            (:OutputPin
              ;[1 1 1] Finished eating - set BiggestNeed to Roam again
              (Variables|/Game/AnimalBehaviorKit/Blueprints/Characters/Animals/GroundAnimals/BP_GroundAnimalBase.BP_GroundAnimalBase_C|SetBiggestNeed (Variables|Default|GetAnimalBase) "NewEnumerator3")
              ;[1 1 1] Resets Hunger
              (Default|EventFinishedEating (Variables|Default|GetNeedSystem))
              (Variables|Default|SetCanEat true)
              (AI|BehaviorTree|FinishExecute true))))
        (:OnFail
          ;[1 1 1] Set Moving to False
          (Class|BTFunctionLibrary|SetBlackboardValueasBool (Variables|Default|GetMoving) false)
          (AI|BehaviorTree|FinishExecute false))))
    (:Is%20Not%20Valid
      (AI|BehaviorTree|FinishExecute false))))