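; Behavior tree task that sends a thirsty ground animal to drink at nearby water.
; A sphere trace gathers BP_AI_Water actors matching the need system's water ID and picks the nearest by closest spline point, retrying a random spline point if the move fails.
; It loops the drink montage for the drinking time, then resets thirst and writes the next roam behavior to the blackboard.
; Without water, the animal dies or resumes roaming.
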(event Custom|EventPlayDrinkAnimation
  (if (Variables|Default|GetCanDrink)
    ;[1 1 1] Check that the Biggest Need is Drinking
    (if (Utilities|Enum|Equal(Enum) (Variables|/Game/AnimalBehaviorKit/Blueprints/Characters/Animals/GroundAnimals/BP_GroundAnimalBase.BP_GroundAnimalBase_C|GetBiggestNeed (Variables|Default|GetAnimalBase)) "NewEnumerator1")
      ;[1 1 1] Play Drink animation
      (Default|EventPlayAnimation (Variables|Default|GetAnimalBase) "NewEnumerator4")
      ;[1 1 1] Wait for the drink animation duration
      (bind _returnvalue (Animation|GetCurrentMontage (Variables|Default|GetAnimalBase) :!class /Script/Engine.Character))
      (Utilities|IsValid _returnvalue
        (:Is%20Valid
          (bind _returnvalue_2 (Animation|GetPlayLength _returnvalue))
          (Utilities|FlowControl|Delay _returnvalue_2))
        (:Is%20Not%20Valid
          (Utilities|FlowControl|Delay 1.0)))
      (CallFunction|EventPlayDrinkAnimation))
    (else
      ;[1 1 1] Stop current animation montage
      (bind _returnvalue_3 (Animation|GetCurrentMontage (Variables|Default|GetAnimalBase) :!class /Script/Engine.Character))
      (Animation|StopAnimMontage (Variables|Default|GetAnimalBase) _returnvalue_3))))

(event EventReceiveExecuteAI
  (params (OwnerController :type AI%20Controller%20Object%20Reference) (ControlledPawn :type Pawn%20Object%20Reference))
  (bind (_found_food _food_location) (CallFunction|FnLookforWater))
  (Variables|Default|SetPawnRef ControlledPawn)
  (bind _asbp_ground_animal_base (Utilities|Casting|CastToBP_GroundAnimalBase (Variables|Default|GetPawnRef)))
  (Variables|Default|SetAnimalBase _asbp_ground_animal_base)
  ;[1 1 1] Check if we have Comp_NeedSystem
  (Utilities|IsValid (Actor|GetComponentbyClass (Variables|Default|GetAnimalBase) "/Game/AnimalBehaviorKit/Blueprints/AI/Components/GroundAnimals/BP_Comp_NeedSystem.BP_Comp_NeedSystem_C")
    (:Is%20Valid
      ;[1 1 1] Save NeedSystem
      (Variables|Default|SetNeedSystem (Actor|GetComponentbyClass (Variables|Default|GetAnimalBase) "/Game/AnimalBehaviorKit/Blueprints/AI/Components/GroundAnimals/BP_Comp_NeedSystem.BP_Comp_NeedSystem_C"))
      ;[1 1 1] Use HomeBase?
      (Variables|Default|SetUseHomeBase? (Variables|/Game/AnimalBehaviorKit/Blueprints/Characters/Animals/GroundAnimals/BP_GroundAnimalBase.BP_GroundAnimalBase_C|GetUseHomeBase? (Variables|Default|GetAnimalBase)))
      ;[1 1 1] Set Acceptance Radius
      (Variables|Default|SetAcceptanceRadius (Variables|/Game/AnimalBehaviorKit/Blueprints/Characters/Animals/GroundAnimals/BP_GroundAnimalBase.BP_GroundAnimalBase_C|GetMovementAcceptanceRadius (Variables|Default|GetAnimalBase)))
      ;[1 1 1] Get water parameters
      (Variables|Default|SetDrinkingTime (.DrinkingTime (Utilities|Struct|BreakBP_Struct_Need_Drink (Variables|/Game/AnimalBehaviorKit/Blueprints/AI/Components/GroundAnimals/BP_Comp_NeedSystem.BP_Comp_NeedSystem_C|GetThristDetails (Variables|Default|GetNeedSystem)))))
      (Variables|Default|SetSearchRadius (.SearchRadius (Utilities|Struct|BreakBP_Struct_Need_Drink (Variables|/Game/AnimalBehaviorKit/Blueprints/AI/Components/GroundAnimals/BP_Comp_NeedSystem.BP_Comp_NeedSystem_C|GetThristDetails (Variables|Default|GetNeedSystem)))))
      (Variables|Default|SetWaterID (.WaterID (Utilities|Struct|BreakBP_Struct_Need_Drink (Variables|/Game/AnimalBehaviorKit/Blueprints/AI/Components/GroundAnimals/BP_Comp_NeedSystem.BP_Comp_NeedSystem_C|GetThristDetails (Variables|Default|GetNeedSystem)))))
      ;[1 1 1] Get nearest water source and Move AI to that location
      (if _found_food
        (AI|AIMoveTo (Variables|Default|GetPawnRef) _food_location 0 (Variables|Default|GetAcceptanceRadius) true
          (:then
            ;[1 1 1] Set Moving to True
            (Class|BTFunctionLibrary|SetBlackboardValueasBool (Variables|Default|GetMoving) true))
          (:OnSuccess
            ;[1 1 1] Set Moving to False
            (Class|BTFunctionLibrary|SetBlackboardValueasBool (Variables|Default|GetMoving) false)
            ;[1 1 1] Play Drink animation
            (CallFunction|EventPlayDrinkAnimation :!label _label)
            ;[1 1 1] Wait WaitAtDestination seconds
            (Utilities|FlowControl|Delay (Variables|Default|GetDrinkingTime))
            ;[1 1 1] Check if we are playing the animation montage and stop it
            (Variables|Default|SetCanDrink false)
            (bind _returnvalue (Animation|GetCurrentMontage (Variables|Default|GetAnimalBase) :!class /Script/Engine.Character))
            (Animation|StopAnimMontage (Variables|Default|GetAnimalBase) _returnvalue)
            ;[1 1 1] This delay accounts for the drinking montage's blend out time. You may need to adjust this depending on your animation
            (Utilities|FlowControl|Delay 1.5)
            (if (Variables|Default|GetUseHomeBase?)
              (Variables|/Game/AnimalBehaviorKit/Blueprints/Characters/Animals/GroundAnimals/BP_GroundAnimalBase.BP_GroundAnimalBase_C|SetRoamBehavior (Variables|Default|GetAnimalBase) "NewEnumerator6"))
            ;[1 1 1] Set next Roam Behavior
            (bind _newroambehavior (Default|FnSetRoamBehavior (Variables|Default|GetAnimalBase)))
            (|SETNEXTBEHAVIORINTHEBLACKBOARD _newroambehavior
              (:OutputPin
                ;[1 1 1] Finished drinking - set BiggestNeed to Roam again
                (Variables|/Game/AnimalBehaviorKit/Blueprints/Characters/Animals/GroundAnimals/BP_GroundAnimalBase.BP_GroundAnimalBase_C|SetBiggestNeed (Variables|Default|GetAnimalBase) "NewEnumerator3")
                ;[1 1 1] Reset Thirst
                (Default|EventFinishedDrinking (Variables|Default|GetNeedSystem))
                (Variables|Default|SetCanDrink true)
                (AI|BehaviorTree|FinishExecute true))))
          (:OnFail
            ;[1 1 1] Set Moving to False
            (Class|BTFunctionLibrary|SetBlackboardValueasBool (Variables|Default|GetMoving) false)
            (|RANDOMLOCATIONINWATERSPLINE
              (:OnSuccess
                (goto _label))
              (:OnFail
                (AI|BehaviorTree|FinishExecute false)))))
        (else
          ;[1 1 1] Check if animal dies from thirst
          (if (Utilities|Struct|BreakBP_Struct_Need_Drink (Variables|/Game/AnimalBehaviorKit/Blueprints/AI/Components/GroundAnimals/BP_Comp_NeedSystem.BP_Comp_NeedSystem_C|GetThristDetails (Variables|Default|GetNeedSystem)))
            ;[1 1 1] Kill animal
            (Default|EventDead (Variables|Default|GetAnimalBase))
            (else
              ;[1 1 1] Set BiggestNeed to Roam again
              (Variables|/Game/AnimalBehaviorKit/Blueprints/Characters/Animals/GroundAnimals/BP_GroundAnimalBase.BP_GroundAnimalBase_C|SetBiggestNeed (Variables|Default|GetAnimalBase) "NewEnumerator3")
              (AI|BehaviorTree|FinishExecute true))))))
    (:Is%20Not%20Valid
      (AI|BehaviorTree|FinishExecute false))))

(fn FnLookforWater
  (bind _animalbase (Variables|Default|GetAnimalBase))
  (bind _returnvalue (Transformation|GetActorLocation _animalbase))
  (bind (_outhits _returnvalue_2) (Collision|MultiSphereTraceForObjects _returnvalue (+ _returnvalue "0, 0,0.010000") (Variables|Default|GetSearchRadius) (Utilities|Array|MakeArray "ObjectTypeQuery7") false 0 "None"))
  (if _returnvalue_2
    (for _array_element _outhits
      (LocalVariables|SetHitActor (.HitActor (Collision|BreakHitResult _array_element)))
      (bind _asbp_ai_water (Utilities|Casting|CastToBP_AI_Water (LocalVariables|GetHitActor)))
      (LocalVariables|SetWater _asbp_ai_water)
      ;[1 1 1] Check the hit actor is water with the correct ID and save it in the Map
      (if (Utilities|Name|Equal(Name) (Variables|/Game/AnimalBehaviorKit/Blueprints/AI/Actors/Ground_AI/NeedSystem/BP_AI_Water.BP_AI_Water_C|GetWaterID (LocalVariables|GetWater)) (Variables|Default|GetWaterID))
        ;[1 1 1] Calculate the distance
        (LocalVariables|SetDistance (Math|Vector|VectorLength (- (Spline|FindLocationClosesttoWorldLocation (Variables|/Game/AnimalBehaviorKit/Blueprints/AI/Actors/Ground_AI/NeedSystem/BP_AI_Water.BP_AI_Water_C|GetSpline (LocalVariables|GetWater)) (Transformation|GetActorLocation (Variables|Default|GetPawnRef)) "World") (Transformation|GetActorLocation (Variables|Default|GetAnimalBase)))))
        ;[1 1 1] Save actor information
        (Utilities|Map|Add (LocalVariables|GetNearbyWater) (LocalVariables|GetWater) (LocalVariables|GetDistance))
        (Utilities|Array|Add (LocalVariables|GetDistances) (LocalVariables|GetDistance))
        (LocalVariables|SetFoundWater true)))
    ;[1 1 1] Do we have at least 1 food nearby?
    (if (Utilities|Array|IsValidIndex (LocalVariables|GetDistances))
      (if (> (Utilities|Map|Length (LocalVariables|GetNearbyWater)) 0)
        ;[1 1 1] Check that the Distance index matches the NearbyWater index
        (if (<= (.IndexOfMinValue (Math|Float|MinOfFloatArray (LocalVariables|GetDistances))) (- (Utilities|Map|Length (LocalVariables|GetNearbyWater)) 1))
          ;[1 1 1] Return the location of the nearest Food
          (bind _keys (Utilities|Map|Keys (LocalVariables|GetNearbyWater)))
          (Utilities|IsValid (Utilities|Array|Get(acopy) _keys (.IndexOfMinValue (Math|Float|MinOfFloatArray (LocalVariables|GetDistances))))
            (:Is%20Valid
              (Variables|Default|SetSelectedWater (Utilities|Array|Get(acopy) _keys (.IndexOfMinValue (Math|Float|MinOfFloatArray (LocalVariables|GetDistances)))))
              (return (LocalVariables|GetFoundWater) (Spline|FindLocationClosesttoWorldLocation (Variables|/Game/AnimalBehaviorKit/Blueprints/AI/Actors/Ground_AI/NeedSystem/BP_AI_Water.BP_AI_Water_C|GetSpline (Utilities|Array|Get(acopy) _keys (.IndexOfMinValue (Math|Float|MinOfFloatArray (LocalVariables|GetDistances))))) (Transformation|GetActorLocation (Variables|Default|GetPawnRef)) "World")))
            (:Is%20Not%20Valid
              (return false "0, 0, 0")))
          (else
            ;[1 1 1] Get the first water actor find and go there
            (bind _keys_2 (Utilities|Map|Keys (LocalVariables|GetNearbyWater)))
            (Variables|Default|SetSelectedWater (Utilities|Array|Get(acopy) _keys_2))
            (return (LocalVariables|GetFoundWater) (Spline|FindLocationClosesttoWorldLocation (Variables|/Game/AnimalBehaviorKit/Blueprints/AI/Actors/Ground_AI/NeedSystem/BP_AI_Water.BP_AI_Water_C|GetSpline (Utilities|Array|Get(acopy) _keys_2)) (Transformation|GetActorLocation (Variables|Default|GetPawnRef)) "World"))))
        (else
          _)))
    (return (LocalVariables|GetFoundWater) "0, 0, 0")))