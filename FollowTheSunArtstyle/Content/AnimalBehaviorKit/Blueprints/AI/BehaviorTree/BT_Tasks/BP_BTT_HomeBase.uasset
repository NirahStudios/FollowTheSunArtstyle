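; Behavior Tree task that sends a ground animal to its Home Base and has it wander inside the base's bounds.
; After arriving, it loops a set number of random moves, each with randomized speed and acceleration, an idle montage and a wait drawn once from POI settings.
; When done, it writes the next roam behavior to the Blackboard, resets movement and succeeds; failed moves end the task as failed.
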(event Custom|EventMoveInsidePOI
  (bind _homebase (Variables|Default|GetHomeBase))
  (bind _bounds (Variables|/Game/AnimalBehaviorKit/Blueprints/AI/Actors/Ground_AI/Navigation/BP_AI_POI_Base.BP_AI_POI_Base_C|GetBounds _homebase))
  (bind _returnvalue (Transformation|GetWorldLocation _bounds))
  (bind _returnvalue_2 (Components|Box|GetScaledBoxExtent _bounds))
  (bind _returnvalue_3 (Math|Random|RandomPointinBoundingBox _returnvalue _returnvalue_2))
  ;[1 1 1] Is the MoveCounter Less Than the TotalMoves?
  (if (< (Variables|Default|GetMoveCounter) (Variables|Default|GetTotalMoves))
    ;[1 1 1] Increase the counter by 1
    (Math|Integer|IncrementInt (Variables|Default|GetMoveCounter)
      (:%20%20
        (|SETRANDOMWALKSPEEDANDACCELERATION_2)
        ;[1 1 1] Get random location inside the POI and move there
        (AI|AIMoveTo (Variables|Default|GetPawnRef) (Math|Vector|MakeVector (.x _returnvalue_3) (.y _returnvalue_3) (.z (Transformation|GetActorLocation (Variables|Default|GetPawnRef)))) 0 (Variables|Default|GetMoveRadius) true
          (:then
            ;[1 1 1] Set Moving to True
            (Class|BTFunctionLibrary|SetBlackboardValueasBool (Variables|Default|GetMoving) true))
          (:OnSuccess
            ;[1 1 1] Set Moving to False
            (Class|BTFunctionLibrary|SetBlackboardValueasBool (Variables|Default|GetMoving) false)
            ;[1 1 1] Play Idle animation
            (Default|EventPlayAnimation (Variables|Default|GetAnimalBase) "NewEnumerator6")
            ;[1 1 1] Wait for the idle animation duration
            (bind _returnvalue_4 (Animation|GetCurrentMontage (Variables|Default|GetAnimalBase) :!class /Script/Engine.Character))
            (Utilities|IsValid _returnvalue_4
              (:Is%20Valid
                (bind _returnvalue_5 (Animation|GetPlayLength _returnvalue_4))
                (Utilities|FlowControl|Delay _returnvalue_5))
              (:Is%20Not%20Valid
                _))
            (Utilities|FlowControl|Delay (Variables|Default|GetWaitTime))
            (|RESETWALKSPEEDANDACCELERATION_2)
            (CallFunction|EventMoveInsidePOI))
          (:OnFail
            ;[1 1 1] Set Moving to False
            (Class|BTFunctionLibrary|SetBlackboardValueasBool (Variables|Default|GetMoving) false)
            (|RESETWALKSPEEDANDACCELERATION_3)
            (AI|BehaviorTree|FinishExecute false)))))
    (else
      ;[1 1 1] Set next Roam Behavior
      (bind _newroambehavior (Default|FnSetRoamBehavior (Variables|Default|GetAnimalBase)))
      (|SETNEXTBEHAVIORINTHEBLACKBOARD _newroambehavior
        (:OutputPin
          ;[1 1 1] Reset Move Counter
          (Variables|Default|SetMoveCounter 0)
          (|RESETWALKSPEEDANDACCELERATION_4)
          ;[1 1 1] Reached total number of moves - Finish Execute
          (AI|BehaviorTree|FinishExecute true))))))

(event EventReceiveExecuteAI
  (params (OwnerController :type AI%20Controller%20Object%20Reference) (ControlledPawn :type Pawn%20Object%20Reference))
  (bind _output_get (Variables|Default|SetPawnRef ControlledPawn))
  (Utilities|IsValid _output_get
    (:Is%20Valid
      (bind _asbp_ground_animal_base (Utilities|Casting|CastToBP_GroundAnimalBase (Variables|Default|GetPawnRef)))
      (Variables|Default|SetAnimalBase _asbp_ground_animal_base)
      ;[1 1 1] Get Total Time spent inside the POI
      (Variables|Default|SetWaitTime (Math|Random|RandomFloatinRange (.x (Utilities|Struct|BreakBP_Struct_GroundAnimalBehavior_POI (Variables|/Game/AnimalBehaviorKit/Blueprints/Characters/Animals/GroundAnimals/BP_GroundAnimalBase.BP_GroundAnimalBase_C|GetBehavior_POI (Variables|Default|GetAnimalBase)))) (.y (Utilities|Struct|BreakBP_Struct_GroundAnimalBehavior_POI (Variables|/Game/AnimalBehaviorKit/Blueprints/Characters/Animals/GroundAnimals/BP_GroundAnimalBase.BP_GroundAnimalBase_C|GetBehavior_POI (Variables|Default|GetAnimalBase))))))
      ;[1 1 1] Get number of moves inside the POI
      (Variables|Default|SetTotalMoves (Utilities|Struct|BreakBP_Struct_GroundAnimalBehavior_POI (Variables|/Game/AnimalBehaviorKit/Blueprints/Characters/Animals/GroundAnimals/BP_GroundAnimalBase.BP_GroundAnimalBase_C|GetBehavior_POI (Variables|Default|GetAnimalBase))))
      ;[1 1 1] Get Movement Acceptance Radius
      (Variables|Default|SetMoveRadius (Variables|/Game/AnimalBehaviorKit/Blueprints/Characters/Animals/GroundAnimals/BP_GroundAnimalBase.BP_GroundAnimalBase_C|GetMovementAcceptanceRadius (Variables|Default|GetAnimalBase)))
      ;[1 1 1] Get Home Base
      (Utilities|IsValid (Variables|/Game/AnimalBehaviorKit/Blueprints/Characters/Animals/GroundAnimals/BP_GroundAnimalBase.BP_GroundAnimalBase_C|GetHomeBase (Variables|Default|GetAnimalBase))
        (:Is%20Valid
          (Variables|Default|SetHomeBase (Variables|/Game/AnimalBehaviorKit/Blueprints/Characters/Animals/GroundAnimals/BP_GroundAnimalBase.BP_GroundAnimalBase_C|GetHomeBase (Variables|Default|GetAnimalBase)))
          (|SETRANDOMWALKSPEEDANDACCELERATION)
          ;[1 1 1] Go to Home Base
          (AI|AIMoveTo (Variables|Default|GetPawnRef) (Transformation|GetActorLocation (Variables|Default|GetHomeBase)) 0 (Variables|Default|GetMoveRadius) true
            (:then
              ;[1 1 1] Set Moving to True
              (Class|BTFunctionLibrary|SetBlackboardValueasBool (Variables|Default|GetMoving) true))
            (:OnSuccess
              ;[1 1 1] Set Moving to False
              (Class|BTFunctionLibrary|SetBlackboardValueasBool (Variables|Default|GetMoving) false)
              (CallFunction|EventMoveInsidePOI))
            (:OnFail
              ;[1 1 1] Set Moving to False
              (Class|BTFunctionLibrary|SetBlackboardValueasBool (Variables|Default|GetMoving) false)
              (|RESETWALKSPEEDANDACCELERATION)
              (AI|BehaviorTree|FinishExecute false))))
        (:Is%20Not%20Valid
          ;[1 1 1] Error Message
          (Development|PrintString (Utilities|String|Append (Utilities|GetDisplayName (Variables|Default|GetAnimalBase)) ": No Home Base found!") true true "(R=1.000000,G=0.000000,B=0.000000,A=1.000000)" 5.0))))))