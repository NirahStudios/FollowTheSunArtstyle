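; Behavior tree task that sends a ground animal to its defense location.
; On execute it randomly scales walk speed and acceleration, runs AIMoveTo with a Moving blackboard flag, and restores engage values when the move ends.
; Tick blocks engaging until the animal is near the location, then waits an inspection delay, re-enables engaging, updates defense state, disengages and finishes the task.
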(event EventReceiveExecuteAI
  (params (OwnerController :type AI%20Controller%20Object%20Reference) (ControlledPawn :type Pawn%20Object%20Reference))
  (bind _output_get (Variables|Default|SetPawnRef ControlledPawn))
  (Utilities|IsValid _output_get
    (:Is%20Valid
      (bind _asbp_ground_animal_base (Utilities|Casting|CastToBP_GroundAnimalBase (Variables|Default|GetPawnRef)))
      (Variables|Default|SetAnimalBase _asbp_ground_animal_base)
      ;[1 1 1] Set Acceptance Radius
      (Variables|Default|SetAcceptanceRadius (Variables|/Game/AnimalBehaviorKit/Blueprints/Characters/Animals/GroundAnimals/BP_GroundAnimalBase.BP_GroundAnimalBase_C|GetMovementAcceptanceRadius (Variables|Default|GetAnimalBase)))
      (|SETRANDOMWALKSPEEDANDACCELERATION)
      ;[1 1 1] Move towards Defense Location
      (AI|AIMoveTo (Variables|Default|GetPawnRef) (Variables|/Game/AnimalBehaviorKit/Blueprints/Characters/Animals/GroundAnimals/BP_GroundAnimalBase.BP_GroundAnimalBase_C|GetDefenseLocation (Variables|Default|GetAnimalBase)) 0 (Variables|Default|GetAcceptanceRadius) true
        (:then
          ;[1 1 1] Set Moving to True
          (Class|BTFunctionLibrary|SetBlackboardValueasBool (Variables|Setup|GetMoving) true))
        (:OnSuccess
          ;[1 1 1] Set Moving to False
          (Class|BTFunctionLibrary|SetBlackboardValueasBool (Variables|Setup|GetMoving) false)
          (|RESETWALKSPEEDANDACCELERATION))
        (:OnFail
          ;[1 1 1] Set Moving to False
          (Class|BTFunctionLibrary|SetBlackboardValueasBool (Variables|Setup|GetMoving) false)
          (|RESETWALKSPEEDANDACCELERATION_2))))))

(event EventReceiveTickAI
  (params (OwnerController :type AI%20Controller%20Object%20Reference) (ControlledPawn :type Pawn%20Object%20Reference) (DeltaSeconds :type Float%20%28single-precision%29))
  (bind _animalbase (Variables|Default|GetAnimalBase))
  ;[1 1 1] Check if animal arrived at Defense Location
  (if (<= (Math|Vector|VectorLength (- (Variables|/Game/AnimalBehaviorKit/Blueprints/Characters/Animals/GroundAnimals/BP_GroundAnimalBase.BP_GroundAnimalBase_C|GetDefenseLocation _animalbase) (Transformation|GetActorLocation _animalbase))) 5e+02)
    ;[1 1 1] Wait InspectionTime
    (Utilities|FlowControl|Delay (Utilities|Struct|BreakBP_Struct_GroundAnimaBehavior_Defend (Variables|/Game/AnimalBehaviorKit/Blueprints/Characters/Animals/GroundAnimals/BP_GroundAnimalBase.BP_GroundAnimalBase_C|GetBehavior_Defend (Variables|Default|GetAnimalBase))))
    (Variables|/Game/AnimalBehaviorKit/Blueprints/Characters/Animals/GroundAnimals/BP_GroundAnimalBase.BP_GroundAnimalBase_C|SetCanEngage (Variables|Default|GetAnimalBase) true)
    (Variables|/Game/AnimalBehaviorKit/Blueprints/Characters/Animals/GroundAnimals/BP_GroundAnimalBase.BP_GroundAnimalBase_C|SetDefenseState (Variables|Default|GetAnimalBase) "NewEnumerator1")
    ;[1 1 1] Set DefenseState to 'Going to Defense Location'
    (Class|BTFunctionLibrary|SetBlackboardValueasEnum (Variables|Setup|GetDefenseState) (Utilities|Enum|LiteralenumBP_Enum_DefenseState "NewEnumerator0"))
    ;[1 1 1] Disengage
    (Default|FnDisengage (Variables|Default|GetAnimalBase))
    (|RESETWALKSPEEDANDACCELERATION_3)
    (AI|BehaviorTree|FinishExecute true)
    (else
      (Variables|/Game/AnimalBehaviorKit/Blueprints/Characters/Animals/GroundAnimals/BP_GroundAnimalBase.BP_GroundAnimalBase_C|SetCanEngage (Variables|Default|GetAnimalBase) false))))