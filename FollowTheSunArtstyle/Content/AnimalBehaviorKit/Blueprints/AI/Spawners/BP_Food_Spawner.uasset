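; Spawner that places BP_AI_Food on tagged static mesh actors and foliage instances, sizing each food's bounds from the source's scale.
; Numbered events gather foliage mesh names into the FoliageMeshes toggle map, then spawn or delete food globally or within the SpawnArea box.
; Area operations use box traces, matching foliage by hit instance index.
; Spawned food is tracked in SpawnedFood for later removal.
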(event Custom|5_DeleteFoodInArea
  ;[1 1 1] Delete food in the area
  (CallFunction|FnDeleteFoodArea))

(event Custom|2_SpawnFood
  ;[1 1 1] Spawn Food on the appropriate actors with tag
  (CallFunction|FnSpawnFood))

(event Custom|1_GetFoliageInfo
  ;[1 1 1] Get current Foliage info and populate the FoliageMeshes Map
  (CallFunction|FnGetFoliageInfo))

(event Custom|3_SpawnFoodInArea
  ;[1 1 1] Spawn food inside area
  (CallFunction|FnSpawnFoodArea))

(event Custom|4_DeleteFood
  ;[1 1 1] Delete all spawned food
  (CallFunction|FnDeleteFood))

(fn ConstructionScript
  (Transformation|SetWorldScale3D (Variables|Default|GetSpawnArea) (Variables|Setup|GetSpawnAreaScale)))

(fn FnSpawnFood
  (bind _outactors (Actor|GetAllActorswithTag (Variables|Setup|GetActor%20Tag)))
  (for _array_element _outactors
    (LocalVariables|SetcActor _array_element)
    (Utilities|FlowControl|Sequence
      (:then_0
        (if (Variables|Setup|GetUseStaticMeshes)
          ;[1 1 1] Is the actor a StaticMeshActor?
          (if (== (Utilities|GetClass (LocalVariables|GetcActor)) "/Script/Engine.StaticMeshActor")
            ;[1 1 1] Spawn BP_AI_Food
            (bind _returnvalue (Game|SpawnActorfromClass (Variables|Setup|GetAIFood_Class) (Math|Transform|MakeTransform (.location (Transformation|GetActorTransform (LocalVariables|GetcActor))) (.rotation (Transformation|GetActorTransform (LocalVariables|GetcActor))) "1,1,1") "AlwaysSpawn" 0 0))
            ;[1 1 1] Add spawned food reference to array
            (Utilities|Array|AddUnique (Variables|Setup|GetSpawnedFood) _returnvalue)
            ;[1 1 1] Set scales
            (bind _asbp_ai_food (Utilities|Casting|CastToBP_AI_Food _returnvalue))
            (LocalVariables|SetcFood _asbp_ai_food)
            (Variables|/Game/AnimalBehaviorKit/Blueprints/AI/Actors/Ground_AI/NeedSystem/BP_AI_Food.BP_AI_Food_C|SetBoundsScale (LocalVariables|GetcFood) (Math|Vector|MakeVector (* (.x (Transformation|GetActorScale3D (LocalVariables|GetcActor))) 2.0) (* (.y (Transformation|GetActorScale3D (LocalVariables|GetcActor))) 2.0) 2.0))
            ;[1 1 1] Scale Bounds
            (Default|FnSetScales (LocalVariables|GetcFood)))))
      (:then_1
        (if (Variables|Setup|GetUseFoliage)
          ;[1 1 1] Is the actor a InstancedFoliageActor?
          (if (== (Utilities|GetClass (LocalVariables|GetcActor)) "/Script/Foliage.InstancedFoliageActor")
            (bind _asinstanced_foliage_actor (Utilities|Casting|CastToInstancedFoliageActor (LocalVariables|GetcActor)))
            ;[1 1 1] Go through each foliage type
            (for _array_element_2 (Actor|GetComponentsByClass _asinstanced_foliage_actor "/Script/Engine.InstancedStaticMeshComponent")
              (bind _output_get (LocalVariables|SetiFoliage _array_element_2))
              ;[1 1 1] Do we spawn Food on this specific Foliage static mesh?
              (if (.Value (Utilities|Map|Find (Variables|Setup|GetFoliageMeshes) (Utilities|McGetFoliageMeshName _output_get)))
                ;[1 1 1] Loop through all instances of this type of Foliage
                (for _index (range 0 (- (Components|InstancedStaticMesh|GetInstanceCount (LocalVariables|GetiFoliage)) 1))
                  ;[1 1 1] Spawn BP_AI_Food
                  (bind _returnvalue_2 (Game|SpawnActorfromClass (Variables|Setup|GetAIFood_Class) (Math|Transform|MakeTransform (.location (.OutInstanceTransform (Components|InstancedStaticMesh|GetInstanceTransform (LocalVariables|GetiFoliage) _index true))) (.rotation (.OutInstanceTransform (Components|InstancedStaticMesh|GetInstanceTransform (LocalVariables|GetiFoliage) _index true))) "1,1,1") "AlwaysSpawn" 0 0))
                  ;[1 1 1] Add spawned food reference to array
                  (Utilities|Array|AddUnique (Variables|Setup|GetSpawnedFood) _returnvalue_2)
                  ;[1 1 1] Set scales
                  (bind _asbp_ai_food_2 (Utilities|Casting|CastToBP_AI_Food _returnvalue_2))
                  (LocalVariables|SetcFood _asbp_ai_food_2)
                  (Variables|/Game/AnimalBehaviorKit/Blueprints/AI/Actors/Ground_AI/NeedSystem/BP_AI_Food.BP_AI_Food_C|SetBoundsScale (LocalVariables|GetcFood) (Math|Vector|MakeVector (* (.x (.scale (.OutInstanceTransform (Components|InstancedStaticMesh|GetInstanceTransform (LocalVariables|GetiFoliage) 0 true)))) 2.0) (* (.y (.scale (.OutInstanceTransform (Components|InstancedStaticMesh|GetInstanceTransform (LocalVariables|GetiFoliage) 0 true)))) 2.0) 2.0))
                  ;[1 1 1] Scale Bounds
                  (Default|FnSetScales (LocalVariables|GetcFood)))))))))))

(fn FnGetFoliageInfo
  (bind _outactors (Actor|GetAllActorswithTag (Variables|Setup|GetActor%20Tag)))
  (for _array_element _outactors
    (LocalVariables|SetcActor _array_element)
    ;[1 1 1] Is the actor a InstancedFoliageActor?
    (if (== (Utilities|GetClass (LocalVariables|GetcActor)) "/Script/Foliage.InstancedFoliageActor")
      (bind _asinstanced_foliage_actor (Utilities|Casting|CastToInstancedFoliageActor (LocalVariables|GetcActor)))
      ;[1 1 1] Go through each foliage type
      (for _array_element_2 (Actor|GetComponentsByClass _asinstanced_foliage_actor "/Script/Engine.InstancedStaticMeshComponent")
        (bind _output_get (LocalVariables|SetiFoliage _array_element_2))
        ;[1 1 1] Add new entry to the FoliageMeshes map
        (Utilities|Map|Add (Variables|Setup|GetFoliageMeshes) (Utilities|McGetFoliageMeshName _output_get) true)))))

(fn FnDeleteFood
  (for _array_element (Variables|Setup|GetSpawnedFood)
    (Actor|DestroyActor _array_element))
  (Utilities|Array|Clear (Variables|Setup|GetSpawnedFood)))

(fn FnSpawnFoodArea
  (bind _spawnarea (Variables|Default|GetSpawnArea))
  (bind _spawnarea_2 (Variables|Default|GetSpawnArea))
  (bind _returnvalue (Transformation|GetWorldLocation _spawnarea))
  (bind _returnvalue_2 (Transformation|GetWorldLocation _spawnarea_2))
  (Utilities|FlowControl|Sequence
    (:then_0
      (if (Variables|Setup|GetUseStaticMeshes)
        ;[1 1 1] Do a multi box trace
        (bind (_outhits _returnvalue_3) (Class|KismetSystemLibrary|BoxTraceMulti _returnvalue_2 (+ _returnvalue_2 "0, 0,0.010000") (Components|Box|GetScaledBoxExtent _spawnarea_2) (Transformation|GetWorldRotation _spawnarea_2) "TraceTypeQuery1" false 0 "None" true))
        ;[1 1 1] Did we hit something?
        (if _returnvalue_3
          ;[1 1 1] For each hit actor
          (for _array_element _outhits
            ;[1 1 1] Check if actor has ActorTag
            (if (Actor|ActorHasTag (.HitActor (Collision|BreakHitResult _array_element)) (Variables|Setup|GetActor%20Tag))
              ;[1 1 1] Is the actor a StaticMeshActor?
              (if (== (Utilities|GetClass (.HitActor (Collision|BreakHitResult _array_element))) "/Script/Engine.StaticMeshActor")
                ;[1 1 1] Add actor to ActorList
                (Utilities|Array|Add (LocalVariables|GetActorList) (.HitActor (Collision|BreakHitResult _array_element))))))
          (if (Utilities|Array|IsValidIndex (LocalVariables|GetActorList))
            (for _array_element_2 (LocalVariables|GetActorList)
              (LocalVariables|SetcActor _array_element_2)
              ;[1 1 1] Spawn BP_AI_Food
              (bind _returnvalue_4 (Game|SpawnActorfromClass (Variables|Setup|GetAIFood_Class) (Math|Transform|MakeTransform (.location (Transformation|GetActorTransform (LocalVariables|GetcActor))) (.rotation (Transformation|GetActorTransform (LocalVariables|GetcActor))) "1,1,1") "AlwaysSpawn" 0 0))
              ;[1 1 1] Add spawned food reference to array
              (Utilities|Array|AddUnique (Variables|Setup|GetSpawnedFood) _returnvalue_4)
              ;[1 1 1] Set scales
              (bind _asbp_ai_food (Utilities|Casting|CastToBP_AI_Food _returnvalue_4))
              (LocalVariables|SetcFood _asbp_ai_food)
              (Variables|/Game/AnimalBehaviorKit/Blueprints/AI/Actors/Ground_AI/NeedSystem/BP_AI_Food.BP_AI_Food_C|SetBoundsScale (LocalVariables|GetcFood) (Math|Vector|MakeVector (* (.x (Transformation|GetActorScale3D (LocalVariables|GetcActor))) 2.0) (* (.y (Transformation|GetActorScale3D (LocalVariables|GetcActor))) 2.0) 2.0))
              ;[1 1 1] Scale Bounds
              (Default|FnSetScales (LocalVariables|GetcFood)))))))
    (:then_1
      (if (Variables|Setup|GetUseFoliage)
        ;[1 1 1] Do a multi box trace
        (bind (_outhits_2 _returnvalue_5) (Class|KismetSystemLibrary|BoxTraceMulti _returnvalue (+ _returnvalue "0, 0,0.010000") (Components|Box|GetScaledBoxExtent _spawnarea) (Transformation|GetWorldRotation _spawnarea) "TraceTypeQuery1" false 0 "None" true))
        ;[1 1 1] Did we hit something?
        (if _returnvalue_5
          ;[1 1 1] For each hit actor
          (for _array_element_3 _outhits_2
            ;[1 1 1] Check if actor has ActorTag
            (if (and (Actor|ActorHasTag (.HitActor (Collision|BreakHitResult _array_element_3)) (Variables|Setup|GetActor%20Tag)) (>= (.HitItem (Collision|BreakHitResult _array_element_3)) 0))
              ;[1 1 1] Save HISMActor
              (LocalVariables|SetHISMActor (.HitActor (Collision|BreakHitResult _array_element_3)))
              ;[1 1 1] Add HISM actor to HISMInstanceList
              (Utilities|Array|Add (LocalVariables|GetHISMInstanceList) (.HitItem (Collision|BreakHitResult _array_element_3)))))
          (Utilities|IsValid (LocalVariables|GetHISMActor)
            (:Is%20Valid
              (bind _asinstanced_foliage_actor (Utilities|Casting|CastToInstancedFoliageActor (LocalVariables|GetHISMActor)))
              ;[1 1 1] Go through each foliage type
              (for _array_element_4 (Actor|GetComponentsByClass _asinstanced_foliage_actor "/Script/Engine.InstancedStaticMeshComponent")
                (bind _output_get (LocalVariables|SetiFoliage _array_element_4))
                ;[1 1 1] Do we spawn Food on this specific Foliage static mesh?
                (if (.Value (Utilities|Map|Find (Variables|Setup|GetFoliageMeshes) (Utilities|McGetFoliageMeshName _output_get)))
                  ;[1 1 1] Loop through all instances of this type of Foliage
                  (for _index (range 0 (- (Components|InstancedStaticMesh|GetInstanceCount (LocalVariables|GetiFoliage)) 1))
                    (LocalVariables|SetInstance _index)
                    ;[1 1 1] Check that this Instance is contained in HISMInstanceList
                    (if (Utilities|Array|ContainsItem (LocalVariables|GetHISMInstanceList) (LocalVariables|GetInstance))
                      ;[1 1 1] Spawn BP_AI_Food
                      (bind _returnvalue_6 (Game|SpawnActorfromClass (Variables|Setup|GetAIFood_Class) (Math|Transform|MakeTransform (.location (.OutInstanceTransform (Components|InstancedStaticMesh|GetInstanceTransform (LocalVariables|GetiFoliage) (LocalVariables|GetInstance) true))) (.rotation (.OutInstanceTransform (Components|InstancedStaticMesh|GetInstanceTransform (LocalVariables|GetiFoliage) (LocalVariables|GetInstance) true))) "1,1,1") "AlwaysSpawn" 0 0))
                      ;[1 1 1] Add spawned food reference to array
                      (Utilities|Array|AddUnique (Variables|Setup|GetSpawnedFood) _returnvalue_6)
                      ;[1 1 1] Set scales
                      (bind _asbp_ai_food_2 (Utilities|Casting|CastToBP_AI_Food _returnvalue_6))
                      (LocalVariables|SetcFood _asbp_ai_food_2)
                      (Variables|/Game/AnimalBehaviorKit/Blueprints/AI/Actors/Ground_AI/NeedSystem/BP_AI_Food.BP_AI_Food_C|SetBoundsScale (LocalVariables|GetcFood) (Math|Vector|MakeVector (* (.x (.scale (.OutInstanceTransform (Components|InstancedStaticMesh|GetInstanceTransform (LocalVariables|GetiFoliage) 0 true)))) 2.0) (* (.y (.scale (.OutInstanceTransform (Components|InstancedStaticMesh|GetInstanceTransform (LocalVariables|GetiFoliage) 0 true)))) 2.0) 2.0))
                      ;[1 1 1] Scale Bounds
                      (Default|FnSetScales (LocalVariables|GetcFood)))))))))))))

(fn FnDeleteFoodArea
  (bind _spawnarea (Variables|Default|GetSpawnArea))
  (bind _returnvalue (Transformation|GetWorldLocation _spawnarea))
  ;[1 1 1] Do a multi box trace
  (bind (_outhits _returnvalue_2) (Class|KismetSystemLibrary|BoxTraceMultiforObjects _returnvalue (+ _returnvalue "0, 0,0.010000") (Components|Box|GetScaledBoxExtent _spawnarea) (Transformation|GetWorldRotation _spawnarea) (Utilities|Array|MakeArray "ObjectTypeQuery1") false 0 "None" true))
  ;[1 1 1] Did we hit something?
  (if _returnvalue_2
    ;[1 1 1] For each hit actor
    (for _array_element _outhits
      (LocalVariables|SetHitActor (.HitActor (Collision|BreakHitResult _array_element)))
      ;[1 1 1] Check if current actor is an instrance of BP_AIFood
      (if (== (Utilities|GetClass (LocalVariables|GetHitActor)) "/Game/AnimalBehaviorKit/Blueprints/AI/Actors/Ground_AI/NeedSystem/BP_AI_Food.BP_AI_Food_C")
        ;[1 1 1] Destroy the AI Food
        (Actor|DestroyActor (LocalVariables|GetHitActor))
        ;[1 1 1] Remove the AI Food from the SpawnedFood array
        (Utilities|Array|RemoveIndex (Variables|Setup|GetSpawnedFood) (Utilities|Array|FindItem (Variables|Setup|GetSpawnedFood) (LocalVariables|GetHitActor)))))))