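; Component on ground animals that lets the level's BP_ActivationManager switch them between active and inactive states to save processing.
; On BeginPlay it sets the owner's sim mode to Activation Manager, starts it inactive and registers it with the manager.
; FnSetAnimalStatus applies InactiveOptions: despawn with population-control cleanup, or toggle visibility, collision, ticks, components and AI controller.
; It also pauses or resumes need, mating, aging and death timers.
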(event EventBeginPlay
  (if (Variables|Setup|GetActive)
    ;[1 1 1] Get owner information
    (bind _asbp_ground_animal_base (Utilities|Casting|CastToBP_GroundAnimalBase (Components|GetOwner)))
    (bind _output_get (Variables|Default|SetOwner _asbp_ground_animal_base))
    (Variables|Default|SetAIController (AI|GetAIController _output_get))
    ;[1 1 1] Set Simulation Mode to Activation Manager
    (Utilities|Struct|SetmembersinBP_Struct_AnimalBase_SimDetails (Variables|/Game/AnimalBehaviorKit/Blueprints/Characters/Animals/BP_AnimalBase.BP_AnimalBase_C|GetSimulation_Details (Variables|Default|GetOwner)) "NewEnumerator2")
    ;[1 1 1] Set Inactive Options
    (Variables|Default|SetInactiveOptions (Utilities|Struct|BreakBP_Struct_AnimalBase_SimDetails (Variables|/Game/AnimalBehaviorKit/Blueprints/Characters/Animals/BP_AnimalBase.BP_AnimalBase_C|GetSimulation_Details (Variables|Default|GetOwner))))
    (Utilities|FlowControl|Sequence
      (:then_0
        ;[1 1 1] Deactivate Animal
        (CallFunction|FnSetAnimalStatus false))
      (:then_1
        ;[1 1 1] Register Animal with Activation Manager
        (CallFunction|FnRegisterAnimal)))))

(fn FnRegisterAnimal
  ;[1 1 1] Get Activation Manager from Level
  (bind _outactors (Actor|GetAllActorsOfClass "/Game/AnimalBehaviorKit/Blueprints/AI/Actors/Ground_AI/BP_ActivationManager.BP_ActivationManager_C"))
  (if (Utilities|Array|IsValidIndex _outactors)
    (Variables|Default|SetActivationManager (Utilities|Array|Get(acopy) _outactors))
    ;[1 1 1] Register Animal
    (Default|FnRegisterAnimal (Variables|Default|GetActivationManager) (Variables|Default|GetOwner))
    (else
      (|PRINTERROR))))

(fn FnSetInactiveOptions
  (bind _owner (Variables|Default|GetOwner))
  (bind _owner_2 (Variables|Default|GetOwner))
  (bind _returnvalue (Actor|GetComponentbyClass _owner_2 "/Game/AnimalBehaviorKit/Blueprints/AI/Components/GroundAnimals/BP_Comp_PopulationControl.BP_Comp_PopulationControl_C"))
  (bind _animal_details (Variables|/Game/AnimalBehaviorKit/Blueprints/Characters/Animals/BP_AnimalBase.BP_AnimalBase_C|GetAnimal_Details _owner))
  (bind (_sex _species) (Utilities|Struct|BreakBP_Struct_AnimalBase_AnimalDetail _animal_details))
  (if (Variables|Default|GetActiveStatus)
    (Utilities|FlowControl|Sequence
      (:then_0
        ;[1 1 1] Hide animal?
        (if (Utilities|Struct|BreakBP_Struct_AnimalBase_InactiveOptions (Variables|Default|GetInactiveOptions))
          (Rendering|SetActorHiddenInGame (Variables|Default|GetOwner) false)))
      (:then_1
        ;[1 1 1] Disable collision
        (if (Utilities|Struct|BreakBP_Struct_AnimalBase_InactiveOptions (Variables|Default|GetInactiveOptions))
          (Collision|SetCollisionEnabled (Variables|/Script/Engine.Character|GetMesh (Variables|Default|GetOwner)) "QueryAndPhysics")
          (Physics|SetEnableGravity (Variables|/Script/Engine.Character|GetCapsuleComponent (Variables|Default|GetOwner)) true)))
      (:then_2
        ;[1 1 1] Stop Actor Tick
        (if (Utilities|Struct|BreakBP_Struct_AnimalBase_InactiveOptions (Variables|Default|GetInactiveOptions))
          (Actor|Tick|SetActorTickEnabled (Variables|Default|GetOwner) true)))
      (:then_3
        (CallFunction|FnDisableAllComponents))
      (:then_4
        (CallFunction|FnDisableAIController)))
    (else
      (Utilities|FlowControl|Sequence
        (:then_0
          ;[1 1 1] Despawn animal
          (if (Utilities|Struct|BreakBP_Struct_AnimalBase_InactiveOptions (Variables|Default|GetInactiveOptions))
            (Utilities|FlowControl|Sequence
              (:then_0
                ;[1 1 1] Check if component Comp_PopulationControl is present
                (Utilities|IsValid _returnvalue
                  (:Is%20Valid
                    (Utilities|IsValid (Variables|/Game/AnimalBehaviorKit/Blueprints/AI/Components/GroundAnimals/BP_Comp_PopulationControl.BP_Comp_PopulationControl_C|GetPopulationControlReference _returnvalue)
                      (:Is%20Valid
                        (Utilities|FlowControl|DoOnce false
                          (:Completed
                            ;[1 1 1] Remove animal from BP_PopulationControl
                            (Default|FnRemoveAnimal (Variables|/Game/AnimalBehaviorKit/Blueprints/AI/Components/GroundAnimals/BP_Comp_PopulationControl.BP_Comp_PopulationControl_C|GetPopulationControlReference _returnvalue) (Utilities|Struct|MakeBP_Struct_Population_AnimalDetails (Variables|Default|GetOwner) _species _sex)))))))))
              (:then_1
                ;[1 1 1] Destroy actor
                (Actor|DestroyActor (Variables|Default|GetOwner))))))
        (:then_1
          ;[1 1 1] Check that actor is valid
          (Utilities|IsValid (Variables|Default|GetOwner)
            (:Is%20Valid
              (Utilities|FlowControl|Sequence
                (:then_0
                  ;[1 1 1] Hide animal?
                  (if (Utilities|Struct|BreakBP_Struct_AnimalBase_InactiveOptions (Variables|Default|GetInactiveOptions))
                    (Rendering|SetActorHiddenInGame (Variables|Default|GetOwner) true)))
                (:then_1
                  ;[1 1 1] Disable collision
                  (if (Utilities|Struct|BreakBP_Struct_AnimalBase_InactiveOptions (Variables|Default|GetInactiveOptions))
                    (Physics|SetEnableGravity (Variables|/Script/Engine.Character|GetCapsuleComponent (Variables|Default|GetOwner)) false)
                    (if (not (Variables|/Game/AnimalBehaviorKit/Blueprints/Characters/Animals/BP_AnimalBase.BP_AnimalBase_C|GetDead (Variables|Default|GetOwner)))
                      (Collision|SetCollisionEnabled (Variables|/Script/Engine.Character|GetMesh (Variables|Default|GetOwner)) "NoCollision"))))
                (:then_2
                  ;[1 1 1] Stop Actor Tick
                  (if (Utilities|Struct|BreakBP_Struct_AnimalBase_InactiveOptions (Variables|Default|GetInactiveOptions))
                    (Actor|Tick|SetActorTickEnabled (Variables|Default|GetOwner))))
                (:then_3
                  (CallFunction|FnDisableAllComponents))
                (:then_4
                  ;[1 1 1] Stop AI Logic
                  (if (Utilities|Struct|BreakBP_Struct_AnimalBase_InactiveOptions (Variables|Default|GetInactiveOptions))
                    (Default|EventSearchforPlayer (Variables|Default|GetOwner))))
                (:then_5
                  (CallFunction|FnDisableAIController))))))))))

(fn FnSetAnimalStatus
  (params (Active :type Boolean))
  (Variables|Default|SetActiveStatus Active)
  (Utilities|FlowControl|Sequence
    (:then_0
      (Variables|/Game/AnimalBehaviorKit/Blueprints/Characters/Animals/BP_AnimalBase.BP_AnimalBase_C|SetActive (Variables|Default|GetOwner) (Variables|Default|GetActiveStatus)))
    (:then_1
      (CallFunction|FnSetInactiveOptions))
    (:then_2
      (CallFunction|FnEnableComponents))))

(fn FnEnableComponents
  (if (Variables|Default|GetActiveStatus)
    (|UNPAUSECOMPONENTSWITHTIMERS)
    (else
      (|PAUSECOMPONENTSWITHTIMERS))))

(fn FnDisableAllComponents
  (if (Utilities|Struct|BreakBP_Struct_AnimalBase_InactiveOptions (Utilities|Struct|BreakBP_Struct_AnimalBase_SimDetails (Variables|/Game/AnimalBehaviorKit/Blueprints/Characters/Animals/BP_AnimalBase.BP_AnimalBase_C|GetSimulation_Details (Variables|Default|GetOwner))))
    (if (Variables|Default|GetActiveStatus)
      (|ENABLEALLCOMPONENTS)
      (else
        (|DISABLEALLCOMPONENTS)))))

(fn FnDisableAIController
  (if (Utilities|Struct|BreakBP_Struct_AnimalBase_InactiveOptions (Utilities|Struct|BreakBP_Struct_AnimalBase_SimDetails (Variables|/Game/AnimalBehaviorKit/Blueprints/Characters/Animals/BP_AnimalBase.BP_AnimalBase_C|GetSimulation_Details (Variables|Default|GetOwner))))
    (if (Variables|Default|GetActiveStatus)
      (|ENABLEAICONTROLLER)
      (else
        (|DISABLEAICONTROLLER)))))