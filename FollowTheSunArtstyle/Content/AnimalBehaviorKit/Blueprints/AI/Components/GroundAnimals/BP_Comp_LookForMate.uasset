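; Ground animal component that drives mate seeking and breeding for its owner.
; On authority, a timer sphere-traces for same-species, opposite-sex animals, chooses one by navmesh path length and flags the owner to breed, if that sex searches.
; EventBreeding halts the animal with optional heart particles for a timed period.
; The non-partner side then, unless engaged, spawns random-sex offspring that can inherit behaviors and tags, or follow the parent via BP_Comp_GrowOld.
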(event EventBeginPlay
  (Utilities|FlowControl|Delay 0.1)
  (|GETOWNERSPECIESANDSEX)
  (if (Variables|Setup-LookForPartner|GetActive)
    ;[1 1 1] Check for Authority
    (if (Default|FnGetAuthority (Variables|Default|GetOwner))
      (|DETERMINEIFNEEDTOSEARCHFORPARTNER)
      (|STARTEVENTSEARCHFORPARTNER))))

(fn FnLookforPartner
  (bind _returnvalue (Components|GetOwner))
  (bind _returnvalue_2 (Transformation|GetActorLocation _returnvalue))
  ;[1 1 1] Check for Authority
  (if (Default|FnGetAuthority (Variables|Default|GetOwner))
    ;[1 1 1] Check that the component is active
    (if (Variables|Setup-LookForPartner|GetActive)
      ;[1 1 1] Do we want to debug partner search?
      (if (Variables|Setup-Debug|GetDebugPartnerSearch)
        ;[1 1 0] Set sphere trace debug mode
        (LocalVariables|SetSphereDebug "ForDuration")
        (else
          (LocalVariables|SetSphereDebug "None")))
      ;[1 1 1] Generate a sphere trace by channel that mimics the Collision_Attack collision sphere
      (bind (_outhits _returnvalue_3) (Collision|MultiSphereTraceForObjects _returnvalue_2 (+ _returnvalue_2 "0, 0,0.010000") (Variables|Setup-LookForPartner|GetPartnerSearchRadius) (Utilities|Array|MakeArray "ObjectTypeQuery3") false 0 (LocalVariables|GetSphereDebug)))
      ;[1 1 1] Did we hit something?
      (if _returnvalue_3
        ;[1 1 1] For each hit actor
        (for _array_element _outhits
          (LocalVariables|SetHitActor (.HitActor (Collision|BreakHitResult _array_element)))
          (bind _asbp_animal_base (Utilities|Casting|CastToBP_AnimalBase (LocalVariables|GetHitActor)))
          ;[1 1 1] Is the Hit Actor the same species as the Owner?
          (if (Utilities|Enum|Equal(Enum) (Variables|Default|GetOwnerSpecies) (Utilities|Struct|BreakBP_Struct_AnimalBase_AnimalDetail (Variables|/Game/AnimalBehaviorKit/Blueprints/Characters/Animals/BP_AnimalBase.BP_AnimalBase_C|GetAnimal_Details _asbp_animal_base)))
            ;[1 1 1] Is the Hit Actor a different Sex than the Owner?
            (if (Utilities|Enum|NotEqual(Enum) (Variables|Default|GetOwnerSex) (Utilities|Struct|BreakBP_Struct_AnimalBase_AnimalDetail (Variables|/Game/AnimalBehaviorKit/Blueprints/Characters/Animals/BP_AnimalBase.BP_AnimalBase_C|GetAnimal_Details _asbp_animal_base)))
              ;[1 1 1] Add Hit Actor to ActorList array
              (Utilities|Array|AddUnique (LocalVariables|GetActorList) (LocalVariables|GetHitActor)))))
        ;[1 1 1] Do we have potential partners nearby?
        (if (> (Utilities|Array|Length (LocalVariables|GetActorList)) 0)
          ;[1 1 1] For each potential Partner
          (for _array_element_2 (LocalVariables|GetActorList)
            (bind _output_get (LocalVariables|SetCurrentActor _array_element_2))
            (Utilities|IsValid _output_get
              (:Is%20Valid
                ;[1 1 1] Get Path Length for current actor in array
                (LocalVariables|SetCurrentPathLength (.PathLength (Class|NavigationSystem|GetPathLength (Transformation|GetActorLocation (Components|GetOwner)) (Transformation|GetActorLocation (LocalVariables|GetCurrentActor)))))
                ;[1 1 1] Check the Nav Mesh path is valid
                (if (Utilities|Enum|Equal(Enum) (.ReturnValue (Class|NavigationSystem|GetPathLength (Transformation|GetActorLocation (Components|GetOwner)) (Transformation|GetActorLocation (LocalVariables|GetCurrentActor)))) "Success")
                  ;[1 1 1] Is Previous Path Length not set yet?
                  (if (== (LocalVariables|GetPreviousPathLength) 0.0)
                    ;[1 1 1] Set PreviousPath to CurrentPath
                    (LocalVariables|SetPreviousPathLength (LocalVariables|GetCurrentPathLength)))
                  ;[1 1 1] Is the CurrentPath shorter or equal than PreviousPath?
                  (if (<= (LocalVariables|GetCurrentPathLength) (LocalVariables|GetPreviousPathLength))
                    ;[1 1 1] Set CurrentActor to ClosestActor
                    (LocalVariables|SetClosestActor (LocalVariables|GetCurrentActor)))))))
          (else
            ;[1 1 1] Reset ClosestActor
            (LocalVariables|SetClosestActor 0 :!label _label)))
        (else
          (goto _label)))
      ;[1 1 0] Debug Nearest Found Prey?
      (if (Variables|Setup-Debug|GetDebugNearestPartner)
        (Development|PrintString (Utilities|String|Append "Closest Partner: " (Utilities|GetDisplayName (LocalVariables|GetClosestActor)))))
      (Utilities|IsValid (LocalVariables|GetClosestActor)
        (:Is%20Valid
          ;[1 1 1] Set ClosestActor to NearbyPartner in the Owner
          (bind _asbp_ground_animal_base (Utilities|Casting|CastToBP_GroundAnimalBase (Components|GetOwner)))
          (Variables|/Game/AnimalBehaviorKit/Blueprints/Characters/Animals/GroundAnimals/BP_GroundAnimalBase.BP_GroundAnimalBase_C|SetNearbyPartner _asbp_ground_animal_base (LocalVariables|GetClosestActor))
          ;[1 1 1] Set Owner's Biggest Need to 'Breed'
          (Variables|/Game/AnimalBehaviorKit/Blueprints/Characters/Animals/GroundAnimals/BP_GroundAnimalBase.BP_GroundAnimalBase_C|SetBiggestNeed _asbp_ground_animal_base "NewEnumerator2")
          ;[1 1 1] Set WantsToBreed to True
          (Variables|/Game/AnimalBehaviorKit/Blueprints/Characters/Animals/GroundAnimals/BP_GroundAnimalBase.BP_GroundAnimalBase_C|SetWantsToBreed _asbp_ground_animal_base true))))))

(fn FnSetAttributes
  (params (Actor :type BP%20Ground%20Animal%20Base%20Object%20Reference))
  (LocalVariables|SetlActor Actor)
  ;[1 1 1] Check for Authority
  (if (Default|FnGetAuthority (Variables|Default|GetOwner))
    (Variables|/Game/AnimalBehaviorKit/Blueprints/Characters/Animals/GroundAnimals/BP_GroundAnimalBase.BP_GroundAnimalBase_C|SetRoamBehavior (LocalVariables|GetlActor) (Variables|Default|GetoRoamBehavior))
    (Variables|/Game/AnimalBehaviorKit/Blueprints/Characters/Animals/GroundAnimals/BP_GroundAnimalBase.BP_GroundAnimalBase_C|SetEngageBehavior (LocalVariables|GetlActor) (Variables|Default|GetoEngageBehavior))
    (Variables|/Game/AnimalBehaviorKit/Blueprints/Characters/Animals/GroundAnimals/BP_GroundAnimalBase.BP_GroundAnimalBase_C|SetBehavior_FollowPath (LocalVariables|GetlActor) (Variables|/Game/AnimalBehaviorKit/Blueprints/Characters/Animals/GroundAnimals/BP_GroundAnimalBase.BP_GroundAnimalBase_C|GetBehavior_FollowPath (Variables|Default|GetOwner)))
    (Variables|/Game/AnimalBehaviorKit/Blueprints/Characters/Animals/GroundAnimals/BP_GroundAnimalBase.BP_GroundAnimalBase_C|SetBehavior_Location (LocalVariables|GetlActor) (Variables|/Game/AnimalBehaviorKit/Blueprints/Characters/Animals/GroundAnimals/BP_GroundAnimalBase.BP_GroundAnimalBase_C|GetBehavior_Location (Variables|Default|GetOwner)))
    (Variables|/Game/AnimalBehaviorKit/Blueprints/Characters/Animals/GroundAnimals/BP_GroundAnimalBase.BP_GroundAnimalBase_C|SetBehavior_POI (LocalVariables|GetlActor) (Variables|/Game/AnimalBehaviorKit/Blueprints/Characters/Animals/GroundAnimals/BP_GroundAnimalBase.BP_GroundAnimalBase_C|GetBehavior_POI (Variables|Default|GetOwner)))))

(fn FnGetSpawnLocation
  (bind _returnvalue (Math|Random|RandomUnitVector))
  (return (+ (Transformation|GetActorLocation (Components|GetOwner)) (Math|Vector|MakeVector (* (Variables|Setup-Breeding|GetSpawnRange) (.x _returnvalue)) (* (Variables|Setup-Breeding|GetSpawnRange) (.y _returnvalue)) (.z (Transformation|GetActorLocation (Components|GetOwner)))))))

(event Custom|EventBreeding
  (params (Partner? :type Boolean))
  (bind _owner (Variables|Default|GetOwner))
  (bind _owner_2 (Variables|Default|GetOwner))
  (bind _minmaxoffspring (Variables|Setup-Breeding|GetMinMaxOffspring))
  (bind _charactermovement (Variables|/Script/Engine.Character|GetCharacterMovement _owner))
  (bind _charactermovement_2 (Variables|/Script/Engine.Character|GetCharacterMovement _owner_2))
  (if (not Partner?)
    ;[1 1 1] Check that Owner is valid
    (Utilities|IsValid (Variables|Default|GetOwner)
      (:Is%20Valid
        ;[1 1 1] Check that Owner is NOT Breeding already
        (if (not (Variables|/Game/AnimalBehaviorKit/Blueprints/Characters/Animals/BP_AnimalBase.BP_AnimalBase_C|GetBreeding (Variables|Default|GetOwner)))
          ;[1 1 1] Set state to Breeding
          (Variables|/Game/AnimalBehaviorKit/Blueprints/Characters/Animals/BP_AnimalBase.BP_AnimalBase_C|SetBreeding (Variables|Default|GetOwner) true)
          ;[1 1 1] Make sure Owner wants to breed
          (if (Variables|/Game/AnimalBehaviorKit/Blueprints/Characters/Animals/GroundAnimals/BP_GroundAnimalBase.BP_GroundAnimalBase_C|GetWantsToBreed (Variables|Default|GetOwner))
            ;[1 1 1] Reset WantsToBreed
            (Variables|/Game/AnimalBehaviorKit/Blueprints/Characters/Animals/GroundAnimals/BP_GroundAnimalBase.BP_GroundAnimalBase_C|SetWantsToBreed (Variables|Default|GetOwner) false))
          ;[1 1 1] Save Roam Behavior, Engage Behavior and Additional Tags to inherit to Offspring
          (Variables|Default|SetoRoamBehavior (Variables|/Game/AnimalBehaviorKit/Blueprints/Characters/Animals/GroundAnimals/BP_GroundAnimalBase.BP_GroundAnimalBase_C|GetRoamBehavior (Variables|Default|GetOwner)))
          (Variables|Default|SetoEngageBehavior (Variables|/Game/AnimalBehaviorKit/Blueprints/Characters/Animals/GroundAnimals/BP_GroundAnimalBase.BP_GroundAnimalBase_C|GetEngageBehavior (Variables|Default|GetOwner)))
          (Variables|Default|SetAdditionalTags (Variables|/Game/AnimalBehaviorKit/Blueprints/Characters/Animals/BP_AnimalBase.BP_AnimalBase_C|GetAdditionalTags (Variables|Default|GetOwner)))
          ;[1 1 1] Make animal stay in place while breeding
          (Variables|/Game/AnimalBehaviorKit/Blueprints/Characters/Animals/GroundAnimals/BP_GroundAnimalBase.BP_GroundAnimalBase_C|SetBiggestNeed (Variables|Default|GetOwner) "NewEnumerator3")
          (Variables|/Game/AnimalBehaviorKit/Blueprints/Characters/Animals/GroundAnimals/BP_GroundAnimalBase.BP_GroundAnimalBase_C|SetRoamBehavior (Variables|Default|GetOwner) "NewEnumerator4")
          ;[1 1 1] Stop movement immediately
          (Variables|Default|SetoWalkSpeed (Variables|/Script/Engine.CharacterMovementComponent|GetMaxWalkSpeed _charactermovement))
          (Variables|/Script/Engine.CharacterMovementComponent|SetMaxWalkSpeed _charactermovement 0.0)
          (if (Variables|Setup-Breeding|GetDisplayParticles)
            ;[1 1 1] Check that no Hearts emitter is spawned
            (if (not (Variables|Default|GetSpawnedHearts))
              (CallFunction|EventDisplayHearts)
              (Variables|Default|SetSpawnedHearts true)))
          ;[1 1 1] Fire custom event
          (Default|BreedingStart (Variables|Default|GetOwner) true)
          ;[1 1 1] Wait BreedingTimer seconds
          (Utilities|FlowControl|RetriggerableDelay (Variables|Setup-Breeding|GetBreedingTimer))
          ;[1 1 1] Fire custom event
          (Default|BreedingEnd (Variables|Default|GetOwner) true)
          (Utilities|IsValid (Variables|Default|GetEmitterRef)
            (:Is%20Valid
              (CallFunction|EventDestroyHearts))
            (:Is%20Not%20Valid
              _))
          ;[1 1 1] Reset Hearts Ref
          (Variables|Default|SetEmitterRef 0)
          (Variables|Default|SetSpawnedHearts false)
          ;[1 1 1] Check animal is NOT engaged
          (if (not (Variables|/Game/AnimalBehaviorKit/Blueprints/Characters/Animals/BP_AnimalBase.BP_AnimalBase_C|GetEngaged (Variables|Default|GetOwner)))
            ;[1 1 1] Spawn random offspring?
            (Variables|Default|SetNumOffspring (Math|Integer|Clamp(Integer) (- (Math|Random|RandomIntegerinRange (Math|Float|Truncate (.x _minmaxoffspring)) (Math|Float|Truncate (.y _minmaxoffspring))) 1) 0 99))
            (for _index (range 0 (Variables|Default|GetNumOffspring))
              ;[1 1 1] Get random Bool to represent sex
              (if (Math|Random|RandomBool)
                ;[1 1 1] Spawn male animal
                (bind _returnvalue (Game|SpawnActorfromClass (Variables|Setup-Breeding|GetMaleClass) (Math|Transform|MakeTransform (CallFunction|FnGetSpawnLocation) (Transformation|GetActorRotation (Variables|Default|GetOwner)) "1,1,1") "AdjustIfPossibleButAlwaysSpawn" 0 0))
                (Variables|Default|SetMaleOffspring _returnvalue)
                (Utilities|FlowControl|Sequence
                  (:then_0
                    (if (Variables|Setup-Breeding|GetInheritBehaviors?)
                      (bind _asbp_ground_animal_base (Utilities|Casting|CastToBP_GroundAnimalBase (Variables|Default|GetMaleOffspring)))
                      ;[1 1 1] Set Roam and Engage Behaviors on offspring
                      (CallFunction|FnSetAttributes _asbp_ground_animal_base)
                      ;[1 1 1] Set all Additional Tags as actor tags for the offspring
                      (for _array_element 0
                        (Utilities|Array|Add (Variables|/Script/Engine.Actor|GetTags (Variables|Default|GetMaleOffspring)) _array_element))))
                  (:then_1
                    (if (Variables|Setup-Breeding|GetOffspringFollowsParent?)
                      (bind _asbp_ground_animal_base_2 (Utilities|Casting|CastToBP_GroundAnimalBase (Variables|Default|GetMaleOffspring)))
                      (Utilities|IsValid (Actor|GetComponentbyClass _asbp_ground_animal_base_2 "/Game/AnimalBehaviorKit/Blueprints/AI/Components/GroundAnimals/BP_Comp_GrowOld.BP_Comp_GrowOld_C")
                        (:Is%20Valid
                          ;[1 1 1] Set owner as child's parent
                          (Variables|/Game/AnimalBehaviorKit/Blueprints/AI/Components/GroundAnimals/BP_Comp_GrowOld.BP_Comp_GrowOld_C|SetParentRef (Actor|GetComponentbyClass _asbp_ground_animal_base_2 "/Game/AnimalBehaviorKit/Blueprints/AI/Components/GroundAnimals/BP_Comp_GrowOld.BP_Comp_GrowOld_C") (Variables|Default|GetOwner))
                          (Default|FnFollowParent (Actor|GetComponentbyClass _asbp_ground_animal_base_2 "/Game/AnimalBehaviorKit/Blueprints/AI/Components/GroundAnimals/BP_Comp_GrowOld.BP_Comp_GrowOld_C")))))))
                (else
                  ;[1 1 1] Spawn female animal
                  (bind _returnvalue_2 (Game|SpawnActorfromClass (Variables|Setup-Breeding|GetFemaleClass) (Math|Transform|MakeTransform (CallFunction|FnGetSpawnLocation) (Transformation|GetActorRotation (Variables|Default|GetOwner)) "1,1,1") "AdjustIfPossibleButAlwaysSpawn" 0 0))
                  (Variables|Default|SetFemaleOffspring _returnvalue_2)
                  (Utilities|FlowControl|Sequence
                    (:then_0
                      (if (Variables|Setup-Breeding|GetInheritBehaviors?)
                        (bind _asbp_ground_animal_base_3 (Utilities|Casting|CastToBP_GroundAnimalBase (Variables|Default|GetFemaleOffspring)))
                        ;[1 1 1] Set Roam and Engage Behaviors on offspring
                        (CallFunction|FnSetAttributes _asbp_ground_animal_base_3)
                        ;[1 1 1] Set all Additional Tags as actor tags for the offspring
                        (for _array_element_2 0
                          (Utilities|Array|Add (Variables|/Script/Engine.Actor|GetTags (Variables|Default|GetFemaleOffspring)) _array_element_2))))
                    (:then_1
                      (if (Variables|Setup-Breeding|GetOffspringFollowsParent?)
                        (bind _asbp_ground_animal_base_4 (Utilities|Casting|CastToBP_GroundAnimalBase (Variables|Default|GetFemaleOffspring)))
                        (Utilities|IsValid (Actor|GetComponentbyClass _asbp_ground_animal_base_4 "/Game/AnimalBehaviorKit/Blueprints/AI/Components/GroundAnimals/BP_Comp_GrowOld.BP_Comp_GrowOld_C")
                          (:Is%20Valid
                            ;[1 1 1] Set owner as child's parent
                            (Variables|/Game/AnimalBehaviorKit/Blueprints/AI/Components/GroundAnimals/BP_Comp_GrowOld.BP_Comp_GrowOld_C|SetParentRef (Actor|GetComponentbyClass _asbp_ground_animal_base_4 "/Game/AnimalBehaviorKit/Blueprints/AI/Components/GroundAnimals/BP_Comp_GrowOld.BP_Comp_GrowOld_C") (Variables|Default|GetOwner))
                            (Default|FnFollowParent (Actor|GetComponentbyClass _asbp_ground_animal_base_4 "/Game/AnimalBehaviorKit/Blueprints/AI/Components/GroundAnimals/BP_Comp_GrowOld.BP_Comp_GrowOld_C"))))))))))
            ;[1 1 1] Reset state Breeding
            (Variables|/Game/AnimalBehaviorKit/Blueprints/Characters/Animals/BP_AnimalBase.BP_AnimalBase_C|SetBreeding (Variables|Default|GetOwner) false)
            ;[1 1 1] Set Roam Behavior
            (Default|FnSetRoamBehavior (Variables|Default|GetOwner))
            (else
              ;[1 1 1] Reset state Breeding
              (Variables|/Game/AnimalBehaviorKit/Blueprints/Characters/Animals/BP_AnimalBase.BP_AnimalBase_C|SetBreeding (Variables|Default|GetOwner) false)
              ;[1 1 1] Set Roam Behavior
              (Default|FnSetRoamBehavior (Variables|Default|GetOwner))
              ;[1 1 1] Restore movement speed
              (Variables|/Script/Engine.CharacterMovementComponent|SetMaxWalkSpeed (Variables|/Script/Engine.Character|GetCharacterMovement (Variables|Default|GetOwner)) (Variables|Default|GetoWalkSpeed)))))))
    (else
      ;[1 1 1] Check that Owner is valid
      (Utilities|IsValid (Variables|Default|GetOwner)
        (:Is%20Valid
          ;[1 1 1] Check that Owner is NOT Breeding already
          (if (not (Variables|/Game/AnimalBehaviorKit/Blueprints/Characters/Animals/BP_AnimalBase.BP_AnimalBase_C|GetBreeding (Variables|Default|GetOwner)))
            ;[1 1 1] Set State to Breeding
            (Variables|/Game/AnimalBehaviorKit/Blueprints/Characters/Animals/BP_AnimalBase.BP_AnimalBase_C|SetBreeding (Variables|Default|GetOwner) true)
            ;[1 1 1] Make sure Owner wants to Breed
            (if (Variables|/Game/AnimalBehaviorKit/Blueprints/Characters/Animals/GroundAnimals/BP_GroundAnimalBase.BP_GroundAnimalBase_C|GetWantsToBreed (Variables|Default|GetOwner))
              ;[1 1 1] Reset WantsToBreed
              (Variables|/Game/AnimalBehaviorKit/Blueprints/Characters/Animals/GroundAnimals/BP_GroundAnimalBase.BP_GroundAnimalBase_C|SetWantsToBreed (Variables|Default|GetOwner) false))
            ;[1 1 1] Make animal stay in place while breeding
            (Variables|/Game/AnimalBehaviorKit/Blueprints/Characters/Animals/GroundAnimals/BP_GroundAnimalBase.BP_GroundAnimalBase_C|SetBiggestNeed (Variables|Default|GetOwner) "NewEnumerator3")
            (Variables|/Game/AnimalBehaviorKit/Blueprints/Characters/Animals/GroundAnimals/BP_GroundAnimalBase.BP_GroundAnimalBase_C|SetRoamBehavior (Variables|Default|GetOwner) "NewEnumerator4")
            ;[1 1 1] Stop movement immediately
            (Variables|Default|SetoWalkSpeed (Variables|/Script/Engine.CharacterMovementComponent|GetMaxWalkSpeed _charactermovement_2))
            (Variables|/Script/Engine.CharacterMovementComponent|SetMaxWalkSpeed _charactermovement_2 0.0)
            (if (Variables|Setup-Breeding|GetDisplayParticles)
              ;[1 1 1] Check that no Hearts emitter is spawned
              (if (not (Variables|Default|GetSpawnedHearts))
                (CallFunction|EventDisplayHearts)
                (Variables|Default|SetSpawnedHearts true)))
            ;[1 1 1] Fire custom event
            (Default|BreedingStart (Variables|Default|GetOwner) false)
            ;[1 1 1] Wait BreedingTimer seconds
            (Utilities|FlowControl|RetriggerableDelay (Variables|Setup-Breeding|GetBreedingTimer))
            ;[1 1 1] Fire custom event
            (Default|BreedingEnd (Variables|Default|GetOwner) false)
            (Utilities|IsValid (Variables|Default|GetEmitterRef)
              (:Is%20Valid
                (CallFunction|EventDestroyHearts))
              (:Is%20Not%20Valid
                _))
            ;[1 1 1] Reset Hearts Ref
            (Variables|Default|SetEmitterRef 0)
            ;[1 1 1] Reset state Breeding
            (Variables|/Game/AnimalBehaviorKit/Blueprints/Characters/Animals/BP_AnimalBase.BP_AnimalBase_C|SetBreeding (Variables|Default|GetOwner) false)
            (Variables|Default|SetSpawnedHearts false)
            ;[1 1 1] Set Roam Behavior
            (Default|FnSetRoamBehavior (Variables|Default|GetOwner))
            ;[1 1 1] Restore movement speed
            (Variables|/Script/Engine.CharacterMovementComponent|SetMaxWalkSpeed (Variables|/Script/Engine.Character|GetCharacterMovement (Variables|Default|GetOwner)) (Variables|Default|GetoWalkSpeed))))))))

(event Custom|EventDestroyHearts
  ;[1 1 1] Destroy Hearts particles
  (Utilities|IsValid (Variables|Default|GetEmitterRef)
    (:Is%20Valid
      (Components|DestroyComponent (Variables|Default|GetEmitterRef)))))

(event Custom|EventDisplayHearts
  ;[1 1 1] Spawn Hearts particle system
  (bind _returnvalue (Effects|SpawnEmitterAttached (Variables|Setup-Breeding|GetBreedingParticles) (Variables|/Script/Engine.Character|GetCapsuleComponent (Variables|Default|GetOwner)) "None" (Variables|Setup-Breeding|GetParticlesLocation)))
  (Variables|Default|SetEmitterRef _returnvalue))

(event Custom|EventSearchForPartner
  (bind _returnvalue (Utilities|Time|SetTimerbyEvent (delegate Custom|EventSearchForPartner) (Variables|Setup-LookForPartner|GetLookForPartnerFrequency) true))
  (Variables|Default|SetPartnerEventHandler _returnvalue)
  (CallFunction|FnLookforPartner))