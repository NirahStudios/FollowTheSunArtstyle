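; Actor component that gives a ground animal a limited lifespan, triggering its death from natural causes.
; On BeginPlay it caches the BP_GroundAnimalBase owner and, if active and with authority, picks a random lifetime between minimum and maximum values.
; A one-second looping timer, set again on each tick, increments a counter until it exceeds that lifetime, then calls EventDead on the animal without clearing the timer.
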(event Custom|EventNaturalDeath
  (if (Default|FnGetAuthority (Variables|Default|GetGroundAnimal))
    ;[1 1 1] Wait TimeToLive seconds
    (Variables|Default|SetRandomTime (Math|Random|RandomFloatinRange (Variables|Setup|GetMinTimeToLive) (Variables|Setup|GetMaxTimeToLive)))
    (CallFunction|EventDie)))

(event Custom|EventDie
  (bind _returnvalue (Utilities|Time|SetTimerbyEvent (delegate Custom|EventDie) 1.0 true))
  (Variables|Default|SetDeathTimerHandler _returnvalue)
  ;[1 1 1] Check if count is less than or equal to random time
  (if (<= (Variables|Default|GetTimerCount) (Variables|Default|GetRandomTime))
    ;[1 1 1] Increase count by 1
    (Math|Float|IncrementFloat (Variables|Default|GetTimerCount))
    (else
      ;[1 1 1] Call EventDead on Ground Animal
      (Default|EventDead (Variables|Default|GetGroundAnimal)))))

(event EventBeginPlay
  ;[1 1 1] Save owner reference
  (bind _asbp_ground_animal_base (Utilities|Casting|CastToBP_GroundAnimalBase (Components|GetOwner)))
  (Variables|Default|SetGroundAnimal _asbp_ground_animal_base)
  ;[1 1 1] Check if component is active
  (if (Variables|Setup|GetActive)
    ;[1 1 1] Check for Authority
    (if (Default|FnGetAuthority (Variables|Default|GetGroundAnimal))
      (CallFunction|EventNaturalDeath))))