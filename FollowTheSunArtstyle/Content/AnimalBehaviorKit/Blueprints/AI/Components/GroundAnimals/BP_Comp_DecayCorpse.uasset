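; Actor component for ground animals that replaces the animal with a decaying corpse actor.
; On BeginPlay it caches the owning BP_GroundAnimalBase.
; EventSpawnCorpse spawns the configured corpse class at the animal's location and rotation, then passes it the decay states, despawn setting and transform.
; It then starts the corpse's server decay event and destroys the animal actor.
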(event EventBeginPlay
  ;[1 1 1] Save owner reference
  (bind _asbp_ground_animal_base (Utilities|Casting|CastToBP_GroundAnimalBase (Components|GetOwner)))
  (Variables|Default|SetGroundAnimal _asbp_ground_animal_base))

(event Custom|EventSpawnCorpse
  (Utilities|FlowControl|Sequence
    (:then_0
      ;[1 1 1] Set Spawn Transform
      (Variables|Default|SetActorTransform (Transformation|GetActorTransform (Variables|Default|GetGroundAnimal)))
      ;[1 1 1] Spawn animal corpse
      (bind _returnvalue (Game|SpawnActorfromClass (Variables|Setup|GetAnimalCorpse) (Math|Transform|MakeTransform (.location (Variables|Default|GetActorTransform)) (.rotation (Variables|Default|GetActorTransform)) "1,1,1") "AdjustIfPossibleButAlwaysSpawn" 0 0))
      (Variables|Default|SetSpawnedCorpse _returnvalue)
      ;[1 1 1] Set the correct parameters
      (Variables|/Game/AnimalBehaviorKit/Blueprints/AI/Actors/Ground_AI/DecaySystem/BP_AnimalCorpseBase.BP_AnimalCorpseBase_C|SetDecayStates (Variables|Default|GetSpawnedCorpse) (Variables|Setup|GetDecayStates))
      (Variables|/Game/AnimalBehaviorKit/Blueprints/AI/Actors/Ground_AI/DecaySystem/BP_AnimalCorpseBase.BP_AnimalCorpseBase_C|SetDespawnAtEnd? (Variables|Default|GetSpawnedCorpse) (Variables|Setup|GetDespawnAtEnd?))
      (Variables|/Game/AnimalBehaviorKit/Blueprints/AI/Actors/Ground_AI/DecaySystem/BP_AnimalCorpseBase.BP_AnimalCorpseBase_C|SetActorTransform (Variables|Default|GetSpawnedCorpse) (Variables|Default|GetActorTransform))
      ;[1 1 1] Start decay process
      (Default|EventStartDecayServer (Variables|Default|GetSpawnedCorpse)))
    (:then_1
      ;[1 1 1] Destroy animal actor
      (Actor|DestroyActor (Variables|Default|GetGroundAnimal)))))