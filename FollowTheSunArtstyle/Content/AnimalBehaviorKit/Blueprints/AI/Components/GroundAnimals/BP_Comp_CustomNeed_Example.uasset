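; Example custom-need component for Animal Behavior Kit ground animals that sends the animal to the player.
; On authority, the need event sets the blackboard's BiggestNeed to a natural-behavior enum value and issues AIMoveTo toward player 0's location.
; A looping timer re-triggers that same event to keep the destination updated.
; On arrival, it pauses the timer, waits the need's TimeAtLocation, then calls EventFinishedNeed to reset the need.
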(event EventBeginPlay
  (|CallParentFunction) ; This node is disabled and will not be called.\nDrag off pins to build functionality.
)

(event EventEventNeedCustomCode
  ;[1 1 1] Check for Authority
  (if (Default|FnGetAuthority (Variables|Default|GetGroundAnimal))
    (bind _returnvalue (Utilities|Time|SetTimerbyEvent (delegate EventEventNeedCustomCode) 0.1 true))
    (Variables|Default|SetTimerHandler _returnvalue)
    ;[1 1 1] Set BT BiggestNeed value to Custom Need
    (AI|Components|Blackboard|SetValueasEnum (Variables|/Script/AIModule.AIController|GetBlackboard (AI|GetAIController (Variables|Default|GetGroundAnimal))) (Variables|Default|GetBiggestNeed) (Utilities|Enum|LiteralenumBP_Enum_GroundNaturalBehaviors "NewEnumerator6"))
    ;[0 1 0] CUSTOM CODE HERE! | Example - Follow Player around
    (AI|AIMoveTo (Variables|Default|GetGroundAnimal) (Transformation|GetActorLocation (Game|Player|GetPlayerPawn 0)) 0 (Variables|Default|GetMovementAcceptanceRadius) true
      (:then
        (Development|PrintString "Going towards Player!" true true "(R=0.000000,G=0.660000,B=1.000000,A=1.000000)" 0.1))
      (:OnSuccess
        (Utilities|Time|PauseTimerbyHandle (Variables|Default|GetTimerHandler))
        ;;[1 1 1] Wait TimeAtLocation seconds
        (Utilities|FlowControl|Delay (Utilities|Struct|BreakBP_Struct_NeedCustom (Variables|Default|GetNeedDetails)))
        ;[1 1 1] Reset Custom Need
        (CallFunction|EventFinishedNeed)))))