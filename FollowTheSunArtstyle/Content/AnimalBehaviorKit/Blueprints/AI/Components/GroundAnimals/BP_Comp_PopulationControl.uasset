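; Component on ground animals that registers its owner with a level's BP_PopulationControl actor for population tracking.
; On BeginPlay, if active and the animal has authority, it finds that manager either as the first actor of its class or by tag, per ReferenceMode.
; After a short delay it registers the animal's reference, species and sex once, or prints an on-screen error if no manager was found.
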(event EventBeginPlay
  (if (Variables|Setup|GetActive)
    ;[1 1 1] Save owner reference
    (bind _asbp_ground_animal_base (Utilities|Casting|CastToBP_GroundAnimalBase (Components|GetOwner)))
    (Variables|Default|SetGroundAnimal _asbp_ground_animal_base)
    ;[1 1 1] Check for Authority
    (if (Default|FnGetAuthority (Variables|Default|GetGroundAnimal))
      ;[1 1 1] Get Population Control reference
      (CallFunction|FnGetPopulationControlRef)
      (Utilities|FlowControl|Delay 0.1)
      ;[1 1 1] Check if we have a valid reference to Population Control
      (Utilities|IsValid (Variables|Setup|GetPopulationControlReference)
        (:Is%20Valid
          ;[1 1 1] Register animal with Population Control
          (CallFunction|FnRegisterAnimal))
        (:Is%20Not%20Valid
          (|DISPLAYERRORMESSAGE))))))

(fn FnRegisterAnimal
  (bind _groundanimal (Variables|Default|GetGroundAnimal))
  (bind _animal_details (Variables|/Game/AnimalBehaviorKit/Blueprints/Characters/Animals/BP_AnimalBase.BP_AnimalBase_C|GetAnimal_Details _groundanimal))
  (bind (_sex _species) (Utilities|Struct|BreakBP_Struct_AnimalBase_AnimalDetail _animal_details))
  (Utilities|FlowControl|DoOnce false
    (:Completed
      ;[1 1 1] Add Owner details to the AnimalDetails Array in Population Control
      (Default|FnRegisterAnimal (Variables|Setup|GetPopulationControlReference) (Utilities|Struct|MakeBP_Struct_Population_AnimalDetails _groundanimal _species _sex)))))

(fn FnGetPopulationControlRef
  (switch Utilities|FlowControl|Switch|SwitchonBP_Enum_ReferenceModePopulation (Variables|Setup|GetReferenceMode)
    (:NewEnumerator0
      (bind _outactors (Actor|GetAllActorsOfClass "/Game/AnimalBehaviorKit/Blueprints/AI/Population_Control/BP_PopulationControl.BP_PopulationControl_C"))
      ;[1 1 1] Check that PopulationControl is found in level
      (if (> (Utilities|Array|Length _outactors) 0)
        ;[1 1 1] Set PopulationControl reference
        (Variables|Setup|SetPopulationControlReference (Utilities|Array|Get(acopy) _outactors))))
    (:NewEnumerator1
      (bind _outactors_2 (Actor|GetAllActorswithTag (Variables|Setup|GetPopulationControlTag)))
      ;[1 1 1] Check that PopulationControl is found in level
      (if (> (Utilities|Array|Length _outactors_2) 0)
        ;[1 1 1] Set PopulationControl reference
        (bind _asbp_population_control (Utilities|Casting|CastToBP_PopulationControl (Utilities|Array|Get(acopy) _outactors_2)))
        (Variables|Setup|SetPopulationControlReference _asbp_population_control)))))