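; Actor component that registers a ground animal with a group and can mark it as the leader.
; On BeginPlay, an active component registers by group mode: manually with an assigned GroupManager (authority-only, after a short delay), or with an auto-group manager found by class or tag, passing sex and species.
; In manual mode, a leader sets CheckLeadership, whose RepNotify prefixes "(L)" to the animal's HUD name.
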(event EventBeginPlay
  (Utilities|FlowControl|Sequence
    (:then_0
      (Components|GetOwner))
    (:then_1
      (|REGISTERWITHGROUP))))

(fn OnRepCheckLeadership
  (CallFunction|FnSetLeaderName))

(fn FnSetLeaderName
  ;[1 1 1] Is this the Group Leader?
  (if (Variables|Setup|GetGroupLeader?)
    (bind _asbp_ground_animal_base (Utilities|Casting|CastToBP_GroundAnimalBase (Components|GetOwner)))
    (LocalVariables|SetAnimal _asbp_ground_animal_base)
    (Utilities|FlowControl|Sequence
      (:then_0
        ;[1 1 1] Change animal name in HUD to include 'L' for leader
        (bind _aswbp_ai_hud (Utilities|Casting|CastToWBP_AI_HUD (UserInterface|GetUserWidgetObject (Variables|/Game/AnimalBehaviorKit/Blueprints/Characters/Animals/BP_AnimalBase.BP_AnimalBase_C|GetWBP_HUD (LocalVariables|GetAnimal)))))
        (Default|FnSetName _aswbp_ai_hud (Utilities|Text|ToText(String) (Utilities|String|Append "(L) " (Utilities|String|ToString(Text) (Utilities|Struct|BreakBP_Struct_AnimalBase_AnimalDetail (Variables|/Game/AnimalBehaviorKit/Blueprints/Characters/Animals/BP_AnimalBase.BP_AnimalBase_C|GetAnimal_Details (LocalVariables|GetAnimal))))))))
      (:then_1
        ;[1 1 1] Change animal name in HUD to include 'L' for leader
        (bind _aswbp_ats_ai_hud (Utilities|Casting|CastToWBP_ATS_AI_HUD (UserInterface|GetUserWidgetObject (Variables|/Game/AnimalBehaviorKit/Blueprints/Characters/Animals/BP_AnimalBase.BP_AnimalBase_C|GetWBP_HUD (LocalVariables|GetAnimal)))))
        (Default|FnSetName _aswbp_ats_ai_hud (Utilities|Text|ToText(String) (Utilities|String|Append "(L) " (Utilities|String|ToString(Text) (Utilities|Struct|BreakBP_Struct_AnimalBase_AnimalDetail (Variables|/Game/AnimalBehaviorKit/Blueprints/Characters/Animals/BP_AnimalBase.BP_AnimalBase_C|GetAnimal_Details (LocalVariables|GetAnimal)))))))))))

(event Custom|EventRegisterWithGroup
  ;[1 1 1] Check for Authority
  (if (Default|FnGetAuthority (Variables|Default|GetOwner))
    (Utilities|FlowControl|Delay 0.2)
    (Utilities|IsValid (Variables|Setup|GetGroupManager)
      (:Is%20Valid
        ;[1 1 1] Add self to group array
        (Utilities|Array|AddUnique (Variables|/Game/AnimalBehaviorKit/Blueprints/AI/Actors/Ground_AI/Group/BP_GroupManager.BP_GroupManager_C|GetGroup (Variables|Setup|GetGroupManager)) (Variables|Default|GetOwner))
        ;[1 1 1] Is this the Herd Leader?
        (if (Variables|Setup|GetGroupLeader?)
          ;[1 1 1] Set self as Group Leader
          (Variables|/Game/AnimalBehaviorKit/Blueprints/AI/Actors/Ground_AI/Group/BP_GroupManager.BP_GroupManager_C|SetGroupLeader (Variables|Setup|GetGroupManager) (Variables|Default|GetOwner))
          (Variables|Default|SetCheckLeadership true)))
      (:Is%20Not%20Valid
        ;[1 1 1] Display error message
        (Development|PrintString (Utilities|String|Append (Utilities|GetDisplayName (Variables|Default|GetOwner)) ": Comp_Group:  MIssing Group Manager reference!") true true "(R=1.000000,G=0.000000,B=0.000000,A=1.000000)" 5.0)))))

(event Custom|EventRegisterWithAutoGroupTag
  (bind _owner (Variables|Default|GetOwner))
  (bind _animal_details (Variables|/Game/AnimalBehaviorKit/Blueprints/Characters/Animals/BP_AnimalBase.BP_AnimalBase_C|GetAnimal_Details _owner))
  (bind (_sex _species) (Utilities|Struct|BreakBP_Struct_AnimalBase_AnimalDetail _animal_details))
  (bind _outactors (Actor|GetAllActorswithTag (Variables|Setup|GetAutoGroupManagerTag)))
  (if (Utilities|Array|IsValidIndex _outactors)
    ;[1 1 1] Register animal with BP_AutoGrouping
    (bind _asbp_auto_group_manager (Utilities|Casting|CastToBP_AutoGroupManager (Utilities|Array|Get(acopy) _outactors)))
    (Default|FnRegisterAnimal _asbp_auto_group_manager _owner _sex _species)))

(event Custom|EventRegisterWithAutoGroup
  (bind _owner (Variables|Default|GetOwner))
  (bind _animal_details (Variables|/Game/AnimalBehaviorKit/Blueprints/Characters/Animals/BP_AnimalBase.BP_AnimalBase_C|GetAnimal_Details _owner))
  (bind (_sex _species) (Utilities|Struct|BreakBP_Struct_AnimalBase_AnimalDetail _animal_details))
  (bind _outactors (Actor|GetAllActorsOfClass "/Game/AnimalBehaviorKit/Blueprints/AI/Actors/Ground_AI/Group/BP_AutoGroupManager.BP_AutoGroupManager_C"))
  (if (Utilities|Array|IsValidIndex _outactors)
    ;[1 1 1] Register animal with BP_AutoGrouping
    (Default|FnRegisterAnimal (Utilities|Array|Get(acopy) _outactors) _owner _sex _species)))