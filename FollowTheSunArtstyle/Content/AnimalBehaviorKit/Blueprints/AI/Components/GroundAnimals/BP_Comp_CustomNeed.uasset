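; Ground animal component that adds a configurable custom need, draining on an authority-side timer while awake and optionally killing the animal.
; Below threshold, it sets BiggestNeed and moves the animal to a set actor or runs an event that child Blueprints override.
; Closest-actor mode sphere-traces for a class and picks by navmesh path length.
; Finishing resets the need, restores roaming and applies an engage cooldown; non-lethal needs pause the timer meanwhile.
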(event EventBeginPlay
  ;[1 1 1] Save owner reference
  (bind _asbp_ground_animal_base (Utilities|Casting|CastToBP_GroundAnimalBase (Components|GetOwner)))
  (Variables|Default|SetGroundAnimal _asbp_ground_animal_base)
  ;[1 1 1] Is the Custom Need Active?
  (if (Variables|Setup|GetActive)
    (if (Default|FnGetAuthority (Variables|Default|GetGroundAnimal))
      ;[1 1 1] Set Custom Need Amount
      (|SetHungerandThirstAmounts)
      (CallFunction|EventDetermineNaturalNeed))
    (else
      (Variables|/Game/AnimalBehaviorKit/Blueprints/Characters/Animals/GroundAnimals/BP_GroundAnimalBase.BP_GroundAnimalBase_C|SetBiggestNeed (Variables|Default|GetGroundAnimal) "NewEnumerator3"))))

(fn FnExecuteCustomNeed
  ;[1 1 1] Switch on Custom Need Mode
  (switch Utilities|FlowControl|Switch|SwitchonBP_Enum_CustomNeedModes (Utilities|Struct|BreakBP_Struct_NeedCustom (Variables|Setup|GetNeedDetails))
    (:NewEnumerator0
      (CallFunction|EventNeedSingleActor))
    (:NewEnumerator1
      (CallFunction|EventNeedClosestActor))
    (:NewEnumerator2
      (CallFunction|EventNeedCustomCode))))

(fn FnGetClosestActor
  (bind _groundanimal (Variables|Default|GetGroundAnimal))
  (bind _returnvalue (Transformation|GetActorLocation _groundanimal))
  ;[1 1 1] Do we want to debug melee range?
  (if (Variables|Debug|GetDebugActorSearch)
    ;[1 1 0] Set sphere trace debug mode
    (LocalVariables|SetSphereDebug "ForDuration")
    (else
      (LocalVariables|SetSphereDebug "None")))
  ;[1 1 1] Generate a sphere trace by channel that mimics the Collision_Attack collision sphere
  (bind (_outhits _returnvalue_2) (Collision|MultiSphereTraceForObjects _returnvalue (+ _returnvalue "0, 0,0.010000") (Variables|Setup|GetActorSearchRadius) (Utilities|Array|MakeArray "ObjectTypeQuery3" "ObjectTypeQuery1" "ObjectTypeQuery2" "ObjectTypeQuery7") false 0 (LocalVariables|GetSphereDebug)))
  ;[1 1 1] Did we hit something?
  (if _returnvalue_2
    ;[1 1 1] For each hit actor
    (for _array_element _outhits
      ;[1 1 1] Check that the hit actor is the same class as the Actor Class in the Custom Need Struct
      (if (== (Utilities|Struct|BreakBP_Struct_NeedCustom (Variables|Setup|GetNeedDetails)) (Utilities|GetClass (.HitActor (Collision|BreakHitResult _array_element))))
        ;[1 1 1] Add HitActor to ActorList array
        (Utilities|Array|AddUnique (LocalVariables|GetActorList) (.HitActor (Collision|BreakHitResult _array_element)))))
    ;[1 1 1] Check that the ActorList has at least 1 actor
    (if (> (Utilities|Array|Length (LocalVariables|GetActorList)) 0)
      ;[1 1 1] For each potential actor
      (for _array_element_2 (LocalVariables|GetActorList)
        (LocalVariables|SetCurrentActor _array_element_2)
        ;[1 1 1] Get Path Length for current actor in array
        (LocalVariables|SetCurrentPathLength (.PathLength (Class|NavigationSystem|GetPathLength (Transformation|GetActorLocation (Variables|Default|GetGroundAnimal)) (Transformation|GetActorLocation (LocalVariables|GetCurrentActor)))))
        ;[1 1 1] Check the Nav Mesh path is valid
        (if (Utilities|Enum|Equal(Enum) (.ReturnValue (Class|NavigationSystem|GetPathLength (Transformation|GetActorLocation (Variables|Default|GetGroundAnimal)) (Transformation|GetActorLocation (LocalVariables|GetCurrentActor)))) "Success")
          ;[1 1 1] Is Previous Path Length not set yet?
          (if (== (LocalVariables|GetPreviousPathLength) 0.0)
            ;[1 1 1] Set PreviousPath to CurrentPath
            (LocalVariables|SetPreviousPathLength (LocalVariables|GetCurrentPathLength)))
          ;[1 1 1] Is the CurrentPath shorter or equal than PreviousPath?
          (if (<= (LocalVariables|GetCurrentPathLength) (LocalVariables|GetPreviousPathLength))
            ;[1 1 1] Set CurrentActor to ClosestActor
            (LocalVariables|SetClosestActor (LocalVariables|GetCurrentActor)))))
      ;[1 1 0] Debug Closest Actor?
      (if (Variables|Debug|GetDebugActorSearch)
        (Development|PrintString (Utilities|String|Append "ClosestActor: " (Utilities|GetDisplayName (LocalVariables|GetClosestActor))) true true "(R=0.000000,G=0.660000,B=1.000000,A=1.000000)" 5.0))
      ;[1 1 1] Check ClosestActor is valid
      (Utilities|IsValid (LocalVariables|GetClosestActor)
        (:Is%20Valid
          ;[1 1 1] Return ClosestActor
          (return (LocalVariables|GetClosestActor)))))))

(event Custom|EventDetermineNaturalNeed
  (bind _returnvalue (Utilities|Time|SetTimerbyEvent (delegate Custom|EventDetermineNaturalNeed) (Variables|Setup|GetNeedsTimer) true))
  (Variables|Setup|SetNaturalNeedTimerHandle _returnvalue)
  ;[1 1 1] Only modify needs if AI is Awake
  (if (Variables|/Game/AnimalBehaviorKit/Blueprints/Characters/Animals/BP_AnimalBase.BP_AnimalBase_C|GetAwake (Variables|Default|GetGroundAnimal))
    (Utilities|FlowControl|Sequence
      (:then_0
        (|DECREASENEED))
      (:then_1
        (|ADJUSTBIGGESTNEED))
      (:then_2
        (|DIEFROMNEEDS?)))))

(event Custom|EventFinishedNeed
  ;[1 1 1] Disable engage
  (Variables|/Game/AnimalBehaviorKit/Blueprints/Characters/Animals/GroundAnimals/BP_GroundAnimalBase.BP_GroundAnimalBase_C|SetCanEngage (Variables|Default|GetGroundAnimal) false)
  ;[1 1 1] Reset CurrentHunger
  (Variables|Setup|SetCurrentNeed (Utilities|Struct|BreakBP_Struct_NeedCustom (Variables|Setup|GetNeedDetails)))
  ;[1 1 1] Unpause Needs Timer
  (Utilities|Time|UnpauseTimerbyHandle (Variables|Setup|GetNaturalNeedTimerHandle))
  ;[1 1 1] Reset Engage Behavior
  (Variables|/Game/AnimalBehaviorKit/Blueprints/Characters/Animals/GroundAnimals/BP_GroundAnimalBase.BP_GroundAnimalBase_C|SetEngageBehavior (Variables|Default|GetGroundAnimal) (Variables|/Game/AnimalBehaviorKit/Blueprints/Characters/Animals/GroundAnimals/BP_GroundAnimalBase.BP_GroundAnimalBase_C|GetOriginalEngageBehavior (Variables|Default|GetGroundAnimal)))
  ;[1 1 1] Wait DisengageCD seconds and allow engaging again
  (Utilities|FlowControl|Delay (.DisengageCD (Utilities|Struct|BreakBP_Struct_GroundAnimalBehavior_AnimalDetails_Attack (Variables|/Game/AnimalBehaviorKit/Blueprints/Characters/Animals/GroundAnimals/BP_GroundAnimalBase.BP_GroundAnimalBase_C|GetBehavior_Details_Attack (Variables|Default|GetGroundAnimal)))))
  (Variables|/Game/AnimalBehaviorKit/Blueprints/Characters/Animals/GroundAnimals/BP_GroundAnimalBase.BP_GroundAnimalBase_C|SetCanEngage (Variables|Default|GetGroundAnimal) true)
  ;[1 1 1] Set BT BiggestNeed value to Roam
  (AI|Components|Blackboard|SetValueasEnum (Variables|/Script/AIModule.AIController|GetBlackboard (AI|GetAIController (Variables|Default|GetGroundAnimal))) (Variables|Default|GetBiggestNeed) (Utilities|Enum|LiteralenumBP_Enum_GroundNaturalBehaviors "NewEnumerator3")))

(event Custom|EventNeed_SingleActor
  ;[1 1 1] Check for Authority
  (if (Default|FnGetAuthority (Variables|Default|GetGroundAnimal))
    ;[1 1 1] Set BT BiggestNeed value to Custom Need
    (AI|Components|Blackboard|SetValueasEnum (Variables|/Script/AIModule.AIController|GetBlackboard (AI|GetAIController (Variables|Default|GetGroundAnimal))) (Variables|Default|GetBiggestNeed) (Utilities|Enum|LiteralenumBP_Enum_GroundNaturalBehaviors "NewEnumerator6"))
    ;[1 1 1] Move AI to Actor's location
    (AI|AIMoveTo (Variables|Default|GetGroundAnimal) (Transformation|GetActorLocation (Utilities|Struct|BreakBP_Struct_NeedCustom (Variables|Setup|GetNeedDetails))) 0 (Variables|Setup|GetMovementAcceptanceRadius) true
      (:OnSuccess
        ;[1 1 1] Wait TimeAtLocation seconds
        (Utilities|FlowControl|Delay (Utilities|Struct|BreakBP_Struct_NeedCustom (Variables|Setup|GetNeedDetails)))
        ;[1 1 1] Set next Roaming Behavior
        (Default|FnSetRoamBehavior (Variables|Default|GetGroundAnimal))
        ;[1 1 1] Reset Custom Need
        (CallFunction|EventFinishedNeed)))))

(event Custom|EventNeed_ClosestActor
  ;[1 1 1] Check for Authority
  (if (Default|FnGetAuthority (Variables|Default|GetGroundAnimal))
    ;[1 1 1] Set BT BiggestNeed value to Custom Need
    (AI|Components|Blackboard|SetValueasEnum (Variables|/Script/AIModule.AIController|GetBlackboard (AI|GetAIController (Variables|Default|GetGroundAnimal))) (Variables|Default|GetBiggestNeed) (Utilities|Enum|LiteralenumBP_Enum_GroundNaturalBehaviors "NewEnumerator6"))
    (bind _nearbyactor (CallFunction|FnGetClosestActor))
    (Utilities|IsValid _nearbyactor
      (:Is%20Valid
        ;[1 1 1] Move AI to Actor's location
        (AI|AIMoveTo (Variables|Default|GetGroundAnimal) (Transformation|GetActorLocation _nearbyactor) 0 (Variables|Setup|GetMovementAcceptanceRadius) true
          (:OnSuccess
            ;[1 1 1] Wait TimeAtLocation seconds
            (Utilities|FlowControl|Delay (Utilities|Struct|BreakBP_Struct_NeedCustom (Variables|Setup|GetNeedDetails)))
            ;[1 1 1] Set next Roaming Behavior
            (Default|FnSetRoamBehavior (Variables|Default|GetGroundAnimal)))))
      (:Is%20Not%20Valid
        _))
    ;[1 1 1] Reset Custom Need
    (CallFunction|EventFinishedNeed)))

(event Custom|EventNeed_CustomCode
  ;[0 1 0] Create Child BP of this component and Override this Event to include your custom code. Make sure you copy the code here as is and insert your custom code between whats here! See example to see how I did it!
  ;[1 1 1] Check for Authority
  (if (Default|FnGetAuthority (Variables|Default|GetGroundAnimal))
    ;[1 1 1] Set BT BiggestNeed value to Custom Need
    (AI|Components|Blackboard|SetValueasEnum (Variables|/Script/AIModule.AIController|GetBlackboard (AI|GetAIController (Variables|Default|GetGroundAnimal))) (Variables|Default|GetBiggestNeed) (Utilities|Enum|LiteralenumBP_Enum_GroundNaturalBehaviors "NewEnumerator6"))
    ;[1 1 1] Reset Custom Need
    (CallFunction|EventFinishedNeed)))