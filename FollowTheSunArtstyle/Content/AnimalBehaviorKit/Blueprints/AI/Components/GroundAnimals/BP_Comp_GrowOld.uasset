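; Ground animal component that, when active, turns its owner into an adult animal after a random growth time.
; On BeginPlay it can set the animal's need to follow its parent and shrink its capsule to overlap pawns and camera, avoiding stuck animals.
; A one-second timer counts up to the random time, then sets GrowUp, whose RepNotify has the authority spawn AdultAnimal in place and destroy the owner.
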(event Custom|EventGrowUp
  (bind _returnvalue (Utilities|Time|SetTimerbyEvent (delegate Custom|EventGrowUp) 1.0 true))
  (Variables|Default|SetGrowUpHandler _returnvalue)
  ;[1 1 1] Check if count is less than or equal to random time
  (if (<= (Variables|Default|GetTimerCount) (Variables|Default|GetRandomTime))
    ;[1 1 1] Increase count by 1
    (Math|Float|IncrementFloat (Variables|Default|GetTimerCount))
    (else
      (Variables|Default|SetGrowUp true))))

(event EventBeginPlay
  (if (Variables|Setup|GetActive)
    (Utilities|FlowControl|Sequence
      (:then_0
        (if (Variables|Setup|GetFollowParent?)
          (CallFunction|FnFollowParent)))
      (:then_1
        (if (Variables|Setup|GetDisableCollision)
          ;[1 1 1] Ignore collision with other pawns. Helps if animals are getting stuck
          (bind _asbp_ground_animal_base (Utilities|Casting|CastToBP_GroundAnimalBase (Components|GetOwner)))
          (Collision|SetCollisionResponsetoChannel (Variables|/Script/Engine.Character|GetCapsuleComponent _asbp_ground_animal_base) "ECC_Pawn" "ECR_Overlap")
          (Collision|SetCollisionResponsetoChannel (Variables|/Script/Engine.Character|GetCapsuleComponent _asbp_ground_animal_base) "ECC_Camera" "ECR_Overlap")
          (Components|Capsule|SetCapsuleRadius (Variables|/Script/Engine.Character|GetCapsuleComponent _asbp_ground_animal_base) 1.0 true)))
      (:then_2
        (Variables|Default|SetRandomTime (Math|Random|RandomFloatinRange (Variables|Setup|GetMinGrowthTime) (Variables|Setup|GetMaxGrowthTime)))
        (CallFunction|EventGrowUp)))))

(fn FnSpawnAdult
  (bind _asbp_animal_base (Utilities|Casting|CastToBP_AnimalBase (Components|GetOwner)))
  (if (Default|FnGetAuthority _asbp_animal_base)
    (Game|SpawnActorfromClass (Variables|Setup|GetAdultAnimal) (Transformation|GetActorTransform (Components|GetOwner)) "AdjustIfPossibleButAlwaysSpawn" 0 0)
    (Actor|DestroyActor (Components|GetOwner))))

(fn OnRepGrowUp
  (CallFunction|FnSpawnAdult))

(fn FnFollowParent
  ;[1 1 1] Check parent reference is valid
  (Utilities|IsValid (Variables|Setup|GetParentRef)
    (:Is%20Valid
      ;[1 1 1] Change animal's need to Follow Parent
      (bind _asbp_ground_animal_base (Utilities|Casting|CastToBP_GroundAnimalBase (Components|GetOwner)))
      (Variables|/Game/AnimalBehaviorKit/Blueprints/Characters/Animals/GroundAnimals/BP_GroundAnimalBase.BP_GroundAnimalBase_C|SetBiggestNeed _asbp_ground_animal_base "NewEnumerator7"))))