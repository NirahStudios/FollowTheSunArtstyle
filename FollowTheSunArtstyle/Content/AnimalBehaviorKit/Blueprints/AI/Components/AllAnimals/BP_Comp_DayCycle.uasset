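; Animal component that switches its owner between active and resting states when day or night starts, supporting diurnal or nocturnal animals.
; It binds to BP_DayNightCycle dispatchers, using a manual or auto-found reference, and relays through Server/Client events.
; Ground animals change behavior, group membership and pause need, mating and optional aging/death timers, resuming only if a montage was playing on waking.
; Flying and swimming animals toggle going to home base, optionally hiding meshes.
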(event Custom|EventBindToDispatchers
  (|BINDEVENTSTODAYNIGHTCYCLEDISPACHERS))

(event EventBeginPlay
  (CallFunction|EventBindtoDispatchers))

(fn FnUnpauseSystems
  (bind _groundanimal (Variables|OwnerReference|GetGroundAnimal))
  (bind _groundanimal_2 (Variables|OwnerReference|GetGroundAnimal))
  (bind _groundanimal_3 (Variables|OwnerReference|GetGroundAnimal))
  (bind _groundanimal_4 (Variables|OwnerReference|GetGroundAnimal))
  (bind _groundanimal_5 (Variables|OwnerReference|GetGroundAnimal))
  (bind _returnvalue (Actor|GetComponentbyClass _groundanimal_3 "/Game/AnimalBehaviorKit/Blueprints/AI/Components/GroundAnimals/BP_Comp_LookForMate.BP_Comp_LookForMate_C"))
  (bind _returnvalue_2 (Actor|GetComponentbyClass _groundanimal "/Game/AnimalBehaviorKit/Blueprints/AI/Components/GroundAnimals/BP_Comp_NeedSystem.BP_Comp_NeedSystem_C"))
  (bind _returnvalue_3 (Actor|GetComponentbyClass _groundanimal_2 "/Game/AnimalBehaviorKit/Blueprints/AI/Components/GroundAnimals/BP_Comp_CustomNeed.BP_Comp_CustomNeed_C"))
  (bind _returnvalue_4 (Actor|GetComponentbyClass _groundanimal_5 "/Game/AnimalBehaviorKit/Blueprints/AI/Components/GroundAnimals/BP_Comp_GrowOld.BP_Comp_GrowOld_C"))
  (bind _returnvalue_5 (Actor|GetComponentbyClass _groundanimal_4 "/Game/AnimalBehaviorKit/Blueprints/AI/Components/GroundAnimals/BP_Comp_NaturalDeath.BP_Comp_NaturalDeath_C"))
  (Utilities|FlowControl|Sequence
    (:then_0
      ;[1 1 1] Unpause Need System
      (Utilities|IsValid _returnvalue_2
        (:Is%20Valid
          (Utilities|Time|UnpauseTimerbyHandle (Variables|/Game/AnimalBehaviorKit/Blueprints/AI/Components/GroundAnimals/BP_Comp_NeedSystem.BP_Comp_NeedSystem_C|GetNaturalNeedTimerHandle _returnvalue_2)))))
    (:then_1
      ;[1 1 1] Unpause Custom Need
      (Utilities|IsValid _returnvalue_3
        (:Is%20Valid
          (Utilities|Time|UnpauseTimerbyHandle (Variables|/Game/AnimalBehaviorKit/Blueprints/AI/Components/GroundAnimals/BP_Comp_CustomNeed.BP_Comp_CustomNeed_C|GetNaturalNeedTimerHandle _returnvalue_3)))))
    (:then_2
      ;[1 1 1] Unpause Look for Mate
      (Utilities|IsValid _returnvalue
        (:Is%20Valid
          (Utilities|Time|UnpauseTimerbyHandle (Variables|/Game/AnimalBehaviorKit/Blueprints/AI/Components/GroundAnimals/BP_Comp_LookForMate.BP_Comp_LookForMate_C|GetPartnerEventHandler _returnvalue))
          (Variables|/Game/AnimalBehaviorKit/Blueprints/AI/Components/GroundAnimals/BP_Comp_LookForMate.BP_Comp_LookForMate_C|SetActive _returnvalue true))))
    (:then_3
      (if (Variables|Setup-Systems|GetPauseNaturalDeath)
        ;[1 1 1] Unpause Natural Death
        (Utilities|IsValid _returnvalue_5
          (:Is%20Valid
            (Utilities|Time|UnpauseTimerbyHandle (Variables|/Game/AnimalBehaviorKit/Blueprints/AI/Components/GroundAnimals/BP_Comp_NaturalDeath.BP_Comp_NaturalDeath_C|GetDeathTimerHandler _returnvalue_5))))))
    (:then_4
      (if (Variables|Setup-Systems|GetPauseGrowOld)
        ;[1 1 1] Unpause Grow Old
        (Utilities|IsValid _returnvalue_4
          (:Is%20Valid
            (Utilities|Time|UnpauseTimerbyHandle (Variables|/Game/AnimalBehaviorKit/Blueprints/AI/Components/GroundAnimals/BP_Comp_GrowOld.BP_Comp_GrowOld_C|GetGrowUpHandler _returnvalue_4))))))))

(fn FnPauseSystems
  (bind _groundanimal (Variables|OwnerReference|GetGroundAnimal))
  (bind _groundanimal_2 (Variables|OwnerReference|GetGroundAnimal))
  (bind _groundanimal_3 (Variables|OwnerReference|GetGroundAnimal))
  (bind _groundanimal_4 (Variables|OwnerReference|GetGroundAnimal))
  (bind _groundanimal_5 (Variables|OwnerReference|GetGroundAnimal))
  (bind _returnvalue (Actor|GetComponentbyClass _groundanimal_3 "/Game/AnimalBehaviorKit/Blueprints/AI/Components/GroundAnimals/BP_Comp_LookForMate.BP_Comp_LookForMate_C"))
  (bind _returnvalue_2 (Actor|GetComponentbyClass _groundanimal "/Game/AnimalBehaviorKit/Blueprints/AI/Components/GroundAnimals/BP_Comp_NeedSystem.BP_Comp_NeedSystem_C"))
  (bind _returnvalue_3 (Actor|GetComponentbyClass _groundanimal_2 "/Game/AnimalBehaviorKit/Blueprints/AI/Components/GroundAnimals/BP_Comp_CustomNeed.BP_Comp_CustomNeed_C"))
  (bind _returnvalue_4 (Actor|GetComponentbyClass _groundanimal_5 "/Game/AnimalBehaviorKit/Blueprints/AI/Components/GroundAnimals/BP_Comp_GrowOld.BP_Comp_GrowOld_C"))
  (bind _returnvalue_5 (Actor|GetComponentbyClass _groundanimal_4 "/Game/AnimalBehaviorKit/Blueprints/AI/Components/GroundAnimals/BP_Comp_NaturalDeath.BP_Comp_NaturalDeath_C"))
  (Utilities|FlowControl|Sequence
    (:then_0
      ;[1 1 1] Pause Need System
      (Utilities|IsValid _returnvalue_2
        (:Is%20Valid
          (Utilities|Time|PauseTimerbyHandle (Variables|/Game/AnimalBehaviorKit/Blueprints/AI/Components/GroundAnimals/BP_Comp_NeedSystem.BP_Comp_NeedSystem_C|GetNaturalNeedTimerHandle _returnvalue_2)))))
    (:then_1
      ;[1 1 1] Pause Custom Need
      (Utilities|IsValid _returnvalue_3
        (:Is%20Valid
          (Utilities|Time|PauseTimerbyHandle (Variables|/Game/AnimalBehaviorKit/Blueprints/AI/Components/GroundAnimals/BP_Comp_CustomNeed.BP_Comp_CustomNeed_C|GetNaturalNeedTimerHandle _returnvalue_3)))))
    (:then_2
      ;[1 1 1] Pause Look for Mate
      (Utilities|IsValid _returnvalue
        (:Is%20Valid
          (Utilities|Time|PauseTimerbyHandle (Variables|/Game/AnimalBehaviorKit/Blueprints/AI/Components/GroundAnimals/BP_Comp_LookForMate.BP_Comp_LookForMate_C|GetPartnerEventHandler _returnvalue))
          (Variables|/Game/AnimalBehaviorKit/Blueprints/AI/Components/GroundAnimals/BP_Comp_LookForMate.BP_Comp_LookForMate_C|SetActive _returnvalue false))))
    (:then_3
      (if (Variables|Setup-Systems|GetPauseNaturalDeath)
        ;[1 1 1] Pause Natural Death
        (Utilities|IsValid _returnvalue_5
          (:Is%20Valid
            (Utilities|Time|PauseTimerbyHandle (Variables|/Game/AnimalBehaviorKit/Blueprints/AI/Components/GroundAnimals/BP_Comp_NaturalDeath.BP_Comp_NaturalDeath_C|GetDeathTimerHandler _returnvalue_5))))))
    (:then_4
      (if (Variables|Setup-Systems|GetPauseGrowOld)
        ;[1 1 1] Pause Grow Old
        (Utilities|IsValid _returnvalue_4
          (:Is%20Valid
            (Utilities|Time|PauseTimerbyHandle (Variables|/Game/AnimalBehaviorKit/Blueprints/AI/Components/GroundAnimals/BP_Comp_GrowOld.BP_Comp_GrowOld_C|GetGrowUpHandler _returnvalue_4))))))))

(fn FnGetDayCycleReference
  ;[1 1 1] Get Day Night Cycle actors
  (bind _outactors (Actor|GetAllActorsOfClass "/Game/AnimalBehaviorKit/Blueprints/AI/Actors/BP_DayNightCycle.BP_DayNightCycle_C"))
  (if (Utilities|Array|IsValidIndex _outactors)
    ;[1 1 1] Set the first actor as the reference
    (Variables|Setup|SetDayNightCycleRef (Utilities|Array|Get(acopy) _outactors))))

(event Custom|BindDayStarted
  ;[1 1 1] Bind EventDayStarted and EventNightStarted to the DayNightCycle event dispachers
  (CallFunction|EventDayStartedServer))

(event Custom|BindNightStarted
  ;[1 1 1] Bind EventDayStarted and EventNightStarted to the DayNightCycle event dispachers
  (CallFunction|EventNightStartedServer))

(event Custom|EventDayStartedClient
  (if (Variables|Setup|GetActive)
    (switch Utilities|FlowControl|Switch|SwitchonBP_Enum_AnimalType (Variables|Setup|GetAnimalType)
      (:NewEnumerator0
        (|GROUNDANIMALCODE))
      (:NewEnumerator1
        (|FLYINGANIMALCODE))
      (:NewEnumerator2
        (|SWIMMINGANIMALCODE)))))

(event Custom|EventDayStartedServer
  (CallFunction|EventDayStartedClient))

(event Custom|EventNightStartedServer
  (CallFunction|EventNightStartedClient))

(event Custom|EventNightStartedClient
  (if (Variables|Setup|GetActive)
    (switch Utilities|FlowControl|Switch|SwitchonBP_Enum_AnimalType (Variables|Setup|GetAnimalType)
      (:NewEnumerator0
        (|GROUNDANIMALCODE_2))
      (:NewEnumerator1
        (|FLYINGANIMALCODE_2))
      (:NewEnumerator2
        (|SWIMMINGANIMALCODE_2)))))