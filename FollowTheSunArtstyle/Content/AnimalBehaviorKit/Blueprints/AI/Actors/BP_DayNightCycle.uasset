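; BP_DayNightCycle is a world actor that runs a configurable-length day/night cycle.
; On the authority, Tick advances the hour, derives the sun angle, fires day/night start dispatchers through DoOnce gates and updates the first player's HUD once per hour.
; The SunAngle RepNotify rotates the sun, updates the sky dome, and uses a curve to scale sunlight color, skylight and atmospheric fog, recapturing the sky.
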(event EventBeginPlay
  ;[1 1 1] Check for Authority
  (Networking|SwitchHasAuthority
    (:Authority
      (Utilities|FlowControl|Sequence
        (:then_0
          (|CALCULATETIMEVARIABLES))
        (:then_1
          (|SAVEPLAYERREFERENCE))
        (:then_2
          (|SAVESUNCOLOR))))))

(event EventTick
  (params (DeltaSeconds :type Float%20%28single-precision%29))
  (Variables|Default|SetDeltaTime DeltaSeconds)
  (Utilities|FlowControl|Sequence
    (:then_0
      ;[1 1 1] Check for Authority
      (Networking|SwitchHasAuthority
        (:Authority
          (if (Variables|Setup|GetActive?)
            (CallFunction|EventCheckTime (Variables|Time|GetHour))
            (CallFunction|FnUpdatePlayerHUD)
            ;[1 1 1] Calculate current Hour of the Day
            (Variables|Time|SetHour (+ (Variables|Time|GetHour) (/ (Variables|Default|GetDeltaTime) (Variables|Time|GetOneHour))))
            ;[1 1 1] Calculate Sun Angle
            (Variables|SunPosition|SetSunAngle (+ (* (/ (Variables|Time|GetHour) 6.0) 9e+01) 9e+01))
            ;[1 1 1] Reset Hour to 0 after 24 hours
            (if (> (Variables|Time|GetHour) 24.0)
              (Variables|Time|SetHour 0.0))))))
    (:then_1
      ;[1 1 0] DEBUG
      (if (Variables|Setup|GetDebugTime)
        (Development|PrintString (Utilities|String|Append "Current Time: " (Utilities|String|ToString(Float) (Variables|Time|GetHour))) true true "(R=0.000000,G=0.660000,B=1.000000,A=1.000000)" (Variables|Default|GetDeltaTime))))))

(fn ConstructionScript)

(fn FnUpdatePlayerHUD
  (bind _playerref (Variables|Default|GetPlayerRef))
  (bind _playerref_2 (Variables|Default|GetPlayerRef))
  (bind _returnvalue (Actor|GetComponentbyClass _playerref "/Game/AdvancedTaming/Blueprints/Characters/Player/Components/BP_Comp_PlayerHUD_ATS.BP_Comp_PlayerHUD_ATS_C"))
  (bind _returnvalue_2 (Actor|GetComponentbyClass _playerref_2 "/Game/AnimalBehaviorKit/Blueprints/Characters/Player/Components/BP_Comp_PlayerHUD.BP_Comp_PlayerHUD_C"))
  (bind _playerhudref (Variables|/Game/AnimalBehaviorKit/Blueprints/Characters/Player/Components/BP_Comp_PlayerHUD.BP_Comp_PlayerHUD_C|GetPlayerHUDRef _returnvalue_2))
  (bind _playerhudref_2 (Variables|/Game/AdvancedTaming/Blueprints/Characters/Player/Components/BP_Comp_PlayerHUD_ATS.BP_Comp_PlayerHUD_ATS_C|GetPlayerHUDRef _returnvalue))
  (if (!= (Math|Float|Floor (Variables|Time|GetHour)) (LocalVariables|GetCalculatedHour))
    (LocalVariables|SetCalculatedHour (Math|Float|Floor (Variables|Time|GetHour)))
    (Utilities|IsValid (Variables|Default|GetPlayerRef)
      (:Is%20Valid
        (Utilities|FlowControl|Sequence
          (:then_0
            (Utilities|IsValid _returnvalue_2
              (:Is%20Valid
                (Utilities|IsValid _playerhudref
                  (:Is%20Valid
                    (Default|FnSetTime _playerhudref (Math|Conversions|ToFloat(Integer) (LocalVariables|GetCalculatedHour))))))))
          (:then_1
            ;[0 1 1] COMPANION CODE
            (Utilities|IsValid _returnvalue
              (:Is%20Valid
                (Utilities|IsValid _playerhudref_2
                  (:Is%20Valid
                    (Default|FnSetTime _playerhudref_2 (Math|Conversions|ToFloat(Integer) (LocalVariables|GetCalculatedHour)))))))))))))

(fn OnRepSunAngle
  (bind _skylightref (Variables|SunPosition|GetSkylightRef))
  (bind _lightcomponent (Variables|/Script/Engine.SkyLight|GetLightComponent _skylightref))
  (Utilities|IsValid (Variables|SunPosition|GetSunRef)
    (:Is%20Valid
      ;[1 1 1] Rotate the sun
      (Transformation|SetActorRotation (Variables|SunPosition|GetSunRef) (Math|Rotator|MakeRotator 0.0 (Variables|SunPosition|GetSunAngle) 0.0))
      ;[1 1 1] Reduce light color intensity as night falls
      (Rendering|Components|Light|SetLightColor (Variables|/Script/Engine.Light|GetLightComponent (Variables|SunPosition|GetSunRef)) (* (Variables|SunPosition|GetSunColor) (Math|Float|Clamp(Float) (Math|Curves|GetFloatValue (Variables|SunPosition|GetSkylightCurve) (Variables|Time|GetHour)) 0.1)) true))
    (:Is%20Not%20Valid
      ;[1 1 1] No Sun reference found!
      (Development|PrintString "No Sun Reference Found" true true "(R=1.000000,G=0.000000,B=0.000000,A=1.000000)" 5.0)))
  (Utilities|IsValid (Variables|SunPosition|GetSkyDomeRef)
    (:Is%20Valid
      ;[1 1 1] Update Skydome
      (Default|UpdateSunDirection (Variables|SunPosition|GetSkyDomeRef)))
    (:Is%20Not%20Valid
      ;[1 1 1] No Skydome reference found!
      (Development|PrintString "No Skydome Reference Found" true true "(R=1.000000,G=0.000000,B=0.000000,A=1.000000)" 5.0)))
  (Utilities|IsValid (Variables|SunPosition|GetSkylightRef)
    (:Is%20Valid
      ;[1 1 1] Set Skylight intensity
      (Class|SkyLightComponent|SetIndirectLightingIntensity _lightcomponent (* (Variables|/Script/Engine.LightComponentBase|GetIntensity _lightcomponent) (Math|Curves|GetFloatValue (Variables|SunPosition|GetSkylightCurve) (Variables|Time|GetHour))))
      ;[1 1 1] Recapture the sky
      (Class|SkyLightComponent|RecaptureSky (Variables|/Script/Engine.SkyLight|GetLightComponent (Variables|SunPosition|GetSkylightRef))))
    (:Is%20Not%20Valid
      _))
  (Utilities|IsValid (Variables|SunPosition|GetAtmosphericFog)
    (:Is%20Valid
      ;[1 1 1] Set sun multiplier on atmospheric fog
      (Class|AtmosphericFogComponent|SetSunMultiplier (Variables|/Script/Engine.AtmosphericFog|GetAtmosphericFogComponent (Variables|SunPosition|GetAtmosphericFog)) (Math|Curves|GetFloatValue (Variables|SunPosition|GetSkylightCurve) (Variables|Time|GetHour))))))

(event Custom|EventCheckTime
  (params (Hour :type Float%20%28single-precision%29))
  ;[1 1 1] Check for Authority
  (Networking|SwitchHasAuthority
    (:Authority
      ;[1 1 1] Check if the current hour is between DayStart and DayEnd
      (if (and (>= Hour (Variables|Setup|GetDayStart)) (<= Hour (Variables|Setup|GetDayEnd)))
        (Utilities|FlowControl|Sequence
          (:then_0
            (Utilities|FlowControl|DoOnce false :!label _label
              (:Completed
                (Default|CallDispDayStarted))))
          (:then_1
            (goto _label_2 Reset)))
        (else
          (Utilities|FlowControl|Sequence
            (:then_0
              (Utilities|FlowControl|DoOnce false :!label _label_2
                (:Completed
                  (Default|CallDispNightStarted))))
            (:then_1
              (goto _label Reset))))))))