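; BP_UnderWaterPPV is an underwater post-process volume actor that pairs with a swimming AI bounds actor.
; Events copy the location and rotation of the referenced SwimmingBounds and resize the root box to match its scaled box extent.
; TogglePPV switches the PostProcess component on or off and tracks the state in PPVActive.
; Nothing in this Blueprint calls these events, and its construction script is empty.
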(event Custom|SetVolumeLocation
  ;[1 1 1] Set Location to BP_AI_SwimmingBounds
  (Transformation|SetActorLocation (Transformation|GetWorldLocation (Variables|/Game/AnimalBehaviorKit/Blueprints/AI/Actors/Swimming_AI/BP_AI_Swimming_BoundingBox.BP_AI_Swimming_BoundingBox_C|GetBounds (Variables|Setup|GetSwimmingBounds))) false true)
  (Transformation|SetActorRotation (Transformation|GetActorRotation (Variables|Setup|GetSwimmingBounds))))

(event Custom|TogglePPV
  ;[1 1 1] Enable and Disable PPV
  (if (Variables|Default|GetPPVActive?)
    (Variables|/Script/Engine.PostProcessComponent|SetbEnabled (Variables|Default|GetPostProcess) false)
    (Variables|Default|SetPPVActive? false)
    (else
      (Variables|/Script/Engine.PostProcessComponent|SetbEnabled (Variables|Default|GetPostProcess) true)
      (Variables|Default|SetPPVActive? true))))

(event Custom|SetVolumeSize
  ;[1 1 1] Set Size to match BP_AI_Swimming_Bounds
  (Components|Box|SetBoxExtent (Variables|Default|GetRoot) (Components|Box|GetScaledBoxExtent (Variables|/Game/AnimalBehaviorKit/Blueprints/AI/Actors/Swimming_AI/BP_AI_Swimming_BoundingBox.BP_AI_Swimming_BoundingBox_C|GetBounds (Variables|Setup|GetSwimmingBounds))) true))

(fn ConstructionScript)