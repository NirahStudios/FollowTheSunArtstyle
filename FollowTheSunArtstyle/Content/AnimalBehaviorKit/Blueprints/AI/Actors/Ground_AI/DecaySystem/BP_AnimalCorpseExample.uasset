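; Example animal corpse Blueprint from the Animal Behavior Kit decay system, showing the decay events it can respond to.
; It handles state started, state ended and decay ended events, printing a debug message for each, with the state index where available.
; The construction script only calls its parent, and no decay logic is implemented in this Blueprint itself.
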(event EventEventStateStarted
  (params (State%20Index :type Integer))
  (Development|PrintString (Utilities|String|Append "State  " (Utilities|String|ToString(Integer) State%20Index) " started!")))

(event EventEventStateEnded
  (params (State%20Index :type Integer))
  (Development|PrintString (Utilities|String|Append "State  " (Utilities|String|ToString(Integer) State%20Index) " ended!")))

(event EventEventDecayEnded
  (Development|PrintString "Decay Ended!"))

(fn ConstructionScript
  (|CallParentFunction))