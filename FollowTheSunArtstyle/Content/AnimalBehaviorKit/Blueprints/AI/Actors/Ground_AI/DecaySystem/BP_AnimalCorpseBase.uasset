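; Base animal corpse actor that steps through an array of decay states after its start event is called.
; Each state traces down for ground height and optional slope alignment, plays a transition particle effect, and replaces the previously spawned actor.
; A delay advances the counter through paired Server and Client events.
; Empty state-start, state-end and decay-end events serve as hooks, with optional despawn after the last state.
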(fn ConstructionScript)

(fn FnGetSpawnLocation
  (bind _actortransform (Variables|Default|GetActorTransform))
  (bind _actortransform_2 (Variables|Default|GetActorTransform))
  (bind _returnvalue (+ (.location _actortransform) "0, 0,20000.000000"))
  ;[1 1 1] Shoot line trace downwards to get floor location
  (bind _outhit (Collision|LineTraceByChannel _returnvalue (+ _returnvalue (* (Math|Vector|GetUpVector (.rotation _actortransform)) -4e+04)) "TraceTypeQuery1" true 0 "None"))
  (LocalVariables|SetImpactLoc (.Location (Collision|BreakHitResult _outhit)))
  (LocalVariables|SetImpactNormal (.Normal (Collision|BreakHitResult _outhit)))
  ;[1 1 1] Do we align to the ground?
  (if (Utilities|Struct|BreakBP_Struct_DecayStateDetails (Utilities|Array|Get(acopy) (Variables|Setup|GetDecayStates) (Variables|Default|GetStateCounter)))
    ;[1 1 1] Set rotation to align to ground
    (LocalVariables|SetRotation (Math|Rotator|MakeRotfromZX (LocalVariables|GetImpactNormal) (Math|Vector|GetForwardVector (.rotation (Variables|Default|GetActorTransform)))))
    (else
      ;[1 1 1] Set rotation to actor's rotation
      (LocalVariables|SetRotation (.rotation (Variables|Default|GetActorTransform)))))
  ;[1 1 1] Set Spawn transform
  (bind _output_get (LocalVariables|SetTransform (Math|Transform|MakeTransform (Math|Vector|MakeVector (.x (.location _actortransform_2)) (.y (.location _actortransform_2)) (+ (.z (LocalVariables|GetImpactLoc)) (Utilities|Struct|BreakBP_Struct_DecayStateDetails (Utilities|Array|Get(acopy) (Variables|Setup|GetDecayStates) (Variables|Default|GetStateCounter))))) (LocalVariables|GetRotation) "1,1,1")))
  (return _output_get))

(event Custom|EventStartDecayServer
  (CallFunction|EventStartDecayClient))

(event Custom|EventStartDecayClient
  (Utilities|FlowControl|Sequence
    (:then_0
      (CallFunction|EventStateStarted (Variables|Default|GetStateCounter))
      ;[1 1 1] Set Spawn Transform
      (bind _spawn_transform (CallFunction|FnGetSpawnLocation))
      (Variables|Default|SetSpawnTransform _spawn_transform))
    (:then_1
      ;[1 1 1] Do we have a valid particle system?
      (Utilities|IsValid (Utilities|Struct|BreakBP_Struct_DecayStateDetails (Utilities|Array|Get(acopy) (Variables|Setup|GetDecayStates) (Variables|Default|GetStateCounter)))
        (:Is%20Valid
          ;[1 1 1] Spawn transition emitter
          (bind _returnvalue (Effects|SpawnEmitteratLocation (Utilities|Struct|BreakBP_Struct_DecayStateDetails (Utilities|Array|Get(acopy) (Variables|Setup|GetDecayStates) (Variables|Default|GetStateCounter))) (.location (Variables|Default|GetSpawnTransform)) (.rotation (Variables|Default|GetSpawnTransform))))
          (Variables|Default|SetSpawnedEmitter _returnvalue)
          ;[1 1 1] Wait for ParticleDuration and then destroy the emitter
          (Utilities|FlowControl|Delay (Utilities|Struct|BreakBP_Struct_DecayStateDetails (Utilities|Array|Get(acopy) (Variables|Setup|GetDecayStates) (Variables|Default|GetStateCounter))))
          (Utilities|IsValid (Variables|Default|GetSpawnedEmitter)
            (:Is%20Valid
              (Components|DestroyComponent (Variables|Default|GetSpawnedEmitter)))))))
    (:then_2
      ;[1 1 1] Do we have a valid actor class?
      (if (Utilities|IsValidClass (Utilities|Struct|BreakBP_Struct_DecayStateDetails (Utilities|Array|Get(acopy) (Variables|Setup|GetDecayStates) (Variables|Default|GetStateCounter))))
        ;[1 1 1] Do we already have a spawned actor? If so, destroy it before spawning the new one
        (Utilities|IsValid (Variables|Default|GetSpawnedActor)
          (:Is%20Valid
            (Actor|DestroyActor (Variables|Default|GetSpawnedActor)))
          (:Is%20Not%20Valid
            _))
        ;[1 1 1] Spawn actor for this state
        (bind _returnvalue_2 (Game|SpawnActorfromClass (Utilities|Struct|BreakBP_Struct_DecayStateDetails (Utilities|Array|Get(acopy) (Variables|Setup|GetDecayStates) (Variables|Default|GetStateCounter))) (Math|Transform|MakeTransform (.location (Variables|Default|GetSpawnTransform)) (.rotation (Variables|Default|GetSpawnTransform)) "1,1,1") "AdjustIfPossibleButAlwaysSpawn" 0 0))
        (Variables|Default|SetSpawnedActor _returnvalue_2)))
    (:then_3
      ;[1 1 1] Wait StateDuration before moving to the next state
      (Utilities|FlowControl|Delay (Utilities|Struct|BreakBP_Struct_DecayStateDetails (Utilities|Array|Get(acopy) (Variables|Setup|GetDecayStates) (Variables|Default|GetStateCounter))))
      ;[1 1 1] Destroy emitter if we spawned one
      (Utilities|IsValid (Variables|Default|GetSpawnedEmitter)
        (:Is%20Valid
          (Components|DestroyComponent (Variables|Default|GetSpawnedEmitter)))
        (:Is%20Not%20Valid
          _))
      ;[1 1 1] Is the StateCounter less than the total number of states?
      (if (< (Variables|Default|GetStateCounter) (- (Utilities|Array|Length (Variables|Setup|GetDecayStates)) 1))
        (CallFunction|EventStateEnded (Variables|Default|GetStateCounter))
        ;[1 1 1] Increase StateCounter by 1
        (Math|Integer|IncrementInt (Variables|Default|GetStateCounter)
          (:%20%20
            (CallFunction|EventStartDecayServer)))
        (else
          (Variables|Default|SetStateCounter 0)
          (CallFunction|EventDecayEnded)
          (if (Variables|Setup|GetDespawnAtEnd?)
            (Actor|DestroyActor (Variables|Default|GetSpawnedActor))
            (Actor|DestroyActor)))))))

(event Custom|EventStateStarted
  (params (State%20Index :type Integer)))

(event Custom|EventStateEnded
  (params (State%20Index :type Integer)))

(event Custom|EventDecayEnded)