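; Activation manager that keeps a registry of animals and switches each between active and inactive.
; Animals register into a unique list, and a supplied active set decides the status pushed to each one's activation component.
; The same pass removes invalid entries from the registry and stores the new active list.
; With DebugStats on, the authority prints active versus total counts on a looping timer.
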(event Custom|EventShowStats
  (Utilities|Time|SetTimerbyEvent (delegate Custom|EventShowStats) (Variables|Default|GetStatUpdateFrequency) true)
  (Utilities|FlowControl|Sequence
    (:then_0
      (Development|PrintString (Utilities|String|Append "Active: " (Utilities|String|ToString(Integer) (Utilities|Array|Length (Variables|Setup|GetActiveAnimalList))) " / " (Utilities|String|ToString(Integer) (Utilities|Array|Length (Variables|Setup|GetTotalAnimalList)))) true true "(R=0.000000,G=0.660000,B=1.000000,A=1.000000)" (Variables|Default|GetStatUpdateFrequency)))
    (:then_1
      (Development|PrintString "Activation Manager" true true "(R=0.000000,G=0.660000,B=1.000000,A=1.000000)" (Variables|Default|GetStatUpdateFrequency)))))

(event EventBeginPlay
  (if (Variables|Setup|GetDebugStats)
    (Networking|SwitchHasAuthority
      (:Authority
        (CallFunction|EventShowStats)))))

(fn ConstructionScript)

(fn FnRegisterAnimal
  (params (Animal :type Actor%20Object%20Reference))
  (Utilities|Array|AddUnique (Variables|Setup|GetTotalAnimalList) Animal))

(fn FnActivateAnimals
  (params (Active%20Animals :type Array%20of%20Actor%20Object%20References))
  (LocalVariables|SetActiveAnimals Active%20Animals)
  ;[1 1 1] Go throught all registered animals
  (for _array_element (Variables|Setup|GetTotalAnimalList)
    (LocalVariables|SetAnimal _array_element)
    (Utilities|IsValid (LocalVariables|GetAnimal)
      (:Is%20Valid
        ;[1 1 1] Check if the current animal is Active
        (if (Utilities|Array|ContainsItem (LocalVariables|GetActiveAnimals) (LocalVariables|GetAnimal))
          ;[1 1 1] Activate Animal
          (Utilities|IsValid (Actor|GetComponentbyClass (LocalVariables|GetAnimal) "/Game/AnimalBehaviorKit/Blueprints/AI/Components/GroundAnimals/BP_Comp_Animal_ActivationManager.BP_Comp_Animal_ActivationManager_C")
            (:Is%20Valid
              (Default|FnSetAnimalStatus (Actor|GetComponentbyClass (LocalVariables|GetAnimal) "/Game/AnimalBehaviorKit/Blueprints/AI/Components/GroundAnimals/BP_Comp_Animal_ActivationManager.BP_Comp_Animal_ActivationManager_C") true)))
          (else
            ;[1 1 1] Deactive Animal
            (Utilities|IsValid (Actor|GetComponentbyClass (LocalVariables|GetAnimal) "/Game/AnimalBehaviorKit/Blueprints/AI/Components/GroundAnimals/BP_Comp_Animal_ActivationManager.BP_Comp_Animal_ActivationManager_C")
              (:Is%20Valid
                (Default|FnSetAnimalStatus (Actor|GetComponentbyClass (LocalVariables|GetAnimal) "/Game/AnimalBehaviorKit/Blueprints/AI/Components/GroundAnimals/BP_Comp_Animal_ActivationManager.BP_Comp_Animal_ActivationManager_C") false))))))
      (:Is%20Not%20Valid
        ;[1 1 1] Animal does not exist - remove it
        (Utilities|Array|RemoveItem (Variables|Setup|GetTotalAnimalList) (LocalVariables|GetAnimal)))))
  ;[1 1 1] Set ActiveAnimalList to the current active animals
  (Utilities|Array|Clear (Variables|Setup|GetActiveAnimalList))
  (Variables|Setup|SetActiveAnimalList (LocalVariables|GetActiveAnimals)))