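; BP_AI_Food is a food actor for the ground AI need system in AnimalBehaviorKit.
; Its construction script calls FnSetScales, which sizes the Bounds component from BoundsScale and the visual Marker at a fixed fraction of that scale.
; The same function pins the text renderer to unit world scale and sets the Marker's editor and in-game visibility from variables.
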(fn ConstructionScript
  (CallFunction|FnSetScales))

(fn FnSetScales
  ;[1 1 1] Set world scale for the text renderer
  (Transformation|SetWorldScale3D (Variables|Default|GetTextRender) "1.000000,1.000000,1.000000")
  ;[1 1 1] Set Bound Scale
  (Transformation|SetWorldScale3D (Variables|Default|GetBounds) (Variables|Setup|GetBoundsScale))
  ;[1 1 1] Scale visual marker
  (Transformation|SetWorldScale3D (Variables|Default|GetMarker) (* (Variables|Setup|GetBoundsScale) 0.625))
  ;[1 1 1] Set Marker visibility
  (Rendering|SetVisibility (Variables|Default|GetMarker) (Variables|Setup|GetMarkerVisible) false)
  (Development|SetHiddeninGame (Variables|Default|GetMarker) (Variables|Setup|GetMarkerHidden) false))