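; Manager actor that automatically forms registered animals into groups by species, with configurable size, leader sex and composition.
; Animals register into per-species male and female lists, which an authority-only looping timer scans when active.
; For viable groups, it picks a leader and members, spawns and configures a BP_GroupManager, and links it through each member's BP_Comp_Group.
; It recurses while enough animals remain and offers debug printouts.
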(event Custom|EventCheckGroups
  (bind _returnvalue (Utilities|Time|SetTimerbyEvent (delegate Custom|EventCheckGroups) (Variables|Setup|GetCheckFrequency) true))
  (Variables|Default|SetCheckHandler _returnvalue)
  (CallFunction|FnManageGroups)
  ;[1 1 1] Check to see if we are debugging
  (if (or (Variables|Debug|GetDebugGroupCreation) (Variables|Debug|GetDebugLooseAnimals))
    (CallFunction|FnCleanDebugInfo)))

(event EventBeginPlay
  ;[1 1 1] Check Auto Grouping is Active
  (if (Variables|Setup|GetActive)
    ;[1 1 1] Check for Authority
    (Networking|SwitchHasAuthority
      (:Authority
        ;[1 1 1] Clear information
        (Variables|Debug|SetTotalGroupsCreated 0)
        (Utilities|Array|Clear (Variables|Debug|GetLeaderList))
        (Utilities|FlowControl|Delay (Variables|Setup|GetCheckFrequency))
        (CallFunction|EventCheckGroups)))))

(fn ConstructionScript
  ;[1 1 1] Add unique tag
  (Utilities|Array|AddUnique (Variables|Actor|GetTags) (Variables|Setup|GetUniqueTag)))

(fn FnRegisterAnimal
  (params (Actor%20reference :type BP%20Ground%20Animal%20Base%20Object%20Reference) (Sex :type BP_Enum_AnimalSex%20Enum :default "NewEnumerator0") (Species :type Text))
  (LocalVariables|SetAnimalReference Actor%20reference)
  (LocalVariables|SetAnimalSex Sex)
  (LocalVariables|SetAnimalSpecies Species)
  (bind (_array_element _array_index) (Utilities|Array|ForEachLoopwithBreak (Variables|Setup|GetSpeciesDetails) :!label _label)
    (:LoopBody
      (LocalVariables|SetCurrentSpecies _array_element)
      (LocalVariables|SetIndex _array_index)
      ;[1 1 1] Is the CurrentSpecies the same as the Animal Species?
      (if (Utilities|Enum|Equal(Enum) (Utilities|Struct|BreakBP_Struct_AutoGroup_SpeciesDetail (LocalVariables|GetCurrentSpecies)) (LocalVariables|GetAnimalSpecies))
        (Utilities|FlowControl|Sequence
          (:then_0
            (switch Utilities|FlowControl|Switch|SwitchonBP_Enum_AnimalSex (LocalVariables|GetAnimalSex)
              (:NewEnumerator0
                (LocalVariables|SetMaleList (Utilities|Struct|BreakBP_Struct_AutoGroup_SpeciesDetail (LocalVariables|GetCurrentSpecies)))
                (Utilities|Array|Add (LocalVariables|GetMaleList) (LocalVariables|GetAnimalReference))
                (bind _structout (Utilities|Struct|SetmembersinBP_Struct_AutoGroup_SpeciesDetail (LocalVariables|GetCurrentSpecies) (LocalVariables|GetMaleList)))
                (Utilities|Array|SetArrayElem (Variables|Setup|GetSpeciesDetails) (LocalVariables|GetIndex) _structout true))
              (:NewEnumerator1
                (LocalVariables|SetFemaleList (Utilities|Struct|BreakBP_Struct_AutoGroup_SpeciesDetail (LocalVariables|GetCurrentSpecies)))
                (Utilities|Array|Add (LocalVariables|GetFemaleList) (LocalVariables|GetAnimalReference))
                (bind _structout_2 (Utilities|Struct|SetmembersinBP_Struct_AutoGroup_SpeciesDetail (LocalVariables|GetCurrentSpecies) (LocalVariables|GetFemaleList)))
                (Utilities|Array|SetArrayElem (Variables|Setup|GetSpeciesDetails) (LocalVariables|GetIndex) _structout_2 true))))
          (:then_1
            (goto _label Break)))))))

(fn FnManageGroups
  ;[1 1 1] Go through all species
  (for (_array_element _array_index) (Variables|Setup|GetSpeciesDetails)
    (LocalVariables|SetCurrentSpecies _array_element)
    (LocalVariables|SetIndex _array_index)
    ;[1 1 1] Save Males and Females for this species
    (LocalVariables|SetMales (.MaleList (Utilities|Struct|BreakBP_Struct_AutoGroup_SpeciesDetail (LocalVariables|GetCurrentSpecies))))
    (LocalVariables|SetFemales (.FemaleList (Utilities|Struct|BreakBP_Struct_AutoGroup_SpeciesDetail (LocalVariables|GetCurrentSpecies))))
    ;[1 1 1] Check that we have the minimum amount of total animals to form a group
    (if (>= (+ (Utilities|Array|Length (LocalVariables|GetMales)) (Utilities|Array|Length (LocalVariables|GetFemales))) (Math|Float|Truncate (.x (Utilities|Struct|BreakBP_Struct_AutoGroup_SpeciesDetail (LocalVariables|GetCurrentSpecies)))))
      ;[1 1 1] Check Male availability
      (if (> (Utilities|Array|Length (LocalVariables|GetMales)) 0)
        (LocalVariables|SetMalesAvailable true)
        (else
          (LocalVariables|SetMalesAvailable false)))
      ;[1 1 1] Check Female availability
      (if (> (Utilities|Array|Length (LocalVariables|GetFemales)) 0)
        (LocalVariables|SetFemalesAvailable true)
        (else
          (LocalVariables|SetFemalesAvailable false)))
      ;[1 1 1] Set random group size
      (LocalVariables|SetGroupSize (Math|Float|Truncate (Math|Random|RandomFloatinRange (Math|Float|Clamp(Float) (.x (Utilities|Struct|BreakBP_Struct_AutoGroup_SpeciesDetail (LocalVariables|GetCurrentSpecies))) 2.0 999.0) (Math|Float|Clamp(Float) (.y (Utilities|Struct|BreakBP_Struct_AutoGroup_SpeciesDetail (LocalVariables|GetCurrentSpecies))) 2.0 999.0))))
      ;[1 1 1] Switch on Leader type
      (switch Utilities|FlowControl|Switch|SwitchonBP_Enum_AutoGroup_AnimalType (Utilities|Struct|BreakBP_Struct_AutoGroup_SpeciesDetail (LocalVariables|GetCurrentSpecies))
        (:NewEnumerator0
          (if (LocalVariables|GetMalesAvailable) :!label _label
            ;[1 1 1] Set Leader
            (bind _output_get (LocalVariables|SetLeader (Utilities|Array|Get(acopy) (LocalVariables|GetMales))))
            ;[1 1 1] Remove actor from array
            (Utilities|Array|RemoveItem (LocalVariables|GetMales) _output_get)
            ;[1 1 1] Populate the rest of the group
            (Utilities|FlowControl|ForLoopwithBreak 0 (- (LocalVariables|GetGroupSize) 2) :!label _label_2
              (:LoopBody
                ;[1 1 1] Switch on Group Composition
                (switch Utilities|FlowControl|Switch|SwitchonBP_Enum_AutoGroup_AnimalType (Utilities|Struct|BreakBP_Struct_AutoGroup_SpeciesDetail (LocalVariables|GetCurrentSpecies))
                  (:NewEnumerator0
                    ;[1 1 1] Check that we have at least 1 actor in the array
                    (if (Utilities|Array|IsValidIndex (LocalVariables|GetMales)) :!label _label_3
                      ;[1 1 1] Add actor to GroupList array
                      (Utilities|Array|Add (LocalVariables|GetGroupList) (Utilities|Array|Get(acopy) (LocalVariables|GetMales)))
                      ;[1 1 1] Remove actor
                      (Utilities|Array|RemoveItem (LocalVariables|GetMales) (Utilities|Array|Get(acopy) (LocalVariables|GetMales)))))
                  (:NewEnumerator1
                    ;[1 1 1] Check that we have at least 1 actor in the array
                    (if (Utilities|Array|IsValidIndex (LocalVariables|GetFemales)) :!label _label_4
                      ;[1 1 1] Add actor to GroupList array
                      (Utilities|Array|Add (LocalVariables|GetGroupList) (Utilities|Array|Get(acopy) (LocalVariables|GetFemales)))
                      ;[1 1 1] Remove actor
                      (Utilities|Array|RemoveItem (LocalVariables|GetFemales) (Utilities|Array|Get(acopy) (LocalVariables|GetFemales)))))
                  (:NewEnumerator2
                    ;[1 1 1] Get random member
                    (if (Math|Random|RandomBool)
                      (goto _label_3)
                      (else
                        (goto _label_4))))))
              (:Completed
                ;[1 1 1] Is the current group size equal or bigger than then min group size?
                (if (>= (+ (Utilities|Array|Length (LocalVariables|GetGroupList)) 1) (Math|Float|Truncate (.x (Utilities|Struct|BreakBP_Struct_AutoGroup_SpeciesDetail (LocalVariables|GetCurrentSpecies)))))
                  (Utilities|FlowControl|Sequence
                    (:then_0
                      ;[1 1 1] Add leader to group
                      (Utilities|Array|AddUnique (LocalVariables|GetGroupList) (LocalVariables|GetLeader))
                      ;[1 1 1] Spawn GroupManager for this group
                      (bind _returnvalue (Game|SpawnActorfromClass "/Game/AnimalBehaviorKit/Blueprints/AI/Actors/Ground_AI/Group/BP_GroupManager.BP_GroupManager_C" (Math|Transform|MakeTransform (Utilities|Struct|BreakBP_Struct_AutoGroup_SpeciesDetail (LocalVariables|GetCurrentSpecies))) "AlwaysSpawn" 0 0))
                      (LocalVariables|SetGroupManager _returnvalue)
                      ;[1 1 1] Deactivate Group Manager
                      (Variables|/Game/AnimalBehaviorKit/Blueprints/AI/Actors/Ground_AI/Group/BP_GroupManager.BP_GroupManager_C|SetActive (LocalVariables|GetGroupManager) false)
                      ;[1 1 1] Set Group Manager Settings
                      (Variables|/Game/AnimalBehaviorKit/Blueprints/AI/Actors/Ground_AI/Group/BP_GroupManager.BP_GroupManager_C|SetEngageBehaviorMethod (LocalVariables|GetGroupManager) (.EngageBehaviorMethod (Utilities|Struct|BreakBP_Struct_GroupManagerSettings (Utilities|Struct|BreakBP_Struct_AutoGroup_SpeciesDetail (LocalVariables|GetCurrentSpecies)))))
                      (Variables|/Game/AnimalBehaviorKit/Blueprints/AI/Actors/Ground_AI/Group/BP_GroupManager.BP_GroupManager_C|SetGroupEngageBehavior (LocalVariables|GetGroupManager) (.GroupEngageBehavior (Utilities|Struct|BreakBP_Struct_GroupManagerSettings (Utilities|Struct|BreakBP_Struct_AutoGroup_SpeciesDetail (LocalVariables|GetCurrentSpecies)))))
                      (Variables|/Game/AnimalBehaviorKit/Blueprints/AI/Actors/Ground_AI/Group/BP_GroupManager.BP_GroupManager_C|SetChooseRandomLeader? (LocalVariables|GetGroupManager) (.Chooserandomleader? (Utilities|Struct|BreakBP_Struct_GroupManagerSettings (Utilities|Struct|BreakBP_Struct_AutoGroup_SpeciesDetail (LocalVariables|GetCurrentSpecies)))))
                      (Variables|/Game/AnimalBehaviorKit/Blueprints/AI/Actors/Ground_AI/Group/BP_GroupManager.BP_GroupManager_C|SetNewLeaderRate (LocalVariables|GetGroupManager) (.Newleaderrate (Utilities|Struct|BreakBP_Struct_GroupManagerSettings (Utilities|Struct|BreakBP_Struct_AutoGroup_SpeciesDetail (LocalVariables|GetCurrentSpecies)))))
                      (Variables|/Game/AnimalBehaviorKit/Blueprints/AI/Actors/Ground_AI/Group/BP_GroupManager.BP_GroupManager_C|SetNoDamageByMembers (LocalVariables|GetGroupManager) (.Nodamagebymembers (Utilities|Struct|BreakBP_Struct_GroupManagerSettings (Utilities|Struct|BreakBP_Struct_AutoGroup_SpeciesDetail (LocalVariables|GetCurrentSpecies)))))
                      (Variables|/Game/AnimalBehaviorKit/Blueprints/AI/Actors/Ground_AI/Group/BP_GroupManager.BP_GroupManager_C|SetGroupTag (LocalVariables|GetGroupManager) (Utilities|String|StringToName (Utilities|GetDisplayName (LocalVariables|GetGroupManager))))
                      ;[1 1 1] Set group members and leader
                      (Variables|/Game/AnimalBehaviorKit/Blueprints/AI/Actors/Ground_AI/Group/BP_GroupManager.BP_GroupManager_C|SetGroup (LocalVariables|GetGroupManager) (LocalVariables|GetGroupList))
                      (Variables|/Game/AnimalBehaviorKit/Blueprints/AI/Actors/Ground_AI/Group/BP_GroupManager.BP_GroupManager_C|SetGroupLeader (LocalVariables|GetGroupManager) (LocalVariables|GetLeader)))
                    (:then_1
                      ;[1 1 1] Go through all group members
                      (for _array_element_2 (LocalVariables|GetGroupList)
                        (LocalVariables|SetCurrentMember _array_element_2)
                        (Utilities|IsValid (LocalVariables|GetCurrentMember)
                          (:Is%20Valid
                            ;[1 1 1] Set Group Manager reference
                            (Utilities|IsValid (Actor|GetComponentbyClass (LocalVariables|GetCurrentMember) "/Game/AnimalBehaviorKit/Blueprints/AI/Components/GroundAnimals/BP_Comp_Group.BP_Comp_Group_C")
                              (:Is%20Valid
                                (Variables|/Game/AnimalBehaviorKit/Blueprints/AI/Components/GroundAnimals/BP_Comp_Group.BP_Comp_Group_C|SetGroupManager (Actor|GetComponentbyClass (LocalVariables|GetCurrentMember) "/Game/AnimalBehaviorKit/Blueprints/AI/Components/GroundAnimals/BP_Comp_Group.BP_Comp_Group_C") (LocalVariables|GetGroupManager)))))))
                      (Utilities|FlowControl|Sequence
                        (:then_0
                          (Utilities|IsValid (LocalVariables|GetLeader)
                            (:Is%20Valid
                              ;[1 1 1] Mark leader appropriately
                              (Utilities|IsValid (Actor|GetComponentbyClass (LocalVariables|GetLeader) "/Game/AnimalBehaviorKit/Blueprints/AI/Components/GroundAnimals/BP_Comp_Group.BP_Comp_Group_C")
                                (:Is%20Valid
                                  (Variables|/Game/AnimalBehaviorKit/Blueprints/AI/Components/GroundAnimals/BP_Comp_Group.BP_Comp_Group_C|SetGroupLeader? (Actor|GetComponentbyClass (LocalVariables|GetLeader) "/Game/AnimalBehaviorKit/Blueprints/AI/Components/GroundAnimals/BP_Comp_Group.BP_Comp_Group_C") true)
                                  (Variables|/Game/AnimalBehaviorKit/Blueprints/AI/Components/GroundAnimals/BP_Comp_Group.BP_Comp_Group_C|SetCheckLeadership (Actor|GetComponentbyClass (LocalVariables|GetLeader) "/Game/AnimalBehaviorKit/Blueprints/AI/Components/GroundAnimals/BP_Comp_Group.BP_Comp_Group_C") true))))))
                        (:then_1
                          ;[1 1 1] Activate the Group Manager
                          (Default|EventSetGroup (LocalVariables|GetGroupManager)))))
                    (:then_2
                      ;[1 1 1] Resize arrays
                      (bind _structout (Utilities|Struct|SetmembersinBP_Struct_AutoGroup_SpeciesDetail (LocalVariables|GetCurrentSpecies) (LocalVariables|GetMales)))
                      (Utilities|Array|SetArrayElem (Variables|Setup|GetSpeciesDetails) (LocalVariables|GetIndex) _structout true)
                      (bind _structout_2 (Utilities|Struct|SetmembersinBP_Struct_AutoGroup_SpeciesDetail (LocalVariables|GetCurrentSpecies) (LocalVariables|GetFemales)))
                      (Utilities|Array|SetArrayElem (Variables|Setup|GetSpeciesDetails) (LocalVariables|GetIndex) _structout_2 true)
                      ;[1 1 1] Increase TotalGroupsCreated
                      (Math|Integer|IncrementInt (Variables|Debug|GetTotalGroupsCreated)
                        (:%20%20
                          ;[1 1 1] Add leader to LeaderList
                          (Utilities|Array|AddUnique (Variables|Debug|GetLeaderList) (LocalVariables|GetLeader)))))
                    (:then_3
                      (if (Variables|Debug|GetDebugGroupCreation)
                        ;[1 1 0] Debug
                        (Development|PrintString (Utilities|String|Append (Utilities|GetDisplayName self) "- Group Size: " (Utilities|String|ToString(Integer) (Utilities|Array|Length (LocalVariables|GetGroupList))) ": Leader: " (Utilities|GetDisplayName (LocalVariables|GetLeader)) " (" (Utilities|String|ToString(Text) (Utilities|Struct|BreakBP_Struct_AutoGroup_SpeciesDetail (LocalVariables|GetCurrentSpecies))) " | " (Utilities|String|EnumtoString (Utilities|Struct|BreakBP_Struct_AnimalBase_AnimalDetail (Variables|/Game/AnimalBehaviorKit/Blueprints/Characters/Animals/BP_AnimalBase.BP_AnimalBase_C|GetAnimal_Details (LocalVariables|GetLeader)))) ")") true true "(R=0.000000,G=1.000000,B=0.000000,A=1.000000)" 1e+01)))
                    (:then_4
                      ;[1 1 1] Check that we have the minimum amount of total animals to form a group
                      (if (>= (+ (Utilities|Array|Length (LocalVariables|GetMales)) (Utilities|Array|Length (LocalVariables|GetFemales))) (Math|Float|Truncate (.x (Utilities|Struct|BreakBP_Struct_AutoGroup_SpeciesDetail (LocalVariables|GetCurrentSpecies)))))
                        ;[1 1 1] Call function again
                        (CallFunction|FnManageGroups))))
                  (else
                    ;[1 1 0] Debug
                    (if (Variables|Debug|GetDebugGroupCreation)
                      (Development|PrintString (Utilities|String|Append (Utilities|GetDisplayName self) " - Could not create group (" (Utilities|String|ToString(Integer) (+ (Utilities|Array|Length (LocalVariables|GetGroupList)) 1)) "/" (Utilities|String|ToString(Integer) (Math|Float|Truncate (.x (Utilities|Struct|BreakBP_Struct_AutoGroup_SpeciesDetail (LocalVariables|GetCurrentSpecies))))) ")") true true "(R=1.000000,G=0.000000,B=0.000000,A=1.000000)" 1e+01))))))))
        (:NewEnumerator1
          (if (LocalVariables|GetFemalesAvailable) :!label _label_5
            ;[1 1 1] Set Leader
            (bind _output_get_2 (LocalVariables|SetLeader (Utilities|Array|Get(acopy) (LocalVariables|GetFemales))))
            ;[1 1 1] Remove actor from array
            (Utilities|Array|RemoveItem (LocalVariables|GetFemales) _output_get_2)
            (goto _label_2)))
        (:NewEnumerator2
          ;[1 1 1] Get random Leader
          (if (Math|Random|RandomBool)
            (goto _label)
            (else
              (goto _label_5)))))
      (elif (Variables|Debug|GetDebugLooseAnimals)
        ;[1 1 0] Debug
        (Development|PrintString (Utilities|String|Append (Utilities|GetDisplayName self) "- Number of animals not enough to create group (" (Utilities|String|ToString(Text) (Utilities|Struct|BreakBP_Struct_AutoGroup_SpeciesDetail (LocalVariables|GetCurrentSpecies))) " | " (Utilities|String|ToString(Integer) (+ (Utilities|Array|Length (LocalVariables|GetMales)) (Utilities|Array|Length (LocalVariables|GetFemales)))) ")") true true "(R=1.000000,G=0.000000,B=0.000000,A=1.000000)" 5.0)))))

(fn FnCleanDebugInfo
  ;[1 1 1] Go thorough all leaders and see if there are some that are invalid
  (for _array_element (Variables|Debug|GetLeaderList)
    (Utilities|IsValid _array_element
      (:Is%20Not%20Valid
        ;[1 1 1] Remove invalid reference
        (Utilities|Array|RemoveItem (Variables|Debug|GetLeaderList) _array_element)))))