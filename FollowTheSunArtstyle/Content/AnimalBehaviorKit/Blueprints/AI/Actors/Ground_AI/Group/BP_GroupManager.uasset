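; BP_GroupManager coordinates a group of animal AI, managing its leader, tags and shared engage behavior.
; After a delayed BeginPlay, the authority sets RepNotify flags whose OnReps add group tags and no-damage tags, and optionally rotate a random leader on a timer.
; Leader changes, also triggered when the leader leaves, retry random picks and mark the HUD name with "(L)".
; Engage behavior follows group, leader or individual settings, and engaging propagates the target to members.
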(event Custom|EventSetGroup
  ;[1 1 1] Check for Authority
  (Networking|SwitchHasAuthority
    (:Authority
      (Utilities|FlowControl|Sequence
        (:then_0
          (Variables|Default|SetAddGroupTag true))
        (:then_1
          (if (Variables|Setup|GetChooseRandomLeader?)
            (CallFunction|EventChooseNewLeader)))
        (:then_2
          (if (Variables|Setup|GetNoDamageByMembers)
            (Variables|Default|SetSetNoDamage true)))
        (:then_3
          (CallFunction|FnPopulateBehavior))))))

(event EventBeginPlay
  (Utilities|FlowControl|Delay 1.0)
  (if (Variables|Setup|GetActive)
    ;[1 1 1] Check for Authority
    (Networking|SwitchHasAuthority
      (:Authority
        (Utilities|FlowControl|Sequence
          (:then_0
            (Variables|Default|SetAddGroupTag true))
          (:then_1
            (if (Variables|Setup|GetChooseRandomLeader?)
              (CallFunction|EventChooseNewLeader)))
          (:then_2
            (if (Variables|Setup|GetNoDamageByMembers)
              (Variables|Default|SetSetNoDamage true)))
          (:then_3
            (CallFunction|FnPopulateBehavior)))))))

(fn ConstructionScript)

(fn FnGetRandomMember
  (return (Utilities|Array|Get(acopy) (Variables|Setup|GetGroup) (Math|Random|RandomIntegerinRange 0 (- (Utilities|Array|Length (Variables|Setup|GetGroup)) 1)))))

(fn FnSetGroupEngageBehavior
  (params (EngagedActor :type Actor%20Object%20Reference))
  (LocalVariables|SeteActor EngagedActor)
  ;[1 1 1] Go through all group members
  (for _array_element (Variables|Setup|GetGroup)
    (LocalVariables|SetMember _array_element)
    ;[1 1 1] Check group member is valid
    (Utilities|IsValid (LocalVariables|GetMember)
      (:Is%20Valid
        (switch Utilities|FlowControl|Switch|SwitchonBP_Enum_GroupManager_EngageBehavior (Variables|Setup|GetEngageBehaviorMethod)
          (:NewEnumerator0
            ;[1 1 1] Set  Engage Behavior to Group Engage Behavior
            (Variables|/Game/AnimalBehaviorKit/Blueprints/Characters/Animals/GroundAnimals/BP_GroundAnimalBase.BP_GroundAnimalBase_C|SetEngageBehavior (LocalVariables|GetMember) (Variables|Setup|GetGroupEngageBehavior))
            (Variables|/Game/AnimalBehaviorKit/Blueprints/Characters/Animals/GroundAnimals/BP_GroundAnimalBase.BP_GroundAnimalBase_C|SetOriginalEngageBehavior (LocalVariables|GetMember) (Variables|Setup|GetGroupEngageBehavior))
            (if (Utilities|Enum|NotEqual(Enum) (Variables|Setup|GetGroupEngageBehavior) "NewEnumerator0")
              ;[1 1 1] Set EngageActor for everyone in the group
              (Variables|/Game/AnimalBehaviorKit/Blueprints/Characters/Animals/GroundAnimals/BP_GroundAnimalBase.BP_GroundAnimalBase_C|SetSensedActor (LocalVariables|GetMember) (LocalVariables|GeteActor) :!label _label)
              (Default|FnSetEngageTarget (LocalVariables|GetMember) (LocalVariables|GeteActor))))
          (:NewEnumerator1
            ;[1 1 1] Set  Engage Behavior to Leader's Engage Behavior
            (Variables|/Game/AnimalBehaviorKit/Blueprints/Characters/Animals/GroundAnimals/BP_GroundAnimalBase.BP_GroundAnimalBase_C|SetEngageBehavior (LocalVariables|GetMember) (Variables|/Game/AnimalBehaviorKit/Blueprints/Characters/Animals/GroundAnimals/BP_GroundAnimalBase.BP_GroundAnimalBase_C|GetEngageBehavior (Variables|Setup|GetGroupLeader)))
            (Variables|/Game/AnimalBehaviorKit/Blueprints/Characters/Animals/GroundAnimals/BP_GroundAnimalBase.BP_GroundAnimalBase_C|SetOriginalEngageBehavior (LocalVariables|GetMember) (Variables|/Game/AnimalBehaviorKit/Blueprints/Characters/Animals/GroundAnimals/BP_GroundAnimalBase.BP_GroundAnimalBase_C|GetEngageBehavior (Variables|Setup|GetGroupLeader)))
            (if (Utilities|Enum|NotEqual(Enum) (Variables|/Game/AnimalBehaviorKit/Blueprints/Characters/Animals/GroundAnimals/BP_GroundAnimalBase.BP_GroundAnimalBase_C|GetEngageBehavior (Variables|Setup|GetGroupLeader)) "NewEnumerator0")
              (goto _label)))
          (:NewEnumerator2
            (if (Utilities|Enum|NotEqual(Enum) (Variables|/Game/AnimalBehaviorKit/Blueprints/Characters/Animals/GroundAnimals/BP_GroundAnimalBase.BP_GroundAnimalBase_C|GetEngageBehavior (LocalVariables|GetMember)) "NewEnumerator0")
              (goto _label))))))))

(fn OnRepChooseLeader
  (CallFunction|FnSetNewLeader))

(fn FnSetNewLeader
  ;[1 1 1] Check that the group has more than 1 member
  (if (> (Utilities|Array|Length (Variables|Setup|GetGroup)) 1)
    ;[1 1 1] Is the Group Leader reference valid?
    (Utilities|IsValid (Variables|Setup|GetGroupLeader)
      (:Is%20Valid
        ;[1 1 1] Save old Group Leader
        (Variables|Default|SetOldGroupLeader (Variables|Setup|GetGroupLeader))
        ;[1 1 1] Demote current group leader
        (Utilities|IsValid (Actor|GetComponentbyClass (Variables|Setup|GetGroupLeader) "/Game/AnimalBehaviorKit/Blueprints/AI/Components/GroundAnimals/BP_Comp_Group.BP_Comp_Group_C")
          (:Is%20Valid
            (Variables|/Game/AnimalBehaviorKit/Blueprints/AI/Components/GroundAnimals/BP_Comp_Group.BP_Comp_Group_C|SetGroupLeader? (Actor|GetComponentbyClass (Variables|Setup|GetGroupLeader) "/Game/AnimalBehaviorKit/Blueprints/AI/Components/GroundAnimals/BP_Comp_Group.BP_Comp_Group_C") false)
            (Utilities|FlowControl|Sequence
              (:then_0
                ;[1 1 1] Reset leader's name to its default name (without the 'L')
                (bind _aswbp_ai_hud (Utilities|Casting|CastToWBP_AI_HUD (UserInterface|GetUserWidgetObject (Variables|/Game/AnimalBehaviorKit/Blueprints/Characters/Animals/BP_AnimalBase.BP_AnimalBase_C|GetWBP_HUD (Variables|Setup|GetGroupLeader)))))
                (Default|FnSetName _aswbp_ai_hud (Utilities|Struct|BreakBP_Struct_AnimalBase_AnimalDetail (Variables|/Game/AnimalBehaviorKit/Blueprints/Characters/Animals/BP_AnimalBase.BP_AnimalBase_C|GetAnimal_Details (Variables|Setup|GetGroupLeader)))))
              (:then_1
                ;[1 1 1] Reset leader's name to its default name (without the 'L')
                (bind _aswbp_ats_ai_hud (Utilities|Casting|CastToWBP_ATS_AI_HUD (UserInterface|GetUserWidgetObject (Variables|/Game/AnimalBehaviorKit/Blueprints/Characters/Animals/BP_AnimalBase.BP_AnimalBase_C|GetWBP_HUD (Variables|Setup|GetGroupLeader)))))
                (Default|FnSetName _aswbp_ats_ai_hud (Utilities|Struct|BreakBP_Struct_AnimalBase_AnimalDetail (Variables|/Game/AnimalBehaviorKit/Blueprints/Characters/Animals/BP_AnimalBase.BP_AnimalBase_C|GetAnimal_Details (Variables|Setup|GetGroupLeader)))))
              (:then_2
                ;[1 1 1] Choose a random leader for the group
                (Variables|Setup|SetGroupLeader (Utilities|Array|Get(acopy) (Variables|Setup|GetGroup) (Math|Random|RandomIntegerinRange 0 (- (Utilities|Array|Length (Variables|Setup|GetGroup)) 1))) :!label _label)
                ;[1 1 1] Make sure the new random leader is NOT the old one
                (if (and (!= (Variables|Setup|GetGroupLeader) (Variables|Default|GetOldGroupLeader)) (Utilities|IsValid (Variables|Setup|GetGroupLeader)))
                  ;[1 1 1] Set new group member as Leader
                  (Utilities|IsValid (Actor|GetComponentbyClass (Variables|Setup|GetGroupLeader) "/Game/AnimalBehaviorKit/Blueprints/AI/Components/GroundAnimals/BP_Comp_Group.BP_Comp_Group_C")
                    (:Is%20Valid
                      (Variables|/Game/AnimalBehaviorKit/Blueprints/AI/Components/GroundAnimals/BP_Comp_Group.BP_Comp_Group_C|SetGroupLeader? (Actor|GetComponentbyClass (Variables|Setup|GetGroupLeader) "/Game/AnimalBehaviorKit/Blueprints/AI/Components/GroundAnimals/BP_Comp_Group.BP_Comp_Group_C") true)
                      (Utilities|FlowControl|Sequence
                        (:then_0
                          ;[1 1 1] Set new leader's name
                          (bind _aswbp_ai_hud_2 (Utilities|Casting|CastToWBP_AI_HUD (UserInterface|GetUserWidgetObject (Variables|/Game/AnimalBehaviorKit/Blueprints/Characters/Animals/BP_AnimalBase.BP_AnimalBase_C|GetWBP_HUD (Variables|Setup|GetGroupLeader)))))
                          (Default|FnSetName _aswbp_ai_hud_2 (Utilities|Text|ToText(String) (Utilities|String|Append "(L) " (Utilities|String|ToString(Text) (Utilities|Struct|BreakBP_Struct_AnimalBase_AnimalDetail (Variables|/Game/AnimalBehaviorKit/Blueprints/Characters/Animals/BP_AnimalBase.BP_AnimalBase_C|GetAnimal_Details (Variables|Setup|GetGroupLeader))))))))
                        (:then_1
                          ;[1 1 1] Set new leader's name
                          (bind _aswbp_ats_ai_hud_2 (Utilities|Casting|CastToWBP_ATS_AI_HUD (UserInterface|GetUserWidgetObject (Variables|/Game/AnimalBehaviorKit/Blueprints/Characters/Animals/BP_AnimalBase.BP_AnimalBase_C|GetWBP_HUD (Variables|Setup|GetGroupLeader)))))
                          (Default|FnSetName _aswbp_ats_ai_hud_2 (Utilities|Text|ToText(String) (Utilities|String|Append "(L) " (Utilities|String|ToString(Text) (Utilities|Struct|BreakBP_Struct_AnimalBase_AnimalDetail (Variables|/Game/AnimalBehaviorKit/Blueprints/Characters/Animals/BP_AnimalBase.BP_AnimalBase_C|GetAnimal_Details (Variables|Setup|GetGroupLeader))))))))
                        (:then_2
                          ;[1 1 1] Reset Old Leader ref
                          (Variables|Default|SetOldGroupLeader 0)))))
                  (else
                    ;[1 1 1] Increase count by 1
                    (Math|Integer|IncrementInt (LocalVariables|GetTryCount)
                      (:%20%20
                        ;[1 1 1] Check that we can still try
                        (if (<= (LocalVariables|GetTryCount) (LocalVariables|GetMaxTries))
                          (goto _label))))))))))))))

(fn OnRepSetNoDamage
  (CallFunction|FnSetNoDamageTags))

(fn FnSetNoDamageTags
  (for _array_element (Variables|Setup|GetGroup)
    (LocalVariables|SetMember _array_element)
    (Utilities|IsValid (LocalVariables|GetMember)
      (:Is%20Valid
        (Utilities|FlowControl|Sequence
          (:then_0
            ;[1 1 1] Get current values from NoDamageTags array
            (LocalVariables|SetTempArray (Utilities|Struct|BreakBP_Struct_AnimalBase_AnimalDetail (Variables|/Game/AnimalBehaviorKit/Blueprints/Characters/Animals/BP_AnimalBase.BP_AnimalBase_C|GetAnimal_Details (LocalVariables|GetMember))))
            ;[1 1 1] Add the Group Manager name as a tag
            (Utilities|Array|Add (LocalVariables|GetTempArray) (Utilities|String|StringToName (Utilities|GetDisplayName self)))
            ;[1 1 1] Set NoDamageTags array to TempArray to include new tag
            (Utilities|Struct|SetmembersinBP_Struct_AnimalBase_AnimalDetail (Variables|/Game/AnimalBehaviorKit/Blueprints/Characters/Animals/BP_AnimalBase.BP_AnimalBase_C|GetAnimal_Details (LocalVariables|GetMember)) (LocalVariables|GetTempArray)))
          (:then_1
            ;[1 1 1] Add an actor tag with the name of the GroupManager
            (Utilities|Array|Add (Variables|/Script/Engine.Actor|GetTags (LocalVariables|GetMember)) (Utilities|String|StringToName (Utilities|GetDisplayName self)))))))))

(fn OnRepAddGroupTag
  (for _array_element (Variables|Setup|GetGroup)
    (LocalVariables|SetMember _array_element)
    (Utilities|IsValid (LocalVariables|GetMember)
      (:Is%20Valid
        ;[1 1 1] Add the Group Tag to the member of the group
        (Utilities|Array|Add (Variables|/Script/Engine.Actor|GetTags (LocalVariables|GetMember)) (Variables|Setup|GetGroupTag))))))

(fn FnPopulateBehavior
  ;[1 1 1] Go through all group members
  (for _array_element (Variables|Setup|GetGroup)
    (LocalVariables|SetMember _array_element)
    ;[1 1 1] Check group member is valid
    (Utilities|IsValid (LocalVariables|GetMember)
      (:Is%20Valid
        (switch Utilities|FlowControl|Switch|SwitchonBP_Enum_GroupManager_EngageBehavior (Variables|Setup|GetEngageBehaviorMethod)
          (:NewEnumerator0
            ;[1 1 1] Set  Engage Behavior to Group Engage Behavior
            (Variables|/Game/AnimalBehaviorKit/Blueprints/Characters/Animals/GroundAnimals/BP_GroundAnimalBase.BP_GroundAnimalBase_C|SetEngageBehavior (LocalVariables|GetMember) (Variables|Setup|GetGroupEngageBehavior))
            (Variables|/Game/AnimalBehaviorKit/Blueprints/Characters/Animals/GroundAnimals/BP_GroundAnimalBase.BP_GroundAnimalBase_C|SetOriginalEngageBehavior (LocalVariables|GetMember) (Variables|Setup|GetGroupEngageBehavior)))
          (:NewEnumerator1
            ;[1 1 1] Set  Engage Behavior to Leader's Engage Behavior
            (Variables|/Game/AnimalBehaviorKit/Blueprints/Characters/Animals/GroundAnimals/BP_GroundAnimalBase.BP_GroundAnimalBase_C|SetEngageBehavior (LocalVariables|GetMember) (Variables|/Game/AnimalBehaviorKit/Blueprints/Characters/Animals/GroundAnimals/BP_GroundAnimalBase.BP_GroundAnimalBase_C|GetEngageBehavior (Variables|Setup|GetGroupLeader)))
            (Variables|/Game/AnimalBehaviorKit/Blueprints/Characters/Animals/GroundAnimals/BP_GroundAnimalBase.BP_GroundAnimalBase_C|SetOriginalEngageBehavior (LocalVariables|GetMember) (Variables|/Game/AnimalBehaviorKit/Blueprints/Characters/Animals/GroundAnimals/BP_GroundAnimalBase.BP_GroundAnimalBase_C|GetEngageBehavior (Variables|Setup|GetGroupLeader)))))))))

(event Custom|EventChooseNewLeader
  (bind _returnvalue (Utilities|Time|SetTimerbyEvent (delegate Custom|EventChooseNewLeader) (Variables|Setup|GetNewLeaderRate) true))
  (Variables|Default|SetLeaderTimerHandle _returnvalue)
  (Variables|Default|SetChooseLeader true))

(event Custom|EventLeaveGroup
  (params (Animal :type BP%20Ground%20Animal%20Base%20Object%20Reference))
  ;[1 1 1] Check if the animal is the group leader
  (if (== Animal (Variables|Setup|GetGroupLeader))
    (CallFunction|FnSetNewLeader)))