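; BP_AI_WayPoint is a waypoint marker for ground AI navigation, identified by a group name and a numeric ID.
; Its construction script writes both values to the PathName and ID text components and applies the TextVisible flag to PathName and its children.
; The fnSetWayPointInfo function repeats the text update without changing visibility, so the labels can be refreshed separately from construction.
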(fn ConstructionScript
  (Rendering|Components|TextRender|SetText (Variables|Default|GetPathName) (Variables|Setup|GetWayPointGroupName))
  (Rendering|Components|TextRender|SetText (Variables|Default|GetID) (Utilities|Text|ToText(Integer) (Variables|Setup|GetWayPointID)))
  (Rendering|SetVisibility (Variables|Default|GetPathName) (Variables|Setup|GetTextVisible) true))

(fn FnSetWayPointInfo
  (Rendering|Components|TextRender|SetText (Variables|Default|GetPathName) (Variables|Setup|GetWayPointGroupName))
  (Rendering|Components|TextRender|SetText (Variables|Default|GetID) (Utilities|Text|ToText(Integer) (Variables|Setup|GetWayPointID))))