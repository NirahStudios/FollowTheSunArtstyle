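; Defense zone actor for ground AI animals that rallies them to a location when a matching actor enters its trigger.
; While active, an overlap compares the intruder's tags against a configured tag list.
; On the first match, every animal in its ground animal array switches to Defend behavior, moves to the defense location and engages the intruder.
; The construction script sizes the trigger from a configurable scale.
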(event OnComponentBeginOverlap(Trigger)
  (params (OverlappedComponent :type Primitive%20Component%20Object%20Reference) (OtherActor :type Actor%20Object%20Reference) (OtherComp :type Primitive%20Component%20Object%20Reference) (OtherBodyIndex :type Integer) (bFromSweep :type Boolean) (SweepResult :type Hit%20Result%20Structure%20%28by%20ref%29))
  (Variables|Default|SetOverlappedActor OtherActor)
  (if (Variables|Setup|GetActive)
    (CallFunction|FnCheckActor (Variables|Default|GetOverlappedActor))))

(fn ConstructionScript
  (Transformation|SetWorldScale3D (Variables|Default|GetTrigger) (Variables|Setup|GetTriggerScale)))

(fn FnCheckActor
  (params (Actor :type Actor%20Object%20Reference))
  (bind _array_element (Utilities|Array|ForEachLoopwithBreak (Variables|/Script/Engine.Actor|GetTags Actor) :!label _label)
    (:LoopBody
      (LocalVariables|Settag _array_element)
      (if (Utilities|Array|ContainsItem (Variables|Setup|GetActorTags) (LocalVariables|Gettag))
        (Utilities|FlowControl|Sequence
          (:then_0
            (CallFunction|FnCallAnimals))
          (:then_1
            (goto _label Break)))))))

(fn FnCallAnimals
  ;[1 1 1] Go through all animals in array
  (for _array_element (Variables|Setup|GetGroundAnimals)
    (LocalVariables|Setanimal _array_element)
    ;[1 1 1] Set EngageBehavior to Defend
    (Variables|/Game/AnimalBehaviorKit/Blueprints/Characters/Animals/GroundAnimals/BP_GroundAnimalBase.BP_GroundAnimalBase_C|SetEngageBehavior (LocalVariables|Getanimal) "NewEnumerator2")
    ;[1 1 1] Make animal come to Defense Location
    (Variables|/Game/AnimalBehaviorKit/Blueprints/Characters/Animals/GroundAnimals/BP_GroundAnimalBase.BP_GroundAnimalBase_C|SetDefenseState (LocalVariables|Getanimal) "NewEnumerator0")
    ;[1 1 1] Set EngagedActor and start engagement
    (Variables|/Game/AnimalBehaviorKit/Blueprints/Characters/Animals/GroundAnimals/BP_GroundAnimalBase.BP_GroundAnimalBase_C|SetEngagedActor (LocalVariables|Getanimal) (Variables|Default|GetOverlappedActor))
    (Default|FnSetEngageParams (LocalVariables|Getanimal))))