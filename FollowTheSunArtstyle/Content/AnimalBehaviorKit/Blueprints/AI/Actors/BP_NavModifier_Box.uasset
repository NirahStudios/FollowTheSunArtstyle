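; Nav modifier box actor that applies a configurable nav area class to a scalable volume, with an option to match an AI swimming bounds actor.
; The construction script scales the root box, keeps the text label at a fixed scale, sets the area class and applies visibility settings.
; Two events copy the swimming bounds' location and rotation, and derive the box scale from its bounds scale using a constant factor.
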(event Custom|SetVolumeLocation
  ;[1 1 1] Set Location to BP_AI_SwimmingBounds
  (Transformation|SetActorLocation (Transformation|GetWorldLocation (Variables|/Game/AnimalBehaviorKit/Blueprints/AI/Actors/Swimming_AI/BP_AI_Swimming_BoundingBox.BP_AI_Swimming_BoundingBox_C|GetBounds (Variables|Setup|GetSwimmingBounds))) false true)
  (Transformation|SetActorRotation (Transformation|GetActorRotation (Variables|Setup|GetSwimmingBounds))))

(event Custom|SetVolumeSize
  ;[1 1 1] Set Size to match BP_AI_Swimming_Bounds
  (Variables|Setup|SetAreaScale (* (Variables|/Game/AnimalBehaviorKit/Blueprints/AI/Actors/Swimming_AI/BP_AI_Swimming_BoundingBox.BP_AI_Swimming_BoundingBox_C|GetBoundsScale (Variables|Setup|GetSwimmingBounds)) 0.625))
  ;[1 1 1] Scale the Box area
  (Transformation|SetWorldScale3D (Variables|Default|GetRoot) (Variables|Setup|GetAreaScale)))

(fn ConstructionScript
  ;[1 1 1] Scale the Box area
  (Transformation|SetWorldScale3D (Variables|Default|GetRoot) (Variables|Setup|GetAreaScale))
  ;[1 1 1] Keep the text at its original scale
  (Transformation|SetWorldScale3D (Variables|Default|GetTextRender) "5.000000,5.000000,5.000000")
  ;[1 1 1] Set the Nav Mesh Modifier to the specified class
  (Class|NavModifierComponent|SetAreaClass (Variables|Default|GetNavModifier) (Variables|Setup|GetNavMesh%20Class))
  ;[1 1 1] Set visibility settings
  (Rendering|SetVisibility (Variables|Default|GetRoot) (Variables|Setup|GetVisibility) false)
  (Development|SetHiddeninGame (Variables|Default|GetRoot) (Variables|Setup|GetHidden) false))