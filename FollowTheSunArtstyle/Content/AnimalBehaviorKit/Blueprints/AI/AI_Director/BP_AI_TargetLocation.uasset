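; BP_AI_TargetLocation is an actor marking a destination for BOID-tagged AI in the Animal Behavior Kit's AI Director system.
; Its collision component's begin-overlap event ignores repeat hits from the same actor by caching the last one.
; When the new actor carries the BOID tag and the director reference is valid, it notifies the AI Director that a boid reached the target.
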(event OnComponentBeginOverlap(Collision)
  (params (OverlappedComponent :type Primitive%20Component%20Object%20Reference) (OtherActor :type Actor%20Object%20Reference) (OtherComp :type Primitive%20Component%20Object%20Reference) (OtherBodyIndex :type Integer) (bFromSweep :type Boolean) (SweepResult :type Hit%20Result%20Structure%20%28by%20ref%29))
  (Variables|Default|SetActor OtherActor)
  (if (!= (Variables|Default|GetActor) (Variables|Default|GetPrevActor))
    (Variables|Default|SetPrevActor (Variables|Default|GetActor))
    ;[1 1 1] Check overlapping actor has BOIDTag
    (if (Actor|ActorHasTag (Variables|Default|GetActor) (Variables|Default|GetBOIDTag))
      ;[1 1 1] Check AI Director is valid
      (Utilities|IsValid (Variables|Setup|GetAIDirector)
        (:Is%20Valid
          (Default|EventBOIDReachedTarget (Variables|Setup|GetAIDirector)))))))

(fn ConstructionScript)