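; Setup diagnostic actor for the Animal Behavior Kit that checks level and player configuration on BeginPlay or through the RunTroubleshooter event.
; FnCheckLevel tests for a NavMeshBoundsVolume, the abkPlayer tag on the player pawn, and the player capsule's Pawn object type and blocking response.
; The resulting flags feed PRINT REPORT, which prints in reverse order, title last, along with a troubleshooter link.
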(event Custom|Run%20Troubleshooter
  (CallFunction|FnCheckLevel))

(event EventBeginPlay
  (CallFunction|FnCheckLevel))

(fn ConstructionScript)

(fn FnCheckLevel
  (bind _returnvalue (Game|GetPlayerCharacter 0))
  (bind _capsulecomponent (Variables|/Script/Engine.Character|GetCapsuleComponent _returnvalue))
  (Utilities|FlowControl|Sequence
    (:then_0
      ;[1 1 1] Check for a Nav Mesh in the level
      (bind _outactors (Actor|GetAllActorsOfClass "/Script/Engine.NavMeshBoundsVolume"))
      (if (Utilities|Array|IsValidIndex _outactors)
        (LocalVariables|SetFoundNavMesh true)
        (else
          (LocalVariables|SetFoundNavMesh false))))
    (:then_1
      ;[1 1 1] Check for Player Tag
      (if (Utilities|Array|ContainsItem (Variables|/Script/Engine.Actor|GetTags (Game|Player|GetPlayerPawn 0)) "abkPlayer")
        (LocalVariables|SetPlayerTagFound true)
        (else
          (LocalVariables|SetPlayerTagFound false))))
    (:then_2
      ;[1 1 1] Check Player collision
      (Utilities|FlowControl|Sequence
        (:then_0
          (if (Utilities|Enum|Equal(Enum) (Collision|GetCollisionResponsetoChannel _capsulecomponent "ECC_Pawn") "ECR_Block")
            (LocalVariables|SetPlayerPawnCollisionBlock true)
            (else
              (LocalVariables|SetPlayerPawnCollisionBlock false))))
        (:then_1
          (if (Utilities|Enum|Equal(Enum) (Collision|GetCollisionObjectType _capsulecomponent) "ECC_Pawn")
            (LocalVariables|SetPlayerCollisionTypePawn true)
            (else
              (LocalVariables|SetPlayerCollisionTypePawn false))))))
    (:then_3
      (|PRINTREPORT))))