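; Blueprint function library of shared helpers for the Advanced Taming System (ATS), covering player HUD setup and companion naming.
; Each function looks up components on the given player and checks validity before acting.
; HUD creation passes prey and predator bait amounts from the taming component, or zeros without one, and another helper updates displayed HP.
; Renaming follows the taming component's companion reference to set the name and trigger a change notification.
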(fn FnCreateHUDATS
  (params (Player :type Pawn%20Object%20Reference))
  (LocalVariables|SetRef Player)
  ;[1 1 1] Do we have component PlayerHUD?
  (Utilities|IsValid (Actor|GetComponentbyClass (LocalVariables|GetRef) "/Game/AdvancedTaming/Blueprints/Characters/Player/Components/BP_Comp_PlayerHUD_ATS.BP_Comp_PlayerHUD_ATS_C")
    (:Is%20Valid
      ;[1 1 1] Do we have component PlayeCanTame
      (Utilities|IsValid (Actor|GetComponentbyClass (LocalVariables|GetRef) "/Game/AdvancedTaming/Blueprints/Characters/Player/Components/BP_Comp_PlayerCanTame.BP_Comp_PlayerCanTame_C")
        (:Is%20Valid
          ;[1 1 1] Create HUD
          (Default|FnCreateHUD (Actor|GetComponentbyClass (LocalVariables|GetRef) "/Game/AdvancedTaming/Blueprints/Characters/Player/Components/BP_Comp_PlayerHUD_ATS.BP_Comp_PlayerHUD_ATS_C") (Variables|/Game/AdvancedTaming/Blueprints/Characters/Player/Components/BP_Comp_PlayerCanTame.BP_Comp_PlayerCanTame_C|GetPreyBaitAmount (Actor|GetComponentbyClass (LocalVariables|GetRef) "/Game/AdvancedTaming/Blueprints/Characters/Player/Components/BP_Comp_PlayerCanTame.BP_Comp_PlayerCanTame_C")) (Variables|/Game/AdvancedTaming/Blueprints/Characters/Player/Components/BP_Comp_PlayerCanTame.BP_Comp_PlayerCanTame_C|GetPredatorBaitAmount (Actor|GetComponentbyClass (LocalVariables|GetRef) "/Game/AdvancedTaming/Blueprints/Characters/Player/Components/BP_Comp_PlayerCanTame.BP_Comp_PlayerCanTame_C"))))
        (:Is%20Not%20Valid
          ;[1 1 1] Create HUD
          (Default|FnCreateHUD (Actor|GetComponentbyClass (LocalVariables|GetRef) "/Game/AdvancedTaming/Blueprints/Characters/Player/Components/BP_Comp_PlayerHUD_ATS.BP_Comp_PlayerHUD_ATS_C")))))))

(fn FnSetHUDPlayerHP
  (params (Player :type Pawn%20Object%20Reference) (New%20HP :type Float%20%28single-precision%29))
  (bind _returnvalue (Actor|GetComponentbyClass Player "/Game/AdvancedTaming/Blueprints/Characters/Player/Components/BP_Comp_PlayerHUD_ATS.BP_Comp_PlayerHUD_ATS_C"))
  (bind _playerhudref (Variables|/Game/AdvancedTaming/Blueprints/Characters/Player/Components/BP_Comp_PlayerHUD_ATS.BP_Comp_PlayerHUD_ATS_C|GetPlayerHUDRef _returnvalue))
  (if (and (Utilities|IsValid _returnvalue) (Utilities|IsValid _playerhudref))
    (Default|FnSetPlayerHP _playerhudref New%20HP)))

(fn FnSetCompanionNameATS
  (params (Player :type Pawn%20Object%20Reference) (Name :type Text))
  (bind _returnvalue (Actor|GetComponentbyClass Player "/Game/AdvancedTaming/Blueprints/Characters/Player/Components/BP_Comp_PlayerCanTame.BP_Comp_PlayerCanTame_C"))
  (bind _companionref (Variables|/Game/AdvancedTaming/Blueprints/Characters/Player/Components/BP_Comp_PlayerCanTame.BP_Comp_PlayerCanTame_C|GetCompanionRef _returnvalue))
  (bind _returnvalue_2 (Actor|GetComponentbyClass _companionref "/Game/AdvancedTaming/Blueprints/AI/Components/GroundAnimals/BP_Comp_Companion.BP_Comp_Companion_C"))
  (Utilities|IsValid _returnvalue
    (:Is%20Valid
      (Utilities|IsValid _companionref
        (:Is%20Valid
          (Utilities|IsValid _returnvalue_2
            (:Is%20Valid
              (Default|FnSetCompanionName _returnvalue_2 Name)
              (Default|FnNotifyNameChange _returnvalue_2))))))))