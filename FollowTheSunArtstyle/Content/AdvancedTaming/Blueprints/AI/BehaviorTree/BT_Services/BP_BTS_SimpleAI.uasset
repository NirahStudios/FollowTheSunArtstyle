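; Behavior tree service that syncs a simple ground animal's state to the Blackboard for its AI.
; Each AI tick stores the controller and pawn, and a DoOnce casts the pawn to BP_SimpleGroundAnimal to cache the reference.
; It then copies the animal's Engaged and MoveAround flags into the Engaged and CanMove keys.
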(event EventReceiveTickAI
  (params (OwnerController :type AI%20Controller%20Object%20Reference) (ControlledPawn :type Pawn%20Object%20Reference) (DeltaSeconds :type Float%20%28single-precision%29))
  (Variables|Default|SetAIController OwnerController)
  (Variables|Default|SetPawnRef ControlledPawn)
  (Utilities|FlowControl|Sequence
    (:then_0
      (Utilities|FlowControl|DoOnce false
        (:Completed
          (bind _asbp_simple_ground_animal (Utilities|Casting|CastToBP_SimpleGroundAnimal (Variables|Default|GetPawnRef)))
          (Variables|Default|SetGroundAnimal _asbp_simple_ground_animal))))
    (:then_1
      ;[1 1 1] Set BB value for Engaged
      (Class|BTFunctionLibrary|SetBlackboardValueasBool (Variables|Setup|GetEngaged) (Variables|/Game/AdvancedTaming/Blueprints/Characters/Animals/GroundAnimals/BP_SimpleGroundAnimal.BP_SimpleGroundAnimal_C|GetEngaged (Variables|Default|GetGroundAnimal)))
      ;[1 1 1] Set BB value for CanMove
      (Class|BTFunctionLibrary|SetBlackboardValueasBool (Variables|Setup|GetCanMove) (Variables|/Game/AdvancedTaming/Blueprints/Characters/Animals/GroundAnimals/BP_SimpleGroundAnimal.BP_SimpleGroundAnimal_C|GetMoveAround (Variables|Default|GetGroundAnimal))))))