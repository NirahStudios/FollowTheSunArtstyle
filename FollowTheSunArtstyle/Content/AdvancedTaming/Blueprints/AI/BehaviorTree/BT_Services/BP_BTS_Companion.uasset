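; Behavior tree service that syncs a tamed companion's current command to the AI blackboard.
; On first tick it caches the pawn's companion component and writes its owner to the blackboard.
; Each tick it maps the component's task to the CurrentTask key, stopping movement for Stay in Place.
; Waiting and StayOnce flags make stay start and end messages to the pawn fire only on transitions.
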(event EventReceiveTickAI
  (params (OwnerController :type AI%20Controller%20Object%20Reference) (ControlledPawn :type Pawn%20Object%20Reference) (DeltaSeconds :type Float%20%28single-precision%29))
  (Variables|Default|SetAIController OwnerController)
  (Variables|Default|SetPawnRef ControlledPawn)
  (Utilities|FlowControl|Sequence
    (:then_0
      (Utilities|FlowControl|DoOnce false
        (:Completed
          (Utilities|IsValid (Actor|GetComponentbyClass (Variables|Default|GetPawnRef) "/Game/AdvancedTaming/Blueprints/AI/Components/GroundAnimals/BP_Comp_Companion.BP_Comp_Companion_C")
            (:Is%20Valid
              (Variables|Default|SetCompanion (Actor|GetComponentbyClass (Variables|Default|GetPawnRef) "/Game/AdvancedTaming/Blueprints/AI/Components/GroundAnimals/BP_Comp_Companion.BP_Comp_Companion_C"))
              ;[1 1 1] Set Owner
              (Utilities|IsValid (Actor|GetComponentbyClass (Variables|Default|GetPawnRef) "/Game/AdvancedTaming/Blueprints/AI/Components/GroundAnimals/BP_Comp_Companion.BP_Comp_Companion_C")
                (:Is%20Valid
                  (Variables|Default|SetOwnerRef (Variables|/Game/AdvancedTaming/Blueprints/AI/Components/GroundAnimals/BP_Comp_Companion.BP_Comp_Companion_C|GetOwnerRef (Actor|GetComponentbyClass (Variables|Default|GetPawnRef) "/Game/AdvancedTaming/Blueprints/AI/Components/GroundAnimals/BP_Comp_Companion.BP_Comp_Companion_C")))
                  ;[1 1 1] Set BB value for Owner
                  (Class|BTFunctionLibrary|SetBlackboardValueasObject (Variables|Setup|GetOwner) (Variables|Default|GetOwnerRef)))))))))
    (:then_1
      (CallFunction|FnSetAITask))))

(fn FnSetAITask
  (switch Utilities|FlowControl|Switch|SwitchonBP_Enum_CompanionTasksATS (Variables|/Game/AdvancedTaming/Blueprints/AI/Components/GroundAnimals/BP_Comp_Companion.BP_Comp_Companion_C|GetCompanionTasks (Variables|Default|GetCompanion))
    (:NewEnumerator0
      ;[1 1 1] Set Current Task to Follow Owner
      (Class|BTFunctionLibrary|SetBlackboardValueasEnum (Variables|Setup|GetCurrentTask) (Utilities|Enum|LiteralenumBP_Enum_CompanionTasksATS "NewEnumerator0"))
      ;[1 1 1] Check if animal was waiting before (command 2)
      (if (Variables|Default|GetWaiting)
        (Variables|Default|SetWaiting false)
        (Variables|Default|SetStayOnce true)
        ;[1 1 1] Fire custom event CompanionStayEnd
        (Class|BPIATSGroundAnimal|FnCompanionStayEndATS(Message) (Variables|Default|GetPawnRef))))
    (:NewEnumerator1
      ;[1 1 1] Set Current Task to Stay In Place
      (Class|BTFunctionLibrary|SetBlackboardValueasEnum (Variables|Setup|GetCurrentTask) (Utilities|Enum|LiteralenumBP_Enum_CompanionTasksATS "NewEnumerator1"))
      ;[1 1 1] Stop AI movement immediately
      (AI|Navigation|StopMovement (Variables|Default|GetAIController))
      ;[1 1 1] Check if animal was waiting before (command 2)
      (if (Variables|Default|GetStayOnce)
        (Variables|Default|SetStayOnce false)
        (Variables|Default|SetWaiting true)
        ;[1 1 1] Fire custom event CompanionStayStart
        (Class|BPIATSGroundAnimal|FnCompanionStayStartATS(Message) (Variables|Default|GetPawnRef))))
    (:NewEnumerator2
      ;[1 1 1] Set Current Task to Go to Location and Wait
      (Class|BTFunctionLibrary|SetBlackboardValueasEnum (Variables|Setup|GetCurrentTask) (Utilities|Enum|LiteralenumBP_Enum_CompanionTasksATS "NewEnumerator2"))
      ;[1 1 1] Check if animal was waiting before (command 2)
      (if (Variables|Default|GetWaiting)
        (Variables|Default|SetWaiting false)
        (Variables|Default|SetStayOnce true)
        ;[1 1 1] Fire custom event CompanionStayEnd
        (Class|BPIATSGroundAnimal|FnCompanionStayEndATS(Message) (Variables|Default|GetPawnRef))))
    (:NewEnumerator3
      ;[1 1 1] Set Current Task to Attack
      (Class|BTFunctionLibrary|SetBlackboardValueasEnum (Variables|Setup|GetCurrentTask) (Utilities|Enum|LiteralenumBP_Enum_CompanionTasksATS "NewEnumerator3"))
      ;[1 1 1] Check if animal was waiting before (command 2)
      (if (Variables|Default|GetWaiting)
        (Variables|Default|SetWaiting false)
        (Variables|Default|SetStayOnce true)
        ;[1 1 1] Fire custom event CompanionStayEnd
        (Class|BPIATSGroundAnimal|FnCompanionStayEndATS(Message) (Variables|Default|GetPawnRef))))
    (:NewEnumerator4
      ;[1 1 1] Set Current Task to Leave
      (Class|BTFunctionLibrary|SetBlackboardValueasEnum (Variables|Setup|GetCurrentTask) (Utilities|Enum|LiteralenumBP_Enum_CompanionTasksATS "NewEnumerator4")))))

(fn OnRepTasks)

(fn OnRepWaiting)

(fn OnRepStayOnce)