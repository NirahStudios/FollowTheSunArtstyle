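; Behavior tree task that makes a simple ground animal wander to a random navigable point and then idle.
; It reads the acceptance radius from the pawn through an ATS message call, and the search radius and idle time from BP_SimpleGroundAnimal.
; A successful move finishes the task after the idle delay, while a failed move fails it immediately.
; Pawns of other classes stop at the cast without finishing the task.
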(event EventReceiveExecuteAI
  (params (OwnerController :type AI%20Controller%20Object%20Reference) (ControlledPawn :type Pawn%20Object%20Reference))
  (Variables|Default|SetPawnRef ControlledPawn)
  ;[1 1 1] Set Acceptance Radius
  (bind _radius (Class|BPIATSGroundAnimal|FnGetMovementAcceptanceRadiusATS(Message) (Variables|Default|GetPawnRef)))
  (Variables|Default|SetAcceptanceRadius _radius)
  ;[1 1 1] Get Search Radius
  (bind _asbp_simple_ground_animal (Utilities|Casting|CastToBP_SimpleGroundAnimal (Variables|Default|GetPawnRef)))
  (Variables|Default|SetGroundAnimal _asbp_simple_ground_animal)
  ;[1 1 1] Set Search Radius
  (Variables|Default|SetRadius (Variables|/Game/AdvancedTaming/Blueprints/Characters/Animals/GroundAnimals/BP_SimpleGroundAnimal.BP_SimpleGroundAnimal_C|GetSearchRadius (Variables|Default|GetGroundAnimal)))
  ;[1 1 1] Set Idle time
  (Variables|Default|SetIdle (Variables|/Game/AdvancedTaming/Blueprints/Characters/Animals/GroundAnimals/BP_SimpleGroundAnimal.BP_SimpleGroundAnimal_C|GetIdleTime (Variables|Default|GetGroundAnimal)))
  ;[1 1 1] Get new random location
  (Variables|Default|SetRandomLocation (.RandomLocation (Class|NavigationSystem|GetRandomPointinNavigableRadius (Transformation|GetActorLocation (Variables|Default|GetPawnRef)) (Variables|Default|GetRadius))))
  ;[1 1 1] Move to random location
  (AI|AIMoveTo (Variables|Default|GetPawnRef) (Variables|Default|GetRandomLocation) 0 (Variables|Default|GetAcceptanceRadius) true
    (:OnSuccess
      ;[1 1 1] Wait Idle seconds
      (Utilities|FlowControl|Delay (Variables|Default|GetIdle))
      (AI|BehaviorTree|FinishExecute true))
    (:OnFail
      (AI|BehaviorTree|FinishExecute false))))