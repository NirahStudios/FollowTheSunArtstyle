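; Behavior tree task that makes a companion animal attack its Engage Actor from the blackboard.
; On execute it sets the attacking state, plays the attack montage, waits out its length plus the attack frequency, then finishes.
; A dead or missing target ends attacking and resets the companion to Follow, highlighting that command in the owner's HUD.
; On tick it moves toward the target and smoothly yaws to face it.
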(event EventReceiveExecuteAI
  (params (OwnerController :type AI%20Controller%20Object%20Reference) (ControlledPawn :type Pawn%20Object%20Reference))
  (Variables|Default|SetPawnRef ControlledPawn)
  ;[1 1 1] Check animal has Companion component
  (Utilities|IsValid (Actor|GetComponentbyClass (Variables|Default|GetPawnRef) "/Game/AdvancedTaming/Blueprints/AI/Components/GroundAnimals/BP_Comp_Companion.BP_Comp_Companion_C")
    (:Is%20Valid
      (Variables|Default|SetCompanion (Actor|GetComponentbyClass (Variables|Default|GetPawnRef) "/Game/AdvancedTaming/Blueprints/AI/Components/GroundAnimals/BP_Comp_Companion.BP_Comp_Companion_C"))
      ;[1 1 1] Set Acceptance Radius
      (bind _radius (Class|BPIATSGroundAnimal|FnGetMovementAcceptanceRadiusATS(Message) (Variables|Default|GetPawnRef)))
      (Variables|Default|SetAcceptanceRadius _radius)
      ;[1 1 1] Set DisengageCD
      (bind _disengagecd (Class|BPIATSGroundAnimal|FnGetDisengageCDATS(Message) (Variables|Default|GetPawnRef)))
      (Variables|Default|SetDisengageCD _disengagecd)
      ;[1 1 1] Check Engage Actor is Valid
      (Utilities|IsValid (AI|BehaviorTree|GetBlackboardValueasActor (Variables|Setup|GetEngageActor))
        (:Is%20Valid
          ;[1 1 1] Check that Engage Actor is NOT Dead
          (if (not (Actor|ActorHasTag (AI|BehaviorTree|GetBlackboardValueasActor (Variables|Setup|GetEngageActor)) "abkDead"))
            ;[1 1 1] Set State to Attacking
            (Class|BPIATSGroundAnimal|FnSetStateAttackingATS(Message) (Variables|Default|GetPawnRef) true)
            ;[1 1 1] Fire custom event
            (Class|BPIATSGroundAnimal|FnCompanionAttackStartATS(Message) (Variables|Default|GetPawnRef))
            ;[1 1 1] Play Attacking animation
            (Class|BPIATSGroundAnimal|FnPlayAttackAnimationATS(Message) (Variables|Default|GetPawnRef))
            ;[1 1 1] Wait for the attack animation duration
            (bind _montage (Class|BPIATSGroundAnimal|FnGetCurrentMontageATS(Message) (Variables|Default|GetPawnRef)))
            (Utilities|IsValid _montage
              (:Is%20Valid
                (bind _returnvalue (Animation|GetPlayLength _montage))
                (Utilities|FlowControl|Delay _returnvalue))
              (:Is%20Not%20Valid
                _))
            ;[1 1 1] Stop attacking
            (Class|BPIATSGroundAnimal|FnSetStateAttackingATS(Message) (Variables|Default|GetPawnRef) false)
            ;[1 1 1] Fire custom event
            (Class|BPIATSGroundAnimal|FnCompanionAttackEndATS(Message) (Variables|Default|GetPawnRef))
            ;[1 1 1] Wait AttackFrequency before stopping the attack
            (bind _frequency (Class|BPIATSGroundAnimal|FnGetAttackFrequencyATS(Message) (Variables|Default|GetPawnRef)))
            (Utilities|FlowControl|Delay _frequency)
            (AI|BehaviorTree|FinishExecute true)
            (else
              ;[1 1 1] Check animal has NeedSystem component
              (Class|BPIATSGroundAnimal|FnFinishedEatingATS(Message) (Variables|Default|GetPawnRef))
              ;[1 1 1] Engage Actor is dead - Disengage
              (Class|BPIATSGroundAnimal|FnDisengageAnimalATS(Message) (Variables|Default|GetPawnRef))
              ;[1 1 1] Stop attacking
              (Class|BPIATSGroundAnimal|FnSetStateAttackingATS(Message) (Variables|Default|GetPawnRef) false)
              ;[1 1 1] Reset Task to Follow Owner
              (Variables|/Game/AdvancedTaming/Blueprints/AI/Components/GroundAnimals/BP_Comp_Companion.BP_Comp_Companion_C|SetCompanionTasks (Variables|Default|GetCompanion) "NewEnumerator0")
              ;[1 1 1] Highlight Follow Command in the Player's HUD
              (Utilities|IsValid (Actor|GetComponentbyClass (Variables|/Game/AdvancedTaming/Blueprints/AI/Components/GroundAnimals/BP_Comp_Companion.BP_Comp_Companion_C|GetOwnerRef (Variables|Default|GetCompanion)) "/Game/AdvancedTaming/Blueprints/Characters/Player/Components/BP_Comp_PlayerHUD_ATS.BP_Comp_PlayerHUD_ATS_C")
                (:Is%20Valid
                  (Default|FnHighlightHUDCommand (Actor|GetComponentbyClass (Variables|/Game/AdvancedTaming/Blueprints/AI/Components/GroundAnimals/BP_Comp_Companion.BP_Comp_Companion_C|GetOwnerRef (Variables|Default|GetCompanion)) "/Game/AdvancedTaming/Blueprints/Characters/Player/Components/BP_Comp_PlayerHUD_ATS.BP_Comp_PlayerHUD_ATS_C") 1))
                (:Is%20Not%20Valid
                  _))
              (AI|BehaviorTree|FinishExecute true))))
        (:Is%20Not%20Valid
          ;[1 1 1] Stop attacking
          (Class|BPIATSGroundAnimal|FnSetStateAttackingATS(Message) (Variables|Default|GetPawnRef) false)
          ;[1 1 1] Reset Task to Follow Owner
          (Variables|/Game/AdvancedTaming/Blueprints/AI/Components/GroundAnimals/BP_Comp_Companion.BP_Comp_Companion_C|SetCompanionTasks (Variables|Default|GetCompanion) "NewEnumerator0")
          ;[1 1 1] Highlight Follow Command in the Player's HUD
          (Utilities|IsValid (Actor|GetComponentbyClass (Variables|/Game/AdvancedTaming/Blueprints/AI/Components/GroundAnimals/BP_Comp_Companion.BP_Comp_Companion_C|GetOwnerRef (Variables|Default|GetCompanion)) "/Game/AdvancedTaming/Blueprints/Characters/Player/Components/BP_Comp_PlayerHUD_ATS.BP_Comp_PlayerHUD_ATS_C")
            (:Is%20Valid
              (Default|FnHighlightHUDCommand (Actor|GetComponentbyClass (Variables|/Game/AdvancedTaming/Blueprints/AI/Components/GroundAnimals/BP_Comp_Companion.BP_Comp_Companion_C|GetOwnerRef (Variables|Default|GetCompanion)) "/Game/AdvancedTaming/Blueprints/Characters/Player/Components/BP_Comp_PlayerHUD_ATS.BP_Comp_PlayerHUD_ATS_C") 1))
            (:Is%20Not%20Valid
              _))
          (AI|BehaviorTree|FinishExecute true))))))

(event EventReceiveTickAI
  (params (OwnerController :type AI%20Controller%20Object%20Reference) (ControlledPawn :type Pawn%20Object%20Reference) (DeltaSeconds :type Float%20%28single-precision%29))
  (bind _pawnref (Variables|Default|GetPawnRef))
  (bind _returnvalue (Transformation|GetActorRotation _pawnref))
  (bind (_roll _pitch) (Math|Rotator|BreakRotator _returnvalue))
  ;[1 1 1] Check Engage Actor is Valid
  (Utilities|IsValid (AI|BehaviorTree|GetBlackboardValueasActor (Variables|Setup|GetEngageActor))
    (:Is%20Valid
      ;[1 1 1] Set actor location to EngageActor
      (AI|AIMoveTo (Variables|Default|GetPawnRef) "0, 0, 0" (AI|BehaviorTree|GetBlackboardValueasActor (Variables|Setup|GetEngageActor)) (* (Variables|Default|GetAcceptanceRadius) 0.25) true
        (:then
          ;[1 1 1] Rotate towards target
          (Transformation|SetActorRotation (Variables|Default|GetPawnRef) (Math|Interpolation|RInterpTo _returnvalue (Math|Rotator|MakeRotator _roll _pitch (.yaw (Math|Rotator|FindLookatRotation (Transformation|GetActorLocation (Variables|Default|GetPawnRef)) (Transformation|GetActorLocation (AI|BehaviorTree|GetBlackboardValueasActor (Variables|Setup|GetEngageActor)))))) (Utilities|Time|GetWorldDeltaSeconds) 2.0)))))))