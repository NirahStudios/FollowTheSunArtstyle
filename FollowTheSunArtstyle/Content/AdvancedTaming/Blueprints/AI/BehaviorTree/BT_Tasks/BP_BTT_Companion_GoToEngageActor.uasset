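; Behavior tree task that moves an AI companion toward its blackboard engage actor until it is within attack range.
; AIMoveTo heads for the actor's location at task start, using a pawn-supplied acceptance radius and updating the Moving key.
; A fast looping timer replaces tick, sphere-tracing around the pawn's attack volume and finishing successfully once the target is hit.
; The range check also computes the target's speed, which goes unused here.
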(event Custom|EventTickReplacement
  (bind _returnvalue (Utilities|Time|SetTimerbyEvent (delegate Custom|EventTickReplacement) 0.01 true))
  (Variables|Default|SetTickHandler _returnvalue)
  ;[1 1 1] Check if we are in melee range
  (if (.Range (CallFunction|FnGetTargetSpeed))
    (AI|BehaviorTree|FinishExecute true)))

(event EventReceiveExecuteAI
  (params (OwnerController :type AI%20Controller%20Object%20Reference) (ControlledPawn :type Pawn%20Object%20Reference))
  (Variables|Default|SetPawnRef ControlledPawn)
  ;[1 1 1] Set Acceptance Radius
  (bind _radius (Class|BPIATSGroundAnimal|FnGetMovementAcceptanceRadiusATS(Message) (Variables|Default|GetPawnRef)))
  (Variables|Default|SetAcceptanceRadius _radius)
  ;[1 1 1] Check Engage Actor is Valid
  (Utilities|IsValid (AI|BehaviorTree|GetBlackboardValueasActor (Variables|Setup|GetEngageActor))
    (:Is%20Valid
      (CallFunction|EventTickReplacement)
      ;[1 1 1] Move towards Engage Actor
      (AI|AIMoveTo (Variables|Default|GetPawnRef) (Transformation|GetActorLocation (AI|BehaviorTree|GetBlackboardValueasActor (Variables|Setup|GetEngageActor))) 0 (Variables|Default|GetAcceptanceRadius) true
        (:then
          ;;[1 1 1] Set Moving to True
          (Class|BTFunctionLibrary|SetBlackboardValueasBool (Variables|Default|GetMoving) true))
        (:OnSuccess
          ;;[1 1 1] Set Moving to False
          (Class|BTFunctionLibrary|SetBlackboardValueasBool (Variables|Default|GetMoving) false)
          (AI|BehaviorTree|FinishExecute true))
        (:OnFail
          ;;[1 1 1] Set Moving to False
          (Class|BTFunctionLibrary|SetBlackboardValueasBool (Variables|Default|GetMoving) false)
          (AI|BehaviorTree|FinishExecute false))))))

(fn FnGetTargetSpeed
  (Utilities|FlowControl|Sequence
    (:then_0
      ;[1 1 1] Check if we are in attack range with target
      (bind _object_types (Class|BPIATSGroundAnimal|FnGetDamageObjectTypesATS(Message) (Variables|Default|GetPawnRef)))
      (bind _collision_attack (Class|BPIATSGroundAnimal|FnGetCollisionAttackVolumeATS(Message) (Variables|Default|GetPawnRef)))
      (bind (_outhits _returnvalue) (Collision|MultiSphereTraceForObjects (Transformation|GetWorldLocation _collision_attack) (+ (Transformation|GetWorldLocation _collision_attack) "0, 0,0.010000") (* (Variables|/Script/Engine.SphereComponent|GetSphereRadius _collision_attack) (Variables|Default|GetCollisionRadiusMultiplier)) _object_types false (Utilities|Array|MakeArray (Variables|Default|GetPawnRef)) (LocalVariables|GetDebugType)))
      (if _returnvalue
        (bind _array_element (Utilities|Array|ForEachLoopwithBreak _outhits :!label _label)
          (:LoopBody
            (if (== (AI|BehaviorTree|GetBlackboardValueasActor (Variables|Setup|GetEngageActor)) (.HitActor (Collision|BreakHitResult _array_element)))
              (LocalVariables|SetInRange true)
              (goto _label Break))))))
    (:then_1
      (if (LocalVariables|GetInRange)
        ;[1 1 1] Get EngageActor's speed and set it for this animal
        (LocalVariables|SetSpeed (Math|Vector|VectorLength (Transformation|GetVelocity (AI|BehaviorTree|GetBlackboardValueasActor (Variables|Setup|GetEngageActor)))))))
    (:then_2
      (return (LocalVariables|GetInRange) (LocalVariables|GetSpeed)))))