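; Behavior tree task that makes a BP_SimpleGroundAnimal attack its engage target.
; On execute it resets aggro, then attacks through pawn interface messages, waiting out the montage and attack frequency before finishing.
; A target tagged dead triggers disengage, while an invalid one just clears the attacking state.
; Each tick reissues AIMoveTo at a quarter of the acceptance radius and smoothly yaws the pawn toward the target.
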(event EventReceiveExecuteAI
  (params (OwnerController :type AI%20Controller%20Object%20Reference) (ControlledPawn :type Pawn%20Object%20Reference))
  (Variables|Default|SetPawnRef ControlledPawn)
  (bind _asbp_simple_ground_animal (Utilities|Casting|CastToBP_SimpleGroundAnimal (Variables|Default|GetPawnRef)))
  (Variables|Default|SetGroundAnimal _asbp_simple_ground_animal)
  (Variables|Default|SetEngageTarget (Variables|/Game/AdvancedTaming/Blueprints/Characters/Animals/GroundAnimals/BP_SimpleGroundAnimal.BP_SimpleGroundAnimal_C|GetEngageTarget (Variables|Default|GetGroundAnimal)))
  ;[1 1 1] Reset Aggro counter
  (Variables|/Game/AdvancedTaming/Blueprints/Characters/Animals/GroundAnimals/BP_SimpleGroundAnimal.BP_SimpleGroundAnimal_C|SetAggroCounter (Variables|Default|GetGroundAnimal) 0.0)
  ;[1 1 1] Set Acceptance Radius
  (bind _radius (Class|BPIATSGroundAnimal|FnGetMovementAcceptanceRadiusATS(Message) (Variables|Default|GetPawnRef)))
  (Variables|Default|SetAcceptanceRadius _radius)
  ;[1 1 1] Set DisengageCD
  (bind _disengagecd (Class|BPIATSGroundAnimal|FnGetDisengageCDATS(Message) (Variables|Default|GetPawnRef)))
  (Variables|Default|SetDisengageCD _disengagecd)
  ;[1 1 1] Check Engage Actor is Valid
  (Utilities|IsValid (Variables|Default|GetEngageTarget)
    (:Is%20Valid
      ;[1 1 1] Check that Engage Actor is NOT Dead
      (if (not (Actor|ActorHasTag (Variables|Default|GetEngageTarget) "abkDead"))
        ;[1 1 1] Set State to Attacking
        (Class|BPIATSGroundAnimal|FnSetStateAttackingATS(Message) (Variables|Default|GetPawnRef) true)
        ;[1 1 1] Fire custom event
        (Class|BPIATSGroundAnimal|FnCompanionAttackStartATS(Message) (Variables|Default|GetPawnRef))
        ;[1 1 1] Play Attacking animation
        (Class|BPIATSGroundAnimal|FnPlayAttackAnimationATS(Message) (Variables|Default|GetPawnRef))
        ;[1 1 1] Wait for the attack animation duration
        (bind _montage (Class|BPIATSGroundAnimal|FnGetCurrentMontageATS(Message) (Variables|Default|GetPawnRef)))
        (Utilities|IsValid _montage
          (:Is%20Valid
            (bind _returnvalue (Animation|GetPlayLength _montage))
            (Utilities|FlowControl|Delay _returnvalue))
          (:Is%20Not%20Valid
            _))
        ;[1 1 1] Stop attacking
        (Class|BPIATSGroundAnimal|FnSetStateAttackingATS(Message) (Variables|Default|GetPawnRef) false)
        ;[1 1 1] Fire custom event
        (Class|BPIATSGroundAnimal|FnCompanionAttackEndATS(Message) (Variables|Default|GetPawnRef))
        ;[1 1 1] Wait AttackFrequency before stopping the attack
        (bind _frequency (Class|BPIATSGroundAnimal|FnGetAttackFrequencyATS(Message) (Variables|Default|GetPawnRef)))
        (Utilities|FlowControl|Delay _frequency)
        (AI|BehaviorTree|FinishExecute true)
        (else
          ;[1 1 1] Engage Actor is dead - Disengage
          (Class|BPIATSGroundAnimal|FnDisengageAnimalATS(Message) (Variables|Default|GetPawnRef))
          ;[1 1 1] Stop attacking
          (Class|BPIATSGroundAnimal|FnSetStateAttackingATS(Message) (Variables|Default|GetPawnRef) false)
          (AI|BehaviorTree|FinishExecute true))))
    (:Is%20Not%20Valid
      ;[1 1 1] Stop attacking
      (Class|BPIATSGroundAnimal|FnSetStateAttackingATS(Message) (Variables|Default|GetPawnRef) false)
      (AI|BehaviorTree|FinishExecute true))))

(event EventReceiveTickAI
  (params (OwnerController :type AI%20Controller%20Object%20Reference) (ControlledPawn :type Pawn%20Object%20Reference) (DeltaSeconds :type Float%20%28single-precision%29))
  (bind _pawnref (Variables|Default|GetPawnRef))
  (bind _returnvalue (Transformation|GetActorRotation _pawnref))
  (bind (_roll _pitch) (Math|Rotator|BreakRotator _returnvalue))
  ;[1 1 1] Check Engage Actor is Valid
  (Utilities|IsValid (Variables|Default|GetEngageTarget)
    (:Is%20Valid
      ;[1 1 1] Set actor location to EngageActor
      (AI|AIMoveTo (Variables|Default|GetPawnRef) "0, 0, 0" (Variables|Default|GetEngageTarget) (* (Variables|Default|GetAcceptanceRadius) 0.25) true
        (:then
          ;[1 1 1] Rotate towards target
          (Transformation|SetActorRotation (Variables|Default|GetPawnRef) (Math|Interpolation|RInterpTo _returnvalue (Math|Rotator|MakeRotator _roll _pitch (.yaw (Math|Rotator|FindLookatRotation (Transformation|GetActorLocation (Variables|Default|GetPawnRef)) (Transformation|GetActorLocation (Variables|Default|GetEngageTarget))))) (Utilities|Time|GetWorldDeltaSeconds) 2.0)))))))