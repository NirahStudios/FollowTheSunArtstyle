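; Behavior tree task that sends a tamed companion animal to a commanded blackboard location or hit actor.
; It gets the acceptance radius from the pawn via message, then runs AI MoveTo and fires start and end events on the pawn.
; On success it notifies the companion component, sets the animal to stay in place and highlights a HUD command.
; On failure it reports the failed movement to the component and fails the task.
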(event EventReceiveExecuteAI
  (params (OwnerController :type AI%20Controller%20Object%20Reference) (ControlledPawn :type Pawn%20Object%20Reference))
  (Variables|Default|SetPawnRef ControlledPawn)
  ;[1 1 1] Set Acceptance Radius
  (bind _radius (Class|BPIATSGroundAnimal|FnGetMovementAcceptanceRadiusATS(Message) (Variables|Default|GetPawnRef)))
  (Variables|Default|SetAcceptanceRadius _radius)
  ;[1 1 1] Check animal has Companion component
  (Utilities|IsValid (Variables|Default|GetPawnRef)
    (:Is%20Valid
      (Utilities|IsValid (Actor|GetComponentbyClass (Variables|Default|GetPawnRef) "/Game/AdvancedTaming/Blueprints/AI/Components/GroundAnimals/BP_Comp_Companion.BP_Comp_Companion_C")
        (:Is%20Valid
          (Variables|Default|SetCompanion (Actor|GetComponentbyClass (Variables|Default|GetPawnRef) "/Game/AdvancedTaming/Blueprints/AI/Components/GroundAnimals/BP_Comp_Companion.BP_Comp_Companion_C"))
          (AI|AIMoveTo (Variables|Default|GetPawnRef) (Class|BTFunctionLibrary|GetBlackboardValueasVector (Variables|Setup|GetTargetLocation)) (select (Utilities|IsValid (Variables|/Game/AdvancedTaming/Blueprints/AI/Components/GroundAnimals/BP_Comp_Companion.BP_Comp_Companion_C|GetHitActor (Variables|Default|GetCompanion))) (Variables|/Game/AdvancedTaming/Blueprints/AI/Components/GroundAnimals/BP_Comp_Companion.BP_Comp_Companion_C|GetHitActor (Variables|Default|GetCompanion)) 0) (Variables|Default|GetAcceptanceRadius) true
            (:then
              (if (Variables|Default|GetGoStart)
                (Variables|Default|SetGoStart false)
                ;[1 1 1] Fire custom events
                (Class|BPIATSGroundAnimal|FnCompanionGoLocStartATS(Message) (Variables|Default|GetPawnRef))))
            (:OnSuccess
              (Variables|Default|SetGoStart true)
              ;[1 1 1] Fire custom events
              (Class|BPIATSGroundAnimal|FnCompanionGoLocEndATS(Message) (Variables|Default|GetPawnRef))
              ;[1 1 1] Custom Event on Comp Companion
              (Default|EventArrivedatLocation (Variables|Default|GetCompanion))
              ;[1 1 1] Set animal to Stay in Place
              (Variables|/Game/AdvancedTaming/Blueprints/AI/Components/GroundAnimals/BP_Comp_Companion.BP_Comp_Companion_C|SetCompanionTasks (Variables|Default|GetCompanion) "NewEnumerator1")
              ;[1 1 1] Highlight Follow Command in the Player's HUD
              (Utilities|IsValid (Actor|GetComponentbyClass (Variables|/Game/AdvancedTaming/Blueprints/AI/Components/GroundAnimals/BP_Comp_Companion.BP_Comp_Companion_C|GetOwnerRef (Variables|Default|GetCompanion)) "/Game/AdvancedTaming/Blueprints/Characters/Player/Components/BP_Comp_PlayerHUD_ATS.BP_Comp_PlayerHUD_ATS_C")
                (:Is%20Valid
                  (Default|FnHighlightHUDCommand (Actor|GetComponentbyClass (Variables|/Game/AdvancedTaming/Blueprints/AI/Components/GroundAnimals/BP_Comp_Companion.BP_Comp_Companion_C|GetOwnerRef (Variables|Default|GetCompanion)) "/Game/AdvancedTaming/Blueprints/Characters/Player/Components/BP_Comp_PlayerHUD_ATS.BP_Comp_PlayerHUD_ATS_C") 2))
                (:Is%20Not%20Valid
                  _))
              (AI|BehaviorTree|FinishExecute true))
            (:OnFail
              (Default|FnMovementFailed (Variables|Default|GetCompanion))
              (AI|BehaviorTree|FinishExecute false))))))))

(fn FnGetTargetLocation
  (params (Initial%20Location :type Vector))
  (LocalVariables|SetLocation Initial%20Location)
  ;[1 1 1] Shoot a trace to hit the floor
  (Collision|LineTraceByChannel (+ (LocalVariables|GetLocation) "0, 0,20000.000000") (+ (+ (LocalVariables|GetLocation) "0, 0,20000.000000") (* (Math|Vector|GetUpVector "0, 0, 0") -4e+04)) "TraceTypeQuery1" true 0 "None" true "(R=1.000000,G=0.000000,B=0.000000,A=1.000000)" "(R=0.000000,G=1.000000,B=0.000000,A=1.000000)" 1e+01))