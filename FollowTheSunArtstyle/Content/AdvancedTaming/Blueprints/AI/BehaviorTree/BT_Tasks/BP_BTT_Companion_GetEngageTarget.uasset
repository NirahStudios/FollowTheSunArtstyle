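; Behavior tree task for the taming system that picks the engage target for a companion AI pawn.
; It reads the attack target from the pawn's companion component and writes it to the EngageActor blackboard key.
; If that target's name matches the pawn's own, it instead switches the companion to stay in place and highlights a command on the owner's HUD.
; The task only finishes, with success, when the companion component exists.
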(event EventReceiveExecuteAI
  (params (OwnerController :type AI%20Controller%20Object%20Reference) (ControlledPawn :type Pawn%20Object%20Reference))
  (Variables|Default|SetPawnRef ControlledPawn)
  ;[1 1 1] Check animal has Companion component
  (Utilities|IsValid (Actor|GetComponentbyClass (Variables|Default|GetPawnRef) "/Game/AdvancedTaming/Blueprints/AI/Components/GroundAnimals/BP_Comp_Companion.BP_Comp_Companion_C")
    (:Is%20Valid
      (Variables|Default|SetCompanion (Actor|GetComponentbyClass (Variables|Default|GetPawnRef) "/Game/AdvancedTaming/Blueprints/AI/Components/GroundAnimals/BP_Comp_Companion.BP_Comp_Companion_C"))
      ;[1 1 1] Check that the AttackTarget is NOT the Companion
      (if (Utilities|Enum|NotEqual(Enum) (Utilities|GetObjectName (Variables|/Game/AdvancedTaming/Blueprints/AI/Components/GroundAnimals/BP_Comp_Companion.BP_Comp_Companion_C|GetCompanionAttackTarget (Variables|Default|GetCompanion))) (Utilities|GetObjectName (Variables|Default|GetPawnRef)))
        ;[1 1 1] Set BB EngageActor to CompanionAttackTarget
        (Class|BTFunctionLibrary|SetBlackboardValueasObject (Variables|Setup|GetEngageActor) (Variables|/Game/AdvancedTaming/Blueprints/AI/Components/GroundAnimals/BP_Comp_Companion.BP_Comp_Companion_C|GetCompanionAttackTarget (Variables|Default|GetCompanion)))
        (else
          ;[1 1 1] Set animal to Stay in Place
          (Variables|/Game/AdvancedTaming/Blueprints/AI/Components/GroundAnimals/BP_Comp_Companion.BP_Comp_Companion_C|SetCompanionTasks (Variables|Default|GetCompanion) "NewEnumerator1")
          ;[1 1 1] Highlight Follow Command in the Player's HUD
          (Utilities|IsValid (Actor|GetComponentbyClass (Variables|/Game/AdvancedTaming/Blueprints/AI/Components/GroundAnimals/BP_Comp_Companion.BP_Comp_Companion_C|GetOwnerRef (Variables|Default|GetCompanion)) "/Game/AdvancedTaming/Blueprints/Characters/Player/Components/BP_Comp_PlayerHUD_ATS.BP_Comp_PlayerHUD_ATS_C")
            (:Is%20Valid
              (Default|FnHighlightHUDCommand (Actor|GetComponentbyClass (Variables|/Game/AdvancedTaming/Blueprints/AI/Components/GroundAnimals/BP_Comp_Companion.BP_Comp_Companion_C|GetOwnerRef (Variables|Default|GetCompanion)) "/Game/AdvancedTaming/Blueprints/Characters/Player/Components/BP_Comp_PlayerHUD_ATS.BP_Comp_PlayerHUD_ATS_C") 2))
            (:Is%20Not%20Valid
              _))))
      (AI|BehaviorTree|FinishExecute true))))