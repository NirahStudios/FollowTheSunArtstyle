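; Behavior Tree task that sends a wild AI with a companion component to bait and has it eat.
; A sphere trace around the pawn picks the first actor tagged as bait, then the pawn moves to it.
; Eating sets a tag and flag for the component's eating time, even when no bait is found.
; Unless tamed by then, it clears both, destroys the component's bait reference and resets Engaged.
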(event EventReceiveExecuteAI
  (params (OwnerController :type AI%20Controller%20Object%20Reference) (ControlledPawn :type Pawn%20Object%20Reference))
  (Variables|Default|SetPawnRef ControlledPawn)
  ;[1 1 1] Check if we have Comp_Companion
  (Utilities|IsValid (Actor|GetComponentbyClass (Variables|Default|GetPawnRef) "/Game/AdvancedTaming/Blueprints/AI/Components/GroundAnimals/BP_Comp_Companion.BP_Comp_Companion_C")
    (:Is%20Valid
      ;[1 1 1] Save Companion
      (Variables|Default|SetCompanion (Actor|GetComponentbyClass (Variables|Default|GetPawnRef) "/Game/AdvancedTaming/Blueprints/AI/Components/GroundAnimals/BP_Comp_Companion.BP_Comp_Companion_C"))
      ;[1 1 1] Get nearest food source and Move AI to that location
      (bind (_found_bait _bait) (CallFunction|FnGetBait))
      (if _found_bait
        (AI|AIMoveTo (Variables|Default|GetPawnRef) (Transformation|GetActorLocation _bait) 0 5e+01 true
          (:OnSuccess
            _)))
      ;[1 1 1] Add tag 'EatingBait'
      (Utilities|Array|Add (Variables|/Script/Engine.Actor|GetTags (Variables|Default|GetPawnRef)) "abkEatingBait")
      ;[1 1 1] Set EatingBait as True
      (Variables|/Game/AdvancedTaming/Blueprints/AI/Components/GroundAnimals/BP_Comp_Companion.BP_Comp_Companion_C|SetEatingBait (Variables|Default|GetCompanion) true)
      ;[1 1 1] Wait BaitEatingTime seconds
      (Utilities|FlowControl|Delay (Utilities|Struct|BreakBP_Struct_Companion_BaitATS (Variables|/Game/AdvancedTaming/Blueprints/AI/Components/GroundAnimals/BP_Comp_Companion.BP_Comp_Companion_C|GetBaitDetails (Variables|Default|GetCompanion))))
      (if (not (Variables|/Game/AdvancedTaming/Blueprints/AI/Components/GroundAnimals/BP_Comp_Companion.BP_Comp_Companion_C|GetIsCompanion (Variables|Default|GetCompanion)))
        ;[1 1 1] Remove tag 'EatingBait'
        (Utilities|Array|RemoveItem (Variables|/Script/Engine.Actor|GetTags (Variables|Default|GetPawnRef)) "abkEatingBait")
        ;[1 1 1] Set EatingBait as False
        (Variables|/Game/AdvancedTaming/Blueprints/AI/Components/GroundAnimals/BP_Comp_Companion.BP_Comp_Companion_C|SetEatingBait (Variables|Default|GetCompanion) false)
        ;[1 1 1] Consume the bait
        (Utilities|IsValid (Variables|/Game/AdvancedTaming/Blueprints/AI/Components/GroundAnimals/BP_Comp_Companion.BP_Comp_Companion_C|GetBaitRef (Variables|Default|GetCompanion))
          (:Is%20Valid
            (Actor|DestroyActor (Variables|/Game/AdvancedTaming/Blueprints/AI/Components/GroundAnimals/BP_Comp_Companion.BP_Comp_Companion_C|GetBaitRef (Variables|Default|GetCompanion))))
          (:Is%20Not%20Valid
            _))
        ;[1 1 1] Reset Engaged to False
        (Class|BTFunctionLibrary|SetBlackboardValueasBool (Variables|Setup|GetEngaged) false)
        (AI|BehaviorTree|FinishExecute true)
        (else
          (AI|BehaviorTree|FinishExecute true))))
    (:Is%20Not%20Valid
      (AI|BehaviorTree|FinishExecute false))))

(fn FnGetBait
  (bind _pawnref (Variables|Default|GetPawnRef))
  (bind _returnvalue (Transformation|GetActorLocation _pawnref))
  (bind (_outhits _returnvalue_2) (Collision|MultiSphereTraceByChannel _returnvalue (+ _returnvalue "0, 0,0.010000") 1e+03 "TraceTypeQuery1" true 0 "None"))
  (if _returnvalue_2
    (bind _array_element (Utilities|Array|ForEachLoopwithBreak _outhits :!label _label)
      (:LoopBody
        (LocalVariables|SetHitActor (.HitActor (Collision|BreakHitResult _array_element)))
        (if (Actor|ActorHasTag (.HitActor (Collision|BreakHitResult _array_element)) "abkBait")
          (LocalVariables|SetFoundIt true)
          (goto _label Break)
          (else
            (LocalVariables|SetFoundIt false))))
      (:Completed
        (return (LocalVariables|GetFoundIt) (LocalVariables|GetHitActor))))))