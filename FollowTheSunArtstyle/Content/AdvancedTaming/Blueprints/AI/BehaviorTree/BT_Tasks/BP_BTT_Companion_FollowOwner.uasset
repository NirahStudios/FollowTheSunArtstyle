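; Behavior tree task that makes a tamed companion AI follow its owner, using settings from its companion component.
; A looping timer re-checks distance and issues AI MoveTo when the owner is at least 500 units away.
; While following, it can teleport to the owner if too far or out of line of sight, when allowed.
; It sends follow start/end messages to the pawn and finishes on arrival.
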(event Custom|EventTeleport
  (if (and (or (>= (Math|Vector|VectorLength (- (Transformation|GetActorLocation (Variables|Default|GetOwnerRef)) (Transformation|GetActorLocation (Variables|Default|GetPawnRef)))) (Variables|Default|GetMinTeleportDist)) (not (CallFunction|FnCanYouSeeOwner))) (Variables|/Game/AdvancedTaming/Blueprints/AI/Components/GroundAnimals/BP_Comp_Companion.BP_Comp_Companion_C|GetCanTeleport (Variables|Default|GetCompanion)))
    (Default|EventCanTeleport (Variables|Default|GetCompanion))
    (Default|EventTeleporttoOwner (Variables|Default|GetCompanion))))

(event Custom|EventMove
  (bind _ownerref (Variables|Default|GetOwnerRef))
  (Utilities|Time|SetTimerbyEvent (delegate Custom|EventMove) 0.1 true)
  ;[1 1 1] Is the distance between the Owner and AI more than 500 units? If so, move towards Owner
  (Utilities|IsValid _ownerref
    (:Is%20Valid
      (if (>= (Math|Vector|VectorLength (- (Transformation|GetActorLocation _ownerref) (Transformation|GetActorLocation (Variables|Default|GetPawnRef)))) 5e+02)
        ;[1 1 1] Move towards Owner
        (AI|AIMoveTo (Variables|Default|GetPawnRef) "0, 0, 0" (Variables|Default|GetOwnerRef) (Variables|Default|GetAcceptanceRadius) true
          (:then
            (if (Variables|Default|GetFollowStart)
              (Variables|Default|SetFollowStart false)
              ;[1 1 1] Fire custom event
              (Class|BPIATSGroundAnimal|FnCompanionFollowStartATS(Message) (Variables|Default|GetPawnRef)))
            ;[1 1 1] Do we teleport?
            (if (Variables|Default|GetTeleport?)
              (CallFunction|EventTeleport)))
          (:OnSuccess
            (Variables|Default|SetFollowStart true)
            ;[1 1 1] Fire custom event
            (Class|BPIATSGroundAnimal|FnCompanionFollowEndATS(Message) (Variables|Default|GetPawnRef))
            (Default|EventArrivedatOwner (Variables|Default|GetCompanion))
            (AI|BehaviorTree|FinishExecute true)))))))

(event EventReceiveExecuteAI
  (params (OwnerController :type AI%20Controller%20Object%20Reference) (ControlledPawn :type Pawn%20Object%20Reference))
  (Variables|Default|SetPawnRef ControlledPawn)
  ;[1 1 1] Check animal has Companion component
  (Utilities|IsValid (Variables|Default|GetPawnRef)
    (:Is%20Valid
      (Utilities|IsValid (Actor|GetComponentbyClass (Variables|Default|GetPawnRef) "/Game/AdvancedTaming/Blueprints/AI/Components/GroundAnimals/BP_Comp_Companion.BP_Comp_Companion_C")
        (:Is%20Valid
          (Variables|Default|SetCompanion (Actor|GetComponentbyClass (Variables|Default|GetPawnRef) "/Game/AdvancedTaming/Blueprints/AI/Components/GroundAnimals/BP_Comp_Companion.BP_Comp_Companion_C"))
          ;[1 1 1] Set Owner Reference
          (Variables|Default|SetOwnerRef (Variables|/Game/AdvancedTaming/Blueprints/AI/Components/GroundAnimals/BP_Comp_Companion.BP_Comp_Companion_C|GetOwnerRef (Variables|Default|GetCompanion)))
          ;[1 1 1] Set Acceptance Radius
          (bind _radius (Class|BPIATSGroundAnimal|FnGetMovementAcceptanceRadiusATS(Message) (Variables|Default|GetPawnRef)))
          (Variables|Default|SetAcceptanceRadius _radius)
          ;[1 1 1] Do we teleport towards Player?
          (Variables|Default|SetTeleport? (.TeleporttoPlayer? (Utilities|Struct|BreakBP_Struct_Companion_TeleportATS (Variables|/Game/AdvancedTaming/Blueprints/AI/Components/GroundAnimals/BP_Comp_Companion.BP_Comp_Companion_C|GetTeleportDetails (Variables|Default|GetCompanion)))))
          ;[1 1 1] Get minimum teleport distance from Player
          (Variables|Default|SetMinTeleportDist (.Mininumteleportdistance? (Utilities|Struct|BreakBP_Struct_Companion_TeleportATS (Variables|/Game/AdvancedTaming/Blueprints/AI/Components/GroundAnimals/BP_Comp_Companion.BP_Comp_Companion_C|GetTeleportDetails (Variables|Default|GetCompanion)))))
          (CallFunction|EventMove))))))

(fn FnCanYouSeeOwner
  (bind (_outhit _returnvalue) (Collision|LineTraceByChannel (Transformation|GetActorLocation (Variables|Default|GetPawnRef)) (Transformation|GetActorLocation (Variables|Default|GetOwnerRef)) "TraceTypeQuery1" true 0 "None"))
  (if _returnvalue
    (return (Actor|ActorHasTag (.HitActor (Collision|BreakHitResult _outhit)) "abkPlayer"))))