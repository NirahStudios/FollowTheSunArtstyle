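; Behavior tree task that moves a simple ground animal toward its current engage target.
; On execute it casts the pawn to BP_SimpleGroundAnimal and gets the acceptance radius through the ATS message function FnGetMovementAcceptanceRadiusATSMessage.
; An AIMoveTo toward EngageTarget, stopping on overlap, finishes the task with success or failure.
; A failed cast never calls FinishExecute.
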(event EventReceiveExecuteAI
  (params (OwnerController :type AI%20Controller%20Object%20Reference) (ControlledPawn :type Pawn%20Object%20Reference))
  (Variables|Default|SetPawnRef ControlledPawn)
  (bind _asbp_simple_ground_animal (Utilities|Casting|CastToBP_SimpleGroundAnimal (Variables|Default|GetPawnRef)))
  (Variables|Default|SetGroundAnimal _asbp_simple_ground_animal)
  ;[1 1 1] Set Acceptance Radius
  (bind _radius (Class|BPIATSGroundAnimal|FnGetMovementAcceptanceRadiusATS(Message) (Variables|Default|GetPawnRef)))
  (Variables|Default|SetAcceptanceRadius _radius)
  ;[1 1 1] Go to Engage Target's location
  (AI|AIMoveTo (Variables|Default|GetPawnRef) "0, 0, 0" (Variables|/Game/AdvancedTaming/Blueprints/Characters/Animals/GroundAnimals/BP_SimpleGroundAnimal.BP_SimpleGroundAnimal_C|GetEngageTarget (Variables|Default|GetGroundAnimal)) (Variables|Default|GetAcceptanceRadius) true
    (:OnSuccess
      (AI|BehaviorTree|FinishExecute true))
    (:OnFail
      (AI|BehaviorTree|FinishExecute false))))