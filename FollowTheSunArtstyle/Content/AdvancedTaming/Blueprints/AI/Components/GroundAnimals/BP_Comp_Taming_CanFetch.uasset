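; Actor component for the taming system that, by its name, marks an object as fetchable by tamed ground animals and handles its highlight.
; On BeginPlay it prints an on-screen error if the owner's root component is not Movable.
; The highlight event saves the owner's static mesh materials, appending to an array that is never cleared, then applies HighlightMaterial to every slot.
; The remove event restores the saved materials by slot index.
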(event Custom|EventSetHighlight
  ;[1 1 1] CUSTOM EVENTS
  (CallFunction|FnSaveMeshMaterials)
  (CallFunction|FnSetHighlightMaterial))

(event Custom|EventRemoveHighlight
  ;[1 1 1] CUSTOM EVENTS
  (CallFunction|FnRemoveHighlight))

(event EventBeginPlay
  ;[1 1 1] Check to see if owner is NOT movable
  (if (Utilities|Enum|NotEqual(Enum) (Variables|/Script/Engine.SceneComponent|GetMobility (Variables|/Script/Engine.Actor|GetRootComponent (Components|GetOwner))) "Movable")
    ;[1 1 1] Print error
    (Development|PrintString (Utilities|String|Append "[Comp_Taming_CanFetch] " (Utilities|GetDisplayName (Components|GetOwner)) " is NOT set to Movable!") true true "(R=1.000000,G=0.000000,B=0.000000,A=1.000000)" 5.0)))

(fn FnSaveMeshMaterials
  ;[1 1 1] Get mesh
  (LocalVariables|SetMesh (Actor|GetComponentbyClass (Components|GetOwner) "/Script/Engine.StaticMeshComponent"))
  ;[1 1 1] Loop through all materials
  (for _index (range 0 (- (Rendering|Material|GetNumMaterials (LocalVariables|GetMesh)) 1))
    ;[1 1 1] Add material to the array
    (Utilities|Array|Add (Variables|Default|GetSavedMaterials) (Rendering|Material|GetMaterial (LocalVariables|GetMesh) _index))))

(fn FnSetHighlightMaterial
  ;[1 1 1] Get mesh
  (LocalVariables|SetMesh (Actor|GetComponentbyClass (Components|GetOwner) "/Script/Engine.StaticMeshComponent"))
  ;[1 1 1] Loop through all materials
  (for _index (range 0 (- (Rendering|Material|GetNumMaterials (LocalVariables|GetMesh)) 1))
    ;[1 1 1] Set the material
    (Rendering|Material|SetMaterial (LocalVariables|GetMesh) _index (Variables|Setup|GetHighlightMaterial))))

(fn FnRemoveHighlight
  ;[1 1 1] Get mesh
  (LocalVariables|SetMesh (Actor|GetComponentbyClass (Components|GetOwner) "/Script/Engine.StaticMeshComponent"))
  ;[1 1 1] Loop through all materials
  (for _index (range 0 (- (Rendering|Material|GetNumMaterials (LocalVariables|GetMesh)) 1))
    ;[1 1 1] Set original material to this index
    (Rendering|Material|SetMaterial (LocalVariables|GetMesh) _index (Utilities|Array|Get(acopy) (Variables|Default|GetSavedMaterials) _index))))