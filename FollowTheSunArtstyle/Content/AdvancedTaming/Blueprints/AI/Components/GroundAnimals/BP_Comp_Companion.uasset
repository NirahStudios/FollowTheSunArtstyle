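; Actor component that makes a ground animal tamable as a player companion in the Advanced Taming system.
; Bait or always-tamable modes lead to companion state, which updates AI controller, movement and widgets, and is undone on release.
; It also handles retaliation, healing, teleporting to the owner and fetching objects via socket attachment.
; Toggled RepNotify booleans propagate state changes; empty start and end events allow child Blueprint overrides.
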(event EventBeginPlay
  (|SAVEOWNERREFERENCE)
  (Utilities|FlowControl|Sequence
    (:then_0
      (|ADDTAMINGTAG))
    (:then_1
      (|CHECKTAMINGMODE))))

(event EventTick
  (params (DeltaSeconds :type Float%20%28single-precision%29))
  (if (Variables|Taming|GetRotateToBait?)
    (CallFunction|FnRotatetoBait)))

(fn FnRotatetoBait
  (bind _animal (Variables|Default|GetAnimal))
  (bind _animal_2 (Variables|Default|GetAnimal))
  (bind _returnvalue (Transformation|GetActorRotation _animal_2))
  ;[1 1 1] Check Bait reference is valid
  (Utilities|IsValid (Variables|Taming|GetBaitRef)
    (:Is%20Valid
      ;[1 1 1] Rotate actor towards the Bait
      (LocalVariables|Setcurrent (.yaw (Transformation|GetActorRotation _animal)))
      (LocalVariables|Settarget (.yaw (Math|Rotator|FindLookatRotation (Transformation|GetActorLocation _animal) (Transformation|GetActorLocation (Variables|Taming|GetBaitRef)))))
      (Transformation|SetActorRotation (Variables|Default|GetAnimal) (Math|Rotator|MakeRotator (.roll _returnvalue) (.pitch _returnvalue) (Math|Interpolation|FInterpTo (LocalVariables|Getcurrent) (LocalVariables|Gettarget) (Utilities|Time|GetWorldDeltaSeconds) 2.0)) true)
      ;[1 1 1] Check if we rotated towards bait
      (if (Math|Float|NearlyEqual(Float) (LocalVariables|Getcurrent) (LocalVariables|Gettarget) 1.0)
        ;[1 1 1] Stop rotating
        (Variables|Taming|SetRotateToBait? false)))))

(fn FnCheckforBait
  (params (Actor :type Actor%20Object%20Reference))
  (LocalVariables|Setbait Actor)
  (if (Actor|ActorHasTag (LocalVariables|Getbait) (Utilities|Struct|BreakBP_Struct_Companion_BaitATS (Variables|Setup|GetBaitDetails)))
    (CallFunction|EventFoundBait (LocalVariables|Getbait))))

(fn FnReceivedDamage
  (params (Damage%20Causer :type Actor%20Object%20Reference))
  (LocalVariables|Setenemy Damage%20Causer)
  (Utilities|FlowControl|Sequence
    (:then_0
      ;[1 1 1] Is animal on Aggressive Stance?
      (if (Utilities|Enum|Equal(Enum) (Utilities|Struct|BreakBP_Struct_Companion_DetailsATS (Variables|Setup|GetCompanionDetails)) "NewEnumerator1")
        ;[1 1 1] Set Attack Target and Set Task to Attack
        (Variables|Setup|SetCompanionAttackTarget (LocalVariables|Getenemy))
        (Variables|Setup|SetCompanionTasks "NewEnumerator3")))
    (:then_1
      ;[1 1 1] Should we auto-heal? If so, call EventStartHealCounter
      (if (Utilities|Struct|BreakBP_Struct_Companion_HealingATS (Variables|Setup|GetHealingDetails))
        (CallFunction|EventStartHealCounter)))))

(fn FnAnimalDied
  (bind _ownerref (Variables|Setup|GetOwnerRef))
  (bind _ownerref_2 (Variables|Setup|GetOwnerRef))
  (bind _returnvalue (Actor|GetComponentbyClass _ownerref "/Game/AdvancedTaming/Blueprints/Characters/Player/Components/BP_Comp_PlayerHUD_ATS.BP_Comp_PlayerHUD_ATS_C"))
  (bind _returnvalue_2 (Actor|GetComponentbyClass _ownerref_2 "/Game/AdvancedTaming/Blueprints/Characters/Player/Components/BP_Comp_PlayerCanTame.BP_Comp_PlayerCanTame_C"))
  (bind _playerhudref (Variables|/Game/AdvancedTaming/Blueprints/Characters/Player/Components/BP_Comp_PlayerHUD_ATS.BP_Comp_PlayerHUD_ATS_C|GetPlayerHUDRef _returnvalue))
  ;[1 1 1] Leave owner
  (Variables|Setup|SetCompanionTasks "NewEnumerator4")
  ;[1 1 1] Check that owner is valid
  (Utilities|IsValid (Variables|Setup|GetOwnerRef)
    (:Is%20Valid
      ;[1 1 1] Do we have component PlayerHUD/
      (Utilities|IsValid _returnvalue
        (:Is%20Valid
          (Utilities|IsValid _playerhudref
            (:Is%20Valid
              ;[1 1 1] Show Companion Commands
              (Widget|SetVisibility (Variables|/Game/AdvancedTaming/Blueprints/Widgets/WBP_ATS_Player_HUD.WBP_ATS_Player_HUD_C|GetWBP_Companion _playerhudref) "Hidden"))
            (:Is%20Not%20Valid
              _)))
        (:Is%20Not%20Valid
          _))
      ;[1 1 1] Reset Companion variables
      (Variables|/Game/AdvancedTaming/Blueprints/Characters/Player/Components/BP_Comp_PlayerCanTame.BP_Comp_PlayerCanTame_C|SetCanTame _returnvalue_2 false)
      (Variables|/Game/AdvancedTaming/Blueprints/Characters/Player/Components/BP_Comp_PlayerCanTame.BP_Comp_PlayerCanTame_C|SetCompanionRef _returnvalue_2 0)
      ;[1 1 1] Get Engage Actor
      (LocalVariables|SetEngageActor (Variables|/Game/AdvancedTaming/Blueprints/Characters/Player/Components/BP_Comp_PlayerCanTame.BP_Comp_PlayerCanTame_C|GetEngageActor _returnvalue_2))
      ;[1 1 1] Hide Animal Marker
      (Utilities|IsValid (LocalVariables|GetEngageActor)
        (:Is%20Valid
          (Class|BPIATSGroundAnimal|FnHideWidgetMarkerATS(Message) (LocalVariables|GetEngageActor)))))))

(fn OnRepNotifyBecameCompanion
  ;[1 1 1] Hide TamingWidget
  (bind _wbp_tame (Class|BPIATSGroundAnimal|FnGetWidgetsATS(Message) (Variables|Default|GetAnimal)))
  (Utilities|IsValid _wbp_tame
    (:Is%20Valid
      (Rendering|SetVisibility _wbp_tame false false))
    (:Is%20Not%20Valid
      _))
  (Utilities|FlowControl|Sequence
    (:then_0
      ;[1 1 1] [BP_SimpleGroundAnimal] Cast to the AI Controller and call function fnSetAsCompanion
      (bind _asbp_ats_aic_base (Utilities|Casting|CastToBP_ATS_AIC_Base (AI|GetAIController (Variables|Default|GetAnimal))))
      (Default|FnSetasCompanion _asbp_ats_aic_base))
    (:then_1
      ;[1 1 1] [BP_GroundAnimalBase] Cast to the AI Controller and call function fnSetAsCompanion
      (bind _asbp_aic_base (Utilities|Casting|CastToBP_AIC_Base (AI|GetAIController (Variables|Default|GetAnimal))))
      (Default|FnSetasCompanion _asbp_aic_base))
    (:then_2
      (Class|BPIATSGroundAnimal|FnSetCompanionNameATS(Message) (Variables|Default|GetAnimal) (Utilities|Struct|BreakBP_Struct_Companion_DetailsATS (Variables|Setup|GetCompanionDetails)))
      (Class|BPIATSGroundAnimal|FnNotifyNameChangeATS(Message) (Variables|Default|GetAnimal))
      ;[1 1 1] Call CompanionStart event
      (CallFunction|EventCompanionStart)
      ;[1 1 1] Leave current group
      (Variables|Default|SetnotifyLeaveGroup false)
      ;[1 1 1] Set Max Land Speed
      (Variables|/Script/Engine.CharacterMovementComponent|SetMaxWalkSpeed (Variables|/Script/Engine.Character|GetCharacterMovement (Variables|Default|GetAnimal)) (Utilities|Struct|BreakBP_Struct_Companion_DetailsATS (Variables|Setup|GetCompanionDetails)))
      ;[1 1 1] Set Max Acceleration
      (Variables|/Script/Engine.CharacterMovementComponent|SetMaxAcceleration (Variables|/Script/Engine.Character|GetCharacterMovement (Variables|Default|GetAnimal)) (Utilities|Struct|BreakBP_Struct_Companion_DetailsATS (Variables|Setup|GetCompanionDetails)))
      ;[1 1 1] Start by following the Owner
      (Variables|Setup|SetCompanionTasks "NewEnumerator0")
      ;[1 1 1] Set text to Companion color
      (if (Variables|Default|GetsetTextToCompanion)
        (Variables|Default|SetsetTextToCompanion false)
        (else
          (Variables|Default|SetsetTextToCompanion true)))
      ;[1 1 1] Show marker?
      (if (Utilities|Struct|BreakBP_Struct_Companion_DetailsATS (Variables|Setup|GetCompanionDetails))
        (CallFunction|EventServerShowMarker))
      ;[1 1 1] If valid, destroy the Bait actor
      (Utilities|IsValid (Variables|Taming|GetBaitRef)
        (:Is%20Valid
          (Actor|DestroyActor (Variables|Taming|GetBaitRef)))
        (:Is%20Not%20Valid
          _))
      ;[1 1 1] Consume the Bait
      (Variables|Taming|SetBaitRef 0)
      (AI|Components|Blackboard|SetValueasBool (Variables|/Script/AIModule.AIController|GetBlackboard (AI|GetAIController (Variables|Default|GetAnimal))) (Variables|Taming|GetFoundBait) false)
      ;[1 1 1] Reset EatingBait values
      (switch Utilities|FlowControl|Switch|SwitchonBP_Enum_Companion_TameModeATS (Utilities|Struct|BreakBP_Struct_Companion_DetailsATS (Variables|Setup|GetCompanionDetails))
        (:NewEnumerator0
          (Variables|Taming|SetEatingBait false)
          (Utilities|Array|RemoveItem (Variables|/Script/Engine.Actor|GetTags (Variables|Default|GetAnimal)) "EatingBait")
          (Utilities|Array|Add (Variables|/Script/Engine.Actor|GetTags (Variables|Default|GetAnimal)) "abkCanTame"))))))

(fn OnRepNotifySetFree
  ;[1 1 1] Change the Animal name and color to default
  (bind _wbp_hud (Class|BPIATSGroundAnimal|FnGetWidgetsATS(Message) (Variables|Default|GetAnimal)))
  (bind _aswbp_ats_ai_hud (Utilities|Casting|CastToWBP_ATS_AI_HUD (UserInterface|GetUserWidgetObject _wbp_hud)))
  (bind _animal_name (Class|BPIATSGroundAnimal|FnGetAnimalNameATS(Message) (Variables|Default|GetAnimal)))
  (Default|FnSetName _aswbp_ats_ai_hud _animal_name)
  (Default|FnSetActive _aswbp_ats_ai_hud)
  (bind (_max_speed _max_acceleration) (Class|BPIATSGroundAnimal|FnGetSpeedandAccelerationATS(Message) (Variables|Default|GetAnimal)))
  ;[1 1 1] Set Max Land Speed
  (Variables|/Script/Engine.CharacterMovementComponent|SetMaxWalkSpeed (Variables|/Script/Engine.Character|GetCharacterMovement (Variables|Default|GetAnimal)) _max_speed)
  ;[1 1 1] Set Max Acceleration
  (Variables|/Script/Engine.CharacterMovementComponent|SetMaxAcceleration (Variables|/Script/Engine.Character|GetCharacterMovement (Variables|Default|GetAnimal)) _max_acceleration)
  ;[1 1 1] Hide Pet Marker widget
  (bind _wbp_pet (Class|BPIATSGroundAnimal|FnGetWidgetsATS(Message) (Variables|Default|GetAnimal)))
  (Rendering|SetVisibility _wbp_pet false false)
  ;[1 1 1] Call CompanionEnd event
  (CallFunction|EventCompanionEnd))

(fn OnRepNotifyLeaveGroup
  (Class|BPIATSGroundAnimal|FnLeaveGroupATS(Message) (Variables|Default|GetAnimal)))

(fn OnRepSetTexttoCompanion
  ;[1 1 1] Change name color to indicate animal is a Companion
  (bind _wbp_hud (Class|BPIATSGroundAnimal|FnGetWidgetsATS(Message) (Variables|Default|GetAnimal)))
  (bind _aswbp_ats_ai_hud (Utilities|Casting|CastToWBP_ATS_AI_HUD (UserInterface|GetUserWidgetObject _wbp_hud)))
  (Default|FnSetasCompanion _aswbp_ats_ai_hud))

(fn OnRepHealCompanion
  (bind _hp (Class|BPIATSGroundAnimal|FnGetAnimalHPATS(Message) (Variables|Default|GetAnimal)))
  (Class|BPIATSGroundAnimal|FnSetAnimalCurrentHPATS(Message) (Variables|Default|GetAnimal) _hp))

(fn FnMovementFailed
  ;[1 1 1] Switch to Follow Owner
  (Default|ServerCommand1 (Actor|GetComponentbyClass (Variables|Setup|GetOwnerRef) "/Game/AdvancedTaming/Blueprints/Characters/Player/Components/BP_Comp_PlayerCanTame.BP_Comp_PlayerCanTame_C") false))

(fn FnRemoveFetchMarker
  (Utilities|IsValid (Variables|CustomCommand|GetMarkerLocRef)
    (:Is%20Valid
      (Actor|DestroyActor (Variables|CustomCommand|GetMarkerLocRef)))))

(fn OnRepOwnerRef)

(fn OnRepCanTeleport)

(fn OnRepCompanionTasks)

(fn OnRepCustomCommand)

(fn OnRepIsCompanion)

(fn OnRepAnimal)

(fn OnRepBActive)

(fn OnRepGettingFetchObject)

(fn OnRepCarryingObject)

(fn OnRepFetchCompRef)

(fn OnRepHitActor)

(fn FnSetTargetLocationinBT
  (params (Animal :type Character%20Object%20Reference))
  (bind _ownerref (Variables|Setup|GetOwnerRef))
  (bind _returnvalue (Actor|GetComponentbyClass _ownerref "/Game/AdvancedTaming/Blueprints/Characters/Player/Components/BP_Comp_PlayerCanTame.BP_Comp_PlayerCanTame_C"))
  ;[1 1 1] Set TargetLocation in Companion's Blackboard
  (AI|Components|Blackboard|SetValueasVector (Variables|/Script/AIModule.AIController|GetBlackboard (AI|GetAIController Animal)) (Variables|/Game/AdvancedTaming/Blueprints/Characters/Player/Components/BP_Comp_PlayerCanTame.BP_Comp_PlayerCanTame_C|GetTargetLocation _returnvalue) (Variables|/Game/AdvancedTaming/Blueprints/Characters/Player/Components/BP_Comp_PlayerCanTame.BP_Comp_PlayerCanTame_C|GetHitLocation _returnvalue)))

(fn FnCheckifActorIsFetchable
  (params (ActorToCheck :type Actor%20Object%20Reference))
  (bind _returnvalue (Actor|GetComponentbyClass ActorToCheck "/Game/AdvancedTaming/Blueprints/AI/Components/GroundAnimals/BP_Comp_Taming_CanFetch.BP_Comp_Taming_CanFetch_C"))
  (Variables|CustomCommand|SetFetchCompRef _returnvalue)
  (if (and (Utilities|IsValid _returnvalue) (Utilities|Enum|Equal(Enum) (Variables|/Script/Engine.SceneComponent|GetMobility (Variables|/Script/Engine.Actor|GetRootComponent ActorToCheck)) "Movable"))
    (return true)
    (else
      (return false))))

(fn OnRepNotifyCustomCommandEnd)

(event Custom|EventMakeCompanion
  (params (Owner :type Actor%20Object%20Reference))
  (CallFunction|EventClientMakeCompanion Owner))

(event Custom|EventClientMakeCompanion
  (params (Owner :type Actor%20Object%20Reference))
  ;[1 1 1] Save owner reference
  (Variables|Setup|SetOwnerRef Owner)
  (if (Variables|Setup|GetActive)
    ;[1 1 1] Set IsCompanion to True
    (Variables|Setup|SetIsCompanion true)
    ;[1 0.5 0] Disable Day Cycle
    (Class|BPIATSGroundAnimal|FnDisableDayCycleATS(Message) (Variables|Default|GetAnimal))
    ;[1 1 1] Fire custom event BecomePet
    (Class|BPIATSGroundAnimal|FnCompanionBecomePetATS(Message) (Variables|Default|GetAnimal))
    (if (Variables|Default|GetnotifyBecameCompanion)
      (Variables|Default|SetnotifyBecameCompanion false)
      (else
        (Variables|Default|SetnotifyBecameCompanion true)))))

(event Custom|EventArrivedAtOwner
  (bind _hitactor (Variables|CustomCommand|GetHitActor))
  (bind _returnvalue (Actor|GetComponentbyClass _hitactor "/Script/Engine.StaticMeshComponent"))
  (Variables|Default|SetnotifyCustomCommandEnd true)
  ;[1 1 1] Check that we are executing a Custom Command
  (if (and (Variables|CustomCommand|GetCustomCommand) (Variables|CustomCommand|GetCarryingObject))
    (Utilities|IsValid (Variables|CustomCommand|GetHitActor)
      (:Is%20Valid
        ;[1 1 1] Detach HitActor
        (Transformation|DetachFromActor (Variables|CustomCommand|GetHitActor) "KeepRelative" "KeepRelative" "KeepRelative")
        ;[1 1 1] Enable collision on HitActor
        (Collision|SetActorEnableCollision (Variables|CustomCommand|GetHitActor) true)
        ;[1 1 1] Simulate Physics on HitActor
        (Utilities|IsValid _returnvalue
          (:Is%20Valid
            (Physics|SetSimulatePhysics _returnvalue true)
            ;[1 1 1] Disable Custom Command Flag
            (Variables|CustomCommand|SetCustomCommand false)
            ;[1 1 1] Reset parameters
            (Variables|CustomCommand|SetCarryingObject false)
            (Variables|CustomCommand|SetGettingFetchObject false)
            ;[1 1 1] Remove Highlight material
            (if (Variables|/Game/AdvancedTaming/Blueprints/AI/Components/GroundAnimals/BP_Comp_Taming_CanFetch.BP_Comp_Taming_CanFetch_C|GetUseHighlightMaterial (Variables|CustomCommand|GetFetchCompRef))
              (Default|EventRemoveHighlight (Variables|CustomCommand|GetFetchCompRef))
              ;[1 1 1] Enable teleporting
              (Variables|Setup-Teleport|SetCanTeleport true))))))))

(event Custom|EventServerShowMarker
  (Class|BPIATSGroundAnimal|FnShowPetMarkerATS(Message) (Variables|Default|GetAnimal)))

(event Custom|Multicast_ChangeAnimalToDefaultState
  (Variables|Setup|SetIsCompanion false)
  ;[1 1 1] Change the Animal name and color to default
  (bind _wbp_hud (Class|BPIATSGroundAnimal|FnGetWidgetsATS(Message) (Variables|Default|GetAnimal)))
  (bind _aswbp_ats_ai_hud (Utilities|Casting|CastToWBP_ATS_AI_HUD (UserInterface|GetUserWidgetObject _wbp_hud)))
  (bind _animal_name (Class|BPIATSGroundAnimal|FnGetAnimalNameATS(Message) (Variables|Default|GetAnimal)))
  (Default|FnSetName _aswbp_ats_ai_hud _animal_name)
  (Default|FnSetActive _aswbp_ats_ai_hud)
  ;[1 1 1] Hide Pet Marker widget
  (bind _wbp_pet (Class|BPIATSGroundAnimal|FnGetWidgetsATS(Message) (Variables|Default|GetAnimal)))
  (Rendering|SetVisibility _wbp_pet false false))

(event Custom|EventLeaveOwner
  ;[1 1 1] Set IsCompanion to False
  (Variables|Setup|SetIsCompanion false)
  ;[1 1 1] Fire custom event Leave
  (Class|BPIATSGroundAnimal|FnCompanionLeaveATS(Message) (Variables|Default|GetAnimal))
  (Utilities|FlowControl|Sequence
    (:then_0
      ;[1 1 1] [BP_SimpleGroundAnimal] Cast to the AI Controller and call function fnSetAsCompanion
      (bind _asbp_ats_aic_base (Utilities|Casting|CastToBP_ATS_AIC_Base (AI|GetAIController (Variables|Default|GetAnimal))))
      (Default|FnSetFree _asbp_ats_aic_base))
    (:then_1
      ;[1 1 1] [BP_GroundAnimalBase] Cast to the AI Controller and call function fnSetAsCompanion
      (bind _asbp_aic_base (Utilities|Casting|CastToBP_AIC_Base (AI|GetAIController (Variables|Default|GetAnimal))))
      (Default|FnSetFree _asbp_aic_base))
    (:then_2
      ;[1 0.5 0] Enable Day Cycle
      (Class|BPIATSGroundAnimal|FnEnableDayCycleATS(Message) (Variables|Default|GetAnimal))
      (if (Variables|Default|GetnotifySetFree)
        (Variables|Default|SetnotifySetFree false)
        (else
          (Variables|Default|SetnotifySetFree true))))))

(event Custom|EventFoundBait
  (params (BaitRef :type Actor%20Object%20Reference))
  (bind _animal (Variables|Default|GetAnimal))
  (bind _returnvalue (AI|GetAIController _animal))
  (Variables|Taming|SetBaitRef BaitRef)
  (if (Variables|Setup|GetActive)
    (Utilities|FlowControl|Sequence
      (:then_0
        (switch Utilities|FlowControl|Switch|SwitchonBP_Enum_Companion_TameModeATS (Utilities|Struct|BreakBP_Struct_Companion_DetailsATS (Variables|Setup|GetCompanionDetails))
          (:NewEnumerator0
            (Utilities|IsValid (Variables|Default|GetAnimal)
              (:Is%20Valid
                ;[1 1 1] Set FoundBait Blackboard value to True
                (Utilities|IsValid _animal
                  (:Is%20Valid
                    (Utilities|IsValid _returnvalue
                      (:Is%20Valid
                        (AI|Components|Blackboard|SetValueasBool (Variables|/Script/AIModule.AIController|GetBlackboard _returnvalue) (Variables|Taming|GetFoundBait) true)
                        ;[1 1 1] Set rotate towards bait
                        (Variables|Taming|SetRotateToBait? (Variables|Taming|GetRotateToBait?)))))))))))
      (:then_1
        (if (and (Utilities|Struct|BreakBP_Struct_Companion_HealingATS (Variables|Setup|GetHealingDetails)) (Variables|Setup|GetIsCompanion))
          (if (Variables|Default|GetHealCompanion)
            (Variables|Default|SetHealCompanion false)
            (else
              (Variables|Default|SetHealCompanion true))))))))

(event EventFnSetCompanionName
  (params (Companion%20Name :type Text))
  (Class|BPIATSGroundAnimal|FnSetCompanionNameATS(Message) (Variables|Default|GetAnimal) Companion%20Name))

(event Custom|EventStartHealCounter
  (Utilities|FlowControl|RetriggerableDelay (Utilities|Struct|BreakBP_Struct_Companion_HealingATS (Variables|Setup|GetHealingDetails)))
  (if (Variables|Default|GetHealCompanion)
    (Variables|Default|SetHealCompanion false)
    (else
      (Variables|Default|SetHealCompanion true))))

(event Custom|fnNotifyNameChange
  (Class|BPIATSGroundAnimal|FnNotifyNameChangeATS(Message) (Variables|Default|GetAnimal)))

(event Custom|EventCompanionEnd
  ;[1 1 1] These custom events are meant to be overriden in a child BP. This allows for custom code to be added when the animal becomes a companion or when it stops being a companion
)

(event Custom|EventCompanionStart
  ;[1 1 1] These custom events are meant to be overriden in a child BP. This allows for custom code to be added when the animal becomes a companion or when it stops being a companion
)

(event Custom|EventCanTeleport
  (if (Variables|Setup-Teleport|GetCanTeleport)
    (Variables|Setup-Teleport|SetCanTeleport false)
    (Utilities|FlowControl|Delay (Utilities|Struct|BreakBP_Struct_Companion_TeleportATS (Variables|Setup|GetTeleportDetails)))
    (Variables|Setup-Teleport|SetCanTeleport true)))

(event Custom|EventTeleportToOwner
  (bind _ownerref (Variables|Setup|GetOwnerRef))
  (bind _returnvalue (Transformation|GetActorRotation _ownerref))
  (Utilities|FlowControl|Delay (Utilities|Struct|BreakBP_Struct_Companion_TeleportATS (Variables|Setup|GetTeleportDetails)))
  (Transformation|Teleport (Variables|Default|GetAnimal) (+ (Transformation|GetActorLocation _ownerref) (* (Math|Vector|GetForwardVector _returnvalue) (Utilities|Struct|BreakBP_Struct_Companion_TeleportATS (Variables|Setup|GetTeleportDetails)))) _returnvalue))

(event Custom|EventArrivedAtLocation
  (bind _hitactor (Variables|CustomCommand|GetHitActor))
  (bind _hitactor_2 (Variables|CustomCommand|GetHitActor))
  ;[1 1 1] Check that we are executing a Custom Command
  (if (Variables|CustomCommand|GetCustomCommand)
    ;[1 1 1] Check that we are near the object
    (Utilities|IsValid _hitactor_2
      (:Is%20Valid
        (if (<= (Math|Vector|VectorLength (- (Transformation|GetActorLocation _hitactor_2) (Transformation|GetActorLocation (Variables|Default|GetAnimal)))) (Variables|CustomCommand|GetMaxObjectDistance))
          ;[1 1 1] Attach HitActor to Animal
          (Transformation|AttachActorToActor (Variables|CustomCommand|GetHitActor) (Variables|Default|GetAnimal) "CarryObject" "SnapToTarget" "SnapToTarget" "KeepWorld" true)
          ;[1 1 1] Disable HitActor collision
          (Collision|SetActorEnableCollision (Variables|CustomCommand|GetHitActor) false)
          ;[1 1 1] Set relative location for the HitActor
          (Transformation|SetActorRelativeLocation _hitactor (Variables|CustomCommand|GetCarryLocation) false true)
          (Transformation|SetActorRelativeRotation _hitactor (Variables|CustomCommand|GetCarryRotation) false true)
          (Variables|CustomCommand|SetCarryingObject true)
          (Utilities|FlowControl|Delay 0.5)
          ;[1 1 1] Follow Player
          (Default|ServerCommand1 (Actor|GetComponentbyClass (Variables|Setup|GetOwnerRef) "/Game/AdvancedTaming/Blueprints/Characters/Player/Components/BP_Comp_PlayerCanTame.BP_Comp_PlayerCanTame_C") false :!label _label)))
      (:Is%20Not%20Valid
        (goto _label)))))

(event Custom|EventStartedAttack)