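; BP_ShowWidget is a trigger actor that shows an on-screen message when a locally controlled pawn tagged abkPlayer overlaps it.
; A client event, with an optional DoOnce gate controlled by ShowOnce, creates a BP_PFT_Message widget with the configured title and description, replacing any existing one.
; The widget is removed from the viewport after the MessageTime delay.
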(event OnComponentBeginOverlap(Trigger)
  (params (OverlappedComponent :type Primitive%20Component%20Object%20Reference) (OtherActor :type Actor%20Object%20Reference) (OtherComp :type Primitive%20Component%20Object%20Reference) (OtherBodyIndex :type Integer) (bFromSweep :type Boolean) (SweepResult :type Hit%20Result%20Structure%20%28by%20ref%29))
  (if (Actor|ActorHasTag OtherActor "abkPlayer")
    (bind _aspawn (Utilities|Casting|CastToPawn OtherActor))
    (if (Pawn|IsLocallyControlled _aspawn)
      (CallFunction|ClientShowMessage))))

(event Custom|EventHideMessage
  (Utilities|FlowControl|Delay (Variables|Setup|GetMessageTime))
  (Widget|RemovefromParent (Variables|Default|GetWBRef)))

(event Custom|Client_ShowMessage
  (if (Variables|Setup|GetShowOnce)
    (Utilities|FlowControl|DoOnce false
      (:Completed
        _)))
  (CallFunction|FnShowMessage)
  (CallFunction|EventHideMessage))

(fn ConstructionScript)

(fn FnShowMessage
  (Utilities|IsValid (Variables|Default|GetWBRef)
    (:Is%20Valid
      (Widget|RemovefromParent (Variables|Default|GetWBRef)))
    (:Is%20Not%20Valid
      _))
  ;[1 1 1] Create a new widget class
  (bind _returnvalue (UserInterface|CreateWidget "/Game/AdvancedTaming/Blueprints/Showcase/BP_PFT_Message.BP_PFT_Message_C"))
  (Variables|Default|SetWBRef _returnvalue)
  ;[1 1 1] Set the title and description of this widget
  (Default|FnSetTitle (Variables|Default|GetWBRef) (Variables|Setup|GetMessageTitle))
  (Default|FnSetDescription (Variables|Default|GetWBRef) (Variables|Setup|GetMessageDescription))
  ;[1 1 1] Add the widget to the viewport and call function fnShowMessage
  (UserInterface|Viewport|AddtoViewport (Variables|Default|GetWBRef) 0)
  (Default|FnShowMessage (Variables|Default|GetWBRef)))

(fn OnRepShowOnce)

(fn OnRepWBRef)