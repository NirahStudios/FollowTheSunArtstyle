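; Showcase trigger actor that slides a referenced Mesh actor by an Offset the first time something overlaps its Trigger.
; The Mesh's start location is cached on BeginPlay, and a DoOnce limits the move to a single activation.
; The TMMove timeline lerps from that start to start plus Offset, teleporting the actor each update without sweep.
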(event OnComponentBeginOverlap(Trigger)
  (params (OverlappedComponent :type Primitive%20Component%20Object%20Reference) (OtherActor :type Actor%20Object%20Reference) (OtherComp :type Primitive%20Component%20Object%20Reference) (OtherBodyIndex :type Integer) (bFromSweep :type Boolean) (SweepResult :type Hit%20Result%20Structure%20%28by%20ref%29))
  (Utilities|FlowControl|DoOnce false
    (:Completed
      (CallFunction|EventMoveObject))))

(event Custom|EventMoveObject
  (bind _startlocation (Variables|Default|GetStartLocation))
  (bind _alpha (Timeline|TMMove PlayFromStart)
    (:Update
      (Transformation|SetActorLocation (Variables|Setup|GetMesh) (Math|Vector|Lerp(Vector) _startlocation (+ _startlocation (Variables|Setup|GetOffset)) _alpha) false true))))

(event EventBeginPlay
  (Variables|Default|SetStartLocation (Transformation|GetActorLocation (Variables|Setup|GetMesh))))

(fn ConstructionScript)