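; Player controller for the taming system that lets the player swap control between their character and the selected companion.
; The ControlCompanion input picks the direction, then server events possess the target pawn, storing the player pawn and the companion's AI controller.
; Returning hands the companion back to that AI controller and disables its camera.
; Switching also toggles companion teleporting, exits aim mode and clears markers on the client.
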(event Custom|Client_ClearMarkerForControl
  (bind _returnvalue (Game|GetPlayerCharacter 0))
  (bind _returnvalue_2 (Actor|GetComponentbyClass _returnvalue "/Game/AdvancedTaming/Blueprints/Characters/Player/Components/BP_Comp_PlayerCanTame.BP_Comp_PlayerCanTame_C"))
  ;[1 0.9117 0] Command Client: remove all marker before control companion
  (Utilities|IsValid _returnvalue_2
    (:Is%20Valid
      (Default|FnRemoveAnyPreviousMarker _returnvalue_2))))

(event Custom|Server_ControlCharacter
  (params (CharacterToControl :type Character%20Object%20Reference) (TargetController :type Player%20Controller%20Object%20Reference))
  ;[1 0 0] Command server: Control Character
  (CallFunction|ControlCharacter CharacterToControl TargetController))

(event Custom|Server_ControlCompanion
  (params (CompanionToControl :type Actor%20Object%20Reference) (PlayerController :type Player%20Controller%20Object%20Reference))
  ;[1 0 0] Command server: Control Companion
  (CallFunction|TakeControlOfCompanion CompanionToControl PlayerController))

(event EventStartControlCompanion
  (params (CompanionToControl :type Actor%20Object%20Reference))
  (bind _returnvalue (Game|GetPlayerCharacter 0))
  ;[1 0.9117 0] Control companion interface call
  (if (Utilities|DoesObjectImplementInterface _returnvalue "/Game/AdvancedTaming/Blueprints/Core/Interfaces/BPI_ATS_HUDAccess.BPI_ATS_HUDAccess_C")
    (bind _bcrosshairactivated (Class|BPIATSHUDAccess|GetShowCrosshairState(Message) _returnvalue))
    (if _bcrosshairactivated
      (Class|BPIATSHUDAccess|ToggleAim(Message) _returnvalue)))
  (CallFunction|ServerControlCompanion CompanionToControl self)
  (CallFunction|ClientClearMarkerforControl))

(event EventStartControlPlayer
  (params (CharacterToControl :type Character%20Object%20Reference) (PlayerController :type Player%20Controller%20Object%20Reference))
  ;[1 0.9117 0] Control companion interface call
  (CallFunction|ServerControlCharacter CharacterToControl PlayerController))

(event Input|ActionEvents|InputActionControlCompanion
  (params (Key :type Key%20Structure))
  (bind _returnvalue (Game|GetPlayerCharacter 0))
  (bind _returnvalue_2 (Actor|GetComponentbyClass _returnvalue "/Game/AdvancedTaming/Blueprints/Characters/Player/Components/BP_Comp_PlayerCanTame.BP_Comp_PlayerCanTame_C"))
  ;[1 1 1] Input call: control companion
  (:Pressed
    (Utilities|IsValid (Actor|GetComponentbyClass _returnvalue "/Game/AdvancedTaming/Blueprints/AI/Components/GroundAnimals/BP_Comp_Companion.BP_Comp_Companion_C")
      (:Is%20Valid
        (Class|BPIATSPlayerActions|StartControlPlayer(Message) self (Variables|Default|GetOwnPawn) self))
      (:Is%20Not%20Valid
        (Utilities|IsValid _returnvalue_2
          (:Is%20Valid
            (if (!= (Variables|/Game/AdvancedTaming/Blueprints/Characters/Player/Components/BP_Comp_PlayerCanTame.BP_Comp_PlayerCanTame_C|GetCurrentCompanions _returnvalue_2) 0)
              (Class|BPIATSPlayerActions|StartControlCompanion(Message) self (Variables|/Game/AdvancedTaming/Blueprints/Characters/Player/Components/BP_Comp_PlayerCanTame.BP_Comp_PlayerCanTame_C|GetSelectedCompanion _returnvalue_2)))))))))

(fn ConstructionScript)

(fn OnRepOwnPawn)

(fn ReleaseCompanionControltoIA
  (params (CharacterRef :type Character%20Object%20Reference) (PlayerControllerRef :type Player%20Controller%20Object%20Reference))
  (bind _returnvalue (Actor|GetComponentbyClass CharacterRef "/Game/AdvancedTaming/Blueprints/Characters/Player/Components/BP_Comp_PlayerCanTame.BP_Comp_PlayerCanTame_C"))
  (bind _selectedcompanion (Variables|/Game/AdvancedTaming/Blueprints/Characters/Player/Components/BP_Comp_PlayerCanTame.BP_Comp_PlayerCanTame_C|GetSelectedCompanion _returnvalue))
  (bind _returnvalue_2 (Actor|GetComponentbyClass _selectedcompanion "/Game/AdvancedTaming/Blueprints/AI/Components/GroundAnimals/BP_Comp_Companion.BP_Comp_Companion_C"))
  (Default|CallCommand2 _returnvalue)
  (Utilities|IsValid _selectedcompanion
    (:Is%20Valid
      (Utilities|IsValid _returnvalue_2
        (:Is%20Valid
          (Variables|/Game/AdvancedTaming/Blueprints/AI/Components/GroundAnimals/BP_Comp_Companion.BP_Comp_Companion_C|SetCanTeleport _returnvalue_2 true)
          (bind _companioncontroller (Class|BPIATSPlayerActions|GetAIControllerRefforCompanion(Message) PlayerControllerRef))
          (bind _aspawn (Utilities|Casting|CastToPawn _selectedcompanion))
          (Pawn|Possess _companioncontroller _aspawn))))))

(fn OnRepCompControllerRef)

(fn ControlCharacter
  (params (CharacterToControl :type Character%20Object%20Reference) (TargetController :type Player%20Controller%20Object%20Reference))
  (LocalVariables|SetTmpActualCompanionControlled (Pawn|GetControlledPawn))
  (LocalVariables|SetTmpCharacterToControl CharacterToControl)
  (LocalVariables|SetTmpTargetController TargetController)
  (CallFunction|ReleaseCompanionControltoIA (LocalVariables|GetTmpCharacterToControl) (LocalVariables|GetTmpTargetController))
  (Pawn|Possess (LocalVariables|GetTmpTargetController) (LocalVariables|GetTmpCharacterToControl))
  ;[1 1 1] Enable companion teleport
  (Utilities|IsValid (Actor|GetComponentbyClass (LocalVariables|GetTmpActualCompanionControlled) "/Game/AdvancedTaming/Blueprints/AI/Components/GroundAnimals/BP_Comp_Companion.BP_Comp_Companion_C")
    (:Is%20Valid
      (Variables|/Game/AdvancedTaming/Blueprints/AI/Components/GroundAnimals/BP_Comp_Companion.BP_Comp_Companion_C|SetCanTeleport (Actor|GetComponentbyClass (LocalVariables|GetTmpActualCompanionControlled) "/Game/AdvancedTaming/Blueprints/AI/Components/GroundAnimals/BP_Comp_Companion.BP_Comp_Companion_C") true)
      ;[1 1 1] [1.3.2] Disable camera components on the companion
      (bind _asbp_ground_animal_base (Utilities|Casting|CastToBP_GroundAnimalBase (LocalVariables|GetTmpActualCompanionControlled)))
      (Default|EventDisableCamera _asbp_ground_animal_base))))

(fn TakeControlOfCompanion
  (params (CompanionToControl :type Actor%20Object%20Reference) (PlayerController :type Player%20Controller%20Object%20Reference))
  (bind _output_get (LocalVariables|SetTmpCompanionRef CompanionToControl))
  (bind _ascharacter (Utilities|Casting|CastToCharacter (Pawn|GetControlledPawn PlayerController)))
  (Variables|Default|SetOwnPawn _ascharacter)
  (Variables|Default|SetCompControllerRef (AI|GetAIController _output_get))
  (bind _aspawn (Utilities|Casting|CastToPawn (LocalVariables|GetTmpCompanionRef)))
  (Pawn|Possess PlayerController _aspawn)
  (Components|Movement|StopMovementImmediately (Variables|/Script/Engine.Character|GetCharacterMovement (Variables|Default|GetOwnPawn)))
  (if (Utilities|DoesObjectImplementInterface (Variables|Default|GetOwnPawn) "/Game/AdvancedTaming/Blueprints/Core/Interfaces/BP_BPI_ATS_PlayerConn.BP_BPI_ATS_PlayerConn_C")
    (bind _falling (Class|BPBPIATSPlayerConn|FnGetIsFalling(Message) (Variables|Default|GetOwnPawn)))
    (if (not _falling)
      ;[1 1 1] Disable companion teleport
      (Utilities|IsValid (Actor|GetComponentbyClass (LocalVariables|GetTmpCompanionRef) "/Game/AdvancedTaming/Blueprints/AI/Components/GroundAnimals/BP_Comp_Companion.BP_Comp_Companion_C")
        (:Is%20Valid
          (Variables|/Game/AdvancedTaming/Blueprints/AI/Components/GroundAnimals/BP_Comp_Companion.BP_Comp_Companion_C|SetCanTeleport (Actor|GetComponentbyClass (LocalVariables|GetTmpCompanionRef) "/Game/AdvancedTaming/Blueprints/AI/Components/GroundAnimals/BP_Comp_Companion.BP_Comp_Companion_C") false))))))

(fn GetAIControllerRefforCompanion
  (return (Variables|Default|GetCompControllerRef)))