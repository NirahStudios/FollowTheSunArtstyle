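; Player component that creates and updates the HUD for the taming system, showing bait amounts and companion status.
; It creates the HUD widget for the owner instigator's player controller, seeds prey and predator bait counts, and adds it to the player screen only if ShowHUD is set.
; Update functions push new bait amounts to the widget and forward the active command and selected companion name to its companion sub-widget.
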(fn FnCreateHUD
  (params (preyBait :type Integer) (predatorBait :type Integer))
  (LocalVariables|SetPreyBaitAmount preyBait)
  (LocalVariables|SetPredatorBaitAmount predatorBait)
  ;[1 1 1] Create Player HUD
  (bind _asplayer_controller (Utilities|Casting|CastToPlayerController (Pawn|GetController (Variables|/Script/Engine.Actor|GetInstigator (Components|GetOwner)))))
  (bind _returnvalue (UserInterface|CreateWidget "/Game/AdvancedTaming/Blueprints/Widgets/WBP_ATS_Player_HUD.WBP_ATS_Player_HUD_C" _asplayer_controller))
  (Variables|Default|SetPlayerHUDRef _returnvalue)
  ;[1 1 1] Show initial Prey and Predator Bait amounts
  (Default|FnSetPreyBait (Variables|Default|GetPlayerHUDRef) (LocalVariables|GetPreyBaitAmount))
  (Default|FnSetPredatorBait (Variables|Default|GetPlayerHUDRef) (LocalVariables|GetPredatorBaitAmount))
  (if (Variables|Setup|GetShowHUD)
    (UserInterface|Viewport|AddtoPlayerScreen (Variables|Default|GetPlayerHUDRef))))

(fn FnUpdateHUDBaitAmounts
  (params (preyBait :type Integer) (predatorBait :type Integer))
  (LocalVariables|SetPreyBaitAmount preyBait)
  (LocalVariables|SetPredatorBaitAmount predatorBait)
  (Utilities|IsValid (Variables|Default|GetPlayerHUDRef)
    (:Is%20Valid
      (Default|FnSetPreyBait (Variables|Default|GetPlayerHUDRef) (LocalVariables|GetPreyBaitAmount))
      (Default|FnSetPredatorBait (Variables|Default|GetPlayerHUDRef) (LocalVariables|GetPredatorBaitAmount)))))

(fn FnHighlightHUDCommand
  (params (ActiveAction :type Integer))
  (LocalVariables|SetaAction ActiveAction)
  (Utilities|IsValid (Variables|Default|GetPlayerHUDRef)
    (:Is%20Valid
      ;[1 1 1] Highlight Action in the HUD
      (Default|FnSetActiveAction (Variables|/Game/AdvancedTaming/Blueprints/Widgets/WBP_ATS_Player_HUD.WBP_ATS_Player_HUD_C|GetWBP_Companion (Variables|Default|GetPlayerHUDRef)) (LocalVariables|GetaAction)))))

(fn FnUpdateSelectedCompanion
  (params (Name :type Text))
  (LocalVariables|SetNewName Name)
  (Utilities|IsValid (Variables|Default|GetPlayerHUDRef)
    (:Is%20Valid
      (Default|FnChangeSelectedName (Variables|/Game/AdvancedTaming/Blueprints/Widgets/WBP_ATS_Player_HUD.WBP_ATS_Player_HUD_C|GetWBP_Companion (Variables|Default|GetPlayerHUDRef)) (LocalVariables|GetNewName)))))