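; Base bait pickup actor for the taming system, granting a set amount of Prey or Predator bait to the player.
; Trigger overlap checks for the player tag, sends type and amount through FnAddBaitMessage once, then destroys the pickup after a short delay.
; The Construction Script shows bait type and amount on text renders.
; The aim, falling and spawn anchor getters are stubs returning false or nothing.
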(event OnComponentBeginOverlap(Trigger)
  (params (OverlappedComponent :type Primitive%20Component%20Object%20Reference) (OtherActor :type Actor%20Object%20Reference) (OtherComp :type Primitive%20Component%20Object%20Reference) (OtherBodyIndex :type Integer) (bFromSweep :type Boolean) (SweepResult :type Hit%20Result%20Structure%20%28by%20ref%29))
  ;[1 1 1] Only overlap Player
  (if (Actor|ActorHasTag OtherActor "abkPlayer")
    (Utilities|FlowControl|DoOnce false
      (:Completed
        (Class|BPBPIATSPlayerConn|FnAddBait(Message) OtherActor (Variables|Setup|GetBaitAmount) (Variables|Setup|GetBaitType))
        (Utilities|FlowControl|Delay 0.2)
        (Actor|DestroyActor)))))

(fn ConstructionScript
  (switch Utilities|FlowControl|Switch|SwitchonBP_Enum_BaitTypeATS (Variables|Setup|GetBaitType)
    (:NewEnumerator0
      (Rendering|Components|TextRender|SetText (Variables|Default|GetRenderType) (Utilities|Text|MakeLiteralText "Prey")))
    (:NewEnumerator1
      (Rendering|Components|TextRender|SetText (Variables|Default|GetRenderType) (Utilities|Text|MakeLiteralText "Predator"))))
  (Rendering|Components|TextRender|SetText (Variables|Default|GetRenderAmount) (Utilities|Text|ToText(Integer) (Variables|Setup|GetBaitAmount))))

(fn FnGetAimMode
  (return false))

(fn FnGetIsFalling
  (return false))

(fn FnGetSpawnAnchor
  (return 0 0))